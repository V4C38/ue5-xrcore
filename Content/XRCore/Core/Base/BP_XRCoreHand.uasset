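; Base XR motion-controller hand that turns two analog inputs into interactions and animates the hand mesh.
; Deadzone-gated primary input interacts or falls back to activating the laser; secondary drives laser or additional interactions.
; Tick feeds the hand AnimBP local or replicated axis values, while BeginPlay mirrors the hand by side and rotates it per XR standard.
; Interaction-sphere feedback for idle, hover and interacting states exists, but its setup is never called.
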(event `XRCoreHandInterface.PrimaryInputAction`
  (params (InAxisValue :type "Float (single-precision)"))
  ;[1 1 1] Input Handling
  (bind _output_get (set `self.LocallyControlled_PrimaryInputAxisValue` InAxisValue))
  (`self.Primary Input` _output_get))

(event `XRCoreHandInterface.SecondaryInputAction`
  (params (InAxisValue :type "Float (single-precision)"))
  ;[1 1 1] Input Handling
  (bind _output_get (set `self.LocallyControlled_SecondaryInputAxisValue` InAxisValue))
  (`self.Secondary Input` _output_get))

(event `self.ReceiveBeginPlay`
  ;[1 1 1] Init
  (`KismetSystemLibrary.Delay` 1.0)
  (`|ExecutionSequence`
    (:`then_0`
      (`XRInteractorComponent.SetPhysicsConstraint` (`XRCoreHandInterface.GetXRInteractor`) (`self.XRInteractor_PhysicsConstraint`)))
    (:`then_1`
      (bind _asabp_xrcore_hand (cast `/XR_Toolkit/XRCore/Assets/Meshes/HandModel/ABP_XRCoreHand` (`SkeletalMeshComponent.GetAnimInstance` (`self.SK_Hand`))))
      (set `self.ABP XRCore Hand` _asabp_xrcore_hand))
    (:`then_2`
      (`self.UpdateHandModelBySide`))
    (:`then_3`
      (`self.UpdateHandRotationByXRStandard`))))

(event `OnHoverStateChanged_Event`
  (params (Sender :type "XRInteractorComponent Object Reference") (HoveredXRInteractionComponent :type "XRInteractionComponent Object Reference") (bHoverState :type Boolean))
  ;[1 1 1] Init
  (`self.Update Interaction State`))

(event `OnStartedInteracting_Event`
  (params (Sender :type "XRInteractorComponent Object Reference") (XRInteractionComponent :type "XRInteractionComponent Object Reference"))
  ;[1 1 1] Init
  (`self.Update Interaction State`))

(event `OnStoppedInteracting_Event`
  (params (Sender :type "XRInteractorComponent Object Reference") (XRInteractionComponent :type "XRInteractionComponent Object Reference"))
  ;[1 1 1] Init
  (`self.Update Interaction State`))

(event `AnimateInteractionSphere`
  (params (InInteractionState :type Integer))
  (bind _interactionrootsphere (`self.InteractionRootSphere`))
  ;[1 1 1] Init
  (bind (_direction _outalpha) (`Timeline|Timeline_InteractionSphere` :!via `PlayFromStart`)
    (:`Update`
      (`SceneComponent.SetRelativeScale3D` _interactionrootsphere (`KismetMathLibrary.VLerp` (`SceneComponent.RelativeScale3D` (`self.InteractionRootSphere`)) (* (`self.DefaultInteractionSphereScale`) (select `int` InInteractionState :`0` 0.05 :`1` 2.0 :`2` 1.0)) _outalpha))
      (bind _output_get (set `self.InteractionSphereOpacity` (`KismetMathLibrary.Lerp` (`self.InteractionSphereOpacity`) (select `int` InInteractionState :`0` 0.05 :`1` 0.25 :`2` 1.0) _outalpha)))
      (`MeshComponent.SetScalarParameterValueOnMaterials` _interactionrootsphere "Opacity" _output_get))))

(event `OnXRLaserStateChanged_Event`
  (params (Sender :type "XRLaserComponent Object Reference") (NewState :type Boolean))
  ;[1 1 1] Init
  (`self.Update Interaction State`))

(event `self.ReceiveTick`
  (params (DeltaSeconds :type "Float (single-precision)"))
  (`parent.ReceiveTick` DeltaSeconds)
  (`self.UpdateHandPose`))

(fn `Primary Input`
  (params (InAxisValue :type "Float (double-precision)"))
  (bind _returnvalue (`XRCoreHandInterface.GetXRInteractor`))
  (if (`self.bIsLocallyControlled`)
    ;[1 1 1] AxisValue Deadzone gate
    (if (`self.bCurrentPrimaryInput`)
      (if (not (> (`local.InAxisValue`) (- (`self.InputAxisDeadzone`) 0.1)))
        (set `self.bCurrentPrimaryInput` false)
        ;[1 1 1] End Interactions
        (if (`XRLaserInterface.IsLaserActive` (`XRCoreHandInterface.GetXRLaser`))
          (message `XRLaserInterface.SetLaserActive` (`XRCoreHandInterface.GetXRLaser`) false)
          (else
            (`XRInteractorComponent.StopAllXRInteractions` (`XRCoreHandInterface.GetXRInteractor`)))))
      (elif (> (`local.InAxisValue`) (`self.InputAxisDeadzone`))
        (set `self.bCurrentPrimaryInput` true)
        ;[1 1 1] Start Interactions
        ; Laser or Interact
        (if (`XRLaserInterface.IsLaserActive` (`XRCoreHandInterface.GetXRLaser`))
          (`XRInteractorComponent.StartXRInteractionByPriority` (`XRCoreHandInterface.GetXRInteractor`) 0 "LowerEqual" :!label _label)
          (elif (or (`.ReturnValue` (`XRInteractorComponent.CanInteract` _returnvalue 0 "LowerEqual")) (`XRInteractorComponent.IsInteracting` _returnvalue))
            (goto _label)
            (else
              (message `XRLaserInterface.SetLaserActive` (`XRCoreHandInterface.GetXRLaser`) true))))))))

(fn `Secondary Input`
  (params (InAxisValue :type "Float (double-precision)"))
  (bind _returnvalue (> (`local.InAxisValue`) (/ (`self.InputAxisDeadzone`) 2.0)))
  (if (`self.bIsLocallyControlled`)
    ;[1 1 1] AxisValue Deadzone gate
    (if (`self.bCurrentSecondaryInput`)
      (if (not _returnvalue)
        (set `self.bCurrentSecondaryInput` false)
        ;[1 1 1] Stop Interactions
        (if (`XRLaserInterface.IsLaserActive` (`XRCoreHandInterface.GetXRLaser`))
          (message `XRInteractionInterface.StopAllInteractions` (`XRCoreHandInterface.GetXRLaser`) null)
          (elif (> (`KismetArrayLibrary.Array_Length` (`XRInteractorComponent.GetActiveInteractions` (`XRCoreHandInterface.GetXRInteractor`))) 1)
            (`XRInteractorComponent.StopXRInteractionByPriority` (`XRCoreHandInterface.GetXRInteractor`) 5 "HigherEqual"))))
      (elif _returnvalue
        (set `self.bCurrentSecondaryInput` true)
        ;[1 1 1] Interactions
        ; Start Next Interaction
        (if (`XRLaserInterface.IsLaserActive` (`XRCoreHandInterface.GetXRLaser`))
          (message `XRInteractionInterface.StartInteractionByPriority` (`XRCoreHandInterface.GetXRLaser`) 0 "LowerEqual")
          (elif (`XRInteractorComponent.IsInteracting` (`XRCoreHandInterface.GetXRInteractor`))
            (`XRInteractorComponent.StartXRInteractionByPriority` (`XRCoreHandInterface.GetXRInteractor`) 0 "LowerEqual")))))))

(fn `Update Interaction State`
  (locals (InteractionState :type Integer :default 0))
  (bind _xrinteractor (`self.XRInteractor`))
  (bind _xrlasercomponent (`self.XRLaserComponent`))
  (bind _returnvalue (`XRLaserInterface.GetXRInteractor` _xrlasercomponent))
  (`/Engine/EditorBlueprintResources/StandardMacros.IsValid` _returnvalue
    (:`Is Valid`
      (bind _output_get (set `local.InteractionState` (select `bool` (or (`XRInteractorComponent.IsInteracting` _xrinteractor) (`XRInteractorComponent.IsInteracting` _returnvalue)) :`false` (select `bool` (or (`.ReturnValue` (`XRInteractorComponent.CanInteract` _xrinteractor 0 "LowerEqual")) (`.ReturnValue` (`XRInteractorComponent.CanInteract` _returnvalue 0 "LowerEqual")) (`XRLaserInterface.IsLaserActive` _xrlasercomponent)) :`true` 1) :`true` 2)))
      (`self.AnimateInteractionSphere` _output_get))))

(fn `UpdateHandModelBySide`
  (`self.SetActorScale3D` (`KismetMathLibrary.MakeVector` 1.0 (select `ESimplifiedControllerHand` (`XRToolsUtilityFunctions.SimplyfyControllerHandEnum` (`XRCoreHandInterface.GetControllerHand`)) :`Left` 1.0 :`Right` -1.0 :`Any` 1.0) 1.0)))

(fn `UpdateHandPose`
  (bind (_returnvalue_location _returnvalue_rotation _returnvalue_primaryinputaxis _returnvalue_secondaryinputaxis) (break `XRCoreHandReplicationData` (`self.GetReplicatedHandData`)))
  (bind _abp_xrcore_hand (`self.ABP XRCore Hand`)
    (:`then`
      (`/XR_Toolkit/XRCore/Assets/Meshes/HandModel/ABP_XRCoreHand.Set ControllerValue_Trigger` _abp_xrcore_hand (select `bool` (`self.bIsLocallyControlled`) :`false` _returnvalue_primaryinputaxis :`true` (`self.LocallyControlled_PrimaryInputAxisValue`) :!type "Float (double-precision)"))
      (`/XR_Toolkit/XRCore/Assets/Meshes/HandModel/ABP_XRCoreHand.Set ControllerValue_Grip` _abp_xrcore_hand (select `bool` (`self.bIsLocallyControlled`) :`false` _returnvalue_secondaryinputaxis :`true` (`self.LocallyControlled_SecondaryInputAxisValue`) :!type "Float (double-precision)")))
    (:`else`)))

(fn `UpdateHandRotationByXRStandard`
  (`SceneComponent.K2_SetRelativeRotation` (`self.MotionControllerRoot`) (select `EXRStandard` (`XRToolsUtilityFunctions.GetXRStandard`) :`MetaXR` (struct :`Pitch` 75.0) :!type "Rotator Structure") false false))

(fn `UserConstructionScript`)
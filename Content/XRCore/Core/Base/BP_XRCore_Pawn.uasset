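; BP_XRCore_Pawn is the base XR player pawn, wiring up floor-relative tracking, Enhanced Input and head replication.
; On BeginPlay it sets the tracking origin, adds its mapping context and initializes a replicator proxy with the camera as local source and HeadContainer as remote target.
; Left and right primary and secondary input actions forward their values to the matching hand, sending zero on cancel or completion.
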(event `self.ReceiveBeginPlay`
  ;[0 0 0] Initial Setup
  (`|ExecutionSequence`
    (:`then_0`
      (`HeadMountedDisplayFunctionLibrary.SetTrackingOrigin` "LocalFloor"))
    (:`then_1`
      ;;[1 1 1] Setup Input
      (bind _asplayer_controller (cast `PlayerController` (`self.GetController`)))
      (bind _returnvalue (pcsubsystem `EnhancedInputLocalPlayerSubsystem` _asplayer_controller))
      (`/Engine/EditorBlueprintResources/StandardMacros.IsValid` _returnvalue
        (:`Is Valid`
          (`EnhancedInputSubsystemInterface.AddMappingContext` _returnvalue (`self.Mapping Context`) 0 (struct)))))
    (:`then_2`
      ;;[1 1 1] Setup Head Replication
      (`/XR_Toolkit/XRCore/Core/Base/BP_ProxyComponentReplicator.Init Components` (`self.BP_ProxyComponentReplicator_Head`) self (`self.Camera`) (`self.Head_Container`)))))

(event `EnhancedInput|/XR_Toolkit/XRCore/Core/Input/InputAction_XR_Primary_L`
  (params (ActionValue :type "Float (double-precision)") (ElapsedSeconds :type "Float (double-precision)") (TriggeredSeconds :type "Float (double-precision)") (InputAction :type "InputAction Object Reference" :default "/XR_Toolkit/XRCore/Core/Input/InputAction_XR_Primary_L.InputAction_XR_Primary_L"))
  (bind _xrcorehand_l (`self.XRCoreHand_L`))
  ;[0 0 0] Input
  (:`Triggered`
    (message `XRCoreHandInterface.PrimaryInputAction` _xrcorehand_l ActionValue))
  (:`Canceled`
    (message `XRCoreHandInterface.PrimaryInputAction` _xrcorehand_l 0.0 :!label _label))
  (:`Completed`
    (goto _label)))

(event `EnhancedInput|/XR_Toolkit/XRCore/Core/Input/InputAction_XR_Primary_R`
  (params (ActionValue :type "Float (double-precision)") (ElapsedSeconds :type "Float (double-precision)") (TriggeredSeconds :type "Float (double-precision)") (InputAction :type "InputAction Object Reference" :default "/XR_Toolkit/XRCore/Core/Input/InputAction_XR_Primary_R.InputAction_XR_Primary_R"))
  (bind _xrcorehand_r (`self.XRCoreHand_R`))
  ;[0 0 0] Input
  (:`Triggered`
    (message `XRCoreHandInterface.PrimaryInputAction` _xrcorehand_r ActionValue))
  (:`Canceled`
    (message `XRCoreHandInterface.PrimaryInputAction` _xrcorehand_r 0.0 :!label _label_2))
  (:`Completed`
    (goto _label_2)))

(event `EnhancedInput|/XR_Toolkit/XRCore/Core/Input/InputAction_XR_Secondary_L`
  (params (ActionValue :type "Float (double-precision)") (ElapsedSeconds :type "Float (double-precision)") (TriggeredSeconds :type "Float (double-precision)") (InputAction :type "InputAction Object Reference" :default "/XR_Toolkit/XRCore/Core/Input/InputAction_XR_Secondary_L.InputAction_XR_Secondary_L"))
  (bind _xrcorehand_l (`self.XRCoreHand_L`))
  ;[0 0 0] Input
  (:`Triggered`
    (message `XRCoreHandInterface.SecondaryInputAction` _xrcorehand_l ActionValue))
  (:`Canceled`
    (message `XRCoreHandInterface.SecondaryInputAction` _xrcorehand_l 0.0 :!label _label_3))
  (:`Completed`
    (goto _label_3)))

(event `EnhancedInput|/XR_Toolkit/XRCore/Core/Input/InputAction_XR_Secondary_R`
  (params (ActionValue :type "Float (double-precision)") (ElapsedSeconds :type "Float (double-precision)") (TriggeredSeconds :type "Float (double-precision)") (InputAction :type "InputAction Object Reference" :default "/XR_Toolkit/XRCore/Core/Input/InputAction_XR_Secondary_R.InputAction_XR_Secondary_R"))
  (bind _xrcorehand_r (`self.XRCoreHand_R`))
  ;[0 0 0] Input
  (:`Triggered`
    (message `XRCoreHandInterface.SecondaryInputAction` _xrcorehand_r ActionValue))
  (:`Canceled`
    (message `XRCoreHandInterface.SecondaryInputAction` _xrcorehand_r 0.0 :!label _label_4))
  (:`Completed`
    (goto _label_4)))

(fn `UserConstructionScript`)
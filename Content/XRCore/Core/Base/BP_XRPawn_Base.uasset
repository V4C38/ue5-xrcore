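; Base VR pawn that sets local-floor tracking, adds its Enhanced Input mapping context and replicates the head from the camera through a proxy replicator component.
; The server spawns left and right replicated XR hand actors owned by the pawn.
; Their OnRep functions attach them to the motion controllers when locally controlled, then fire initialization events that derived classes can override.
; Helper functions look up hands, lasers and interactors by controller hand.
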(event `self.ReceiveBeginPlay`
  ;[0 0 0] Initial Setup
  (`|ExecutionSequence`
    (:`then_0`
      (`HeadMountedDisplayFunctionLibrary.SetTrackingOrigin` "LocalFloor"))
    (:`then_1`
      ;;[1 1 1] Setup Input
      (bind _asplayer_controller (cast `PlayerController` (`self.GetController`)))
      (bind _returnvalue (pcsubsystem `EnhancedInputLocalPlayerSubsystem` _asplayer_controller))
      (`/Engine/EditorBlueprintResources/StandardMacros.IsValid` _returnvalue
        (:`Is Valid`
          (`EnhancedInputSubsystemInterface.AddMappingContext` _returnvalue (`self.Mapping Context`) 0 (struct)))))
    (:`then_2`
      (if (`KismetSystemLibrary.IsServer`)
        (`self.Server_SpawnXRHands`)))
    (:`then_3`
      ;;[1 1 1] Setup Head Replication
      (`/XR_Toolkit/XRCore/Core/Utilities/BP_ProxyComponentReplicator.Init Components` (`self.BP_ProxyComponentReplicator_Head`) self (`self.Camera`) (`self.Head_Container`)))
    (:`then_4`
      (`/XR_Toolkit/XRCore/Core/Utilities/FL_XRUtilityFunctions.CustomDebugWarning` "NewEnumerator3" (`GameplayStatics.GetPlayerController` 0) "VR Mode: Using " (`KismetSystemLibrary.GetDisplayName` self)))))

(event `Server_SpawnXRHands`
  ;[1 1 1] Spawn XRHands
  (`|ExecutionSequence`
    (:`then_0`
      (bind _returnvalue (`|SpawnActorFromClass` (`self.XRHandType`) (`KismetMathLibrary.MakeTransform` (0.0 0.0 0.0)) "Undefined" "MultiplyWithRoot" self null))
      (bind _output_get (set `self.XRHand_Right` _returnvalue))
      (`self.SetReplicates` _output_get true)
      (`/XR_Toolkit/XRCore/Core/Hands/BP_XRHand.SetControllerHand` _output_get "Right"))
    (:`then_1`
      (bind _returnvalue_2 (`|SpawnActorFromClass` (`self.XRHandType`) (`KismetMathLibrary.MakeTransform` (0.0 0.0 0.0)) "Undefined" "MultiplyWithRoot" self null))
      (bind _output_get_2 (set `self.XRHand_Left` _returnvalue_2))
      (`self.SetReplicates` _output_get_2 true)
      (`/XR_Toolkit/XRCore/Core/Hands/BP_XRHand.SetControllerHand` _output_get_2 "Left"))))

(event `OnXRHandInitialized_Event`
  (params (XRHand :type "/XR_Toolkit/XRCore/Core/Hands/BP_XRHand Object Reference (by ref)"))
  ;[1 1 1] Spawn XRHands
)

(fn `Get XRInteractor By Hand`
  (params (InControllerHand :type "EControllerHand Enum" :default "Left"))
  (returns (OutXRInteractor :type "XRInteractorComponent Object Reference"))
  (bind _xrhand_right (`self.XRHand_Right`))
  (bind _xrhand_left (`self.XRHand_Left`))
  (switch `/XR_Toolkit/XRCore/Core/Utilities/EN_ReducedControllerHand` (`/XR_Toolkit/XRCore/Core/Utilities/FL_XRUtilityFunctions.XRCore_ReduceControllerHandEnum` InControllerHand)
    (:`NewEnumerator0`
      (`/Engine/EditorBlueprintResources/StandardMacros.IsValid` _xrhand_left
        (:`Is Valid`
          (return (`/XR_Toolkit/XRCore/Core/Hands/BP_XRHand.XRInteractor` _xrhand_left)))))
    (:`NewEnumerator1`
      (`/Engine/EditorBlueprintResources/StandardMacros.IsValid` _xrhand_right
        (:`Is Valid`
          (return (`/XR_Toolkit/XRCore/Core/Hands/BP_XRHand.XRInteractor` _xrhand_right)))))))

(fn `Get XRLaser By Hand`
  (params (InControllerHand :type "EControllerHand Enum" :default "Left"))
  (returns (OutXRLaser :type "XRLaserComponent Object Reference"))
  (bind _returnvalue (`self.GetXRHand` InControllerHand))
  (bind _xrlaser (`/XR_Toolkit/XRCore/Core/Hands/BP_XRHand.XRLaser` _returnvalue))
  (`/Engine/EditorBlueprintResources/StandardMacros.IsValid` _returnvalue
    (:`Is Valid`
      (`/Engine/EditorBlueprintResources/StandardMacros.IsValid` _xrlaser
        (:`Is Valid`
          (return _xrlaser))
        (:`Is Not Valid`
          _)))
    (:`Is Not Valid`
      _))
  (`/XR_Toolkit/XRCore/Core/Utilities/FL_XRUtilityFunctions.CustomDebugWarning` "NewEnumerator0" self "Failed to return valid XRLaser for XRHand: ")
  (return null))

(fn `GetXRHand`
  (params (InControllerHand :type "EControllerHand Enum" :default "Left"))
  (returns (ReturnValue :type "/XR_Toolkit/XRCore/Core/Hands/BP_XRHand Object Reference"))
  (return (select `/XR_Toolkit/XRCore/Core/Utilities/EN_ReducedControllerHand` (`/XR_Toolkit/XRCore/Core/Utilities/FL_XRUtilityFunctions.XRCore_ReduceControllerHandEnum` InControllerHand) :`NewEnumerator0` (`self.XRHand_Left`) :`NewEnumerator1` (`self.XRHand_Right`))))

(fn `OnRep_XRHand_Left`
  (bind _xrhand_left (`self.XRHand_Left`))
  (`|ExecutionSequence`
    (:`then_0`
      (if (`self.IsLocallyControlled`)
        (`SceneComponent.K2_AttachToComponent` (`/XR_Toolkit/XRCore/Core/Hands/BP_XRHand.MotionController_Root` (`self.XRHand_Left`)) (`self.MotionController_L`) "None" "SnapToTarget" "SnapToTarget" "KeepRelative" true)))
    (:`then_1`
      (`self.OnXRHandInitialized` _xrhand_left)
      (`self.OnXRHandInitialized_Event` _xrhand_left))))

(fn `OnRep_XRHand_Right`
  (bind _xrhand_right (`self.XRHand_Right`))
  (`|ExecutionSequence`
    (:`then_0`
      (if (`self.IsLocallyControlled`)
        (`SceneComponent.K2_AttachToComponent` (`/XR_Toolkit/XRCore/Core/Hands/BP_XRHand.MotionController_Root` (`self.XRHand_Right`)) (`self.MotionController_R`) "None" "SnapToTarget" "SnapToTarget" "KeepRelative" true)))
    (:`then_1`
      (`self.OnXRHandInitialized` _xrhand_right)
      (`self.OnXRHandInitialized_Event` _xrhand_right))))

(fn `UserConstructionScript`)
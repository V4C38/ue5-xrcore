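; XR hand for one controller side that turns trigger and grip input into interactions and hand poses, with switchable hand tracking.
; Trigger starts an XRInteractor interaction or falls back to XRLaser; grip starts further interactions.
; The interactor smoothly follows a root between thumb and index sockets, or from hand tracking.
; The local client sends transform and pose by server RPC each tick; receivers apply the transform directly and interpolate the pose.
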(event `EnhancedInput|/XR_Toolkit/XRCore/Core/Input/InputAction_OpenMenu`
  (params (ActionValue :type Boolean) (ElapsedSeconds :type "Float (double-precision)") (TriggeredSeconds :type "Float (double-precision)") (InputAction :type "InputAction Object Reference" :default "/XR_Toolkit/XRCore/Core/Input/InputAction_OpenMenu.InputAction_OpenMenu"))
  (bind _handtrackingsystem (`self.HandTrackingSystem`))
  ;[0 0 0] Temporary switch to manually toggle HandTracking
  (:`Completed`
    (`/XR_Toolkit/XRCore/Core/Hands/HandTracking/BP_XRCore_HandTrackingSystem.SetIsHandTracking` _handtrackingsystem (not (`/XR_Toolkit/XRCore/Core/Hands/HandTracking/BP_XRCore_HandTrackingSystem.GetIsHandTracking` _handtrackingsystem)))))

(event `EnhancedInput|/XR_Toolkit/XRCore/Core/Input/InputAction_XR_Primary_Touched_L`
  (params (ActionValue :type "Float (double-precision)") (ElapsedSeconds :type "Float (double-precision)") (TriggeredSeconds :type "Float (double-precision)") (InputAction :type "InputAction Object Reference" :default "/XR_Toolkit/XRCore/Core/Input/InputAction_XR_Primary_Touched_L.InputAction_XR_Primary_Touched_L"))
  ;[0 0 0] Input
  (:`Triggered`
    (`self.IsValidInput` "Left" :!label _label
      (:`true`
        (`self.Input Set Controller Value Trigger Touched` ActionValue))))
  (:`Started`
    (goto _label))
  (:`Canceled`
    (`self.IsValidInput` "Left" :!label _label_2
      (:`true`
        (`self.Input Set Controller Value Trigger Touched` 0.0))))
  (:`Completed`
    (goto _label_2)))

(event `EnhancedInput|/XR_Toolkit/XRCore/Core/Input/InputAction_XR_Primary_Touched_R`
  (params (ActionValue :type "Float (double-precision)") (ElapsedSeconds :type "Float (double-precision)") (TriggeredSeconds :type "Float (double-precision)") (InputAction :type "InputAction Object Reference" :default "/XR_Toolkit/XRCore/Core/Input/InputAction_XR_Primary_Touched_R.InputAction_XR_Primary_Touched_R"))
  ;[0 0 0] Input
  (:`Triggered`
    (`self.IsValidInput` "Right" :!label _label_3
      (:`true`
        (`self.Input Set Controller Value Trigger Touched` ActionValue))))
  (:`Started`
    (goto _label_3))
  (:`Canceled`
    (`self.IsValidInput` "Right" :!label _label_4
      (:`true`
        (`self.Input Set Controller Value Trigger Touched` 0.0))))
  (:`Completed`
    (goto _label_4)))

(event `EnhancedInput|/XR_Toolkit/XRCore/Core/Input/InputAction_XR_Primary_R`
  (params (ActionValue :type "Float (double-precision)") (ElapsedSeconds :type "Float (double-precision)") (TriggeredSeconds :type "Float (double-precision)") (InputAction :type "InputAction Object Reference" :default "/XR_Toolkit/XRCore/Core/Input/InputAction_XR_Primary_R.InputAction_XR_Primary_R"))
  ;[0 0 0] Input
  (:`Triggered`
    (`self.IsValidInput` "Right"
      (:`true`
        (`self.PrimaryInput_Triggered` ActionValue))))
  (:`Canceled`
    (`self.IsValidInput` "Right" :!label _label_5
      (:`true`
        (`self.PrimaryInput_Triggered` 0.0))))
  (:`Completed`
    (goto _label_5)))

(event `EnhancedInput|/XR_Toolkit/XRCore/Core/Input/InputAction_XR_Primary_L`
  (params (ActionValue :type "Float (double-precision)") (ElapsedSeconds :type "Float (double-precision)") (TriggeredSeconds :type "Float (double-precision)") (InputAction :type "InputAction Object Reference" :default "/XR_Toolkit/XRCore/Core/Input/InputAction_XR_Primary_L.InputAction_XR_Primary_L"))
  ;[0 0 0] Input
  (:`Triggered`
    (`self.IsValidInput` "Left"
      (:`true`
        (`self.PrimaryInput_Triggered` ActionValue))))
  (:`Canceled`
    (`self.IsValidInput` "Left" :!label _label_6
      (:`true`
        (`self.PrimaryInput_Triggered` 0.0))))
  (:`Completed`
    (goto _label_6)))

(event `EnhancedInput|/XR_Toolkit/XRCore/Core/Input/InputAction_XR_Secondary_L`
  (params (ActionValue :type "Float (double-precision)") (ElapsedSeconds :type "Float (double-precision)") (TriggeredSeconds :type "Float (double-precision)") (InputAction :type "InputAction Object Reference" :default "/XR_Toolkit/XRCore/Core/Input/InputAction_XR_Secondary_L.InputAction_XR_Secondary_L"))
  ;[0 0 0] Input
  (:`Triggered`
    (`self.IsValidInput` "Left"
      (:`true`
        (`self.SecondaryInput_Triggered` ActionValue))))
  (:`Canceled`
    (`self.IsValidInput` "Left" :!label _label_7
      (:`true`
        (`self.SecondaryInput_Triggered` 0.0))))
  (:`Completed`
    (goto _label_7)))

(event `EnhancedInput|/XR_Toolkit/XRCore/Core/Input/InputAction_XR_Secondary_R`
  (params (ActionValue :type "Float (double-precision)") (ElapsedSeconds :type "Float (double-precision)") (TriggeredSeconds :type "Float (double-precision)") (InputAction :type "InputAction Object Reference" :default "/XR_Toolkit/XRCore/Core/Input/InputAction_XR_Secondary_R.InputAction_XR_Secondary_R"))
  ;[0 0 0] Input
  (:`Triggered`
    (`self.IsValidInput` "Right"
      (:`true`
        (`self.SecondaryInput_Triggered` ActionValue))))
  (:`Canceled`
    (`self.IsValidInput` "Right" :!label _label_8
      (:`true`
        (`self.SecondaryInput_Triggered` 0.0))))
  (:`Completed`
    (goto _label_8)))

(event `self.ReceiveBeginPlay`
  (bind _bp_xrcore_handtrackingsystem (`self.BP_XRCore_HandTrackingSystem`))
  ;[1 1 1] Init
  (bind _aspawn (cast `Pawn` (`self.GetOwner`)))
  (set `self.OwningPawn` _aspawn)
  (`|ExecutionSequence`
    (:`then_0`
      (set `self.bIsLocallyControlled` (`Pawn.IsLocallyControlled` (`self.OwningPawn`))))
    (:`then_1`
      (`XRInteractorComponent.SetPhysicsConstraint` (`self.XRInteractor`) (`self.XRInteractor_PhysicsConstraint`)))
    (:`then_2`
      (bind _asabp_xrcore_hand (cast `/XR_Toolkit/XRCore/Assets/Meshes/HandModel/ABP_XRCoreHand` (`SkeletalMeshComponent.GetAnimInstance` (`self.SK_Hand`))))
      (bind _output_get (set `self.ABP XRCore Hand` _asabp_xrcore_hand))
      (`/XR_Toolkit/XRCore/Core/Hands/HandTracking/BP_XRCore_HandTrackingSystem.AssignAnimBP` _bp_xrcore_handtrackingsystem _output_get)
      (set `self.HandTrackingSystem` _bp_xrcore_handtrackingsystem))
    (:`then_3`
      (`self.OnInitComplete` self))))

(event `self.ReceiveTick`
  (params (DeltaSeconds :type "Float (single-precision)"))
  (bind _motioncontroller_root (`self.MotionController_Root`))
  (bind (_latestreplicationdata_location_worldspace _latestreplicationdata_rotation_worldspace) (break `/XR_Toolkit/XRCore/Core/Hands/F_XRHand_ReplicationData` (`self.LatestReplicationData`)))
  (`|ExecutionSequence`
    (:`then_0`
      (`self.UpdateInteractionRoot`))
    (:`then_1`
      (`self.InterpolateXRInteractorTransform`))
    (:`then_2`
      (if (`self.bIsLocallyControlled`)
        ;[1 1 1] Sending Client
        (bind _motioncontrollerdata (`HeadMountedDisplayFunctionLibrary.GetMotionControllerData` self (`self.ControllerHand`)))
        (if (`.bValid` (break `XRMotionControllerData` _motioncontrollerdata))
          (`self.Server_SetReplicationData` (make `/XR_Toolkit/XRCore/Core/Hands/F_XRHand_ReplicationData` (`SceneComponent.K2_GetComponentLocation` _motioncontroller_root) (`SceneComponent.K2_GetComponentRotation` _motioncontroller_root) (make `/XR_Toolkit/XRCore/Core/Hands/F_XRHand_HandPoseReplicationData` (`self.Local_TriggerAxis`) (`self.Local_TriggerTouch`) (`self.Local_GripAxis`))))
          (`SceneComponent.SetVisibility` (`self.SK_Hand`) (not (`/XR_Toolkit/XRCore/Core/Hands/HandTracking/BP_XRCore_HandTrackingSystem.GetIsHandTracking` (`self.HandTrackingSystem`))) false))
        (else
          ;[1 1 1] Receivers
          (`|ExecutionSequence`
            (:`then_0`
              (`SceneComponent.K2_SetWorldLocationAndRotation` (`self.MotionController_Root`) _latestreplicationdata_location_worldspace _latestreplicationdata_rotation_worldspace false false))
            (:`then_1`
              (`self.Update Hand Pose`))))))))

(event `Server_SetReplicationData`
  (params (InReplicationData :type "/XR_Toolkit/XRCore/Core/Hands/F_XRHand_ReplicationData Structure"))
  ;[0 0 0] RPC
  (set `self.LatestReplicationData` InReplicationData))

(fn `GetControllerHand`
  (returns (OutControllerHand :type "EControllerHand Enum"))
  (return (`self.ControllerHand`)))

(fn `Input Set Controller Value Grip`
  (params (InAxisValue :type "Float (double-precision)"))
  (set `self.Local_GripAxis` InAxisValue)
  (bind _abp_xrcore_hand (`self.ABP XRCore Hand`)
    (:`then`
      (`/XR_Toolkit/XRCore/Assets/Meshes/HandModel/ABP_XRCoreHand.Set ControllerValue_Grip` _abp_xrcore_hand InAxisValue))
    (:`else`)))

(fn `Input Set Controller Value Trigger`
  (params (InAxisValue :type "Float (double-precision)"))
  (set `self.Local_TriggerAxis` InAxisValue)
  (bind _abp_xrcore_hand (`self.ABP XRCore Hand`)
    (:`then`
      (`/XR_Toolkit/XRCore/Assets/Meshes/HandModel/ABP_XRCoreHand.Set ControllerValue_Trigger` _abp_xrcore_hand InAxisValue))
    (:`else`)))

(fn `Input Set Controller Value Trigger Touched`
  (params (Local_TriggerTouch :type "Float (double-precision)"))
  (bind _abp_xrcore_hand (`self.ABP XRCore Hand`)
    (:`then`
      (set `/XR_Toolkit/XRCore/Assets/Meshes/HandModel/ABP_XRCoreHand.Input_Trigger_Touch` Local_TriggerTouch _abp_xrcore_hand))
    (:`else`)))

(fn `InterpolateXRInteractorTransform`
  (bind _returnvalue (`GameplayStatics.GetWorldDeltaSeconds`))
  (bind _xrinteractor (`self.XRInteractor`))
  (bind _xrinteractorroot (`self.XRInteractorRoot`))
  (`SceneComponent.K2_SetWorldLocationAndRotation` (`self.XRInteractor`) (`KismetMathLibrary.VInterpTo` (`SceneComponent.K2_GetComponentLocation` _xrinteractor) (`SceneComponent.K2_GetComponentLocation` _xrinteractorroot) _returnvalue 30.0) (`KismetMathLibrary.RInterpTo` (`SceneComponent.K2_GetComponentRotation` _xrinteractor) (`SceneComponent.K2_GetComponentRotation` _xrinteractorroot) _returnvalue 7.0) false false))

(fn `ModifyMotionControllerRoot_LocationRotation`
  (return))

(fn `OnRep_ControllerHand`
  (`self.SetMotionControllerRoot_Scale` false)
  (`XRLaserInterface.SetControllerHand` (`self.XRLaser`) (`self.ControllerHand`))
  ;[1 1 1] HandTracking
  (`/XR_Toolkit/XRCore/Core/Hands/HandTracking/BP_XRCore_HandTrackingSystem.SetControllerHand` (`self.BP_XRCore_HandTrackingSystem`) (`self.ControllerHand`)))

(fn `PrimaryInput_End`
  (`|ExecutionSequence`
    (:`then_0`
      (set `self.bCurrentPrimaryInput` false))
    (:`then_1`
      ;[1 1 1] Handle Interactions
      (if (`XRLaserInterface.IsLaserActive` (`self.XRLaser`))
        (message `XRLaserInterface.SetLaserActive` (`self.XRLaser`) false)
        (else
          (`XRInteractorComponent.StopAllXRInteractions` (`self.XRInteractor`)))))
    (:`then_2`
      ;[1 1 1] HandPose
      (set `self.Local_TriggerAxis` 0.0)
      (bind _abp_xrcore_hand (`self.ABP XRCore Hand`)
        (:`then`
          (`/XR_Toolkit/XRCore/Assets/Meshes/HandModel/ABP_XRCoreHand.Set ControllerValue_Trigger` _abp_xrcore_hand 0.0))
        (:`else`)))))

(fn `PrimaryInput_Triggered`
  (params (InAxisValue :type "Float (double-precision)"))
  (bind _inaxisvalue (`local.InAxisValue`))
  (bind _xrinteractor (`self.XRInteractor`))
  (`|ExecutionSequence`
    (:`then_0`
      (`self.UpdateInteractionRoot`))
    (:`then_1`
      ;[1 1 1] AxisValue Deadzone gate
      (if (`self.bCurrentPrimaryInput`)
        (if (not (> (`local.InAxisValue`) (- (`self.InputAxisDeadzone`) 0.1)))
          (set `self.bCurrentPrimaryInput` false)
          ;[1 1 1] End Interactions
          (if (`XRLaserInterface.IsLaserActive` (`self.XRLaser`))
            (message `XRLaserInterface.SetLaserActive` (`self.XRLaser`) false)
            (else
              (`XRInteractorComponent.StopAllXRInteractions` (`self.XRInteractor`)))))
        (elif (> (`local.InAxisValue`) (`self.InputAxisDeadzone`))
          (set `self.bCurrentPrimaryInput` true)
          ;[1 1 1] Start Interactions
          ; Laser or Interact
          (if (`XRLaserInterface.IsLaserActive` (`self.XRLaser`))
            (`XRInteractorComponent.StartXRInteractionByPriority` (`self.XRInteractor`) 0 "LowerEqual" :!label _label)
            (elif (or (`.ReturnValue` (`XRInteractorComponent.CanInteract` _xrinteractor 0 "LowerEqual")) (`XRInteractorComponent.IsInteracting` _xrinteractor))
              (goto _label)
              (else
                (message `XRLaserInterface.SetLaserActive` (`self.XRLaser`) true)))))))
    (:`then_2`
      ;[1 1 1] HandPose
      (set `self.Local_TriggerAxis` _inaxisvalue)
      (bind _abp_xrcore_hand (`self.ABP XRCore Hand`)
        (:`then`
          (`/XR_Toolkit/XRCore/Assets/Meshes/HandModel/ABP_XRCoreHand.Set ControllerValue_Trigger` _abp_xrcore_hand _inaxisvalue))
        (:`else`)))))

(fn `SecondaryInput_End`
  (bind _returnvalue (`XRLaserInterface.GetXRInteractor` (`self.XRLaser`)))
  (`|ExecutionSequence`
    (:`then_0`
      (set `self.bCurrentSecondaryInput` false))
    (:`then_1`
      ;[1 1 1] Handle Interactions
      (if (`XRLaserInterface.IsLaserActive` (`self.XRLaser`))
        (`/Engine/EditorBlueprintResources/StandardMacros.IsValid` _returnvalue
          (:`Is Valid`
            (`XRInteractorComponent.StopAllXRInteractions` _returnvalue)))
        (else
          (`XRInteractorComponent.StopXRInteractionByPriority` (`self.XRInteractor`) 2 "HigherEqual"))))
    (:`then_2`
      ;[1 1 1] HandPose
      (set `self.Local_GripAxis` 0.0)
      (bind _abp_xrcore_hand (`self.ABP XRCore Hand`)
        (:`then`
          (`/XR_Toolkit/XRCore/Assets/Meshes/HandModel/ABP_XRCoreHand.Set ControllerValue_Grip` _abp_xrcore_hand 0.0))
        (:`else`)))))

(fn `SecondaryInput_Triggered`
  (params (InAxisValue :type "Float (double-precision)"))
  (bind _inaxisvalue (`local.InAxisValue`))
  (bind _returnvalue (> (`local.InAxisValue`) (/ (`self.InputAxisDeadzone`) 2.0)))
  (`|ExecutionSequence`
    (:`then_0`
      ;[1 1 1] AxisValue Deadzone gate
      (if (`self.bCurrentSecondaryInput`)
        (if (not _returnvalue)
          (set `self.bCurrentSecondaryInput` false)
          ;[1 1 1] Stop Interactions
          (if (`XRLaserInterface.IsLaserActive` (`self.XRLaser`))
            (message `XRInteractionInterface.StopAllInteractions` (`self.XRLaser`) null)
            (elif (> (`KismetArrayLibrary.Array_Length` (`XRInteractorComponent.GetActiveInteractions` (`self.XRInteractor`))) 1)
              (`XRInteractorComponent.StopXRInteractionByPriority` (`self.XRInteractor`) 5 "HigherEqual"))))
        (elif _returnvalue
          (set `self.bCurrentSecondaryInput` true)
          ;[1 1 1] Interactions
          ; Start Next Interaction
          (if (`XRLaserInterface.IsLaserActive` (`self.XRLaser`))
            (message `XRInteractionInterface.StartInteractionByPriority` (`self.XRLaser`) 0 "LowerEqual")
            (elif (`XRInteractorComponent.IsInteracting` (`self.XRInteractor`))
              (`XRInteractorComponent.StartXRInteractionByPriority` (`self.XRInteractor`) 0 "LowerEqual"))))))
    (:`then_1`
      ;[1 1 1] HandPose
      (set `self.Local_GripAxis` _inaxisvalue)
      (bind _abp_xrcore_hand (`self.ABP XRCore Hand`)
        (:`then`
          (`/XR_Toolkit/XRCore/Assets/Meshes/HandModel/ABP_XRCoreHand.Set ControllerValue_Grip` _abp_xrcore_hand _inaxisvalue))
        (:`else`)))))

(fn `SetControllerHand`
  (params (ControllerHand :type "EControllerHand Enum" :default "Left"))
  (set `self.ControllerHand` ControllerHand))

(fn `SetMotionControllerRoot_Scale`
  (params (bIsHandTracking :type Boolean))
  (bind _returnvalue (`KismetMathLibrary.MakeVector` 1.0 (select `/XR_Toolkit/XRCore/Core/Utilities/EN_ReducedControllerHand` (`/XR_Toolkit/XRCore/Core/Utilities/FL_XRUtilityFunctions.XRCore_ReduceControllerHandEnum` (`self.ControllerHand`)) :`NewEnumerator0` 1.0 :`NewEnumerator1` -1.0) 1.0))
  (`SceneComponent.K2_SetRelativeTransform` (`self.MotionController_Root`) (select `bool` (`local.bIsHandTracking`) :`false` (select `EXRStandard` (`XRToolsUtilityFunctions.GetXRStandard`) :`OpenXR` (`KismetMathLibrary.MakeTransform` (0.0 0.0 0.0) (struct) _returnvalue) :`MetaXR` (`KismetMathLibrary.MakeTransform` (-3.0 0.0 -5.0) (struct :`Pitch` 75.0) _returnvalue)) :`true` (`KismetMathLibrary.MakeTransform` (0.0 0.0 0.0))) false false))

(fn `ShouldReplicate`
  (params (InDeltaTime :type "Float (double-precision)"))
  (returns (OutShouldReplicate :type Boolean)))

(fn `Update Hand Pose`
  (bind _returnvalue (`GameplayStatics.GetWorldDeltaSeconds`))
  (bind (_triggeraxis _triggertouched _gripaxis) (break `/XR_Toolkit/XRCore/Core/Hands/F_XRHand_HandPoseReplicationData` (`.HandPoseAxis_11_0280A96848F6A398B1E653B05B765F49` (break `/XR_Toolkit/XRCore/Core/Hands/F_XRHand_ReplicationData` (`self.LatestReplicationData`)))))
  (`|ExecutionSequence`
    (:`then_0`
      (`self.Input Set Controller Value Trigger` (`KismetMathLibrary.FInterpTo` (`self.Local_TriggerAxis`) _triggeraxis _returnvalue 1.0)))
    (:`then_1`
      (`self.Input Set Controller Value Grip` (`KismetMathLibrary.FInterpTo` (`self.Local_GripAxis`) _gripaxis _returnvalue 1.0)))
    (:`then_2`
      (`/XR_Toolkit/XRCore/Assets/Meshes/HandModel/ABP_XRCoreHand.Set ControllerValue_Trigger_Touched` (`self.ABP XRCore Hand`) (`KismetMathLibrary.FInterpTo` (`self.Local_TriggerTouch`) _triggertouched _returnvalue 1.0)))))

(fn `UpdateInteractionRoot`
  (bind _handtrackingsystem (`self.HandTrackingSystem`))
  (bind _sk_hand (`self.SK_Hand`))
  (bind _boutishandtracking (`/XR_Toolkit/XRCore/Core/Hands/HandTracking/BP_XRCore_HandTrackingSystem.GetIsHandTracking` _handtrackingsystem))
  (`|ExecutionSequence`
    (:`then_0`
      (`SceneComponent.K2_SetWorldLocationAndRotation` (`self.XRInteractorRoot`) (select `bool` _boutishandtracking :`false` (/ (+ (`SceneComponent.GetSocketLocation` _sk_hand "b_l_thumb_nullSocket") (`SceneComponent.GetSocketLocation` _sk_hand "b_l_index_nullSocket")) 2.0) :`true` (`/XR_Toolkit/XRCore/Core/Hands/HandTracking/BP_XRCore_HandTrackingSystem.GetInteractionRootLocation` _handtrackingsystem)) (select `bool` _boutishandtracking :`true` (`/XR_Toolkit/XRCore/Core/Hands/HandTracking/BP_XRCore_HandTrackingSystem.GetInteractionRootRotation` _handtrackingsystem)) false false)
      (if (not (`/XR_Toolkit/XRCore/Core/Hands/HandTracking/BP_XRCore_HandTrackingSystem.GetIsHandTracking` (`self.HandTrackingSystem`)))
        (`SceneComponent.K2_SetRelativeRotation` (`self.XRInteractorRoot`) (`KismetMathLibrary.MakeRotator` -6.723 -17.578 (select `/XR_Toolkit/XRCore/Core/Utilities/EN_ReducedControllerHand` (`/XR_Toolkit/XRCore/Core/Utilities/FL_XRUtilityFunctions.XRCore_ReduceControllerHandEnum` (`self.GetControllerHand`)) :`NewEnumerator0` 41.607 :`NewEnumerator1` -41.607 :!type "Float (single-precision)")) false false)))
    (:`then_1`
      (`SceneComponent.SetVisibility` (`self.RootSphere`) (`self.bCurrentPrimaryInput`) false))))

(fn `UserConstructionScript`
  (`SceneComponent.SetHiddenInGame` (`self.Arrow1`) (not (`self.bDebugMode`)) false)
  (`SceneComponent.SetHiddenInGame` (`self.Arrow`) (not (`self.bDebugMode`)) false)
  (`SceneComponent.SetHiddenInGame` (`self.XRInteractor`) (not (`self.bDebugMode`)) false))
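; BP_DEBUG_StringBillboard is a debug actor in the XRCore hand tracking folder that displays up to three strings as in-world text.
; Every Tick it rotates to face the player 0 camera using a look-at rotation.
; UpdateText writes each non-empty input to its matching TextRender component, so an empty string leaves that line's previous text in place.
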(event `self.ReceiveTick`
  (params (DeltaSeconds :type "Float (single-precision)"))
  (`self.K2_SetActorRotation` (`KismetMathLibrary.FindLookAtRotation` (`self.K2_GetActorLocation`) (`PlayerCameraManager.GetCameraLocation` (`GameplayStatics.GetPlayerCameraManager` 0)))))

(event `UpdateText`
  (params (InString_1 :type String) (InString_2 :type String) (InString_3 :type String))
  (`|ExecutionSequence`
    (:`then_0`
      (if (not (`KismetStringLibrary.IsEmpty` InString_1))
        (`TextRenderComponent.K2_SetText` (`self.TextRender_1`) (`KismetTextLibrary.Conv_StringToText` InString_1))))
    (:`then_1`
      (if (not (`KismetStringLibrary.IsEmpty` InString_2))
        (`TextRenderComponent.K2_SetText` (`self.TextRender_2`) (`KismetTextLibrary.Conv_StringToText` InString_2))))
    (:`then_2`
      (if (not (`KismetStringLibrary.IsEmpty` InString_3))
        (`TextRenderComponent.K2_SetText` (`self.TextRender_3`) (`KismetTextLibrary.Conv_StringToText` InString_3))))))

(fn `UserConstructionScript`)
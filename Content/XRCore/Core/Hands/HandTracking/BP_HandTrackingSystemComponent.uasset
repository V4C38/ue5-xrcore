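; Hand tracking component for XRCore that appears to be an unfinished stub for feeding tracked hand data to a hand Anim Blueprint.
; Tick reads right-hand motion controller data when an assigned hand AnimBP is valid, but does nothing with the result.
; The stored controller hand is ignored, AssignAnimBP is empty, and the index-tip transform and debug prints are disconnected.
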(event `self.ReceiveBeginPlay`)

(event `self.ReceiveTick`
  (params (DeltaSeconds :type "Float (single-precision)"))
  (`self.Assigned ABP XRCore Hand`
    (:`then`
      (bind _motioncontrollerdata (`HeadMountedDisplayFunctionLibrary.GetMotionControllerData` self "Right")))
    (:`else`)))

(fn `AssignAnimBP`
  (params (`InABP XRCore Hand` :type "Object Object Reference")))

(fn `SetControllerHand`
  (params (InControllerHand :type "EControllerHand Enum" :default "Left"))
  (set `self.ControllerHand` InControllerHand))
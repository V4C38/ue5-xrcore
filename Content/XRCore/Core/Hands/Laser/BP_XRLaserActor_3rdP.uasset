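; Third-person XR hand laser actor that holds its pre-interaction length while interacting, scaled by an adjustable modifier.
; On laser state changes it captures the current length when Interacting starts, and resets the modifier when Inactive, Seeking or Hovering.
; SetDynamicLength returns the BehaviorTip location outside interaction, otherwise a point along the Root-to-Direction vector at the scaled stored length.
; EnsureInteractionValidity is left empty.
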(event `self.ReceiveBeginPlay`
  (`parent.ReceiveBeginPlay`)
  (add `self.OnLaserStateChanged` (delegate `OnLaserStateChanged_Event`)))

(event `OnLaserStateChanged_Event` :!signature `self.OnLaserStateChanged`
  (params (Sender :type "/XR_Toolkit/XRCore/Core/Hands/Laser/BP_XRLaserActor Object Reference") (NewState :type "EXRLaserState Enum" :default "Inactive"))
  (switch `EXRLaserState` NewState
    (:`Inactive`
      (set `self.bDirtyPreInteractionLength` true :!label _label)
      (set `self.Length Modifier` 1.0))
    (:`Seeking`
      (goto _label))
    (:`Hovering`
      (goto _label))
    (:`Interacting`
      (set `self.PreInteractionLength` (`self.GetCurrentLength`))
      (set `self.bDirtyPreInteractionLength` false))))

(event `self.ReceiveTick`
  (params (DeltaSeconds :type "Float (single-precision)"))
  (`parent.ReceiveTick` DeltaSeconds))

(fn `EnsureInteractionValidity`)

(fn `GetLengthModifier`
  (returns (OutLengthModifier :type "Float (double-precision)"))
  (return (`self.Length Modifier`)))

(fn `SetDynamicLength`
  (returns (OutDesiredTipLocation :type "Vector Structure"))
  (bind _returnvalue (`SceneComponent.K2_GetComponentLocation` (`self.Root`)))
  (if (`self.bDirtyPreInteractionLength`)
    (return (`SceneComponent.K2_GetComponentLocation` (`self.BehaviorTip`)))
    (else
      (return (+ _returnvalue (* (`KismetMathLibrary.GetDirectionUnitVector` _returnvalue (`SceneComponent.K2_GetComponentLocation` (`self.Direction`))) (`self.PreInteractionLength`) (`self.Length Modifier`)))))))

(fn `SetLengthModifier`
  (params (InLengthModifier :type "Float (double-precision)"))
  (set `self.Length Modifier` InLengthModifier))

(fn `UserConstructionScript`
  (`parent.UserConstructionScript`))
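; XRCore scene component that requests required runtime permissions on Android as part of its load step.
; On load it sets an in-progress LoadState, collects ungranted permissions and requests them together asynchronously.
; The response callback advances LoadState and fires OnPermissionsGranted without checking the grant results.
; Other platforms advance immediately, while Android with nothing to request never advances LoadState in this graph.
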(event `/XR_Toolkit/XRCore/Core/Scene/BPI_XRCoreScene_LoadComponent.OnLoadComponent`
  (bind _permissionstorequest (`self.PermissionsToRequest`))
  (if (`KismetStringLibrary.EqualEqual_StrStr` (`GameplayStatics.GetPlatformName`) "Android")
    (set `self.Load State` "NewEnumerator2")
    (for _array_element (`self.RequiredPermissions`)
      (bind _returnvalue (`AndroidPermissionFunctionLibrary.CheckPermission` _array_element))
      (if (not _returnvalue)
        (`KismetArrayLibrary.Array_AddUnique` (`self.PermissionsToRequest`) _array_element)))
    (if (> (`KismetArrayLibrary.Array_Length` _permissionstorequest) 0)
      (bind _returnvalue_2 (`AndroidPermissionFunctionLibrary.AcquirePermissions` _permissionstorequest))
      (add `AndroidPermissionCallbackProxy.OnPermissionsGrantedDynamicDelegate` _returnvalue_2 (delegate `OnPermissionsGrantedDynamicDelegate_Event`)))
    (else
      (set `self.Load State` "NewEnumerator3"))))

(event `OnPermissionsGrantedDynamicDelegate_Event`
  (params (Permissions :type "Array of String (by ref)") (GrantResults :type "Array of Boolean (by ref)"))
  (set `self.Load State` "NewEnumerator3")
  (`self.OnPermissionsGranted` self))
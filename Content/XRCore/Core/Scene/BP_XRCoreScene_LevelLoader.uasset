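; BP_XRCoreScene_LevelLoader is an XRCore scene-loading component that opens a configured level by object reference.
; OnLoadComponent updates LoadState and, when LoadWhenFinishedLoadScene is set, calls LoadLevel immediately and advances the state.
; LoadLevel can also be triggered as its own event and performs an absolute OpenLevel.
; GetLoadPriority reports zero with no group, and GetLoadState returns a fixed enum value rather than the LoadState variable.
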(event `/XR_Toolkit/XRCore/Core/Scene/BPI_XRCoreScene_LoadComponent.OnLoadComponent`
  (set `self.Load State` "NewEnumerator2")
  (if (`self.bLoadWhenFinishedLoadScene`)
    (`self.LoadLevel`)
    (set `self.Load State` "NewEnumerator3")))

(event `LoadLevel`
  (`GameplayStatics.OpenLevelBySoftObjectPtr` (`self.Level`)))

(fn `GetLoadPriority`
  (returns (OutLoadPriority :type Integer) (OutGroupName :type Name))
  (return 0 "None"))

(fn `GetLoadState`
  (returns (OutLoadState :type "/XR_Toolkit/XRCore/Core/Scene/EN_XRCoreScene_LoadState Enum"))
  (return "NewEnumerator0"))
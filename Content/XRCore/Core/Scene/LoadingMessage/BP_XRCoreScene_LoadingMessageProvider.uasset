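; BP_XRCoreScene_LoadingMessageProvider shows and updates an in-world loading message while an XRCore scene loads.
; On BeginPlay, outside dedicated servers and unless suppressed, it spawns a BP_XRCoreScene_LoadingMessage in front of the player camera, titled with the level name.
; Events forward load group name, component name and progress to that message actor.
; Finishing the scene load or unloading the component hides the message and updates the load state.
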(event `self.ReceiveBeginPlay`
  (bind _distancetocamera (`self.DistanceToCamera`))
  (bind _returnvalue (`Actor.GetComponentByClass` (`GameplayStatics.GetPlayerPawn` 0) "/Script/Engine.CameraComponent"))
  (if (`KismetSystemLibrary.IsDedicatedServer`)
    _
    (elif (not (`self.bSupressLoading`))
      (bind _returnvalue_2 (`|SpawnActorFromClass` "/XR_Toolkit/XRCore/Core/Scene/LoadingMessage/BP_XRCoreScene_LoadingMessage.BP_XRCoreScene_LoadingMessage_C" (`KismetMathLibrary.MakeTransform` (+ (`SceneComponent.K2_GetComponentLocation` _returnvalue) (* (`SceneComponent.GetForwardVector` _returnvalue) _distancetocamera)) (struct) (`KismetMathLibrary.Conv_DoubleToVector` (`self.SpawnSize`))) "Undefined" "MultiplyWithRoot" null _distancetocamera (`self.LevelName`) null))
      (bind _output_get (set `self.SceneLoadingMessage` _returnvalue_2))
      (set `self.Load State` "NewEnumerator3")
      (message `/XR_Toolkit/XRCore/Core/Utilities/XRAnnotation/BPI_XRCoreUI.SetTitle` _output_get (`self.LevelName`)))))

(event `/XR_Toolkit/XRCore/Core/Scene/BPI_XRCoreScene_LoadComponent.OnFinishedLoadingScene`
  (message `/XR_Toolkit/XRCore/Core/Utilities/XRAnnotation/BPI_XRCoreUI.Hide` (`self.SceneLoadingMessage`) :!label _label)
  (set `self.Load State` "NewEnumerator0"))

(event `/XR_Toolkit/XRCore/Core/Scene/BPI_XRCoreScene_LoadComponent.OnUnloadComponent`
  (goto _label))

(event `SetCurrentLoadGroupName`
  (params (InName :type Text))
  (bind _sceneloadingmessage (`self.SceneLoadingMessage`)
    (:`then`
      (message `/XR_Toolkit/XRCore/Core/Utilities/XRAnnotation/BPI_XRCoreUI.SetSubtitle` _sceneloadingmessage InName))
    (:`else`)))

(event `SetCurrentLoadingComponentName`
  (params (InName :type Text))
  (bind _sceneloadingmessage (`self.SceneLoadingMessage`)
    (:`then`
      (`/XR_Toolkit/XRCore/Core/Scene/LoadingMessage/BP_XRCoreScene_LoadingMessage.SetTitle` _sceneloadingmessage InName))
    (:`else`)))

(event `/XR_Toolkit/XRCore/Core/Utilities/XRAnnotation/BPI_XRCoreUI.SetFloatValueAtIndex`
  (params (InIndex :type Integer) (InFloatValue :type "Float (double-precision)"))
  ;[1 1 1] Update Progress Bar
  (bind _sceneloadingmessage (`self.SceneLoadingMessage`)
    (:`then`
      (message `/XR_Toolkit/XRCore/Core/Utilities/XRAnnotation/BPI_XRCoreUI.SetFloatValueAtIndex` _sceneloadingmessage 0 InFloatValue))
    (:`else`)))
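; XR loading message actor that floats in front of the player camera, showing title, subtitle, elapsed time and progress.
; Tick feeds delta time to the info widget and, unless grabbed, eases the actor toward the view direction, facing the camera.
; Interface messages route text and progress to title, info and background widgets.
; Hide waits for any grab to end, fills progress, hides the widgets and destroys the actor on a timer.
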(event `self.ReceiveBeginPlay`
  (bind _camera (`self.Camera`))
  (bind _returnvalue (`self.GetComponentByClass` (`GameplayStatics.GetPlayerPawn` 0) "/Script/Engine.CameraComponent"))
  (`|ExecutionSequence`
    (:`then_0`
      ;[1 1 1] Rotate to Player Camera
      (`/Engine/EditorBlueprintResources/StandardMacros.IsValid` _returnvalue
        (:`Is Valid`
          (set `self.Camera` _returnvalue)
          (`self.SetActorTickEnabled` true)
          (`self.K2_SetActorLocation` (+ (`SceneComponent.K2_GetComponentLocation` _camera) (* (`SceneComponent.GetForwardVector` _camera) (`self.DistanceToCamera`)))))))
    (:`then_1`
      ;[1 1 1] Update Elapsed time
      (message `/XR_Toolkit/XRCore/Core/Utilities/XRAnnotation/BPI_XRCoreUI.SetFloatValueAtIndex` (`WidgetComponent.GetUserWidgetObject` (`self.Widget_Info`)) 0 (stale `self.ReceiveTick` DeltaSeconds) :!label _label))))

(event `self.ReceiveTick`
  (params (DeltaSeconds :type "Float (single-precision)"))
  (bind _returnvalue (`self.K2_GetActorLocation`))
  (bind _camera (`self.Camera`))
  (`|ExecutionSequence`
    (:`then_0`
      (goto _label))
    (:`then_1`
      (if (not (`XRInteractionComponent.IsInteractedWith` (`self.XRInteractionGrab`)))
        (`self.K2_SetActorLocationAndRotation` (`KismetMathLibrary.VInterpTo` _returnvalue (+ (`SceneComponent.K2_GetComponentLocation` _camera) (* (`SceneComponent.GetForwardVector` _camera) (`self.DistanceToCamera`))) DeltaSeconds 2.0) (`KismetMathLibrary.FindLookAtRotation` _returnvalue (`SceneComponent.K2_GetComponentLocation` (`self.Camera`))))))))

(event `/XR_Toolkit/XRCore/Core/Utilities/XRAnnotation/BPI_XRCoreUI.SetSubtitle`
  (params (InSubtitle :type Text))
  (message `/XR_Toolkit/XRCore/Core/Utilities/XRAnnotation/BPI_XRCoreUI.SetSubtitle` (`WidgetComponent.GetUserWidgetObject` (`self.Widget_Info`)) InSubtitle))

(event `/XR_Toolkit/XRCore/Core/Utilities/XRAnnotation/BPI_XRCoreUI.SetTitle`
  (params (InTitle :type Text))
  (message `/XR_Toolkit/XRCore/Core/Utilities/XRAnnotation/BPI_XRCoreUI.SetTitle` (`WidgetComponent.GetUserWidgetObject` (`self.Widget_Title`)) InTitle))

(event `/XR_Toolkit/XRCore/Core/Utilities/XRAnnotation/BPI_XRCoreUI.Hide`
  (bind _returnvalue (`WidgetComponent.GetUserWidgetObject` (`self.Widget_Background`)))
  (if (`XRInteractionComponent.IsInteractedWith` (`self.XRInteractionGrab`))
    (add `XRInteractionComponent.OnInteractionEnded` (`self.XRInteractionGrab`) (delegate `OnInteractionEnded_Event`))
    (else
      (bind _returnvalue_2 (`KismetSystemLibrary.K2_SetTimerDelegate` (delegate `DestroyMessage`) (`self.DestroyTime`) :!label _label_2))
      (set `self.DestroyTimer` _returnvalue_2)
      (message `/XR_Toolkit/XRCore/Core/Utilities/XRAnnotation/BPI_XRCoreUI.SetFloatValueAtIndex` _returnvalue 0 1.0)
      (message `/XR_Toolkit/XRCore/Core/Utilities/XRAnnotation/BPI_XRCoreUI.Hide` _returnvalue)
      (message `/XR_Toolkit/XRCore/Core/Utilities/XRAnnotation/BPI_XRCoreUI.Hide` (`WidgetComponent.GetUserWidgetObject` (`self.Widget_Info`)))
      (message `/XR_Toolkit/XRCore/Core/Utilities/XRAnnotation/BPI_XRCoreUI.Hide` (`WidgetComponent.GetUserWidgetObject` (`self.Widget_Title`))))))

(event `OnInteractionEnded_Event`
  (params (Sender :type "XRInteractionComponent Object Reference") (XRInteractorComponent :type "XRInteractorComponent Object Reference"))
  (`ActorComponent.Deactivate` (`self.XRInteractionGrab`))
  (goto _label_2))

(event `DestroyMessage`
  (`self.K2_DestroyActor`))

(event `/XR_Toolkit/XRCore/Core/Utilities/XRAnnotation/BPI_XRCoreUI.SetFloatValueAtIndex`
  (params (InIndex :type Integer) (InFloatValue :type "Float (double-precision)"))
  ;[1 1 1] Update Progress Bar
  (message `/XR_Toolkit/XRCore/Core/Utilities/XRAnnotation/BPI_XRCoreUI.SetFloatValueAtIndex` (`WidgetComponent.GetUserWidgetObject` (`self.Widget_Background`)) 0 InFloatValue))

(fn `UserConstructionScript`)
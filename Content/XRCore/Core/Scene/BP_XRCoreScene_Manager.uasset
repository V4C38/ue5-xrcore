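; XRCore scene manager that, on BeginPlay, loads its own scene components in priority-ordered groups and broadcasts loading start and completion.
; Components implementing BPI_XRCoreScene_LoadComponent are bucketed by priority into group UObjects, skipping suppressed ones.
; Groups load sequentially from highest priority, polled by a looping timer because Blueprint UObjects lack timers, while progress feeds a loading message provider.
; An optional timeout auto-completes the scene load.
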(event `self.ReceiveBeginPlay`
  (`self.SetLoadState` "NewEnumerator1")
  (`self.CacheLoadingGroups`)
  (`self.LoadScene`))

(event `LoadScene`
  ;[0 0 0] Load Scene
  (`self.SetLoadState` "NewEnumerator2")
  (`|ExecutionSequence`
    (:`then_0`
      (`self.OnLoadingScene` self))
    (:`then_1`
      (bind _returnvalue (`KismetSystemLibrary.K2_SetTimerDelegate` (delegate `OnLoadTimerFinished`) (`self.AutoCompleteSceneLoadAfterSeconds`)))
      (set `self.Timer_SceneLoadDuration` _returnvalue))
    (:`then_2`
      (bind _values (`BlueprintMapLibrary.Map_Values` (`self.ComponentGroups`)))
      (for _array_element _values
        (`/XR_Toolkit/XRCore/Core/Scene/BP_XRCoreScene_ComponentLoadingGroup.QueueGroup` _array_element))
      (`self.LoadNextGroup`) ; Start Loading all groups sequentially
    )
    (:`then_3`
      (`KismetSystemLibrary.PrintString` (`KismetStringLibrary.Concat_StrStr` "XRCore Scene: Loading " (`KismetStringLibrary.Conv_IntToString` (`BlueprintMapLibrary.Map_Length` (`self.ComponentGroups`))) " component groups.") true true (struct :`G` 0.5 :`A` 1.0) 5.0 "XRCoreScene_Init"))))

(event `OnLoadTimerFinished`
  ;[0 0 0] Load Scene
  (if (`self.bAutoCompleteSceneLoad`)
    (`self.LoadSceneCompleted`)))

(event `LoadNextGroup`
  (bind (_success _outloadinggroup) (`self.GetHighestPriorityLoadingGroup`))
  ;[1 1 1] Load Group
  (if _success
    (bind _output_get (`self.SetCurrentLoadGroup` _outloadinggroup))
    (`/Engine/EditorBlueprintResources/StandardMacros.IncrementInt` (`self.LoadedGroups`)
      (:`  `
        (`/XR_Toolkit/XRCore/Core/Scene/BP_XRCoreScene_ComponentLoadingGroup.LoadGroup` _output_get)
        (add `/XR_Toolkit/XRCore/Core/Scene/BP_XRCoreScene_ComponentLoadingGroup.OnGroupLoadStateChanged` _output_get (delegate `OnGroupLoadStateChanged_Event`))
        (`KismetSystemLibrary.PrintString` (`KismetStringLibrary.Concat_StrStr` "XRCore Scene: " (`KismetStringLibrary.Concat_StrStr` "loading group: " (`KismetStringLibrary.Conv_NameToString` (`/XR_Toolkit/XRCore/Core/Scene/BP_XRCoreScene_ComponentLoadingGroup.GroupName` (`self.CurrentLoadGroup`))))) true true (struct :`G` 0.5 :`A` 1.0) 2.0 "XRCoreScene_LoaderDetail")
        ;[0.3 0.3 0.3] Force check group load state as UObject cannot have timers in BP
        ; (if this is moved to C++ this can be moved to the group directly)
        (bind _returnvalue (`KismetSystemLibrary.K2_SetTimerDelegate` (delegate `CheckGroupLoadState`) 0.4 true))
        (set `self.Timer_CheckGroupLoadState` _returnvalue)))
    (else
      (`self.SetCurrentLoadGroup` null)
      (`self.LoadSceneCompleted`))))

(event `CheckGroupLoadState`
  ;[0.3 0.3 0.3] Force check group load state as UObject cannot have timers in BP
  ; (if this is moved to C++ this can be moved to the group directly)
  (`/XR_Toolkit/XRCore/Core/Scene/BP_XRCoreScene_ComponentLoadingGroup.CheckGroupLoadState` (`self.CurrentLoadGroup`)))

(event `OnGroupLoadStateChanged_Event`
  (params (Sender :type "/XR_Toolkit/XRCore/Core/Scene/BP_XRCoreScene_ComponentLoadingGroup Object Reference") (OutLoadState :type "/XR_Toolkit/XRCore/Core/Scene/EN_XRCoreScene_LoadState Enum" :default "NewEnumerator0"))
  ;[1 1 1] Once this group is loaded, unbind all and load next group
  (if (`|EnumEquality` OutLoadState "NewEnumerator3")
    (clear `/XR_Toolkit/XRCore/Core/Scene/BP_XRCoreScene_ComponentLoadingGroup.OnGroupLoadStateChanged` Sender)
    (`KismetSystemLibrary.K2_ClearAndInvalidateTimerHandle` (`self.Timer_CheckGroupLoadState`))
    (`self.LoadNextGroup`)
    (`KismetSystemLibrary.PrintString` (`KismetStringLibrary.Concat_StrStr` "XRCore Scene: finished loading group: " (`KismetStringLibrary.Conv_NameToString` (`/XR_Toolkit/XRCore/Core/Scene/BP_XRCoreScene_ComponentLoadingGroup.GroupName` Sender))) true true (struct :`G` 0.5 :`A` 1.0) 2.0 "XRCoreScene_LoaderDetail")))

(event `LoadSceneCompleted`
  ;[0 0 0] Finished Load Scene
  (`KismetSystemLibrary.K2_ClearAndInvalidateTimerHandle` (`self.Timer_CheckGroupLoadState`))
  (`|ExecutionSequence`
    (:`then_0`
      (`self.OnLoadingSceneCompleted` self))
    (:`then_1`
      (bind _values (`BlueprintMapLibrary.Map_Values` (`self.ComponentGroups`)))
      (for _array_element _values
        (`/XR_Toolkit/XRCore/Core/Scene/BP_XRCoreScene_ComponentLoadingGroup.CompleteGroup` _array_element)))
    (:`then_2`
      (`KismetSystemLibrary.PrintString` (`KismetStringLibrary.Concat_StrStr` "XRCore Scene: Finished Loading.  \nLoaded a total of " (`KismetStringLibrary.Conv_IntToString` (`BlueprintMapLibrary.Map_Length` (`self.ComponentGroups`))) " SceneComponent groups took " (`KismetStringLibrary.Conv_DoubleToString` (`KismetSystemLibrary.K2_GetTimerElapsedTimeHandle` (`self.Timer_SceneLoadDuration`))) " Seconds." (select `bool` (`self.bAutoCompleteSceneLoad`) :`true` " \n(Autocompleted)")) true true (struct :`G` 0.5 :`A` 1.0) 5.0 "XRCoreScene_Init")
      (`KismetSystemLibrary.K2_ClearAndInvalidateTimerHandle` (`self.Timer_SceneLoadDuration`)))
    (:`then_3`
      (`self.SetLoadState` "NewEnumerator3"))))

(fn `CacheLoadingGroups`
  (locals (Loc_UnsortedLoadingGroups :type "Map of Integer to /XR_Toolkit/XRCore/Core/Scene/BP_XRCoreScene_ComponentLoadingGroup Object Reference"))
  (for _array_element (`self.GetComponentsByInterface` "/XR_Toolkit/XRCore/Core/Scene/BPI_XRCoreScene_LoadComponent.BPI_XRCoreScene_LoadComponent_C")
    (bind _bsupressloading (message `/XR_Toolkit/XRCore/Core/Scene/BPI_XRCoreScene_LoadComponent.GetSupressesLoading` _array_element))
    (if _bsupressloading
      ;[1 1 1] Component is supressed manually (Does not load)
      (message `/XR_Toolkit/XRCore/Core/Scene/BPI_XRCoreScene_LoadComponent.OnSupressedLoading` _array_element)
      (`KismetSystemLibrary.PrintString` (`KismetStringLibrary.Concat_StrStr` "XRCore Scene: did not load component (supressed load): " (`KismetSystemLibrary.GetDisplayName` _array_element)) true true (struct :`G` 0.5 :`A` 1.0) 2.0 "XRCoreScene_LoaderDetail")
      (else
        (bind (_outloadpriority _outgroupname) (message `/XR_Toolkit/XRCore/Core/Scene/BPI_XRCoreScene_LoadComponent.GetLoadPriority` _array_element))
        (bind (_value _returnvalue) (`BlueprintMapLibrary.Map_Find` (`local.Loc_UnsortedLoadingGroups`) _outloadpriority))
        (if _returnvalue
          ;[1 1 1] Add to existing group
          (`/XR_Toolkit/XRCore/Core/Scene/BP_XRCoreScene_ComponentLoadingGroup.AddXRCoreSceneComponent` _value _array_element "NewEnumerator0")
          (else
            ;[1 1 1] Group does not exist yet -> make new and add component
            (bind _returnvalue_2 (`|GenericCreateObject` self "/XR_Toolkit/XRCore/Core/Scene/BP_XRCoreScene_ComponentLoadingGroup.BP_XRCoreScene_ComponentLoadingGroup_C" _outloadpriority _outgroupname))
            (`/XR_Toolkit/XRCore/Core/Scene/BP_XRCoreScene_ComponentLoadingGroup.AddXRCoreSceneComponent` _returnvalue_2 _array_element "NewEnumerator0")
            (`BlueprintMapLibrary.Map_Add` (`local.Loc_UnsortedLoadingGroups`) _outloadpriority _returnvalue_2))))))
  (set `self.ComponentGroups` (`local.Loc_UnsortedLoadingGroups`))
  (set `self.LoadedGroups` 0)
  (return))

(fn `GetHighestPriorityLoadingGroup`
  (returns (Success :type Boolean) (OutLoadingGroup :type "/XR_Toolkit/XRCore/Core/Scene/BP_XRCoreScene_ComponentLoadingGroup Object Reference"))
  (locals (Loc_HighestPriority :type Integer :default -1) (Loc_OutGroup :type "/XR_Toolkit/XRCore/Core/Scene/BP_XRCoreScene_ComponentLoadingGroup Object Reference"))
  (bind (_value _returnvalue) (`BlueprintMapLibrary.Map_Find` (`self.ComponentGroups`) (`local.Loc_HighestPriority`)))
  (bind _values (`BlueprintMapLibrary.Map_Values` (`self.ComponentGroups`)))
  (for _array_element _values
    (switch `/XR_Toolkit/XRCore/Core/Scene/EN_XRCoreScene_LoadState` (`/XR_Toolkit/XRCore/Core/Scene/BP_XRCoreScene_ComponentLoadingGroup.GetGroupLoadedState` _array_element)
      (:`NewEnumerator0`
        _)
      (:`NewEnumerator1`
        _))
    (bind _priority (`/XR_Toolkit/XRCore/Core/Scene/BP_XRCoreScene_ComponentLoadingGroup.Priority` _array_element))
    (if (> _priority (`local.Loc_HighestPriority`))
      (set `local.Loc_HighestPriority` _priority)))
  (if _returnvalue
    (return true _value)
    (else
      (return false null))))

(fn `GetLoadState`
  (returns (OutLoadState :type "/XR_Toolkit/XRCore/Core/Scene/EN_XRCoreScene_LoadState Enum"))
  (return (`self.LoadState`)))

(fn `SetCurrentLoadGroup`
  (params (CurrentLoadGroup :type "/XR_Toolkit/XRCore/Core/Scene/BP_XRCoreScene_ComponentLoadingGroup Object Reference"))
  (returns (Output_Get :type "/XR_Toolkit/XRCore/Core/Scene/BP_XRCoreScene_ComponentLoadingGroup Object Reference"))
  (bind _bp_xrcorescene_loadingmessageprovider (`self.BP_XRCoreScene_LoadingMessageProvider`))
  (bind _output_get (set `self.CurrentLoadGroup` CurrentLoadGroup))
  (`/Engine/EditorBlueprintResources/StandardMacros.IsValid` _output_get
    (:`Is Valid`
      (`/XR_Toolkit/XRCore/Core/Scene/LoadingMessage/BP_XRCoreScene_LoadingMessageProvider.SetCurrentLoadGroupName` _bp_xrcorescene_loadingmessageprovider (`KismetTextLibrary.Conv_NameToText` (`/XR_Toolkit/XRCore/Core/Scene/BP_XRCoreScene_ComponentLoadingGroup.GroupName` _output_get))))
    (:`Is Not Valid`
      _))
  (message `/XR_Toolkit/XRCore/Core/Utilities/XRAnnotation/BPI_XRCoreUI.SetFloatValueAtIndex` _bp_xrcorescene_loadingmessageprovider 0 (/ (`KismetMathLibrary.Conv_IntToDouble` (`self.LoadedGroups`)) (`KismetMathLibrary.Conv_IntToDouble` (`BlueprintMapLibrary.Map_Length` (`self.ComponentGroups`)))))
  (return (`self.CurrentLoadGroup`)))

(fn `SetLoadState`
  (params (InLoadState :type "/XR_Toolkit/XRCore/Core/Scene/EN_XRCoreScene_LoadState Enum" :default "NewEnumerator0"))
  (if (`|EnumInequality` InLoadState (`self.LoadState`))
    (set `self.LoadState` InLoadState)))

(fn `UserConstructionScript`)
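; VR teleport pointer actor that shows an aiming arc and landing circle, and exposes target validity, location and rotation.
; While active, Tick eases aim toward its parent root and predicts a gravity projectile path, validating hit actors by tag.
; Each tick rebuilds the path as spline meshes sharing a dynamic material, dimmed when invalid.
; Starting plays a distance-scaled reveal timeline, then scales up the circle; stopping hides the actor and disables Tick.
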(event `self.ReceiveBeginPlay`
  ;[1 1 1] INIT
  (`self.Init Dyna Material`))

(event `self.ReceiveTick`
  (params (DeltaSeconds :type "Float (single-precision)"))
  ;[1 1 1] TICK
  ; Only active while Teleporting
  (`|ExecutionSequence`
    (:`then_0`
      (`self.SmoothTeleportDirection` DeltaSeconds))
    (:`then_1`
      (`self.TraceTeleportLocation`)
      (`self.Update Visuals`))))

(event `StartTeleporter`
  (bind _attachedtoparent_root (`self.AttachedToParent_Root`))
  ;[0 0 0] Start
  ; - TeleportStart Buildup Animation
  (`|ExecutionSequence`
    (:`then_0`
      (`SceneComponent.SetRelativeScale3D` (`self.TeleportCylinder`) (0.0 0.0 0.0))
      (`self.SetActorTickEnabled` true)
      (`self.SetActorHiddenInGame` false)
      (set `self.bBuildupComplete` false)
      (`SceneComponent.K2_SetWorldLocationAndRotation` (`self.FollowingRoot`) (`SceneComponent.K2_GetComponentLocation` _attachedtoparent_root) (`SceneComponent.K2_GetComponentRotation` _attachedtoparent_root) false false :!label _label))
    (:`then_1`
      (`TimelineComponent.SetPlayRate` (`self.Timeline_BuildUp`) (`self.GetBuildUpSpeedByDistance`))
      (bind (_direction _curve_range) (`Timeline|Timeline_BuildUp` :!via `PlayFromStart`)
        (:`Update`
          (`MaterialInstanceDynamic.SetScalarParameterValue` (`self.DynaMat_Arc`) "VisibilityDistance" (`self.GetBuildupVisibilityDistance` _curve_range))
          (goto _label))
        (:`Finished`
          (`TimelineComponent.SetPlayRate` (`self.Timeline_ScaleUp`) 6.0)
          (bind (_direction_2 _teleportcircle_scale) (`Timeline|Timeline_ScaleUp` :!via `PlayFromStart`)
            (:`Update`
              (`SceneComponent.SetRelativeScale3D` (`self.TeleportCylinder`) (`KismetMathLibrary.Conv_DoubleToVector` _teleportcircle_scale)))
            (:`Finished`
              (set `self.bBuildupComplete` true))))))))

(event `StopTeleporter`
  ;[0 0 0] Stop
  (`self.SetActorHiddenInGame` true)
  (`self.SetActorTickEnabled` false)
  (`self.ClearArc`)
  (`TimelineComponent.Stop` (`self.Timeline_BuildUp`))
  (`TimelineComponent.Stop` (`self.Timeline_ScaleUp`)))

(fn `CheckActorForValidTags`
  (params (InActorToCheck :type "Actor Object Reference"))
  (returns (bHasValidTag :type Boolean))
  (locals (bLocal_FoundTag :type Boolean :default false))
  (`/Engine/EditorBlueprintResources/StandardMacros.IsValid` InActorToCheck
    (:`Is Valid`
      (for _array_element (`Actor.Tags` InActorToCheck)
        (if (`KismetArrayLibrary.Array_Contains` (`self.AllowTeleportOnActorsWithTags`) _array_element)
          (set `local.bLocal_FoundTag` true)))
      (return (`local.bLocal_FoundTag`)))))

(fn `ClearArc`
  (bind _splinemeshes (`self.SplineMeshes`))
  (`ActorComponent.K2_DestroyComponent` _splinemeshes)
  (`KismetArrayLibrary.Array_Clear` _splinemeshes)
  (`SplineComponent.ClearSplinePoints` (`self.ArcSpline`) true))

(fn `GetBuildUpSpeedByDistance`
  (returns (OutPlayRate :type "Float (double-precision)"))
  (bind _buildupspeed (`self.BuildUpSpeed`))
  (bind _skipbuildupdistancetreshold (`self.SkipBuildupDistanceTreshold`))
  (bind (_traceresult_pathpoints _traceresult_lasttracedestination) (break `/XR_Toolkit/XRCore/Core/Utilities/VRLocomotion/Teleport/FTeleportTraceResult_BP` (`self.TraceResult`)))
  (return (`KismetMathLibrary.MapRangeClamped` (`KismetMathLibrary.Vector_Distance` _traceresult_lasttracedestination (`SceneComponent.K2_GetComponentLocation` (`self.ArcDirection`))) _skipbuildupdistancetreshold (* _skipbuildupdistancetreshold 5.0) (* 5.0 _buildupspeed) _buildupspeed)))

(fn `GetBuildupVisibilityDistance`
  (params (InAlpha :type "Float (double-precision)"))
  (returns (OutDistance :type "Float (double-precision)"))
  (bind (_traceresult_pathpoints _traceresult_lasttracedestination) (break `/XR_Toolkit/XRCore/Core/Utilities/VRLocomotion/Teleport/FTeleportTraceResult_BP` (`self.TraceResult`)))
  (return (* InAlpha (`KismetMathLibrary.Vector_Distance` _traceresult_lasttracedestination (`SceneComponent.K2_GetComponentLocation` (`self.ArcDirection`))) 1.1)))

(fn `GetTeleportData`
  (returns (`Trace Result Is Valid Location` :type Boolean) (TeleportLocation :type "Vector Structure") (TeleportRotation :type "Rotator Structure"))
  (bind (_traceresult_pathpoints _traceresult_lasttracedestination _traceresult_bisvalidlocation) (break `/XR_Toolkit/XRCore/Core/Utilities/VRLocomotion/Teleport/FTeleportTraceResult_BP` (`self.TraceResult`)))
  (return _traceresult_bisvalidlocation _traceresult_lasttracedestination (`self.TeleportRotation`)))

(fn `Init Dyna Material`
  (bind _returnvalue (`KismetMaterialLibrary.CreateDynamicMaterialInstance` "/XR_Toolkit/XRCore/Assets/MaterialLibrary/Laser/MI_TeleportSpline.MI_TeleportSpline"))
  (bind _output_get (set `self.DynaMat_Arc` _returnvalue))
  (`MaterialInstanceDynamic.SetScalarParameterValue` _output_get "Thickness" -0.25))

(fn `Is Teleporter Active`
  (returns (bIsActive :type Boolean))
  (return (`self.IsActorTickEnabled`)))

(fn `SetTeleportRotation`
  (params (TeleportRotation :type "Rotator Structure"))
  (set `self.TeleportRotation` TeleportRotation))

(fn `SmoothTeleportDirection`
  (params (InDeltaTime :type "Float (single-precision)"))
  (bind _attachedtoparent_root (`self.AttachedToParent_Root`))
  (`SceneComponent.K2_SetWorldLocationAndRotation` (`self.FollowingRoot`) (`SceneComponent.K2_GetComponentLocation` _attachedtoparent_root) (`KismetMathLibrary.RInterpTo` (`SceneComponent.K2_GetComponentRotation` (`self.FollowingRoot`)) (`SceneComponent.K2_GetComponentRotation` _attachedtoparent_root) (`local.InDeltaTime`) 7.5) false false))

(fn `TraceTeleportLocation`
  (bind _arcdirection (`self.ArcDirection`))
  (bind (_traceresult_pathpoints _traceresult_lasttracedestination) (break `/XR_Toolkit/XRCore/Core/Utilities/VRLocomotion/Teleport/FTeleportTraceResult_BP` (`self.TraceResult`)))
  (bind (_outhit _outpathpositions _outlasttracedestination _returnvalue) (`GameplayStatics.Blueprint_PredictProjectilePath_ByObjectType` (`SceneComponent.K2_GetComponentLocation` _arcdirection) (* (`SceneComponent.GetForwardVector` _arcdirection) (`self.TeleportLaunchVelocity`)) true 0.0 (`|MakeArray` "ObjectTypeQuery1" :!type "EObjectTypeQuery Enum") false (`|MakeArray` (`self.GetOwner`)) "None" 0.0 30.0)) ; Simulate throwing a projectile (including gravity) to find a teleport location.
  (if _returnvalue
    (bind (_bblockinghit _binitialoverlap _time _distance _location _impactpoint _normal _impactnormal _physmat _hitactor) (`GameplayStatics.BreakHitResult` _outhit))
    (set `self.TraceResult` (make `/XR_Toolkit/XRCore/Core/Utilities/VRLocomotion/Teleport/FTeleportTraceResult_BP` _outpathpositions _impactpoint (`self.CheckActorForValidTags` _hitactor)))
    (else
      (set `self.TraceResult` (make `/XR_Toolkit/XRCore/Core/Utilities/VRLocomotion/Teleport/FTeleportTraceResult_BP` _traceresult_pathpoints _traceresult_lasttracedestination))))
  (return))

(fn `Update Visuals`
  (bind _dynamat_arc (`self.DynaMat_Arc`))
  (bind _teleportcylinder (`self.TeleportCylinder`))
  (bind (_traceresult_pathpoints _traceresult_lasttracedestination _traceresult_bisvalidlocation) (break `/XR_Toolkit/XRCore/Core/Utilities/VRLocomotion/Teleport/FTeleportTraceResult_BP` (`self.TraceResult`)))
  (bind (_traceresult_pathpoints_2 _traceresult_lasttracedestination_2 _traceresult_bisvalidlocation_2) (break `/XR_Toolkit/XRCore/Core/Utilities/VRLocomotion/Teleport/FTeleportTraceResult_BP` (`self.TraceResult`)))
  (`|ExecutionSequence`
    (:`then_0`
      ;[0 0 0] Setup Arc
      (`self.ClearArc`)
      (`self.UpdateArc`))
    (:`then_1`
      ;[0 0 0] Only Set Circle visible when location is valid
      (`SceneComponent.SetVisibility` _teleportcylinder _traceresult_bisvalidlocation_2 false)
      (`SceneComponent.SetVisibility` (`self.RotationIndicator`) _traceresult_bisvalidlocation_2 false)
      (bind _output_get (set `self.LastValidLocation` _traceresult_lasttracedestination_2))
      (`SceneComponent.K2_SetWorldLocation` _teleportcylinder _output_get false false)
      (`SceneComponent.K2_SetWorldRotation` _teleportcylinder (`self.TeleportRotation`) false false))
    (:`then_2`
      (if (`self.bBuildupComplete`)
        ;[0 0 0] Materials
        (`MaterialInstanceDynamic.SetScalarParameterValue` (`self.DynaMat_Arc`) "VisibilityDistance" 100000.0))
      (`MaterialInstanceDynamic.SetVectorParameterValue` _dynamat_arc "AWP_Root" (`KismetMathLibrary.Conv_VectorToLinearColor` (`SceneComponent.K2_GetComponentLocation` (`self.FollowingRoot`))))
      (`MaterialInstanceDynamic.SetScalarParameterValue` _dynamat_arc "Opacity" (select `bool` _traceresult_bisvalidlocation :`false` 0.15 :`true` 1.0)))))

(fn `UpdateArc`
  (bind _traceresult_pathpoints (break `/XR_Toolkit/XRCore/Core/Utilities/VRLocomotion/Teleport/FTeleportTraceResult_BP` (`self.TraceResult`)))
  (bind _arcspline (`self.ArcSpline`))
  (bind (_traceresult_pathpoints_2 _traceresult_lasttracedestination _traceresult_bisvalidlocation) (break `/XR_Toolkit/XRCore/Core/Utilities/VRLocomotion/Teleport/FTeleportTraceResult_BP` (`self.TraceResult`)))
  (bind _arcspline_2 (`self.ArcSpline`))
  (bind _traceresult_pathpoints_3 (break `/XR_Toolkit/XRCore/Core/Utilities/VRLocomotion/Teleport/FTeleportTraceResult_BP` (`self.TraceResult`)))
  ;[1 1 1] Add Spline points
  ; (+ configure last point)
  (for _array_element _traceresult_pathpoints_3
    (`SplineComponent.AddSplinePoint` _arcspline_2 _array_element "Local" false) ; Build a spline from all trace points. This generates tangets we can use to build a smoothly curved spline mesh
  )
  (`SplineComponent.SetSplinePointType` _arcspline_2 (`KismetArrayLibrary.Array_LastIndex` _traceresult_pathpoints_3) "CurveClamped" true) ; Update the point type to create the curve
  ;[1 1 1] Set Spline MeshComponents
  (for _index (range (+ (- (`SplineComponent.GetNumberOfSplinePoints` (`self.ArcSpline`)) 2) 1))
    (bind _returnvalue (`AddComponent|NODE_AddSplineMeshComponent-0` :`bManualAttachment` true :`RelativeTransform` (`KismetMathLibrary.MakeTransform` (0.0 0.0 0.0)))) ; Add new cylinder mesh
    (`PrimitiveComponent.SetMaterial` _returnvalue 0 (`self.DynaMat_Arc`))
    (`KismetArrayLibrary.Array_Add` (`self.SplineMeshes`) _returnvalue)
    (bind _returnvalue_2 (+ _index 1))
    (`SplineMeshComponent.SetStartAndEnd` _returnvalue (`|GetArrayItem` _traceresult_pathpoints _index) (`SplineComponent.GetTangentAtSplinePoint` _arcspline _index "Local") (`|GetArrayItem` _traceresult_pathpoints _returnvalue_2) (`SplineComponent.GetTangentAtSplinePoint` _arcspline _returnvalue_2 "Local") true) ; Set the tangents and position to build slightly bend the cylinder. All cylinders combined create a smooth arc.
    ;[1 1 1] Set EndPoint to Teleport Location
    (`SceneComponent.SetVisibility` (`self.TipSphere`) (xor _traceresult_bisvalidlocation false) false)))

(fn `UserConstructionScript`)
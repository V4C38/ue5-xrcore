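; Pawn component that runs networked VR teleportation through a replicated BP_XRTeleportOrigin actor spawned by the server.
; Start, rotation, execute and abort requests go through server events to multicasts that drive that actor, whose settings are pushed on RepNotify.
; The teleporter starts only for the local player unless flagged visible to other clients.
; Execute moves the owner to the traced location if valid, then reports success or failure.
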(event `self.ReceiveBeginPlay`
  ;[1 1 1] Init
  (`|ExecutionSequence`
    (:`then_0`
      (bind _aspawn (cast `Pawn` (`self.GetOwner`)))
      (set `self.bIsLocalTeleporter` (`Pawn.IsLocallyControlled` _aspawn)))
    (:`then_1`
      (if (`KismetSystemLibrary.IsServer`)
        (`self.BP_XRTeleportOrigin`
          (:`then`)
          (:`else`
            (bind _returnvalue (`|SpawnActorFromClass` "/XR_Toolkit/XRCore/Core/Utilities/VRLocomotion/Teleport/BP_XRTeleportOrigin.BP_XRTeleportOrigin_C" (`KismetMathLibrary.MakeTransform` (0.0 0.0 0.0)) "Undefined" "OverrideRootScale" (`self.GetOwner`) null))
            (`Actor.SetReplicates` _returnvalue true)
            (set `self.BP_XRTeleportOrigin` _returnvalue)))))))

(event `Server_RequestTeleport_SetRotation`
  (params (TeleportRotation :type "Rotator Structure"))
  ;[0 0 0] Rotation
  (bind _output_get (set `self.TeleportRotation` TeleportRotation))
  (`self.Multicast_RequestTeleport_SetRotation` _output_get))

(event `Server_RequestTeleport_Start`
  (params (InRequestingHand :type "EControllerHand Enum" :default "Left") (RootComponent :type "SceneComponent Object Reference") (PlayerCamera :type "SceneComponent Object Reference"))
  ;[0 0 0] Request Start
  (set `self.TeleportHand` InRequestingHand)
  (`self.Multicast_RequestTeleport_Start` RootComponent PlayerCamera))

(event `Multicast_RequestTeleport_SetRotation`
  (params (TeleportRotation :type "Rotator Structure"))
  ;[0 0 0] Rotation
  (bind _bp_xrteleportorigin (`self.BP_XRTeleportOrigin`)
    (:`then`
      (`/XR_Toolkit/XRCore/Core/Utilities/VRLocomotion/Teleport/BP_XRTeleportOrigin.SetTeleportRotation` _bp_xrteleportorigin TeleportRotation))
    (:`else`)))

(event `Multicast_RequestTeleport_Start`
  (params (RootComponent :type "SceneComponent Object Reference") (PlayerCamera :type "SceneComponent Object Reference"))
  (bind (_returnvalue_roll _returnvalue_pitch _returnvalue_yaw) (`KismetMathLibrary.BreakRotator` (`SceneComponent.K2_GetComponentRotation` PlayerCamera)))
  ;[0 0 0] Request Start
  (if (`self.IsActive`)
    (if (`self.IsTeleporterVisibleOnThisClient`)
      (`|ExecutionSequence`
        (:`then_0`
          (bind _bp_xrteleportorigin (`self.BP_XRTeleportOrigin`)
            (:`then`
              (`SceneComponent.K2_AttachToComponent` (`/XR_Toolkit/XRCore/Core/Utilities/VRLocomotion/Teleport/BP_XRTeleportOrigin.AttachedToParent_Root` _bp_xrteleportorigin) RootComponent "None" "SnapToTarget" "SnapToTarget" "KeepWorld" true))
            (:`else`)))
        (:`then_1`
          (bind _bp_xrteleportorigin_2 (`self.BP_XRTeleportOrigin`)
            (:`then`
              (`/XR_Toolkit/XRCore/Core/Utilities/VRLocomotion/Teleport/BP_XRTeleportOrigin.StartTeleporter` _bp_xrteleportorigin_2)
              (`self.Server_RequestTeleport_SetRotation` (`KismetMathLibrary.MakeRotator` 0.0 0.0 _returnvalue_yaw)))
            (:`else`)))
        (:`then_2`
          (`self.OnSeekingTeleportTarget` self))))
    (else
      (`self.Server_RequestTeleport_Abort`))))

(event `Server_RequestTeleport_Execute`
  ;[0 0 0] Execute Teleport
  (`self.Multicast_RequestTeleport_Execute`))

(event `Multicast_RequestTeleport_Execute`
  (bind (_trace_result_is_valid_location _teleportlocation _teleportrotation) (`/XR_Toolkit/XRCore/Core/Utilities/VRLocomotion/Teleport/BP_XRTeleportOrigin.GetTeleportData` (`self.BP_XRTeleportOrigin`)))
  ;[0 0 0] Execute Teleport
  (if (`/XR_Toolkit/XRCore/Core/Utilities/VRLocomotion/Teleport/BP_XRTeleportOrigin.Is Teleporter Active` (`self.BP_XRTeleportOrigin`))
    (`|ExecutionSequence`
      (:`then_0`
        (`/XR_Toolkit/XRCore/Core/Utilities/VRLocomotion/Teleport/BP_XRTeleportOrigin.StopTeleporter` (`self.BP_XRTeleportOrigin`) :!label _label))
      (:`then_1`
        ;;[1 1 1] Execute Teleport for Owning Pawn
        (if _trace_result_is_valid_location
          (`Actor.K2_SetActorLocationAndRotation` (`self.GetOwner`) _teleportlocation _teleportrotation false false)
          (`self.OnTeleported` self true)
          (else
            (`self.OnTeleported` self :!label _label_2)))))
    (else
      (`|ExecutionSequence`
        (:`then_0`
          (goto _label))
        (:`then_1`
          (goto _label_2))))))

(event `Server_RequestTeleport_Abort`
  ;[0 0 0] Execute Teleport
  ;;[0 0 0] Abort
  (`self.Multicast_RequestTeleport_Abort`))

(event `Multicast_RequestTeleport_Abort`
  ;[0 0 0] Execute Teleport
  ;;[0 0 0] Abort
  (`|ExecutionSequence`
    (:`then_0`
      (bind _bp_xrteleportorigin (`self.BP_XRTeleportOrigin`)
        (:`then`
          (`/XR_Toolkit/XRCore/Core/Utilities/VRLocomotion/Teleport/BP_XRTeleportOrigin.StopTeleporter` _bp_xrteleportorigin))
        (:`else`)))
    (:`then_1`
      (`self.OnTeleported` self))))

(fn `Get Teleporter Actor`
  (returns (OutXRTeleportOrigin :type "/XR_Toolkit/XRCore/Core/Utilities/VRLocomotion/Teleport/BP_XRTeleportOrigin Object Reference"))
  (return (`self.BP_XRTeleportOrigin`)))

(fn `GetIsTeleportActive`
  (returns (bTeleportActive :type Boolean))
  (bind _bp_xrteleportorigin (`self.BP_XRTeleportOrigin`)
    (:`then`
      (return (`/XR_Toolkit/XRCore/Core/Utilities/VRLocomotion/Teleport/BP_XRTeleportOrigin.Is Teleporter Active` _bp_xrteleportorigin)))
    (:`else`
      (return false))))

(fn `GetTeleportHand`
  (returns (OutTeleportingHand :type "EControllerHand Enum"))
  (return (`self.TeleportHand`)))

(fn `GetTeleportRotation`
  (returns (`Teleport Rotation` :type "Rotator Structure"))
  (return (`self.TeleportRotation`)))

(fn `IsTeleporterVisibleOnThisClient`
  (returns (bIsVisibleOnClient :type Boolean))
  (return (or (`self.bVisibleToOtherClients`) (`self.bIsLocalTeleporter`))))

(fn `OnRep_BP_XRTeleportOrigin`
  (bind _bp_xrteleportorigin (`self.BP_XRTeleportOrigin`)
    (:`then`
      (set `/XR_Toolkit/XRCore/Core/Utilities/VRLocomotion/Teleport/BP_XRTeleportOrigin.BuildUpSpeed` (`self.BuildupSpeed`) _bp_xrteleportorigin)
      (set `/XR_Toolkit/XRCore/Core/Utilities/VRLocomotion/Teleport/BP_XRTeleportOrigin.AllowTeleportOnActorsWithTags` (`self.AllowTeleportOnActorsWithTags`) _bp_xrteleportorigin))
    (:`else`)))
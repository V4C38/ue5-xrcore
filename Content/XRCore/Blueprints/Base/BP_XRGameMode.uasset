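; XR base game mode that spawns and possesses a pawn of XRPawnClass for each player who logs in.
; PostLogin spawns the pawn at the location and rotation of the PlayerStart returned by GetSpawnPoint, owned by the new controller.
; GetSpawnPoint caches all PlayerStarts on first use, then rotates through them round-robin by moving the chosen start to the end of the array.
; CreateAndPosessPawn is an empty stub.
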(event `self.K2_PostLogin`
  (params (NewPlayer :type "PlayerController Object Reference"))
  (bind _outputpin (`self.GetSpawnPoint`))
  (bind (_returnvalue_location _returnvalue_rotation) (`KismetMathLibrary.BreakTransform` (`self.GetTransform` _outputpin)))
  (bind _returnvalue (`|SpawnActorFromClass` (`self.XRPawnClass`) (`KismetMathLibrary.MakeTransform` _returnvalue_location _returnvalue_rotation) "Undefined" "OverrideRootScale" NewPlayer null))
  (`Controller.Possess` NewPlayer _returnvalue))

(fn `Create And Posess Pawn`
  (params (InPlayerController :type "PlayerController Object Reference") (InPawnClass :type "Pawn Class Reference")))

(fn `GetSpawnPoint`
  (returns (OutputPin :type "PlayerStart Object Reference"))
  (locals (OutPlayerStart :type "PlayerStart Object Reference"))
  (if (`KismetArrayLibrary.Array_IsEmpty` (`self.AllPlayerStarts`))
    ;[1 1 1] Cache Player Starts
    (bind _outactors (`GameplayStatics.GetAllActorsOfClass` "/Script/Engine.PlayerStart"))
    (set `self.AllPlayerStarts` _outactors))
  ;[1 1 1] Get the first player spawner in the array, and move it to the end (iE. wrap)
  (set `local.OutPlayerStart` (`|GetArrayItem` (`self.AllPlayerStarts`)))
  (`KismetArrayLibrary.Array_Remove` (`self.AllPlayerStarts`))
  (`KismetArrayLibrary.Array_AddUnique` (`self.AllPlayerStarts`) (`local.OutPlayerStart`))
  (return (`local.OutPlayerStart`)))

(fn `UserConstructionScript`)
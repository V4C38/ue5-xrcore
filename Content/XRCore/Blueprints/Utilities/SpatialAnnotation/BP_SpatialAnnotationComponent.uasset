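; Scene component that displays a title and subtitle annotation on an XR actor through a spawned BP_SpatialAnnotationActor.
; It binds to a given interaction or the owner's priority one, toggling the message on hover, start and end per InteractionBehavior.
; Show spawns the annotation actor if missing, while Hide starts a delayed destroy that Show cancels.
; Interaction handlers and BeginPlay call the actor directly, without creating or validating it.
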(event `BindToInteraction`
  (params (InInteraction :type "XRInteractionComponent Object Reference"))
  (bind _returnvalue (`self.GetOwner`))
  (bind (_outxrinteractions _returnvalue_2) (`XRToolsUtilityFunctions.IsActorInteractive` _returnvalue))
  ;[1 1 1] Bind To Interactions
  (`/Engine/EditorBlueprintResources/StandardMacros.IsValid` InInteraction
    (:`Is Valid`
      (set `self.AssignedInteraction` InInteraction)
      (add `XRInteractionComponent.OnInteractionHovered` (`self.AssignedInteraction`) (delegate `OnInteractionHovered_Event`) :!label _label)
      (add `XRInteractionComponent.OnInteractionStarted` (`self.AssignedInteraction`) (delegate `OnInteractionStarted_Event`))
      (add `XRInteractionComponent.OnInteractionEnded` (`self.AssignedInteraction`) (delegate `OnInteractionEnded_Event`)))
    (:`Is Not Valid`
      (`/Engine/EditorBlueprintResources/StandardMacros.IsValid` _returnvalue
        (:`Is Valid`
          (if _returnvalue_2
            (set `self.AssignedInteraction` (`XRToolsUtilityFunctions.GetXRInteractionByPriority` _outxrinteractions null))
            (goto _label)))))))

(event `self.ReceiveBeginPlay`
  (`|ExecutionSequence`
    (:`then_0`
      (if (`self.bInitiallyVisible`)
        (message `/XRCore/XRCore/Blueprints/Utilities/SpatialAnnotation/BPI_XRCoreUI.Show` (`self.AnnotationActor`))))
    (:`then_1`
      (if (`self.bAutoBindToInteraction`)
        (`self.BindToInteraction` null)))))

(event `OnInteractionStarted_Event`
  (params (Sender :type "XRInteractionComponent Object Reference") (XRInteractorComponent :type "XRInteractorComponent Object Reference"))
  (bind _annotationactor (`self.AnnotationActor`))
  ;[1 1 1] Bind To Interactions
  (switch `/XRCore/XRCore/Blueprints/Utilities/SpatialAnnotation/EN_SpatialAnnotationInteractionBehavior` (`self.InteractionBehavior`)
    (:`NewEnumerator1`
      (message `/XRCore/XRCore/Blueprints/Utilities/SpatialAnnotation/BPI_XRCoreUI.Hide` _annotationactor :!label _label_2))
    (:`NewEnumerator2`
      (goto _label_2))
    (:`NewEnumerator3`
      (message `/XRCore/XRCore/Blueprints/Utilities/SpatialAnnotation/BPI_XRCoreUI.Show` _annotationactor :!label _label_3))
    (:`NewEnumerator4`
      (goto _label_3))))

(event `OnInteractionEnded_Event`
  (params (Sender :type "XRInteractionComponent Object Reference") (XRInteractorComponent :type "XRInteractorComponent Object Reference"))
  (bind _assignedinteraction (`self.AssignedInteraction`))
  (bind _annotationactor (`self.AnnotationActor`))
  ;[1 1 1] Bind To Interactions
  (switch `/XRCore/XRCore/Blueprints/Utilities/SpatialAnnotation/EN_SpatialAnnotationInteractionBehavior` (`self.InteractionBehavior`)
    (:`NewEnumerator1`
      (if (not (`XRInteractionComponent.IsInteractedWith` (`self.AssignedInteraction`)))
        (message `/XRCore/XRCore/Blueprints/Utilities/SpatialAnnotation/BPI_XRCoreUI.Show` _annotationactor)))
    (:`NewEnumerator3`
      (if (not (`XRInteractionComponent.IsInteractedWith` (`self.AssignedInteraction`)))
        (message `/XRCore/XRCore/Blueprints/Utilities/SpatialAnnotation/BPI_XRCoreUI.Hide` _annotationactor)))
    (:`NewEnumerator4`
      (if (not (or (`XRInteractionComponent.IsInteractedWith` _assignedinteraction) (`.ReturnValue` (`XRInteractionComponent.IsHovered` _assignedinteraction))))
        (message `/XRCore/XRCore/Blueprints/Utilities/SpatialAnnotation/BPI_XRCoreUI.Hide` (`self.AnnotationActor`))))))

(event `OnInteractionHovered_Event`
  (params (Sender :type "XRInteractionComponent Object Reference") (HoveringXRInteractor :type "XRInteractorComponent Object Reference") (bHovered :type Boolean))
  (bind _annotationactor (`self.AnnotationActor`))
  ;[1 1 1] Bind To Interactions
  (if bHovered
    (switch `/XRCore/XRCore/Blueprints/Utilities/SpatialAnnotation/EN_SpatialAnnotationInteractionBehavior` (`self.InteractionBehavior`)
      (:`NewEnumerator0`
        (message `/XRCore/XRCore/Blueprints/Utilities/SpatialAnnotation/BPI_XRCoreUI.Show` _annotationactor :!label _label_4))
      (:`NewEnumerator1`
        (message `/XRCore/XRCore/Blueprints/Utilities/SpatialAnnotation/BPI_XRCoreUI.Hide` _annotationactor))
      (:`NewEnumerator2`
        (goto _label_4))
      (:`NewEnumerator4`
        (goto _label_4)))
    (else
      (switch `/XRCore/XRCore/Blueprints/Utilities/SpatialAnnotation/EN_SpatialAnnotationInteractionBehavior` (`self.InteractionBehavior`)
        (:`NewEnumerator1`
          (if (not (`XRInteractionComponent.IsInteractedWith` (`self.AssignedInteraction`)))
            (message `/XRCore/XRCore/Blueprints/Utilities/SpatialAnnotation/BPI_XRCoreUI.Show` (`self.AnnotationActor`))))
        (:`NewEnumerator2`
          (message `/XRCore/XRCore/Blueprints/Utilities/SpatialAnnotation/BPI_XRCoreUI.Hide` (`self.AnnotationActor`)))
        (:`NewEnumerator4`
          (if (not (`XRInteractionComponent.IsInteractedWith` (`self.AssignedInteraction`)))
            (message `/XRCore/XRCore/Blueprints/Utilities/SpatialAnnotation/BPI_XRCoreUI.Hide` (`self.AnnotationActor`))))))))

(event `self.Show`
  ;[1 1 1] Show / Hide
  (`KismetSystemLibrary.K2_ClearAndInvalidateTimerHandle` (`self.Timer_AnnotationDelete`))
  (bind _annotationactor (`self.AnnotationActor`)
    (:`then`
      (message `/XRCore/XRCore/Blueprints/Utilities/SpatialAnnotation/BPI_XRCoreUI.Show` _annotationactor))
    (:`else`
      (bind _annotationactor_2 (`self.CreateAnnotationActor`))
      (message `/XRCore/XRCore/Blueprints/Utilities/SpatialAnnotation/BPI_XRCoreUI.Show` _annotationactor_2))))

(event `self.Hide`
  ;[1 1 1] Show / Hide
  (bind _annotationactor (`self.AnnotationActor`)
    (:`then`
      (message `/XRCore/XRCore/Blueprints/Utilities/SpatialAnnotation/BPI_XRCoreUI.Hide` _annotationactor)
      (bind _returnvalue (`KismetSystemLibrary.K2_SetTimerDelegate` (delegate `DeleteAnnotation`) 5.0))
      (set `self.Timer_AnnotationDelete` _returnvalue))
    (:`else`)))

(event `DeleteAnnotation`
  ;[1 1 1] Show / Hide
  (bind _annotationactor (`self.AnnotationActor`)
    (:`then`
      (`Actor.K2_DestroyActor` _annotationactor))
    (:`else`)))

(event `self.SetTitle`
  (params (InTitle :type Text))
  ;[1 1 1] Set Content
  (bind _annotationactor (`self.AnnotationActor`)
    (:`then`
      (message `/XRCore/XRCore/Blueprints/Utilities/SpatialAnnotation/BPI_XRCoreUI.SetTitle` _annotationactor InTitle))
    (:`else`)))

(event `self.SetSubtitle`
  (params (InSubtitle :type Text))
  ;[1 1 1] Set Content
  (bind _annotationactor (`self.AnnotationActor`)
    (:`then`
      (message `/XRCore/XRCore/Blueprints/Utilities/SpatialAnnotation/BPI_XRCoreUI.SetSubtitle` _annotationactor InSubtitle))
    (:`else`)))

(fn `CreateAnnotationActor`
  (returns (AnnotationActor :type "/XRCore/XRCore/Blueprints/Utilities/SpatialAnnotation/BP_SpatialAnnotationActor Object Reference"))
  (bind _returnvalue (`|SpawnActorFromClass` "/XRCore/XRCore/Blueprints/Utilities/SpatialAnnotation/BP_SpatialAnnotationActor.BP_SpatialAnnotationActor_C" (`KismetMathLibrary.MakeTransform` (`self.K2_GetComponentLocation`) (struct) (`KismetMathLibrary.Conv_DoubleToVector` (`self.Scale`))) "Undefined" "MultiplyWithRoot" (`self.GetOwner`) false (`self.Title`) (`self.Subtitle`) (`self.Offset`) self (`self.FollowSpeed`) null))
  (bind _output_get (set `self.AnnotationActor` _returnvalue))
  (return _output_get))
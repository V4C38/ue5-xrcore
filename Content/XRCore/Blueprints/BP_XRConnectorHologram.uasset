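; XR connector hologram actor that displays a preview mesh in visible, highlighted or hidden states.
; On BeginPlay it applies a dynamic instance of the hologram base material to its mesh.
; State changes play or reverse a fade timeline that drives opacity and actor scale, with brighter illumination and a lower exponent when highlighted.
; It passes the target state to the parent class once the fade finishes.
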(event `self.ReceiveBeginPlay`
  (bind _returnvalue (`PrimitiveComponent.CreateDynamicMaterialInstance` (`self.MeshComponent`) 0 "/XR_Toolkit/XRCore/Assets/MaterialLibrary/Holograms/MI_XRConnector_Hologram_Base.MI_XRConnector_Hologram_Base" "None"))
  (set `self.DynaMat` _returnvalue)
  (`PrimitiveComponent.SetMaterial` (`self.MeshComponent`) 0 (`self.DynaMat`)))

(event `XRHologramInterface.InitHologram`
  (params (InConnector :type "XRConnectorComponent Object Reference") (InHologramMesh :type "StaticMesh Object Reference") (InHologramMeshScale :type "Float (single-precision)"))
  (`parent.InitHologram` InConnector InHologramMesh InHologramMeshScale))

(event `XRHologramInterface.SetHologramState`
  (params (InState :type "EXRHologramState Enum" :default "Visible"))
  (bind _dynamat (`self.DynaMat`))
  (bind _targetstate (`self.TargetState`))
  (bind _output_get (set `self.TargetState` InState))
  (switch `EXRHologramState` _output_get
    (:`Visible`
      (`self.SetActorHiddenInGame` false :!label _label)
      (bind (_direction _opacity _scale) (`Timeline|Timeline_Fade` :!label _label_2)
        (:`Update`
          (`MaterialInstanceDynamic.SetScalarParameterValue` (`self.DynaMat`) "Opacity" _opacity)
          (`self.SetActorScale3D` (`KismetMathLibrary.Conv_DoubleToVector` (* _scale (`self.HologramMeshScale`))))
          ;[1 1 1] Handle highlighted state
          (`MaterialInstanceDynamic.SetScalarParameterValue` _dynamat "ExponentIn" (select `EXRHologramState` _targetstate :`Visible` 5.0 :`Highlighted` 1.0 :`Hidden` 5.0))
          (`MaterialInstanceDynamic.SetScalarParameterValue` _dynamat "Illum" (select `EXRHologramState` _targetstate :`Visible` 1.25 :`Highlighted` 2.0 :`Hidden` 1.25)))
        (:`Finished`
          (`parent.SetHologramState` (`self.TargetState`)))))
    (:`Highlighted`
      (goto _label))
    (:`Hidden`
      (goto _label_2 :!via `Reverse`))))

(fn `UserConstructionScript`)
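; Scene component that shows a spatial title and subtitle annotation at its location, driven by an XR interaction on its owner.
; It binds to a given interaction or the owner's highest-priority one, optionally on BeginPlay.
; Hover, start and end events show or hide the annotation according to an InteractionBinding mode.
; The annotation actor is spawned on first show and destroyed by a timer some seconds after hiding, cancelled if shown again.
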(event `BindToInteraction`
  (params (InInteraction :type "XRInteractionComponent Object Reference"))
  (bind _returnvalue (`self.GetOwner`))
  (bind (_outxrinteractions _returnvalue_2) (`XRToolsUtilityFunctions.IsActorInteractive` _returnvalue))
  ;[1 1 1] Bind To Interactions
  (`/Engine/EditorBlueprintResources/StandardMacros.IsValid` InInteraction
    (:`Is Valid`
      (set `self.AssignedInteraction` InInteraction)
      (add `XRInteractionComponent.OnInteractionHovered` (`self.AssignedInteraction`) (delegate `OnInteractionHovered_Event`) :!label _label)
      (add `XRInteractionComponent.OnInteractionStarted` (`self.AssignedInteraction`) (delegate `OnInteractionStarted_Event`))
      (add `XRInteractionComponent.OnInteractionEnded` (`self.AssignedInteraction`) (delegate `OnInteractionEnded_Event`)))
    (:`Is Not Valid`
      (`/Engine/EditorBlueprintResources/StandardMacros.IsValid` _returnvalue
        (:`Is Valid`
          (if _returnvalue_2
            (set `self.AssignedInteraction` (`XRToolsUtilityFunctions.GetXRInteractionByPriority` _outxrinteractions null))
            (goto _label)))))))

(event `self.ReceiveBeginPlay`
  (`|ExecutionSequence`
    (:`then_0`
      (if (`self.bInitiallyVisible`)
        (`self.Show`)))
    (:`then_1`
      (if (`self.bAutoBindToInteraction`)
        (`self.BindToInteraction` null)))))

(event `OnInteractionStarted_Event`
  (params (Sender :type "XRInteractionComponent Object Reference") (XRInteractorComponent :type "XRInteractorComponent Object Reference"))
  ;[1 1 1] Bind To Interactions
  (switch `/XR_Toolkit/XRCore/Blueprints/SpatialAnnotation/EN_SpatialAnnotationInteractionBehavior` (`self.InteractionBinding`)
    (:`NewEnumerator1`
      (`self.Hide` :!label _label_2))
    (:`NewEnumerator2`
      (goto _label_2))
    (:`NewEnumerator3`
      (`self.Show` :!label _label_3))
    (:`NewEnumerator4`
      (goto _label_3))))

(event `OnInteractionEnded_Event`
  (params (Sender :type "XRInteractionComponent Object Reference") (XRInteractorComponent :type "XRInteractorComponent Object Reference"))
  (bind _assignedinteraction (`self.AssignedInteraction`))
  ;[1 1 1] Bind To Interactions
  (switch `/XR_Toolkit/XRCore/Blueprints/SpatialAnnotation/EN_SpatialAnnotationInteractionBehavior` (`self.InteractionBinding`)
    (:`NewEnumerator1`
      (if (not (`XRInteractionComponent.IsInteractedWith` (`self.AssignedInteraction`)))
        (`self.Show`)))
    (:`NewEnumerator3`
      (if (not (`XRInteractionComponent.IsInteractedWith` (`self.AssignedInteraction`)))
        (`self.Hide`)))
    (:`NewEnumerator4`
      (if (not (or (`XRInteractionComponent.IsInteractedWith` _assignedinteraction) (`.ReturnValue` (`XRInteractionComponent.IsHovered` _assignedinteraction))))
        (`self.Hide`)))))

(event `OnInteractionHovered_Event`
  (params (Sender :type "XRInteractionComponent Object Reference") (HoveringXRInteractor :type "XRInteractorComponent Object Reference") (bHovered :type Boolean))
  ;[1 1 1] Bind To Interactions
  (if bHovered
    (switch `/XR_Toolkit/XRCore/Blueprints/SpatialAnnotation/EN_SpatialAnnotationInteractionBehavior` (`self.InteractionBinding`)
      (:`NewEnumerator0`
        (`self.Show` :!label _label_4))
      (:`NewEnumerator1`
        (`self.Hide`))
      (:`NewEnumerator2`
        (goto _label_4))
      (:`NewEnumerator4`
        (`self.Show`)))
    (else
      (switch `/XR_Toolkit/XRCore/Blueprints/SpatialAnnotation/EN_SpatialAnnotationInteractionBehavior` (`self.InteractionBinding`)
        (:`NewEnumerator1`
          (if (not (`XRInteractionComponent.IsInteractedWith` (`self.AssignedInteraction`)))
            (`self.Show`)))
        (:`NewEnumerator2`
          (`self.Hide`))
        (:`NewEnumerator4`
          (if (not (`XRInteractionComponent.IsInteractedWith` (`self.AssignedInteraction`)))
            (`self.Hide`)))))))

(event `/XR_Toolkit/XRCore/Blueprints/SpatialAnnotation/BPI_XRCoreUI.Show`
  ;[1 1 1] Show / Hide
  (`KismetSystemLibrary.K2_ClearAndInvalidateTimerHandle` (`self.Timer_AnnotationDelete`))
  (`self.AnnotationActor`
    (:`then`
      (`/XR_Toolkit/XRCore/Blueprints/SpatialAnnotation/BPI_XRCoreUI.Show` (`self.AnnotationActor`)))
    (:`else`
      (bind _outannotationactor (`self.CreateAnnotationActor`))
      (`/XR_Toolkit/XRCore/Blueprints/SpatialAnnotation/BPI_XRCoreUI.Show` _outannotationactor))))

(event `/XR_Toolkit/XRCore/Blueprints/SpatialAnnotation/BPI_XRCoreUI.Hide`
  ;[1 1 1] Show / Hide
  (bind _annotationactor (`self.AnnotationActor`)
    (:`then`
      (`/XR_Toolkit/XRCore/Blueprints/SpatialAnnotation/BPI_XRCoreUI.Hide` _annotationactor)
      (bind _returnvalue (`KismetSystemLibrary.K2_SetTimerDelegate` (delegate `DeleteAnnotation`) 5.0))
      (set `self.Timer_AnnotationDelete` _returnvalue))
    (:`else`)))

(event `DeleteAnnotation`
  ;[1 1 1] Show / Hide
  (bind _annotationactor (`self.AnnotationActor`)
    (:`then`
      (`Actor.K2_DestroyActor` _annotationactor))
    (:`else`)))

(event `/XR_Toolkit/XRCore/Blueprints/SpatialAnnotation/BPI_XRCoreUI.SetTitle`
  (params (InTitle :type Text))
  ;[1 1 1] Set Content
  (bind _annotationactor (`self.AnnotationActor`)
    (:`then`
      (message `/XR_Toolkit/XRCore/Blueprints/SpatialAnnotation/BPI_XRCoreUI.SetTitle` _annotationactor InTitle))
    (:`else`)))

(event `/XR_Toolkit/XRCore/Blueprints/SpatialAnnotation/BPI_XRCoreUI.SetSubtitle`
  (params (InSubtitle :type Text))
  ;[1 1 1] Set Content
  (bind _annotationactor (`self.AnnotationActor`)
    (:`then`
      (message `/XR_Toolkit/XRCore/Blueprints/SpatialAnnotation/BPI_XRCoreUI.SetSubtitle` _annotationactor InSubtitle))
    (:`else`)))

(fn `CreateAnnotationActor`
  (returns (OutAnnotationActor :type "/XR_Toolkit/XRCore/Blueprints/SpatialAnnotation/BP_SpatialAnnotationActor Object Reference"))
  (bind _returnvalue (`|SpawnActorFromClass` "/XR_Toolkit/XRCore/Blueprints/SpatialAnnotation/BP_SpatialAnnotationActor.BP_SpatialAnnotationActor_C" (`KismetMathLibrary.MakeTransform` (`self.K2_GetComponentLocation`) (struct) (`KismetMathLibrary.Conv_DoubleToVector` (`self.Scale`))) "Undefined" "MultiplyWithRoot" null false (`self.Title`) (`self.Subtitle`) (`self.Offset`) self (`self.FollowSpeed`) null))
  (set `self.AnnotationActor` _returnvalue)
  (return (`self.AnnotationActor`)))
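; Floating XR annotation actor that displays a title and subtitle on paired title and background widgets, anchored to an owning component.
; While visible and non-static, Tick follows the component's location plus an offset and turns toward the player camera, interpolated by FollowSpeed or snapping when zero.
; Show snaps into place before revealing the widgets; Hide stops ticking.
; Text updates shift the widget root sideways based on the Title variable's length.
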(event `self.ReceiveBeginPlay`
  (`self.CacheAndConfigureWidget`)
  (if (not (`self.bInitiallyVisible`))
    (`/XR_Toolkit/XRCore/Blueprints/SpatialAnnotation/BPI_XRCoreUI.Hide`)))

(event `/XR_Toolkit/XRCore/Blueprints/SpatialAnnotation/BPI_XRCoreUI.Show`
  ;[0 0 0] Show
  (if (not (`self.bIsStatic`))
    (`self.K2_SetActorLocationAndRotation` (+ (`SceneComponent.K2_GetComponentLocation` (`self.OwningComponent`)) (`self.Offset`)) (`KismetMathLibrary.FindLookAtRotation` (`self.K2_GetActorLocation`) (`PlayerCameraManager.GetCameraLocation` (`GameplayStatics.GetPlayerCameraManager` 0))))
    (`|ExecutionSequence`
      (:`then_0`
        (`self.SetActorTickEnabled` true))
      (:`then_1`
        (message `/XR_Toolkit/XRCore/Blueprints/SpatialAnnotation/BPI_XRCoreUI.Show` (`WidgetComponent.GetUserWidgetObject` (`self.Widget_Title`)))
        (message `/XR_Toolkit/XRCore/Blueprints/SpatialAnnotation/BPI_XRCoreUI.Show` (`WidgetComponent.GetUserWidgetObject` (`self.Widget_Background`)))))))

(event `/XR_Toolkit/XRCore/Blueprints/SpatialAnnotation/BPI_XRCoreUI.SetTitle`
  (params (InTitle :type Text))
  ;[1 1 1] Update Contents
  (message `/XR_Toolkit/XRCore/Blueprints/SpatialAnnotation/BPI_XRCoreUI.SetTitle` (`WidgetComponent.GetUserWidgetObject` (`self.Widget_Title`)) InTitle)
  (message `/XR_Toolkit/XRCore/Blueprints/SpatialAnnotation/BPI_XRCoreUI.SetTitle` (`WidgetComponent.GetUserWidgetObject` (`self.Widget_Background`)) InTitle)
  (`self.RepositionWidgetRoot` :!label _label))

(event `/XR_Toolkit/XRCore/Blueprints/SpatialAnnotation/BPI_XRCoreUI.SetSubtitle`
  (params (InSubtitle :type Text))
  ;[1 1 1] Update Contents
  (message `/XR_Toolkit/XRCore/Blueprints/SpatialAnnotation/BPI_XRCoreUI.SetSubtitle` (`WidgetComponent.GetUserWidgetObject` (`self.Widget_Title`)) InSubtitle)
  (message `/XR_Toolkit/XRCore/Blueprints/SpatialAnnotation/BPI_XRCoreUI.SetSubtitle` (`WidgetComponent.GetUserWidgetObject` (`self.Widget_Background`)) InSubtitle)
  (goto _label))

(event `/XR_Toolkit/XRCore/Blueprints/SpatialAnnotation/BPI_XRCoreUI.Hide`
  ;[0 0 0] Hide
  (if (not (`self.bIsStatic`))
    (message `/XR_Toolkit/XRCore/Blueprints/SpatialAnnotation/BPI_XRCoreUI.Hide` (`WidgetComponent.GetUserWidgetObject` (`self.Widget_Title`)))
    (message `/XR_Toolkit/XRCore/Blueprints/SpatialAnnotation/BPI_XRCoreUI.Hide` (`WidgetComponent.GetUserWidgetObject` (`self.Widget_Background`)))
    (`self.SetActorTickEnabled` false)))

(event `self.ReceiveTick`
  (params (DeltaSeconds :type "Float (single-precision)"))
  (bind _returnvalue (> (`self.FollowSpeed`) 0.0))
  (bind _returnvalue_2 (`KismetMathLibrary.FindLookAtRotation` (`self.K2_GetActorLocation`) (`PlayerCameraManager.GetCameraLocation` (`GameplayStatics.GetPlayerCameraManager` 0))))
  (bind _returnvalue_3 (+ (`SceneComponent.K2_GetComponentLocation` (`self.OwningComponent`)) (`self.Offset`)))
  ;[1 1 1] Move to Target Loc
  (if (not (`self.bIsStatic`))
    (`self.K2_SetActorLocationAndRotation` (select `bool` _returnvalue :`false` _returnvalue_3 :`true` (`KismetMathLibrary.VInterpTo` (`self.K2_GetActorLocation`) _returnvalue_3 DeltaSeconds (* (`self.FollowSpeed`) 10.0))) (select `bool` _returnvalue :`false` _returnvalue_2 :`true` (`KismetMathLibrary.RInterpTo` (`self.K2_GetActorRotation`) _returnvalue_2 DeltaSeconds (* (`self.FollowSpeed`) 6.0))))))

(fn `CacheAndConfigureWidget`
  (`/XR_Toolkit/XRCore/Blueprints/SpatialAnnotation/BPI_XRCoreUI.SetTitle` (`self.Title`))
  (`/XR_Toolkit/XRCore/Blueprints/SpatialAnnotation/BPI_XRCoreUI.SetSubtitle` (`self.Subtitle`))
  (`self.RepositionWidgetRoot`))

(fn `RepositionWidgetRoot`
  (`SceneComponent.K2_SetRelativeLocation` (`self.WidgetRoot`) (`KismetMathLibrary.MakeVector` 0.0 (`KismetMathLibrary.MapRangeClamped` (`KismetMathLibrary.Conv_IntToDouble` (`KismetStringLibrary.Len` (`KismetTextLibrary.Conv_TextToString` (`self.Title`)))) 0.0 30.0 -11.0 5.0)) false false))

(fn `UserConstructionScript`)
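; XR laser pointer actor for hovering and grabbing XR interaction components at range, or clicking widgets.
; An Inactive/Active/Hover/Interact state drives tracing, tip smoothing, beam opacity and timeline build-up/retract animations.
; While interacting, the visual tip attaches to the target and Go-Go-style hand motion changes beam length, releasing if the tips separate too far.
; The curved beam is rebuilt from spline meshes on every update, using a dynamic material.
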(event `self.ReceiveBeginPlay`
  ;[0 0 0] Initial Config
  (`|ExecutionSequence`
    (:`then_0`
      (`XRInteractorComponent.SetPhysicsConstraint` (`self.XRInteractor`) (`self.XRInteractor_PhysicsConstraint_Laser`)))
    (:`then_1`
      (`self.CreateDynamicMaterials`))
    (:`then_2`
      (set `self.InitialSphereScale` (`SceneComponent.RelativeScale3D` (`self.TipSphere`)))
      (set `self.MaxDragDistance` (* (`self.MaxDragDistance`) 2.0)))))

(event `XRLaserInterface.SetControllerHand`
  (params (InXRControllerHand :type "EControllerHand Enum" :default "Left"))
  ;[0 0 0] Initial Config
  (if (`KismetSystemLibrary.IsServer`)
    (`XRInteractorComponent.Server_SetXRControllerHand` (`self.XRInteractor`) InXRControllerHand)))

(event `XRLaserInterface.ProvideAttachmentRoot`
  (params (InComponent :type "SceneComponent Object Reference"))
  ;[0 0 0] Initial Config
  (`SceneComponent.K2_AttachToComponent` (`self.Root`) InComponent "None" "SnapToTarget" "SnapToTarget" "KeepWorld" true))

(event `self.ReceiveTick`
  (params (DeltaSeconds :type "Float (single-precision)"))
  ;[0 0 0] Tick
  (switch `EXRLaserState` (`self.LaserState`)
    (:`Active`
      (bind _outdesiredtiplocation (`self.LineTrace` :!label _label))
      (`self.Update Tip Position` _outdesiredtiplocation true))
    (:`Hover`
      (goto _label))
    (:`Interact`
      (bind _outdesiredtiplocation_2 (`self.SetDynamicLength`))
      (`self.Update Tip Position` _outdesiredtiplocation_2)
      (`self.EnsureInteractionValidity`)))
  (`self.UpdateBeam`))

(event `self.XRInteractor.OnStartedInteracting`
  (params (Sender :type "XRInteractorComponent Object Reference") (XRInteractionComponent :type "XRInteractionComponent Object Reference"))
  ;[1 1 1] Interaction
  (`self.SetState` "Interact")
  (`self.HandleVisualTipAttachment` XRInteractionComponent)
  (set `self.DynamicLengthCooldown` 0.0))

(event `self.XRInteractor.OnStoppedInteracting`
  (params (Sender :type "XRInteractorComponent Object Reference") (XRInteractionComponent :type "XRInteractionComponent Object Reference"))
  ;[1 1 1] Interaction
  (`self.SetState` (select `EXRLaserState` (`self.LaserState`) :`Inactive` "Inactive" :`Active` "Active" :`Hover` "Active" :`Interact` "Active" :!type "EXRLaserState Enum"))
  (`self.HandleVisualTipAttachment` null))

(event `XRInteractionInterface.StartInteractionByPriority`
  (params (InPriority :type Integer) (InPrioritySelectionCondition :type "EXRInteractionPrioritySelection Enum" :default "Equal"))
  ;[0 0 0] Interaction Interface
  (if (`self.CanInteractWithWidget`)
    (`WidgetInteractionComponent.PressPointerKey` (`self.WidgetInteraction`) "LeftMouseButton")
    (else
      (`XRInteractorComponent.StartXRInteractionByPriority` (`self.XRInteractor`) InPriority InPrioritySelectionCondition))))

(event `self.XRInteractor.OnHoverStateChanged`
  (params (Sender :type "XRInteractorComponent Object Reference") (HoveredXRInteractionComponent :type "XRInteractionComponent Object Reference") (bHoverState :type Boolean))
  (bind _returnvalue (`XRInteractorComponent.IsInteracting` Sender))
  ;[1 1 1] Interaction
  (if (`|EnumInequality` (`self.LaserState`) "Inactive")
    (if bHoverState
      (if (not _returnvalue)
        (`self.SetState` "Hover"))
      (elif _returnvalue
        (`self.SetState` "Interact")
        (else
          (`self.SetState` "Active"))))))

(event `XRInteractionInterface.StopInteractionByPriority`
  (params (InPriority :type Integer) (InPrioritySelectionCondition :type "EXRInteractionPrioritySelection Enum" :default "Equal"))
  ;[0 0 0] Interaction Interface
  (`XRInteractorComponent.StopXRInteractionByPriority` (`self.XRInteractor`) InPriority InPrioritySelectionCondition)
  (`WidgetInteractionComponent.ReleasePointerKey` (`self.WidgetInteraction`) "LeftMouseButton" :!label _label_2))

(event `XRInteractionInterface.StopAllInteractions`
  (params (InInteractor :type "XRInteractorComponent Object Reference"))
  ;[0 0 0] Interaction Interface
  (`XRInteractorComponent.StopAllXRInteractions` (`self.XRInteractor`))
  (goto _label_2))

(event `XRLaserInterface.SetLaserActive`
  (params (bInState :type Boolean))
  (bind _animationplaybackrate (`self.AnimationPlaybackRate`))
  (bind _maxlength (`self.MaxLength`))
  ;[1 1 1] Activate/Deactivate Animation
  (if bInState
    (`self.SetState` "Active")
    (bind _outanimationplaybackrate (`self.Animation_Activate_SetInitialState`))
    (`TimelineComponent.SetPlayRate` (`self.Timeline_BuildUpAnimation`) _outanimationplaybackrate)
    (bind (_direction _progress _linearprogress) (`Timeline|Timeline_BuildUpAnimation` :!label _label_3)
      (:`Update`
        (switch `EXRLaserState` (`self.LaserState`)
          (:`Inactive`
            (`self.Animation_Deactivate` _progress _linearprogress))
          (:`Active`
            (`self.Animation_Activate` _progress _linearprogress :!label _label_4))
          (:`Hover`
            (goto _label_4))
          (:`Interact`
            (goto _label_4))))
      (:`Finished`
        (switch `EXRLaserState` (`self.LaserState`)
          (:`Inactive`
            (`self.Animation_ResetToDefaultState`))
          (:`Active`
            (`self.SetActorTickEnabled` true :!label _label_5))
          (:`Hover`
            (goto _label_5))
          (:`Interact`
            (goto _label_5)))))
    (else
      (`XRInteractorComponent.StopAllXRInteractions` (`self.XRInteractor`))
      (`WidgetInteractionComponent.ReleasePointerKey` (`self.WidgetInteraction`) "LeftMouseButton")
      (`self.SetState` "Inactive")
      (`TimelineComponent.SetPlayRate` (`self.Timeline_BuildUpAnimation`) (`KismetMathLibrary.MapRangeClamped` (`self.CurrentLength`) (* 0.25 _maxlength) _maxlength (* _animationplaybackrate 4.0) (* _animationplaybackrate 1.0)))
      (goto _label_3 :!via `Reverse`))))

(event `AnimateTipSphere`
  (params (InLaserState :type "EXRLaserState Enum" :default "Inactive"))
  (bind _visualtip (`self.VisualTip`))
  ;[1 1 1] Animate Tip Sphere
  (bind (_direction _outalpha) (`Timeline|Timeline` :!via `PlayFromStart`)
    (:`Update`
      (`SceneComponent.SetRelativeScale3D` _visualtip (`KismetMathLibrary.VLerp` (`SceneComponent.RelativeScale3D` _visualtip) (* (`self.InitialSphereScale`) (select `EXRLaserState` InLaserState :`Active` 0.5 :`Hover` 3.0 :`Interact` 1.0)) _outalpha)))))

(fn `Animation_Activate`
  (params (InProgress :type "Float (double-precision)") (InLinearProgress :type "Float (double-precision)"))
  (bind _dynamat_beam (`self.DynaMat_Beam`))
  (bind (_returnvalue_x _returnvalue_y _returnvalue_z) (`KismetMathLibrary.BreakVector` (`SceneComponent.K2_GetComponentLocation` (`self.Root`))))
  (`SceneComponent.K2_SetWorldRotation` (`self.BehaviorTip`) (`SceneComponent.K2_GetComponentRotation` (`self.Root`)) false false)
  (`SceneComponent.K2_SetWorldRotation` (`self.VisualTip`) (`SceneComponent.K2_GetComponentRotation` (`self.Root`)) false false)
  (bind (_outdesiredtiplocation _outdistance) (`self.LineTrace`))
  (set `self.CurrentLength` _outdistance)
  (`SceneComponent.K2_SetWorldLocationAndRotation` (`self.VisualTip`) (`KismetMathLibrary.VLerp` (`SceneComponent.K2_GetComponentLocation` (`self.BehaviorTip`)) _outdesiredtiplocation (`local.InProgress`)) (`KismetMathLibrary.RLerp` (`SceneComponent.K2_GetComponentRotation` (`self.BehaviorTip`)) (`SceneComponent.K2_GetComponentRotation` (`self.Root`)) (`local.InProgress`) true) false false)
  (`SceneComponent.K2_SetWorldLocationAndRotation` (`self.BehaviorTip`) (`KismetMathLibrary.VLerp` (`SceneComponent.K2_GetComponentLocation` (`self.BehaviorTip`)) _outdesiredtiplocation (`local.InProgress`)) (`KismetMathLibrary.RLerp` (`SceneComponent.K2_GetComponentRotation` (`self.BehaviorTip`)) (`SceneComponent.K2_GetComponentRotation` (`self.Root`)) (`local.InProgress`) true) false false)
  (`self.UpdateBeam`)
  ;[1 1 1] Material settings -> Lerp to visibility
  (`|ExecutionSequence`
    (:`then_0`
      (`MaterialInstanceDynamic.SetVectorParameterValue` _dynamat_beam "AWP_Root" (make `LinearColor` _returnvalue_x _returnvalue_y _returnvalue_z 1.0)))
    (:`then_1`
      (`MaterialInstanceDynamic.SetScalarParameterValue` _dynamat_beam "VisibilityDistance" (`KismetMathLibrary.Lerp` 0.0 (* (`self.CurrentLength`) 1.5) (`local.InLinearProgress`))))
    (:`then_2`
      (`MaterialInstanceDynamic.SetScalarParameterValue` (`self.DynaMat_Beam`) "Opacity" (`KismetMathLibrary.Lerp` 0.0 (`self.Get Opacity by State`) (`local.InProgress`))))))

(fn `Animation_Activate_SetInitialState`
  (returns (OutAnimationPlaybackRate :type "Float (double-precision)"))
  (bind _animationplaybackrate (`self.AnimationPlaybackRate`))
  (bind _maxlength (`self.MaxLength`))
  (`self.SetActorHiddenInGame` false)
  (`SceneComponent.K2_SetWorldLocation` (`self.BehaviorTip`) (`SceneComponent.K2_GetComponentLocation` (`self.Root`)) false false)
  (`SceneComponent.K2_SetWorldLocation` (`self.VisualTip`) (`SceneComponent.K2_GetComponentLocation` (`self.Root`)) false false)
  ;[1 1 1] Distance based buildup speed
  (bind (_outdesiredtiplocation _outdistance) (`self.LineTrace`))
  (return (`KismetMathLibrary.MapRangeClamped` _outdistance (* _maxlength 0.25) _maxlength (* _animationplaybackrate 4.0) _animationplaybackrate)))

(fn `Animation_Deactivate`
  (params (InProgress :type "Float (double-precision)") (InLinearProgress :type "Float (double-precision)"))
  (bind _dynamat_beam (`self.DynaMat_Beam`))
  (bind (_returnvalue_x _returnvalue_y _returnvalue_z) (`KismetMathLibrary.BreakVector` (`SceneComponent.K2_GetComponentLocation` (`self.Root`))))
  (bind _returnvalue (`SceneComponent.K2_GetComponentLocation` (`self.Root`)))
  (bind _outdesiredtiplocation (`self.LineTrace`))
  (set `self.CurrentLength` (`KismetMathLibrary.Vector_Distance` _returnvalue (`SceneComponent.K2_GetComponentLocation` (`self.BehaviorTip`))))
  (`SceneComponent.K2_SetWorldLocationAndRotation` (`self.VisualTip`) (`KismetMathLibrary.VLerp` _returnvalue _outdesiredtiplocation (`local.InProgress`)) (`KismetMathLibrary.RLerp` (`SceneComponent.K2_GetComponentRotation` (`self.Root`)) (`SceneComponent.K2_GetComponentRotation` (`self.BehaviorTip`)) (`local.InProgress`) true) false false)
  (`SceneComponent.K2_SetWorldLocationAndRotation` (`self.BehaviorTip`) (`KismetMathLibrary.VLerp` _returnvalue _outdesiredtiplocation (`local.InProgress`)) (`KismetMathLibrary.RLerp` (`SceneComponent.K2_GetComponentRotation` (`self.Root`)) (`SceneComponent.K2_GetComponentRotation` (`self.BehaviorTip`)) (`local.InProgress`) true) false false)
  (`self.UpdateBeam`)
  ;[1 1 1] Material settings -> Lerp to invisibility
  (`|ExecutionSequence`
    (:`then_0`
      (`MaterialInstanceDynamic.SetVectorParameterValue` _dynamat_beam "AWP_Root" (make `LinearColor` _returnvalue_x _returnvalue_y _returnvalue_z 1.0)))
    (:`then_1`
      (`MaterialInstanceDynamic.SetScalarParameterValue` _dynamat_beam "VisibilityDistance" (`KismetMathLibrary.Lerp` (`self.MaxLength`) 0.0 (`local.InProgress`))))
    (:`then_2`
      (`MaterialInstanceDynamic.SetScalarParameterValue` (`self.DynaMat_Beam`) "Opacity" (`KismetMathLibrary.Lerp` (select `EXRLaserState` (`self.LaserState`) :`Active` 0.15 :`Hover` 0.5 :`Interact` 1.0 :!type "Float (single-precision)") 0.0 (`local.InProgress`))))))

(fn `Animation_ResetToDefaultState`
  (bind (_returnvalue_location _returnvalue_rotation) (`KismetMathLibrary.BreakTransform` (`SceneComponent.K2_GetComponentToWorld` (`self.Root`))))
  (`self.SetActorHiddenInGame` true)
  (`SceneComponent.K2_SetWorldLocationAndRotation` (`self.BehaviorTip`) _returnvalue_location _returnvalue_rotation false false)
  (`SceneComponent.K2_SetWorldLocationAndRotation` (`self.VisualTip`) _returnvalue_location _returnvalue_rotation false false))

(fn `CanInteractWithWidget`
  (returns (bCanInteract :type Boolean))
  (return (`KismetSystemLibrary.IsValid` (`WidgetInteractionComponent.GetHoveredWidgetComponent` (`self.WidgetInteraction`)))))

(fn `CreateDynamicMaterials`
  (`|ExecutionSequence`
    (:`then_0`
      ;[1 1 1] Beam
      (bind _returnvalue (`KismetMaterialLibrary.CreateDynamicMaterialInstance` "/XR_Toolkit/XRCore/Assets/MaterialLibrary/Laser/MI_XRLaserBeam.MI_XRLaserBeam"))
      (bind _output_get (set `self.DynaMat_Beam` _returnvalue))
      (`MaterialInstanceDynamic.SetScalarParameterValue` _output_get "LaserLength_Max" (`self.MaxLength`)) ; Used to determine Laser Thickness in the Shader
      (`MaterialInstanceDynamic.SetScalarParameterValue` _output_get "Thickness" (`self.Thickness`)) ; Used to determine Laser Thickness in the Shader
    )))

(fn `EnsureInteractionValidity`
  (if (> (`KismetMathLibrary.Vector_DistanceSquared` (`SceneComponent.K2_GetComponentLocation` (`self.BehaviorTip`)) (`SceneComponent.K2_GetComponentLocation` (`self.VisualTip`))) (`self.MaxDragDistance`))
    (`XRInteractorComponent.StopAllXRInteractions` (`self.XRInteractor`))))

(fn `Get Opacity by State`
  (returns (OutOpacity :type "Float (double-precision)"))
  (return (select `EXRLaserState` (`self.LaserState`) :`Active` 0.15 :`Hover` 0.5 :`Interact` 1.0 :!type "Float (single-precision)")))

(fn `GetControllerHand`
  (returns (ReturnValue :type "EControllerHand Enum"))
  (return "Left"))

(fn `GetCurrentLength`
  (returns (OutCurrentLength :type "Float (double-precision)"))
  (return (`self.CurrentLength`)))

(fn `GetLaserState`
  (returns (ReturnValue :type "EXRLaserState Enum"))
  (return (`self.LaserState`)))

(fn `GetXRInteractor`
  (returns (ReturnValue :type "XRInteractorComponent Object Reference"))
  (return (`self.XRInteractor`)))

(fn `GetXRLaserActor`
  (returns (ReturnValue :type "Actor Object Reference"))
  (return null))

(fn `HandleLaserInteraction`)

(fn `HandleVisualTipAttachment`
  (params (Parent :type "SceneComponent Object Reference"))
  (`/Engine/EditorBlueprintResources/StandardMacros.IsValid` Parent
    (:`Is Valid`
      (`SceneComponent.K2_AttachToComponent` (`self.VisualTip`) Parent "None" "KeepWorld" "KeepWorld" "KeepWorld" false))
    (:`Is Not Valid`
      (`SceneComponent.K2_DetachFromComponent` (`self.VisualTip`) "KeepWorld" "KeepWorld" "KeepWorld" true))))

(fn `IsLaserActive`
  (returns (ReturnValue :type Boolean))
  (return (select `EXRLaserState` (`self.LaserState`) :`Active` true :`Hover` true :`Interact` true)))

(fn `LineTrace`
  (returns (OutDesiredTipLocation :type "Vector Structure") (OutDistance :type "Float (single-precision)"))
  (locals (Loc_MaxLengthVector :type "Vector Structure"))
  (bind _returnvalue (`SceneComponent.K2_GetComponentLocation` (`self.Root`)))
  (bind _returnvalue_2 (+ _returnvalue (* (`KismetMathLibrary.GetDirectionUnitVector` _returnvalue (`SceneComponent.K2_GetComponentLocation` (`self.Direction`))) (`self.MaxLength`))))
  (set `local.Loc_MaxLengthVector` _returnvalue_2)
  (bind (_outhit _returnvalue_3) (`KismetSystemLibrary.LineTraceSingle` (`SceneComponent.K2_GetComponentLocation` (`self.Root`)) _returnvalue_2 "TraceTypeQuery1" true (`|MakeArray` (`self.GetOwner`))))
  (if _returnvalue_3
    (bind (_bblockinghit _binitialoverlap _time _distance _location) (`GameplayStatics.BreakHitResult` _outhit))
    ;[1 1 1] Valid hit - return impact point
    (if (<= _distance (`self.MaxLength`))
      (return _location _distance)
      (else
        _)))
  ;[1 1 1] Not (valid) hit - set to max length forward
  (return (`local.Loc_MaxLengthVector`) (`self.MaxLength`)))

(fn `SetDynamicLength`
  (returns (OutDesiredTipLocation :type "Vector Structure"))
  (locals (Loc_CurrentLaserRootLocation :type "Vector Structure" :default (0.0 0.0 0.0)) (Loc_DirectionDOT :type "Float (double-precision)" :default 0.0) (Loc_MoveVelocity :type "Float (double-precision)" :default 0.0) (Loc_LengthModifier :type "Float (double-precision)"))
  (bind _loc_directiondot (`local.Loc_DirectionDOT`))
  (bind _returnvalue (`SceneComponent.K2_GetComponentLocation` (`self.Root`)))
  (bind _returnvalue_2 (`SceneComponent.K2_GetComponentLocation` (`self.Root`)))
  ;[1 1 1] RampUp Dynamic Length (this is effectively a multiplier)
  (set `self.DynamicLengthCooldown` (+ (`self.DynamicLengthCooldown`) (`GameplayStatics.GetWorldDeltaSeconds`)))
  (set `local.Loc_CurrentLaserRootLocation` (`SceneComponent.K2_GetComponentLocation` (`self.Root`)))
  ;[0 0 0] Cache Movement Data
  (set `local.Loc_DirectionDOT` (`KismetMathLibrary.Dot_VectorVector` (`KismetMathLibrary.GetDirectionUnitVector` (`local.Loc_CurrentLaserRootLocation`) (`self.LastLaserRootLocation`)) (`KismetMathLibrary.GetDirectionUnitVector` (`SceneComponent.K2_GetComponentLocation` (`self.Root`)) (`SceneComponent.K2_GetComponentLocation` (`self.BehaviorTip`)))))
  (set `local.Loc_MoveVelocity` (`KismetMathLibrary.VSize` (- (`local.Loc_CurrentLaserRootLocation`) (`self.LastLaserRootLocation`))))
  (set `self.LastLaserRootLocation` (`SceneComponent.K2_GetComponentLocation` (`self.Root`)))
  ;[1 1 1] Only apply GoGo when moving in Object Direction
  ; - more leeway when moving towards
  (if (or (> _loc_directiondot 0.45) (< _loc_directiondot -0.35))
    (bind _output_get (set `local.Loc_LengthModifier` (* (`KismetMathLibrary.MapRangeClamped` (`self.CurrentLength`) 25.0 (`self.MaxLength`) 0.5 3.0) (`KismetMathLibrary.MapRangeClamped` (`local.Loc_MoveVelocity`) 0.001 0.333 0.0 3.5) (select `bool` (> (`local.Loc_DirectionDOT`) 0.0) :`false` 1 :`true` -1) (`KismetMathLibrary.MapRangeClamped` (`self.DynamicLengthCooldown`) 0.0 (`self.InitialDynamicLengthCooldown`) 0.0 1.0))))
    (if (> (+ _output_get (`self.CurrentLength`)) 1.0)
      ;[0 0 0] Modified Length
      (set `self.CurrentLength` (+ (`self.CurrentLength`) (`local.Loc_LengthModifier`)))
      (return (+ _returnvalue_2 (* (`KismetMathLibrary.GetDirectionUnitVector` _returnvalue_2 (`SceneComponent.K2_GetComponentLocation` (`self.Direction`))) (+ (`self.CurrentLength`) (`local.Loc_LengthModifier`)))))
      (else
        _)))
  ;[0 0 0] Default, unchanged length
  (return (+ _returnvalue (* (`KismetMathLibrary.GetDirectionUnitVector` _returnvalue (`SceneComponent.K2_GetComponentLocation` (`self.Direction`))) (`self.CurrentLength`)))))

(fn `SetState`
  (params (InLaserState :type "EXRLaserState Enum" :default "Inactive"))
  (if (`KismetSystemLibrary.IsServer`)
    (if (`|EnumInequality` (`local.InLaserState`) (`self.LaserState`))
      (set `self.LaserState` (`local.InLaserState`))
      (`|ExecutionSequence`
        (:`then_0`
          (switch `EXRLaserState` (`local.InLaserState`)
            (:`Inactive`
              (`self.SetActorTickEnabled` false))))
        (:`then_1`
          (`self.OnLaserStateChanged` self (`local.InLaserState`) :!label _label))))
    (else
      (`self.AnimateTipSphere` InLaserState)
      (goto _label))))

(fn `Update Tip Position`
  (params (InDesiredTipLocation :type "Vector Structure") (InSyncVisualAndBehavioralTip :type Boolean))
  (locals (Loc_TargetLocation :type "Vector Structure" :default (0.0 0.0 0.0)))
  (`|ExecutionSequence`
    (:`then_0`
      (set `local.Loc_TargetLocation` (`KismetMathLibrary.VInterpTo` (`SceneComponent.K2_GetComponentLocation` (`self.BehaviorTip`)) (`local.InDesiredTipLocation`) (`GameplayStatics.GetWorldDeltaSeconds`) (select `EXRLaserState` (`self.LaserState`) :`Active` 15.0 :`Hover` 35.0 :`Interact` 15.0 :!type "Float (single-precision)")))
      (`|ExecutionSequence`
        (:`then_0`
          (if (`local.InSyncVisualAndBehavioralTip`)
            (`SceneComponent.K2_SetWorldLocation` (`self.VisualTip`) (`KismetMathLibrary.VInterpTo` (`SceneComponent.K2_GetComponentLocation` (`self.BehaviorTip`)) (`local.InDesiredTipLocation`) (`GameplayStatics.GetWorldDeltaSeconds`) 5.0) false false)))
        (:`then_1`
          (`SceneComponent.K2_SetWorldLocation` (`self.BehaviorTip`) (`local.Loc_TargetLocation`) false false)
          (set `self.CurrentLength` (`KismetMathLibrary.Vector_Distance` (`SceneComponent.K2_GetComponentLocation` (`self.Root`)) (`local.Loc_TargetLocation`))))))
    (:`then_1`
      ;[1 1 1] Rotation
      (`SceneComponent.K2_SetWorldRotation` (`self.BehaviorTip`) (`KismetMathLibrary.RInterpTo` (`SceneComponent.K2_GetComponentRotation` (`self.BehaviorTip`)) (`SceneComponent.K2_GetComponentRotation` (`self.Root`)) (`GameplayStatics.GetWorldDeltaSeconds`) 4.5) false false))))

(fn `UpdateBeam`
  (`self.UpdateSpline`)
  (`self.UpdateSplineMesh`)
  (`self.UpdateBeamMaterials`))

(fn `UpdateBeamMaterials`
  (bind _dynamat_beam (`self.DynaMat_Beam`))
  (bind (_returnvalue_x _returnvalue_y _returnvalue_z) (`KismetMathLibrary.BreakVector` (`SceneComponent.K2_GetComponentLocation` (`self.Root`))))
  (`|ExecutionSequence`
    (:`then_0`
      (`MaterialInstanceDynamic.SetVectorParameterValue` _dynamat_beam "AWP_Root" (make `LinearColor` _returnvalue_x _returnvalue_y _returnvalue_z 1.0)))
    (:`then_1`
      (`MaterialInstanceDynamic.SetScalarParameterValue` _dynamat_beam "VisibilityDistance" 100000.0))
    (:`then_2`
      (`MaterialInstanceDynamic.SetScalarParameterValue` (`self.DynaMat_Beam`) "Opacity" (`self.Get Opacity by State`)))))

(fn `UpdateSpline`
  (bind _spline (`self.Spline`))
  (bind _returnvalue (* (`KismetMathLibrary.GetDirectionUnitVector` (`SceneComponent.K2_GetComponentLocation` (`self.Root`)) (`SceneComponent.K2_GetComponentLocation` (`self.Direction`))) (* (`self.CurrentLength`) 0.2)))
  (`SplineComponent.ClearSplinePoints` (`self.Spline`) true)
  (`|ExecutionSequence`
    (:`then_0`
      (`SplineComponent.AddSplinePoint` (`self.Spline`) (`SceneComponent.K2_GetComponentLocation` (`self.Root`)) "World" false))
    (:`then_1`
      ;[1 1 1] Midpoint based on distance to the Target
      (`SplineComponent.AddSplinePoint` _spline (+ _returnvalue (`SceneComponent.K2_GetComponentLocation` (`self.Root`))) "World" false)
      ;;[0 0 0] Smooth Tangent
      (`SplineComponent.SetTangentAtSplinePoint` _spline 1 (* _returnvalue (`KismetMathLibrary.MapRangeClamped` (`self.CurrentLength`) 0.0 (`self.MaxLength`) 4.0 10.0)) "World" false))
    (:`then_2`
      (`SplineComponent.AddSplinePoint` (`self.Spline`) (`SceneComponent.K2_GetComponentLocation` (`self.VisualTip`)) "World" true))
    (:`then_3`
      (return))))

(fn `UpdateSplineMesh`
  (bind _splinemeshes_beam (`self.SplineMeshes_Beam`))
  (bind _spline (`self.Spline`))
  ;[1 1 1] Clear Spline Meshes
  (for _array_element _splinemeshes_beam
    (`ActorComponent.K2_DestroyComponent` _array_element))
  (`KismetArrayLibrary.Array_Clear` _splinemeshes_beam)
  ;[1 1 1] Set Spline MeshComponents
  (for _index (range (+ (- (`SplineComponent.GetNumberOfSplinePoints` (`self.Spline`)) 2) 1))
    (bind _returnvalue (`AddComponent|NODE_AddSplineMeshComponent-1` :`bManualAttachment` true :`RelativeTransform` (`KismetMathLibrary.MakeTransform` (0.0 0.0 0.0)))) ; Add new cylinder mesh
    (`PrimitiveComponent.SetMaterial` _returnvalue 0 (`self.DynaMat_Beam`))
    (`KismetArrayLibrary.Array_Add` (`self.SplineMeshes_Beam`) _returnvalue)
    (bind _returnvalue_2 (+ _index 1))
    (`SplineMeshComponent.SetStartAndEnd` _returnvalue (`SplineComponent.GetLocationAtSplinePoint` (`self.Spline`) _index "Local") (`SplineComponent.GetTangentAtSplinePoint` _spline _index "Local") (`SplineComponent.GetLocationAtSplinePoint` (`self.Spline`) _returnvalue_2 "Local") (`SplineComponent.GetTangentAtSplinePoint` _spline _returnvalue_2 "Local") true) ; Set the tangents and position to build slightly bend the cylinder. All cylinders combined create a smooth arc.
  )
  (return))

(fn `UserConstructionScript`)
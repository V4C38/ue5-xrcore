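; Actor component in XR Toolkit that lets its owning actor be staged by the scene manager's actor loading system.
; On BeginPlay it optionally registers with BP_XRCore_ActorInitializer, warning if that is missing, and tracks a load state.
; UnInitialize hides the owner and disables collision; Initialize can attach its XRConnectorComponent to a target actor's socket, by ID or first found, and restore visibility and collision.
; The load getters return constants, and a scale-up timeline sits unwired.
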(event `self.ReceiveBeginPlay`
  (set `self.LoadState` "NewEnumerator0")
  (if (`self.bRegisterWithSceneManager`)
    (bind _output_get (set `self.XRCoreSceneManager` (`/XR_Toolkit/XR_Toolkit/Core/Utilities/FL_XRUtilityFunctions.XRCoreScene_GetSceneManager`)))
    (bind _returnvalue (`Actor.GetComponentByClass` _output_get "/XR_Toolkit/XR_Toolkit/Core/Scene/ActorLoading/BP_XRCore_ActorInitializer.BP_XRCore_ActorInitializer_C"))
    (`/Engine/EditorBlueprintResources/StandardMacros.IsValid` _returnvalue
      (:`Is Valid`
        (`/XR_Toolkit/XR_Toolkit/Core/Scene/ActorLoading/BP_XRCore_ActorInitializer.RegisterComponent` _returnvalue self)
        (set `self.LoadState` "NewEnumerator2"))
      (:`Is Not Valid`
        (`/XR_Toolkit/XR_Toolkit/Core/Utilities/FL_XRUtilityFunctions.CustomDebugWarning` "NewEnumerator1" self "XRCore_ActorInitializer component not found on XRCreSceneManager.")
        (set `self.LoadState` "NewEnumerator4")))))

(event `UnInitialize`
  (bind _returnvalue (`self.GetOwner`))
  ;[0 0 0] Called by ActorInitializer
  (set `self.LoadState` "NewEnumerator1")
  (`Actor.SetActorHiddenInGame` _returnvalue true)
  (`Actor.SetActorEnableCollision` _returnvalue false)
  (`/Engine/EditorBlueprintResources/StandardMacros.IsValid` (`Actor.GetComponentByClass` (`self.GetOwner`) "/Script/XR_Toolkit.XRConnectorComponent")))

(event `Initialize`
  (bind _returnvalue (`self.GetOwner`))
  (bind _returnvalue_2 (`Actor.GetComponentByClass` (`self.GetOwner`) "/Script/XR_Toolkit.XRConnectorComponent"))
  ;[0 0 0] Called by ActorInitializer
  ;[1 1 1] Replace with XRCore Utility TryConnectToActor
  (bind _connecttoactor (`self.ConnectToActor`)
    (:`then`
      (if (> (`KismetStringLibrary.Len` (`self.ConnectionSocketID`)) 0)
        (bind _returnvalue_3 (`Actor.K2_GetComponentsByClass` _connecttoactor "/Script/XR_Toolkit.XRConnectorSocket"))
        (for _array_element _returnvalue_3
          (if (`KismetStringLibrary.EqualEqual_StrStr` (`XRConnectorSocket.GetSocketID` _array_element) (`self.ConnectionSocketID`))
            (`XRConnectorComponent.ConnectToSocket` _returnvalue_2 _array_element)))
        (`Actor.SetActorHiddenInGame` _returnvalue false :!label _label)
        (`Actor.SetActorEnableCollision` _returnvalue true)
        (set `self.LoadState` "NewEnumerator3")
        (else
          (bind _output (`|GetArrayItem` _returnvalue_3))
          (`/Engine/EditorBlueprintResources/StandardMacros.IsValid` _output
            (:`Is Valid`
              (`XRConnectorComponent.ConnectToSocket` _returnvalue_2 _output))))))
    (:`else`
      (goto _label))))

(fn `GetLoadPriority`
  (returns (OutLoadPriority :type Integer) (OutGroupName :type Name))
  (return 0 "None"))

(fn `GetLoadState`
  (returns (OutLoadState :type "/XR_Toolkit/XR_Toolkit/Core/Scene/EN_XRCoreScene_LoadState Enum"))
  (return "NewEnumerator0"))

(fn `GetSupressesLoading`
  (returns (bSupressLoading :type Boolean))
  (return false))
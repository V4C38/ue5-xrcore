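; XR Toolkit initializer that ties component initialization to the scene manager's loading process.
; It keeps a list of unique registered components, immediately initializing each new one if the scene is already loaded and uninitializing it otherwise.
; On its load event it initializes every registered component, moving its own state from Loading to Loaded.
; It also exposes that state, plus a load priority and group name.
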(event `self.ReceiveBeginPlay`
  (set `self.XRCore Scene Manager` (`/XR_Toolkit/XR_Toolkit/Core/Utilities/FL_XRUtilityFunctions.XRCoreScene_GetSceneManager`)))

(event `/XR_Toolkit/XR_Toolkit/Core/Scene/BPI_XRCore_SceneLoadComponent.OnLoadComponent`
  (set `self.Load State` "NewEnumerator2")
  (for _array_element (`self.RegisteredComponents`)
    (`/XR_Toolkit/XR_Toolkit/Core/Scene/ActorLoading/BP_XRCore_InitializationComponent.Initialize` _array_element))
  (set `self.Load State` "NewEnumerator3"))

(event `/XR_Toolkit/XR_Toolkit/Core/Scene/BPI_XRCore_SceneLoadComponent.OnFinishedLoadingScene`)

(fn `GetLoadPriority`
  (returns (OutLoadPriority :type Integer) (OutGroupName :type Name))
  (return (`self.LoadPriority`) (`self.LoadGroupName`)))

(fn `GetLoadState`
  (returns (OutLoadState :type "/XR_Toolkit/XR_Toolkit/Core/Scene/EN_XRCoreScene_LoadState Enum"))
  (return (`self.Load State`)))

(fn `RegisterComponent`
  (params (InComponent :type "/XR_Toolkit/XR_Toolkit/Core/Scene/ActorLoading/BP_XRCore_InitializationComponent Object Reference"))
  (`/Engine/EditorBlueprintResources/StandardMacros.IsValid` InComponent
    (:`Is Valid`
      (if (not (`KismetArrayLibrary.Array_Contains` (`self.RegisteredComponents`) (`local.InComponent`)))
        (`KismetArrayLibrary.Array_Add` (`self.RegisteredComponents`) (`local.InComponent`))
        (switch `/XR_Toolkit/XR_Toolkit/Core/Scene/EN_XRCoreScene_LoadState` (`/XR_Toolkit/XR_Toolkit/Core/Scene/BP_XRCore_SceneManager.GetLoadState` (`self.XRCore Scene Manager`))
          (:`NewEnumerator0`
            (`/XR_Toolkit/XR_Toolkit/Core/Scene/ActorLoading/BP_XRCore_InitializationComponent.Un-Initialize` (`local.InComponent`) :!label _label))
          (:`NewEnumerator1`
            (goto _label))
          (:`NewEnumerator2`
            (goto _label))
          (:`NewEnumerator3`
            (`/XR_Toolkit/XR_Toolkit/Core/Scene/ActorLoading/BP_XRCore_InitializationComponent.Initialize` (`local.InComponent`))))))))
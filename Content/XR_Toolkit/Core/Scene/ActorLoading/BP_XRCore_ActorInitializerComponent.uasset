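; Actor component that lets the XR scene manager's initialization manager stage the loading of its owning actor, tracking a load state throughout.
; On BeginPlay it optionally registers with that manager, warning if none exists.
; UnInitialize hides the owner, disables collision and hides its spatial annotations.
; Initialize can connect the owner to a target actor's socket, then restores visibility, collision and initially visible annotations; scale-in timeline and disconnect logic are unwired.
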(event `self.ReceiveBeginPlay`
  (set `self.LoadState` "NewEnumerator0")
  (if (`self.bRegisterWithSceneManager`)
    (bind _output_get (set `self.XRCoreSceneManager` (`/XR_Toolkit/XR_Toolkit/Core/Utilities/FL_XRUtilityFunctions.XRCoreScene_GetSceneManager`)))
    (bind _returnvalue (`Actor.GetComponentByClass` _output_get "/XR_Toolkit/XR_Toolkit/Core/Scene/ActorLoading/BP_XRCore_ActorInitializationManager.BP_XRCore_ActorInitializationManager_C"))
    (`/Engine/EditorBlueprintResources/StandardMacros.IsValid` _returnvalue
      (:`Is Valid`
        (`/XR_Toolkit/XR_Toolkit/Core/Scene/ActorLoading/BP_XRCore_ActorInitializationManager.RegisterComponent` _returnvalue self)
        (set `self.LoadState` "NewEnumerator2"))
      (:`Is Not Valid`
        (`/XR_Toolkit/XR_Toolkit/Core/Utilities/FL_XRUtilityFunctions.CustomDebugWarning` "NewEnumerator1" self "XRCore_ActorInitializer component not found on XRCreSceneManager.")
        (set `self.LoadState` "NewEnumerator4")))))

(event `UnInitialize`
  (bind _returnvalue (`self.GetOwner`))
  ;[0 0 0] Called by ActorInitializer
  (set `self.LoadState` "NewEnumerator1")
  (`Actor.SetActorHiddenInGame` _returnvalue true)
  (`Actor.SetActorEnableCollision` _returnvalue false)
  (`|ExecutionSequence`
    (:`then_0`
      (`/Engine/EditorBlueprintResources/StandardMacros.IsValid` (`Actor.GetComponentByClass` (`self.GetOwner`) "/Script/XR_Toolkit.XRConnectorComponent")))
    (:`then_1`
      (for _array_element (`Actor.K2_GetComponentsByClass` (`self.GetOwner`) "/XR_Toolkit/XR_Toolkit/Core/Utilities/XRAnnotation/BP_SpatialAnnotation.BP_SpatialAnnotation_C")
        (message `/XR_Toolkit/XR_Toolkit/Core/Utilities/XRAnnotation/BPI_XRCoreUI.Hide` _array_element)))))

(event `Initialize`
  (bind _returnvalue (`self.GetOwner`))
  ;[0 0 0] Called by ActorInitializer
  (bind _connecttoactor (`self.ConnectToActor`)
    (:`then`
      (`XRToolsUtilityFunctions.TryConnectToActor` (`Actor.GetComponentByClass` (`self.GetOwner`) "/Script/XR_Toolkit.XRConnectorComponent") _connecttoactor (`self.ConnectionSocketID`)))
    (:`else`
      _))
  (`Actor.SetActorHiddenInGame` _returnvalue false)
  (`Actor.SetActorEnableCollision` _returnvalue true)
  (`|ExecutionSequence`
    (:`then_0`
      (for _array_element (`Actor.K2_GetComponentsByClass` (`self.GetOwner`) "/XR_Toolkit/XR_Toolkit/Core/Utilities/XRAnnotation/BP_SpatialAnnotation.BP_SpatialAnnotation_C")
        (if (`/XR_Toolkit/XR_Toolkit/Core/Utilities/XRAnnotation/BP_SpatialAnnotation.bInitiallyVisible` _array_element)
          (message `/XR_Toolkit/XR_Toolkit/Core/Utilities/XRAnnotation/BPI_XRCoreUI.Show` _array_element))))
    (:`then_1`
      (set `self.LoadState` "NewEnumerator3"))))

(fn `GetLoadPriority`
  (returns (OutLoadPriority :type Integer) (OutGroupName :type Name))
  (return 0 "None"))

(fn `GetLoadState`
  (returns (OutLoadState :type "/XR_Toolkit/XR_Toolkit/Core/Scene/EN_XRCoreScene_LoadState Enum"))
  (return "NewEnumerator0"))

(fn `GetSupressesLoading`
  (returns (bSupressLoading :type Boolean))
  (return false))
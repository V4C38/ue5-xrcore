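; XR Toolkit scene manager that loads its scene components in priority-ordered groups on BeginPlay.
; It sorts its components implementing BPI_XRCore_SceneComponent into loading-group objects keyed by priority, then loads them sequentially, highest first.
; A looping timer polls the current group, since UObjects lack Blueprint timers, and its Loaded event starts the next.
; It updates loading messages and broadcasts start and completion, with an optional timeout that auto-completes loading.
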(event `self.ReceiveBeginPlay`
  (`self.CacheXRCoreSceneComponents`)
  (`self.LoadScene`))

(event `LoadScene`
  ;[0 0 0] Load Scene
  (`|ExecutionSequence`
    (:`then_0`
      (`self.OnLoadingScene` self))
    (:`then_1`
      (bind _returnvalue (`KismetSystemLibrary.K2_SetTimerDelegate` (delegate `OnLoadTimerFinished`) (`self.AutoCompleteSceneLoadAfterSeconds`)))
      (set `self.Timer_SceneLoadDuration` _returnvalue))
    (:`then_2`
      (bind _values (`BlueprintMapLibrary.Map_Values` (`self.ComponentGroups`)))
      (for _array_element _values
        (`/XR_Toolkit/XR_Toolkit/Core/Scene/BP_XRCoreSceneComponentLoadingGroup.QueueGroup` _array_element))
      (`self.LoadNextGroup`) ; Start Loading all groups sequentially
    )
    (:`then_3`
      (`KismetSystemLibrary.PrintString` (`KismetStringLibrary.Concat_StrStr` "XRCore Scene: Loading " (`KismetStringLibrary.Conv_IntToString` (`BlueprintMapLibrary.Map_Length` (`self.ComponentGroups`))) " component groups.") true true (struct :`G` 0.5 :`A` 1.0) 5.0 "XRCoreScene_Init"))))

(event `OnLoadTimerFinished`
  ;[0 0 0] Load Scene
  (if (`self.bAutoCompleteSceneLoad`)
    (`self.LoadSceneCompleted`)))

(event `LoadNextGroup`
  (bind (_success _outloadinggroup) (`self.GetHighestPriorityLoadingGroup`))
  (bind _returnvalue (`KismetStringLibrary.Concat_StrStr` "Group: " (`KismetStringLibrary.Conv_NameToString` (`/XR_Toolkit/XR_Toolkit/Core/Scene/BP_XRCoreSceneComponentLoadingGroup.GroupName` (`self.CurrentLoadGroup`)))))
  ;[1 1 1] Load Group
  (if _success
    (bind _output_get (set `self.CurrentLoadGroup` _outloadinggroup))
    (`/XR_Toolkit/XR_Toolkit/Core/Scene/BP_XRCoreSceneComponentLoadingGroup.LoadGroup` _output_get)
    (add `/XR_Toolkit/XR_Toolkit/Core/Scene/BP_XRCoreSceneComponentLoadingGroup.OnGroupLoadStateChanged` _output_get (delegate `OnGroupLoadStateChanged_Event`))
    (`/XR_Toolkit/XR_Toolkit/Core/Scene/LoadingMessage/BP_XRCore_LoadingMessageProvider.UpdateMessage` (`self.BP_XRCore_LoadingMessageProvider`) (`KismetTextLibrary.Conv_StringToText` _returnvalue))
    (`KismetSystemLibrary.PrintString` (`KismetStringLibrary.Concat_StrStr` "XRCore Scene: " _returnvalue) true true (struct :`G` 0.5 :`A` 1.0) 2.0 "XRCoreScene_LoaderDetail")
    ;[0.3 0.3 0.3] Force check group load state as UObject cannot have timers in BP
    ; (if this is moved to C++ this can be moved to the group directly)
    (bind _returnvalue_2 (`KismetSystemLibrary.K2_SetTimerDelegate` (delegate `CheckGroupLoadState`) 0.5 true))
    (set `self.Timer_CheckGroupLoadState` _returnvalue_2)
    (else
      (set `self.CurrentLoadGroup` null)
      (`self.LoadSceneCompleted`))))

(event `CheckGroupLoadState`
  ;[0.3 0.3 0.3] Force check group load state as UObject cannot have timers in BP
  ; (if this is moved to C++ this can be moved to the group directly)
  (`/XR_Toolkit/XR_Toolkit/Core/Scene/BP_XRCoreSceneComponentLoadingGroup.CheckGroupLoadState` (`self.CurrentLoadGroup`)))

(event `OnGroupLoadStateChanged_Event`
  (params (Sender :type "/XR_Toolkit/XR_Toolkit/Core/Scene/BP_XRCoreSceneComponentLoadingGroup Object Reference") (OutLoadState :type "/XR_Toolkit/XR_Toolkit/Core/Scene/EN_XRCoreSceneComponent_LoadState Enum" :default "NewEnumerator0"))
  ;[1 1 1] Load Group
  (if (`|EnumEquality` OutLoadState "NewEnumerator3")
    (clear `/XR_Toolkit/XR_Toolkit/Core/Scene/BP_XRCoreSceneComponentLoadingGroup.OnGroupLoadStateChanged` Sender)
    (`KismetSystemLibrary.K2_ClearAndInvalidateTimerHandle` (`self.Timer_CheckGroupLoadState`))
    (`self.LoadNextGroup`)
    (`KismetSystemLibrary.PrintString` (`KismetStringLibrary.Concat_StrStr` "XRCore Scene: finished loading group: " (`KismetStringLibrary.Conv_NameToString` (`/XR_Toolkit/XR_Toolkit/Core/Scene/BP_XRCoreSceneComponentLoadingGroup.GroupName` Sender))) true true (struct :`G` 0.5 :`A` 1.0) 2.0 "XRCoreScene_LoaderDetail")))

(event `LoadSceneCompleted`
  ;[0 0 0] Finished Load Scene
  (`KismetSystemLibrary.K2_ClearAndInvalidateTimerHandle` (`self.Timer_CheckGroupLoadState`))
  (`|ExecutionSequence`
    (:`then_0`
      (`/XR_Toolkit/XR_Toolkit/Core/Scene/LoadingMessage/BP_XRCore_LoadingMessageProvider.UpdateMessage` (`self.BP_XRCore_LoadingMessageProvider`) "Completed."))
    (:`then_1`
      (`self.OnLoadingSceneCompleted` self))
    (:`then_2`
      (bind _values (`BlueprintMapLibrary.Map_Values` (`self.ComponentGroups`)))
      (for _array_element _values
        (`/XR_Toolkit/XR_Toolkit/Core/Scene/BP_XRCoreSceneComponentLoadingGroup.CompleteGroup` _array_element)))
    (:`then_3`
      (`KismetSystemLibrary.PrintString` (`KismetStringLibrary.Concat_StrStr` "XRCore Scene: Finished Loading.  \nLoaded a total of " (`KismetStringLibrary.Conv_IntToString` (`BlueprintMapLibrary.Map_Length` (`self.ComponentGroups`))) " SceneComponent groups took " (`KismetStringLibrary.Conv_DoubleToString` (`KismetSystemLibrary.K2_GetTimerElapsedTimeHandle` (`self.Timer_SceneLoadDuration`))) " Seconds." (select `bool` (`self.bAutoCompleteSceneLoad`) :`true` " \n(Autocompleted)")) true true (struct :`G` 0.5 :`A` 1.0) 5.0 "XRCoreScene_Init")
      (`KismetSystemLibrary.K2_ClearAndInvalidateTimerHandle` (`self.Timer_SceneLoadDuration`)))))

(fn `CacheXRCoreSceneComponents`
  (locals (Loc_UnsortedLoadingGroups :type "Map of Integer to /XR_Toolkit/XR_Toolkit/Core/Scene/BP_XRCoreSceneComponentLoadingGroup Object Reference"))
  (for _array_element (`self.GetComponentsByInterface` "/XR_Toolkit/XR_Toolkit/Core/Scene/BPI_XRCore_SceneComponent.BPI_XRCore_SceneComponent_C")
    (bind (_outloadpriority _outgroupname) (message `/XR_Toolkit/XR_Toolkit/Core/Scene/BPI_XRCore_SceneComponent.GetLoadPriority` _array_element))
    (bind (_value _returnvalue) (`BlueprintMapLibrary.Map_Find` (`local.Loc_UnsortedLoadingGroups`) _outloadpriority))
    (if _returnvalue
      (`/XR_Toolkit/XR_Toolkit/Core/Scene/BP_XRCoreSceneComponentLoadingGroup.AddXRCoreSceneComponent` _value _array_element "NewEnumerator0")
      (else
        (bind _returnvalue_2 (`|GenericCreateObject` self "/XR_Toolkit/XR_Toolkit/Core/Scene/BP_XRCoreSceneComponentLoadingGroup.BP_XRCoreSceneComponentLoadingGroup_C" _outloadpriority _outgroupname))
        (`/XR_Toolkit/XR_Toolkit/Core/Scene/BP_XRCoreSceneComponentLoadingGroup.AddXRCoreSceneComponent` _returnvalue_2 _array_element "NewEnumerator0")
        (`BlueprintMapLibrary.Map_Add` (`local.Loc_UnsortedLoadingGroups`) _outloadpriority _returnvalue_2))))
  (set `self.ComponentGroups` (`local.Loc_UnsortedLoadingGroups`))
  (return))

(fn `GetHighestPriorityLoadingGroup`
  (returns (Success :type Boolean) (OutLoadingGroup :type "/XR_Toolkit/XR_Toolkit/Core/Scene/BP_XRCoreSceneComponentLoadingGroup Object Reference"))
  (locals (Loc_HighestPriority :type Integer :default -1) (Loc_OutGroup :type "/XR_Toolkit/XR_Toolkit/Core/Scene/BP_XRCoreSceneComponentLoadingGroup Object Reference"))
  (bind (_value _returnvalue) (`BlueprintMapLibrary.Map_Find` (`self.ComponentGroups`) (`local.Loc_HighestPriority`)))
  (bind _values (`BlueprintMapLibrary.Map_Values` (`self.ComponentGroups`)))
  (for _array_element _values
    (switch `/XR_Toolkit/XR_Toolkit/Core/Scene/EN_XRCoreSceneComponent_LoadState` (`/XR_Toolkit/XR_Toolkit/Core/Scene/BP_XRCoreSceneComponentLoadingGroup.GetGroupLoadedState` _array_element)
      (:`NewEnumerator0`
        _)
      (:`NewEnumerator1`
        _))
    (bind _priority (`/XR_Toolkit/XR_Toolkit/Core/Scene/BP_XRCoreSceneComponentLoadingGroup.Priority` _array_element))
    (if (> _priority (`local.Loc_HighestPriority`))
      (set `local.Loc_HighestPriority` _priority)))
  (if _returnvalue
    (return true _value)
    (else
      (return false null))))

(fn `UserConstructionScript`)
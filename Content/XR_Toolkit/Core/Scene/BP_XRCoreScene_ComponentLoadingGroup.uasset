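; A loading group for XR Toolkit scenes that tracks a set of XR core scene components and a shared load state.
; Queue, load, complete and unload events drive the group, relaying load, finished-loading and unload messages to each registered component.
; CheckGroupLoadState queries every component and, once all report Loaded, marks the group Loaded and fires its state-changed dispatcher.
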(event `QueueGroup`
  (`self.SetGroupLoadedState` "NewEnumerator1"))

(event `LoadGroup`
  (`self.SetGroupLoadedState` "NewEnumerator2")
  (for _array_element (`self.XRCoreSceneComponents`)
    (message `/XR_Toolkit/XR_Toolkit/Core/Scene/BPI_XRCoreScene_LoadComponent.OnLoadComponent` _array_element)))

(event `CompleteGroup`
  (for _array_element (`self.XRCoreSceneComponents`)
    (message `/XR_Toolkit/XR_Toolkit/Core/Scene/BPI_XRCoreScene_LoadComponent.OnFinishedLoadingScene` _array_element)))

(event `UnloadGroup`
  (`self.SetGroupLoadedState` "NewEnumerator0"))

(fn `AddXRCoreSceneComponent`
  (params (InComponent :type "ActorComponent Object Reference") (InCurrentLoadState :type "/XR_Toolkit/XR_Toolkit/Core/Scene/EN_XRCoreScene_LoadState Enum" :default "NewEnumerator0"))
  (`KismetArrayLibrary.Array_AddUnique` (`self.XRCoreSceneComponents`) (`local.InComponent`)))

(fn `CheckGroupLoadState`
  (returns (bOutLoaded :type Boolean))
  (locals (bLoc_Loaded :type Boolean))
  (set `local.bLoc_Loaded` true)
  (for _array_element (`self.XRCoreSceneComponents`)
    (bind _outloadstate (message `/XR_Toolkit/XR_Toolkit/Core/Scene/BPI_XRCoreScene_LoadComponent.GetLoadState` _array_element))
    (if (not (`|EnumEquality` _outloadstate "NewEnumerator3"))
      (set `local.bLoc_Loaded` false)))
  (if (`local.bLoc_Loaded`)
    (bind _output_get (set `self.LoadState` "NewEnumerator3"))
    (`self.OnGroupLoadStateChanged` self _output_get)
    (return true)
    (else
      (return false))))

(fn `GetAllXRSceneComponents`
  (returns (OutComponents :type "Array of ActorComponent Object Reference"))
  (return (`self.XRCoreSceneComponents`)))

(fn `GetGroupLoadedState`
  (returns (OutLoadState :type "/XR_Toolkit/XR_Toolkit/Core/Scene/EN_XRCoreScene_LoadState Enum"))
  (return (`self.LoadState`)))

(fn `RemoveXRCoreSceneComponent`
  (params (InComponent :type "ActorComponent Object Reference"))
  (`KismetArrayLibrary.Array_RemoveItem` (`self.XRCoreSceneComponents`) InComponent))

(fn `SetGroupLoadedState`
  (params (InState :type "/XR_Toolkit/XR_Toolkit/Core/Scene/EN_XRCoreScene_LoadState Enum" :default "NewEnumerator0"))
  (if (`|EnumInequality` InState (`self.LoadState`))
    (bind _output_get (set `self.LoadState` InState))
    (switch `/XR_Toolkit/XR_Toolkit/Core/Scene/EN_XRCoreScene_LoadState` _output_get
      (:`NewEnumerator0`
        (for _array_element (`self.XRCoreSceneComponents`)
          (message `/XR_Toolkit/XR_Toolkit/Core/Scene/BPI_XRCoreScene_LoadComponent.OnUnloadComponent` _array_element))))))
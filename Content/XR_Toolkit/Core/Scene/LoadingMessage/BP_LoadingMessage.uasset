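; BP_LoadingMessage is a floating text message, likely shown during scene loading in the XR toolkit, that hovers in front of the player's camera.
; Tick eases it toward a point ahead of the camera and turns it to face the player, pausing while it is grabbed.
; UpdateMessage refreshes the text render.
; RemoveMessage starts a timer whose remaining time shrinks the actor's scale until it is destroyed.
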(event `self.ReceiveBeginPlay`
  (bind _camera (`self.Camera`))
  (bind _returnvalue (`self.GetComponentByClass` (`GameplayStatics.GetPlayerPawn` 0) "/Script/Engine.CameraComponent"))
  (`|ExecutionSequence`
    (:`then_0`
      ;[1 1 1] Rotate to Player Camera
      (`/Engine/EditorBlueprintResources/StandardMacros.IsValid` _returnvalue
        (:`Is Valid`
          (set `self.Camera` _returnvalue)
          (`self.SetActorTickEnabled` true)
          (`self.K2_SetActorLocation` (+ (`SceneComponent.K2_GetComponentLocation` _camera) (* (`SceneComponent.GetForwardVector` _camera) (`self.DistanceToCamera`)))))))
    (:`then_1`
      (`TextRenderComponent.K2_SetText` (`self.TextRender_SceneName`) (`self.DescriptionText`) :!label _label))))

(event `UpdateMessage`
  (params (DescriptionText :type Text))
  (set `self.DescriptionText` DescriptionText)
  (goto _label))

(event `RemoveMessage`
  (bind _returnvalue (`KismetSystemLibrary.K2_SetTimerDelegate` (delegate `DestroyMessage`) (`self.DestroyTime`)))
  (set `self.DestroyTimer` _returnvalue))

(event `DestroyMessage`
  (`self.K2_DestroyActor`))

(event `self.ReceiveTick`
  (params (DeltaSeconds :type "Float (single-precision)"))
  (bind _returnvalue (`self.K2_GetActorLocation`))
  (bind _camera (`self.Camera`))
  (bind _destroytimer (`self.DestroyTimer`))
  (if (not (`XRInteractionComponent.IsInteractedWith` (`self.XRInteractionGrab`)))
    (`self.K2_SetActorLocationAndRotation` (`KismetMathLibrary.VInterpTo` _returnvalue (+ (`SceneComponent.K2_GetComponentLocation` _camera) (* (`SceneComponent.GetForwardVector` _camera) (`self.DistanceToCamera`))) DeltaSeconds 2.0) (`KismetMathLibrary.FindLookAtRotation` _returnvalue (`SceneComponent.K2_GetComponentLocation` (`self.Camera`))))
    (if (`KismetSystemLibrary.K2_IsTimerActiveHandle` _destroytimer)
      (`self.SetActorScale3D` (`KismetMathLibrary.Conv_DoubleToVector` (`KismetMathLibrary.MapRangeClamped` (`KismetSystemLibrary.K2_GetTimerRemainingTimeHandle` _destroytimer) 0.0 (`self.DestroyTime`) 0.0 1.0))))))

(fn `UserConstructionScript`)
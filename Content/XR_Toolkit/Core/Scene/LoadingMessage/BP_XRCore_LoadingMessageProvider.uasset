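; BP_XRCore_LoadingMessageProvider shows a loading message in front of the player's camera while an XR Toolkit scene loads.
; On BeginPlay, unless on a dedicated server or suppressed, it spawns a BP_LoadingMessage along the camera's forward vector, titled with the level name.
; It forwards load group names and background progress to that message.
; Finishing the scene load or unloading the component removes the message and resets the load state.
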(event `self.ReceiveBeginPlay`
  (bind _distancetocamera (`self.DistanceToCamera`))
  (bind _returnvalue (`Actor.GetComponentByClass` (`GameplayStatics.GetPlayerPawn` 0) "/Script/Engine.CameraComponent"))
  (if (`KismetSystemLibrary.IsDedicatedServer`)
    _
    (elif (not (`self.bSupressLoading`))
      (bind _returnvalue_2 (`|SpawnActorFromClass` "/XR_Toolkit/XR_Toolkit/Core/Scene/LoadingMessage/BP_LoadingMessage.BP_LoadingMessage_C" (`KismetMathLibrary.MakeTransform` (+ (`SceneComponent.K2_GetComponentLocation` _returnvalue) (* (`SceneComponent.GetForwardVector` _returnvalue) _distancetocamera)) (struct) (`KismetMathLibrary.Conv_DoubleToVector` (`self.SpawnSize`))) "Undefined" "MultiplyWithRoot" null _distancetocamera (`self.LevelName`) null))
      (bind _output_get (set `self.SceneLoadingMessage` _returnvalue_2))
      (set `self.Load State` "NewEnumerator3")
      (`/XR_Toolkit/XR_Toolkit/Core/Scene/LoadingMessage/BPI_XRCore_LoadingMessage.UpdateTitle` _output_get (`self.LevelName`)))))

(event `/XR_Toolkit/XR_Toolkit/Core/Scene/BPI_XRCore_SceneLoadComponent.OnFinishedLoadingScene`
  (`/XR_Toolkit/XR_Toolkit/Core/Scene/LoadingMessage/BPI_XRCore_LoadingMessage.RemoveMessage` (`self.SceneLoadingMessage`) :!label _label)
  (set `self.Load State` "NewEnumerator0"))

(event `/XR_Toolkit/XR_Toolkit/Core/Scene/BPI_XRCore_SceneLoadComponent.OnUnloadComponent`
  (goto _label))

(event `SetCurrentLoadGroup`
  (params (InLoadingGroup :type "/XR_Toolkit/XR_Toolkit/Core/Scene/BP_XRCoreSceneComponentLoadingGroup Object Reference"))
  (bind _sceneloadingmessage (`self.SceneLoadingMessage`))
  (`self.SceneLoadingMessage`
    (:`then`
      (`/Engine/EditorBlueprintResources/StandardMacros.IsValid` InLoadingGroup
        (:`Is Valid`
          (`/XR_Toolkit/XR_Toolkit/Core/Scene/LoadingMessage/BPI_XRCore_LoadingMessage.UpdateInfo` _sceneloadingmessage (`KismetTextLibrary.Conv_NameToText` (`/XR_Toolkit/XR_Toolkit/Core/Scene/BP_XRCoreSceneComponentLoadingGroup.GroupName` InLoadingGroup))))
        (:`Is Not Valid`
          (`/XR_Toolkit/XR_Toolkit/Core/Scene/LoadingMessage/BPI_XRCore_LoadingMessage.UpdateInfo` _sceneloadingmessage "Final"))))
    (:`else`)))

(event `/XR_Toolkit/XR_Toolkit/Core/Scene/LoadingMessage/BPI_XRCore_LoadingMessage.UpdateBackground`
  (params (InProgress :type "Float (double-precision)"))
  (bind _sceneloadingmessage (`self.SceneLoadingMessage`)
    (:`then`
      (`/XR_Toolkit/XR_Toolkit/Core/Scene/LoadingMessage/BPI_XRCore_LoadingMessage.UpdateBackground` _sceneloadingmessage InProgress))
    (:`else`)))
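; XR persistence manager that owns the XRCore save game and relays per-object save and load requests to it by UUID.
; On BeginPlay it async-loads the existing save, or creates one and assigns random-integer string UUIDs to all actors with a BP_XRPersistentObject component.
; It also keeps a UUID-keyed registry of persistent objects for lookup and can delete the save slot.
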(event `self.ReceiveBeginPlay`
  (`|ExecutionSequence`
    (:`then_0`
      (bind _returnvalue (`GameplayStatics.DoesSaveGameExist` (`self.SlotName`)))
      (if _returnvalue
        (bind (_savegame _bsuccess) (`AsyncActionHandleSaveGame.AsyncLoadGameFromSlot` "XRCore")
          (:`Completed`
            (if _bsuccess
              (bind _asbp_xrcore_save_game (cast `/XR_Toolkit/XR_Toolkit/Core/Scene/Persistence/BP_XRCore_SaveGame` _savegame))
              (set `self.XRCore Save Game` _asbp_xrcore_save_game))))
        (else
          (bind _returnvalue_2 (`GameplayStatics.CreateSaveGameObject` "/XR_Toolkit/XR_Toolkit/Core/Scene/Persistence/BP_XRCore_SaveGame.BP_XRCore_SaveGame_C"))
          (`GameplayStatics.SaveGameToSlot` _returnvalue_2 "XRCore")
          (set `self.XRCore Save Game` _returnvalue_2)
          (`self.ProvideUUIDs`))))))

(event `ClearSaveData`
  (`GameplayStatics.DeleteGameInSlot` (`self.SlotName`)))

(event `ProvideUUIDs`
  (bind _outactors (`GameplayStatics.GetAllActorsOfClass` "/Script/Engine.Actor"))
  (for _array_element _outactors
    (bind _returnvalue (`Actor.GetComponentByClass` _array_element "/XR_Toolkit/XR_Toolkit/Core/Scene/Persistence/BP_XRPersistentObject.BP_XRPersistentObject_C"))
    (`/Engine/EditorBlueprintResources/StandardMacros.IsValid` _returnvalue
      (:`Is Valid`
        (bind _outuuid (`self.MakeUUID`))
        (set `/XR_Toolkit/XR_Toolkit/Core/Scene/Persistence/BP_XRPersistentObject.UUID` _outuuid _returnvalue)
        (`KismetSystemLibrary.PrintString` (`KismetStringLibrary.Concat_StrStr` "Provided " (`KismetSystemLibrary.GetDisplayName` _returnvalue) " PersistentObjects with UUID: " _outuuid) true true (struct :`G` 1.0 :`A` 1.0))))))

(fn `Get Persistent Object By UUID`
  (params (InUUID :type String))
  (returns (OutPersistentObject :type "/XR_Toolkit/XR_Toolkit/Core/Scene/Persistence/BP_XRPersistentObject Soft Object Reference"))
  (return (`BlueprintMapLibrary.Map_Find` (`self.PersistentActors`) InUUID)))

(fn `LoadPersistentObject`
  (params (InUUID :type String))
  (returns (bOutSuccess :type Boolean) (OutObjectData :type "/XR_Toolkit/XR_Toolkit/Core/Scene/Persistence/FXRPersistentObjectData Structure"))
  (bind _xrcore_save_game (`self.XRCore Save Game`)
    (:`then`
      (bind (_boutsucces _outobjectdata) (`/XR_Toolkit/XR_Toolkit/Core/Scene/Persistence/BP_XRCore_SaveGame.LoadPersistentObject` _xrcore_save_game InUUID))
      (return _boutsucces _outobjectdata))
    (:`else`
      (return false))))

(fn `MakeUUID`
  (returns (OutUUID :type String))
  (locals (Iter :type Integer))
  (return (`KismetStringLibrary.Conv_IntToString` (`KismetMathLibrary.RandomIntegerInRange` -214748364 214748364))))

(fn `RegisterPersistentObject`
  (params (InUUID :type String) (InPersistantObject :type "/XR_Toolkit/XR_Toolkit/Core/Scene/Persistence/BP_XRPersistentObject Soft Object Reference"))
  (bind _persistentactors (`self.PersistentActors`))
  (if (not (`.ReturnValue` (`BlueprintMapLibrary.Map_Find` _persistentactors InUUID)))
    (`BlueprintMapLibrary.Map_Add` _persistentactors InUUID InPersistantObject)))

(fn `SavePersistentObject`
  (params (InObjectData :type "/XR_Toolkit/XR_Toolkit/Core/Scene/Persistence/FXRPersistentObjectData Structure"))
  (bind _xrcore_save_game (`self.XRCore Save Game`)
    (:`then`
      (`/XR_Toolkit/XR_Toolkit/Core/Scene/Persistence/BP_XRCore_SaveGame.SavePersistentObject` _xrcore_save_game InObjectData))
    (:`else`)))
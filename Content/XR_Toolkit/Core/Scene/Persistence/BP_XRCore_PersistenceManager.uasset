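; Scene manager that saves and restores persistent XR objects through an XRCore SaveGame slot, loaded or created on BeginPlay.
; On load it caches actors with a PersistentObject component by UUID, applies saved transforms, then reconnects connectors to sockets in a second pass.
; Objects hidden during loading are revealed afterwards.
; Saving runs on EndPlay or a trigger interaction, another trigger clears data, and an editor tool assigns random UUIDs.
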(event `self.ReceiveBeginPlay`
  (bind _output (`|ConvertAsset` (`self.Trigger_ForceSave`)))
  (bind _output_2 (`|ConvertAsset` (`self.Trigger_ForceClear`)))
  (bind _bsupressloading (`/XR_Toolkit/XR_Toolkit/Core/Scene/BPI_XRCore_SceneLoadComponent.GetSupressesLoading`))
  (if (not _bsupressloading)
    (`|ExecutionSequence`
      (:`then_0`
        ;[0 0 0] Initial Load
        (bind _returnvalue (`GameplayStatics.DoesSaveGameExist` (`self.SaveGame_SlotName`)))
        (if _returnvalue
          (bind (_savegame _bsuccess) (`AsyncActionHandleSaveGame.AsyncLoadGameFromSlot` (`self.SaveGame_SlotName`))
            (:`Completed`
              (if _bsuccess
                (bind _asbp_xrcore_save_game (cast `/XR_Toolkit/XR_Toolkit/Core/Scene/Persistence/BP_XRCore_SaveGame` _savegame))
                (set `self.XRCore Save Game` _asbp_xrcore_save_game)
                (`KismetSystemLibrary.PrintString` "XRCore: Loaded Persistent Data from SaveGame" false true (struct :`R` 0.4 :`G` 0.4 :`B` 0.4 :`A` 1.0) 5.0))))
          (else
            (bind _returnvalue_2 (`GameplayStatics.CreateSaveGameObject` "/XR_Toolkit/XR_Toolkit/Core/Scene/Persistence/BP_XRCore_SaveGame.BP_XRCore_SaveGame_C"))
            (`GameplayStatics.SaveGameToSlot` _returnvalue_2 (`self.SaveGame_SlotName`))
            (set `self.XRCore Save Game` _returnvalue_2)
            (`KismetSystemLibrary.PrintString` "XRCore: Created new Persistent Data in SaveGame" false true (struct :`R` 0.4 :`G` 0.4 :`B` 0.4 :`A` 1.0) 5.0))))
      (:`then_1`
        ;[0 0 0] Assign to Triggers
        (`|ExecutionSequence`
          (:`then_0`
            (`/Engine/EditorBlueprintResources/StandardMacros.IsValid` _output
              (:`Is Valid`
                (add `XRInteractionComponent.OnInteractionStarted` (`/XR_Toolkit/XR_Toolkit/Demo/Blueprints/BP_XRTriggerable.XRInteractionTrigger` _output) (delegate `OnInteractionStarted_Event`)))))
          (:`then_1`
            (`/Engine/EditorBlueprintResources/StandardMacros.IsValid` _output_2
              (:`Is Valid`
                (add `XRInteractionComponent.OnInteractionStarted` (`/XR_Toolkit/XR_Toolkit/Demo/Blueprints/BP_XRTriggerable.XRInteractionTrigger` _output_2) (delegate `OnInteractionStarted_Event_0`))))))))))

(event `OnInteractionStarted_Event`
  (params (Sender :type "XRInteractionComponent Object Reference") (XRInteractorComponent :type "XRInteractorComponent Object Reference"))
  ;[0 0 0] Assign to Triggers
  (`self.SaveAllPersistentObjects`))

(event `OnInteractionStarted_Event_0`
  (params (Sender :type "XRInteractionComponent Object Reference") (XRInteractorComponent :type "XRInteractorComponent Object Reference"))
  ;[0 0 0] Assign to Triggers
  (`self.ClearSaveData`))

(event `/XR_Toolkit/XR_Toolkit/Core/Scene/BPI_XRCore_SceneLoadComponent.OnLoadComponent`
  ;[1 1 1] Load All Persistent Objects
  (set `self.Load State` "NewEnumerator2")
  (`self.CachePersistentObjectsInLevel`)
  (`self.LoadPersistentObjects`)
  (`self.Load Persistent Connections`)
  (set `self.Load State` "NewEnumerator3"))

(event `/XR_Toolkit/XR_Toolkit/Core/Scene/BPI_XRCore_SceneLoadComponent.OnFinishedLoadingScene`
  ;[1 1 1] Load All Persistent Objects
  (`self.FinishLoadPersistentObject`))

(event `/XR_Toolkit/XR_Toolkit/Core/Scene/BPI_XRCore_SceneLoadComponent.OnSupressedLoading`
  ;[1 1 1] Load All Persistent Objects
  (`KismetSystemLibrary.Delay` 1.0)
  (`self.Force Persistent Object Visibility`))

(event `self.ReceiveEndPlay`
  (params (EndPlayReason :type "EEndPlayReason Enum" :default "Destroyed"))
  (`self.SaveAllPersistentObjects`))

(event `SaveAllPersistentObjects`
  ;[1 1 1] Save / Clear
  (bind _keys (`BlueprintMapLibrary.Map_Keys` (`self.PersistentObjects`)))
  (for (_ _array_index) _keys
    (bind _values (`BlueprintMapLibrary.Map_Values` (`self.PersistentObjects`)))
    (bind _output (`|ConvertAsset` (`|GetArrayItem` _values _array_index)))
    (`/Engine/EditorBlueprintResources/StandardMacros.IsValid` _output
      (:`Is Valid`
        (`self.SavePersistentObject` (`/XR_Toolkit/XR_Toolkit/Core/Scene/Persistence/BP_XRCore_PersistentObject.Construct XRPersistent Object Data` _output))))))

(event `ClearSaveData`
  ;[1 1 1] Save / Clear
  (bind _keys (`BlueprintMapLibrary.Map_Keys` (`self.PersistentObjects`)))
  (for (_array_element _array_index) _keys
    (bind _values (`BlueprintMapLibrary.Map_Values` (`self.PersistentObjects`)))
    (`/Engine/EditorBlueprintResources/StandardMacros.IsValid` (`|ConvertAsset` (`|GetArrayItem` _values _array_index))
      (:`Is Valid`
        (`self.RemovePersistentObject` _array_element))
      (:`Is Not Valid`
        _))
    (`BlueprintMapLibrary.Map_Remove` (`self.PersistentObjects`) _array_element))
  (bind _xrcore_save_game (`self.XRCore Save Game`)
    (:`then`
      (`/XR_Toolkit/XR_Toolkit/Core/Scene/Persistence/BP_XRCore_SaveGame.ClearAllData` _xrcore_save_game))
    (:`else`)))

(event `ProvideUUIDs`
  ;[0 0 0] Editor Tools
  (bind _outactors (`GameplayStatics.GetAllActorsOfClass` "/Script/Engine.Actor"))
  (for _array_element _outactors
    (bind _returnvalue (`Actor.GetComponentByClass` _array_element "/XR_Toolkit/XR_Toolkit/Core/Scene/Persistence/BP_XRCore_PersistentObject.BP_XRCore_PersistentObject_C"))
    (`/Engine/EditorBlueprintResources/StandardMacros.IsValid` _returnvalue
      (:`Is Valid`
        (bind _outuuid (`self.MakeUUID`))
        (set `/XR_Toolkit/XR_Toolkit/Core/Scene/Persistence/BP_XRCore_PersistentObject.UUID` _outuuid _returnvalue)
        (`KismetSystemLibrary.PrintString` (`KismetStringLibrary.Concat_StrStr` "XRCore: Provided " (`KismetSystemLibrary.GetDisplayName` _returnvalue) " PersistentObjects with UUID: " _outuuid) true true (struct :`G` 1.0 :`A` 1.0))))))

(fn `CachePersistentObjectsInLevel`
  (bind _outactors (`GameplayStatics.GetAllActorsOfClass` "/Script/Engine.Actor"))
  (for _array_element _outactors
    (bind _returnvalue (`Actor.GetComponentByClass` _array_element "/XR_Toolkit/XR_Toolkit/Core/Scene/Persistence/BP_XRCore_PersistentObject.BP_XRCore_PersistentObject_C"))
    (`/Engine/EditorBlueprintResources/StandardMacros.IsValid` _returnvalue
      (:`Is Valid`
        (`BlueprintMapLibrary.Map_Add` (`self.PersistentObjects`) (`/XR_Toolkit/XR_Toolkit/Core/Scene/Persistence/BP_XRCore_PersistentObject.UUID` _returnvalue) (`|ConvertAsset` _returnvalue)))))
  (return))

(fn `FinishLoadPersistentObject`
  (bind _values (`BlueprintMapLibrary.Map_Values` (`self.PersistentObjects`)))
  (for _array_element _values
    (bind _output (`|ConvertAsset` _array_element))
    (`/Engine/EditorBlueprintResources/StandardMacros.IsValid` _output
      (:`Is Valid`
        (set `/XR_Toolkit/XR_Toolkit/Core/Scene/Persistence/BP_XRCore_PersistentObject.bLoaded` true _output)
        (if (`/XR_Toolkit/XR_Toolkit/Core/Scene/Persistence/BP_XRCore_PersistentObject.bHideWhileLoading` _output)
          (`Actor.SetActorHiddenInGame` (`self.GetOwner` _output) false))))))

(fn `Force Persistent Object Visibility`
  (bind _outactors (`GameplayStatics.GetAllActorsOfClass` "/Script/Engine.Actor"))
  (for _array_element _outactors
    (`/Engine/EditorBlueprintResources/StandardMacros.IsValid` (`Actor.GetComponentByClass` _array_element "/XR_Toolkit/XR_Toolkit/Core/Scene/Persistence/BP_XRCore_PersistentObject.BP_XRCore_PersistentObject_C")
      (:`Is Valid`
        (`Actor.SetActorHiddenInGame` _array_element false)))))

(fn `Get Persistent Object By UUID`
  (params (InUUID :type String))
  (returns (OutPersistentObject :type "/XR_Toolkit/XR_Toolkit/Core/Scene/Persistence/BP_XRCore_PersistentObject Soft Object Reference"))
  (return (`BlueprintMapLibrary.Map_Find` (`self.PersistentObjects`) InUUID)))

(fn `Load Persistent Connections`
  (bind _keys (`BlueprintMapLibrary.Map_Keys` (`self.PersistentObjects`)))
  (for _array_element _keys
    (bind (_boutsucces _outobjectdata) (`/XR_Toolkit/XR_Toolkit/Core/Scene/Persistence/BP_XRCore_SaveGame.LoadPersistentObject` (`self.XRCore Save Game`) _array_element))
    (if _boutsucces
      (bind (_objectuuid _transformdata _connectiondata) (break `/XR_Toolkit/XR_Toolkit/Core/Scene/Persistence/FXRPersistentObjectData` _outobjectdata))
      ;[1 1 1] Connected objects deferred
      (if (`.bIsConnected_13_2B5778B747D58B159B807D86E5D9AF56` (break `/XR_Toolkit/XR_Toolkit/Core/Scene/Persistence/FXRCore_ConnectionData` _connectiondata))
        (bind _returnvalue (`Actor.GetComponentByClass` (`self.GetOwner` (`|ConvertAsset` (`self.Get Persistent Object By UUID` _objectuuid))) "/Script/XR_Toolkit.XRConnectorComponent"))
        ;;[1 1 1] Get Connector on loaded object
        (`/Engine/EditorBlueprintResources/StandardMacros.IsValid` _returnvalue
          (:`Is Valid`
            (bind (_bisconnected _conectedactoruuid _connectedsocketid) (break `/XR_Toolkit/XR_Toolkit/Core/Scene/Persistence/FXRCore_ConnectionData` _connectiondata))
            ;;[1 1 1] Get Socket to Attach to
            (for _array_element_2 (`Actor.K2_GetComponentsByClass` (`self.GetOwner` (`|ConvertAsset` (`self.Get Persistent Object By UUID` _conectedactoruuid))) "/Script/XR_Toolkit.XRConnectorSocket")
              (if (`KismetStringLibrary.EqualEqual_StrStr` (`XRConnectorSocket.GetSocketID` _array_element_2) _connectedsocketid)
                (`XRConnectorComponent.ConnectToSocket` _returnvalue _array_element_2)))))))))

(fn `LoadPersistentObject`
  (params (InUUID :type String))
  (returns (bOutSuccess :type Boolean) (OutObjectData :type "/XR_Toolkit/XR_Toolkit/Core/Scene/Persistence/FXRPersistentObjectData Structure"))
  (bind _xrcore_save_game (`self.XRCore Save Game`)
    (:`then`
      (`|ExecutionSequence`
        (:`then_0`
          (bind (_boutsucces _outobjectdata) (`/XR_Toolkit/XR_Toolkit/Core/Scene/Persistence/BP_XRCore_SaveGame.LoadPersistentObject` _xrcore_save_game InUUID))
          (`KismetSystemLibrary.PrintString` (`KismetStringLibrary.Concat_StrStr` "XRCore SaveGame - " "Loaded Object: " (`.ObjectUUID_15_6A6D29464501F7B43E267790ACB8EC47` (break `/XR_Toolkit/XR_Toolkit/Core/Scene/Persistence/FXRPersistentObjectData` _outobjectdata))) false true (struct :`R` 0.2 :`G` 0.2 :`B` 0.2 :`A` 1.0)))
        (:`then_1`
          (return _boutsucces _outobjectdata))))
    (:`else`
      (return false))))

(fn `LoadPersistentObjects`
  (bind _keys (`BlueprintMapLibrary.Map_Keys` (`self.PersistentObjects`)))
  (for _array_element _keys
    (bind (_boutsucces _outobjectdata) (`/XR_Toolkit/XR_Toolkit/Core/Scene/Persistence/BP_XRCore_SaveGame.LoadPersistentObject` (`self.XRCore Save Game`) _array_element))
    (if _boutsucces
      (bind (_objectuuid _transformdata) (break `/XR_Toolkit/XR_Toolkit/Core/Scene/Persistence/FXRPersistentObjectData` _outobjectdata))
      (bind _output (`|ConvertAsset` (`self.Get Persistent Object By UUID` _objectuuid)))
      ;[1 1 1] Load Transform from persistent data
      (`/XR_Toolkit/XR_Toolkit/Core/Scene/Persistence/BP_XRCore_PersistentObject.ForceDisconnectOwner` _output)
      (`Actor.K2_SetActorTransform` (`self.GetOwner` _output) (`.Transform_2_5632505340EC93BF860305919E032C59` (break `/XR_Toolkit/XR_Toolkit/Core/Scene/Persistence/FXRCore_TransformData` _transformdata)) false false)))
  (return))

(fn `MakeUUID`
  (returns (OutUUID :type String))
  (locals (Iter :type Integer))
  (return (`KismetStringLibrary.Conv_IntToString` (`KismetMathLibrary.RandomIntegerInRange` -214748364 214748364))))

(fn `RegisterPersistentObject`
  (params (InUUID :type String) (InPersistantObject :type "/XR_Toolkit/XR_Toolkit/Core/Scene/Persistence/BP_XRCore_PersistentObject Soft Object Reference"))
  (bind _persistentobjects (`self.PersistentObjects`))
  (if (not (`.ReturnValue` (`BlueprintMapLibrary.Map_Find` _persistentobjects InUUID)))
    (`BlueprintMapLibrary.Map_Add` _persistentobjects InUUID InPersistantObject)))

(fn `RemovePersistentObject`
  (params (InUUID :type String))
  (bind _xrcore_save_game (`self.XRCore Save Game`)
    (:`then`
      (`/XR_Toolkit/XR_Toolkit/Core/Scene/Persistence/BP_XRCore_SaveGame.RemoveObjectFromSaveGame` _xrcore_save_game InUUID)
      (`KismetSystemLibrary.PrintString` (`KismetStringLibrary.Concat_StrStr` "XRCore SaveGame - " "Removed Object: " InUUID) true true (struct :`R` 0.2 :`G` 0.2 :`B` 0.2 :`A` 1.0)))
    (:`else`)))

(fn `SavePersistentObject`
  (params (InObjectData :type "/XR_Toolkit/XR_Toolkit/Core/Scene/Persistence/FXRPersistentObjectData Structure"))
  (bind _xrcore_save_game (`self.XRCore Save Game`)
    (:`then`
      (`/XR_Toolkit/XR_Toolkit/Core/Scene/Persistence/BP_XRCore_SaveGame.SavePersistentObject` _xrcore_save_game InObjectData)
      (`KismetSystemLibrary.PrintString` (`KismetStringLibrary.Concat_StrStr` "XRCore SaveGame - " "Saved Object: " (`.ObjectUUID_15_6A6D29464501F7B43E267790ACB8EC47` (break `/XR_Toolkit/XR_Toolkit/Core/Scene/Persistence/FXRPersistentObjectData` InObjectData))) true true (struct :`R` 0.2 :`G` 0.2 :`B` 0.2 :`A` 1.0)))
    (:`else`)))
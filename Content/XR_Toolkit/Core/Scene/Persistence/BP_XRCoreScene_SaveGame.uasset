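; SaveGame object for the XR Toolkit core scene that stores persistent object data in an array, keyed by each object's UUID.
; A linear lookup by UUID backs saving, which replaces any existing entry, and removal.
; Saves and successful removals write the object to its slot immediately.
; Clearing deletes the slot but leaves the in-memory array untouched.
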(event `SavePersistentObject`
  (params (InObjectData :type "/XR_Toolkit/XR_Toolkit/Core/Scene/Persistence/FXRCoreScene_PersistentObjectData Structure"))
  (bind (_boutsucces _outobjectdata _outindex) (`self.LoadPersistentObject` (`.ObjectUUID_15_6A6D29464501F7B43E267790ACB8EC47` (break `/XR_Toolkit/XR_Toolkit/Core/Scene/Persistence/FXRCoreScene_PersistentObjectData` InObjectData))))
  (if _boutsucces
    (`KismetArrayLibrary.Array_Remove` (`self.PersistentObjects`) _outindex))
  (`KismetArrayLibrary.Array_Add` (`self.PersistentObjects`) InObjectData)
  (`GameplayStatics.SaveGameToSlot` self (`self.Slot Name`)))

(event `RemoveObjectFromSaveGame`
  (params (InUUID :type String))
  (bind (_boutsucces _outobjectdata) (`self.LoadPersistentObject` InUUID))
  (if _boutsucces
    (`KismetArrayLibrary.Array_RemoveItem` (`self.PersistentObjects`) _outobjectdata)
    (`GameplayStatics.SaveGameToSlot` self (`self.Slot Name`))))

(event `ClearAllData`
  (`GameplayStatics.DeleteGameInSlot` (`self.Slot Name`)))

(fn `LoadPersistentObject`
  (params (InUUID :type String))
  (returns (bOutSucces :type Boolean) (OutObjectData :type "/XR_Toolkit/XR_Toolkit/Core/Scene/Persistence/FXRCoreScene_PersistentObjectData Structure") (OutIndex :type Integer))
  (for (_array_element _array_index) (`self.PersistentObjects`)
    (if (`KismetStringLibrary.EqualEqual_StrStr` (`.ObjectUUID_15_6A6D29464501F7B43E267790ACB8EC47` (break `/XR_Toolkit/XR_Toolkit/Core/Scene/Persistence/FXRCoreScene_PersistentObjectData` _array_element)) (`local.InUUID`))
      (return true _array_element _array_index)))
  (return false (struct) -1))
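; Actor component that persists its owner's transform and XR socket connection by UUID.
; On BeginPlay it hides the owner and registers with the scene manager's persistence manager, unhiding on post scene initialize.
; Scene initialize optionally loads saved data, reconnecting to the saved socket on another persistent object, or restoring the transform if no connection was saved.
; It saves every Tick and on EndPlay.
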(event `self.ReceiveBeginPlay`
  (`|ExecutionSequence`
    (:`then_0`
      (`Actor.SetActorHiddenInGame` (`self.GetOwner`) true))
    (:`then_1`
      (bind _ourxrscenemanager (`self.RegisterWithXRSceneManager`))
      (add `/XR_Toolkit/XR_Toolkit/Core/Scene/BP_XRCore_SceneManager.OnSceneInitialize` _ourxrscenemanager (delegate `OnSceneInitialize_Event`))
      (add `/XR_Toolkit/XR_Toolkit/Core/Scene/BP_XRCore_SceneManager.OnPostSceneInitialize` _ourxrscenemanager (delegate `OnPostSceneInitialize_Event`)))))

(event `OnSceneInitialize_Event`
  (params (Sender :type "/XR_Toolkit/XR_Toolkit/Core/Scene/BP_XRCore_SceneManager Object Reference"))
  (if (`self.bAutomaticallyLoadPersistentData`)
    (`self.Load Persistent Object`)))

(event `OnPostSceneInitialize_Event`
  (params (Sender :type "/XR_Toolkit/XR_Toolkit/Core/Scene/BP_XRCore_SceneManager Object Reference"))
  (`Actor.SetActorHiddenInGame` (`self.GetOwner`) false))

(event `self.ReceiveTick`
  (params (DeltaSeconds :type "Float (single-precision)"))
  (`self.Save Persistent Object`))

(event `self.ReceiveEndPlay`
  (params (EndPlayReason :type "EEndPlayReason Enum" :default "Destroyed"))
  (`self.Save Persistent Object`))

(fn `ForceDisconnectOwner`
  (bind _returnvalue (`Actor.GetComponentByClass` (`self.GetOwner`) "/Script/XR_Toolkit.XRConnectorComponent"))
  (`/Engine/EditorBlueprintResources/StandardMacros.IsValid` _returnvalue
    (:`Is Valid`
      (`XRConnectorComponent.DisconnectFromSocket` _returnvalue))
    (:`Is Not Valid`
      _))
  (return))

(fn `GetOwnerTransformData`
  (returns (OutTransformData :type "/XR_Toolkit/XR_Toolkit/Core/Scene/Persistence/FXRCore_TransformData Structure"))
  (bind _returnvalue (`self.GetOwner`))
  (`/Engine/EditorBlueprintResources/StandardMacros.IsValid` _returnvalue
    (:`Is Valid`
      (return (make `/XR_Toolkit/XR_Toolkit/Core/Scene/Persistence/FXRCore_TransformData` (`Actor.GetTransform` _returnvalue))))
    (:`Is Not Valid`
      (return))))

(fn `GetUUID`
  (returns (OutUUID :type String))
  (return (`self.UUID`)))

(fn `GetXRConnectionData`
  (returns (bOutIsConnected :type Boolean) (OutConnectionData :type "/XR_Toolkit/XR_Toolkit/Core/Scene/Persistence/FXRCore_ConnectionData Structure"))
  (bind _returnvalue (`Actor.GetComponentByClass` (`self.GetOwner`) "/Script/XR_Toolkit.XRConnectorComponent"))
  (bind (_outconnectedsocket _returnvalue_2) (`XRConnectorComponent.IsConnected` _returnvalue))
  (bind _returnvalue_3 (`Actor.GetComponentByClass` (`self.GetOwner` _outconnectedsocket) "BP_XRPersistentObject_C"))
  (`/Engine/EditorBlueprintResources/StandardMacros.IsValid` _returnvalue
    (:`Is Valid`
      (if _returnvalue_2
        ;[1 1 1] Check if connected to a persistable Object
        (`/Engine/EditorBlueprintResources/StandardMacros.IsValid` _returnvalue_3
          (:`Is Valid`
            (return true (make `/XR_Toolkit/XR_Toolkit/Core/Scene/Persistence/FXRCore_ConnectionData` (`self.GetUUID` _returnvalue_3) (`XRConnectorSocket.GetSocketID` _outconnectedsocket))))
          (:`Is Not Valid`
            _))))
    (:`Is Not Valid`
      _))
  (return false))

(fn `Load Persistent Object`
  (bind _returnvalue (`Actor.GetComponentByClass` (`self.GetOwner`) "/Script/XR_Toolkit.XRConnectorComponent"))
  (bind _xrcore_persistence_manager (`self.XRCore Persistence Manager`)
    (:`then`
      (bind (_boutsuccess _outobjectdata) (`/XR_Toolkit/XR_Toolkit/Core/Scene/Persistence/BP_XRPersistenceManager.LoadPersistentObject` _xrcore_persistence_manager (`self.UUID`)))
      (if _boutsuccess
        (bind (_objectuuid _transformdata _connectiondata) (break `/XR_Toolkit/XR_Toolkit/Core/Scene/Persistence/FXRPersistentObjectData` _outobjectdata))
        (if (`KismetArrayLibrary.Array_IsValidIndex` _connectiondata)
          (bind (_conectedactoruuid _connectedsocketid) (break `/XR_Toolkit/XR_Toolkit/Core/Scene/Persistence/FXRCore_ConnectionData` (`|GetArrayItem` _connectiondata)))
          ;[1 1 1] Load XRConnection
          (bind _outpersistentobject (`/XR_Toolkit/XR_Toolkit/Core/Scene/Persistence/BP_XRPersistenceManager.Get Persistent Object By UUID` (`self.XRCore Persistence Manager`) _conectedactoruuid))
          (bind _output (`|ConvertAsset` _outpersistentobject))
          (`/Engine/EditorBlueprintResources/StandardMacros.IsValid` _output
            (:`Is Valid`
              (for _array_element (`Actor.K2_GetComponentsByClass` (`self.GetOwner` _output) "/Script/XR_Toolkit.XRConnectorSocket")
                (if (`KismetStringLibrary.EqualEqual_StrStr` (`XRConnectorSocket.GetSocketID` _array_element) _connectedsocketid)
                  (`/Engine/EditorBlueprintResources/StandardMacros.IsValid` _returnvalue
                    (:`Is Valid`
                      (`self.ForceDisconnectOwner`)
                      (`XRConnectorComponent.ConnectToSocket` _returnvalue _array_element)
                      ;[0 0 0] Debug
                      (`KismetSystemLibrary.PrintString` (`KismetStringLibrary.Concat_StrStr` "Restored " (`KismetSystemLibrary.GetDisplayName` (`self.GetOwner`)) " from persistant data.") true true (struct :`R` 0.2 :`G` 0.2 :`B` 0.2 :`A` 1.0) 4.0 :!label _label)))))))
          (else
            ;[1 1 1] Load Transform
            (`self.ForceDisconnectOwner`)
            (`Actor.K2_SetActorTransform` (`self.GetOwner`) (`.Transform_2_5632505340EC93BF860305919E032C59` (break `/XR_Toolkit/XR_Toolkit/Core/Scene/Persistence/FXRCore_TransformData` _transformdata)) false false)
            (goto _label)))))
    (:`else`)))

(fn `RegisterWithXRSceneManager`
  (returns (OurXRSceneManager :type "/XR_Toolkit/XR_Toolkit/Core/Scene/BP_XRCore_SceneManager Object Reference") (OutPersistenceManager :type "/XR_Toolkit/XR_Toolkit/Core/Scene/Persistence/BP_XRPersistenceManager Object Reference") (bOutSuccess :type Boolean))
  (bind _returnvalue (`GameplayStatics.GetActorOfClass` "/XR_Toolkit/XR_Toolkit/Core/Scene/BP_XRCore_SceneManager.BP_XRCore_SceneManager_C"))
  (`/Engine/EditorBlueprintResources/StandardMacros.IsValid` _returnvalue
    (:`Is Valid`
      (bind _output_get (set `self.XRCore Persistence Manager` (`/XR_Toolkit/XR_Toolkit/Core/Scene/BP_XRCore_SceneManager.BP_XRCore_PersistenceManager` _returnvalue)))
      (`/XR_Toolkit/XR_Toolkit/Core/Scene/Persistence/BP_XRPersistenceManager.RegisterPersistentObject` _output_get (`self.UUID`) (`|ConvertAsset` self))
      (return _returnvalue _output_get true))
    (:`Is Not Valid`
      (`KismetSystemLibrary.PrintString` (`KismetStringLibrary.Concat_StrStr` (`KismetSystemLibrary.GetDisplayName` self) " ERROR: Failed to find XRCore_SceneManager") true true (struct :`R` 1.0 :`A` 1.0) 4.0 "None")
      (return null null false))))

(fn `Save Persistent Object`
  (bind (_boutisconnected _outconnectiondata) (`self.GetXRConnectionData`))
  (bind _xrcore_persistence_manager (`self.XRCore Persistence Manager`)
    (:`then`
      (`/XR_Toolkit/XR_Toolkit/Core/Scene/Persistence/BP_XRPersistenceManager.SavePersistentObject` _xrcore_persistence_manager (make `/XR_Toolkit/XR_Toolkit/Core/Scene/Persistence/FXRPersistentObjectData` (`self.UUID`) (`self.GetOwnerTransformData`) (select `bool` _boutisconnected :`true` (`|MakeArray` _outconnectiondata)))))
    (:`else`)))
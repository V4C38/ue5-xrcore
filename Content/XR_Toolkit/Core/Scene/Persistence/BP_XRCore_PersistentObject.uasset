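; Actor component that makes its owning XR actor persistable, identified by a UUID.
; It packages the owner's transform and XRConnector socket link into a save struct and passes it to the XRCore Persistence Manager.
; Connections are recorded as target UUID plus socket ID, only when the target actor also has this component.
; It can optionally hide the owner on BeginPlay for loading and exposes functions to force socket connection or disconnection.
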(event `self.ReceiveBeginPlay`
  (if (`self.bHideWhileLoading`)
    (`Actor.SetActorHiddenInGame` (`self.GetOwner`) true)))

(fn `Construct XRPersistent Object Data`
  (returns (FXRPersistentObjectData :type "/XR_Toolkit/XR_Toolkit/Core/Scene/Persistence/FXRPersistentObjectData Structure"))
  (return (make `/XR_Toolkit/XR_Toolkit/Core/Scene/Persistence/FXRPersistentObjectData` (`self.UUID`) (`self.GetOwnerTransformData`) (`self.GetXRConnectionData`))))

(fn `ForceConnectOwner`
  (params (InSocket :type "XRConnectorSocket Object Reference"))
  (bind _returnvalue (`Actor.GetComponentByClass` (`self.GetOwner`) "/Script/XR_Toolkit.XRConnectorComponent"))
  (`/Engine/EditorBlueprintResources/StandardMacros.IsValid` _returnvalue
    (:`Is Valid`
      (`XRConnectorComponent.ConnectToSocket` _returnvalue InSocket))))

(fn `ForceDisconnectOwner`
  (bind _returnvalue (`Actor.GetComponentByClass` (`self.GetOwner`) "/Script/XR_Toolkit.XRConnectorComponent"))
  (`/Engine/EditorBlueprintResources/StandardMacros.IsValid` _returnvalue
    (:`Is Valid`
      (if (`.ReturnValue` (`XRConnectorComponent.IsConnected` _returnvalue))
        (`XRConnectorComponent.DisconnectFromSocket` _returnvalue)
        (return)))
    (:`Is Not Valid`
      (return))))

(fn `GetOwnerTransformData`
  (returns (OutTransformData :type "/XR_Toolkit/XR_Toolkit/Core/Scene/Persistence/FXRCore_TransformData Structure"))
  (bind _returnvalue (`self.GetOwner`))
  (`/Engine/EditorBlueprintResources/StandardMacros.IsValid` _returnvalue
    (:`Is Valid`
      (return (make `/XR_Toolkit/XR_Toolkit/Core/Scene/Persistence/FXRCore_TransformData` (`Actor.GetTransform` _returnvalue))))
    (:`Is Not Valid`
      (return))))

(fn `GetUUID`
  (returns (OutUUID :type String))
  (return (`self.UUID`)))

(fn `GetXRConnectionData`
  (returns (OutConnectionData :type "/XR_Toolkit/XR_Toolkit/Core/Scene/Persistence/FXRCore_ConnectionData Structure"))
  (bind _returnvalue (`Actor.GetComponentByClass` (`self.GetOwner`) "/Script/XR_Toolkit.XRConnectorComponent"))
  (bind (_outconnectedsocket _returnvalue_2) (`XRConnectorComponent.IsConnected` _returnvalue))
  (bind _returnvalue_3 (`Actor.GetComponentByClass` (`self.GetOwner` _outconnectedsocket) "BP_XRCore_PersistentObject_C"))
  (`/Engine/EditorBlueprintResources/StandardMacros.IsValid` _returnvalue
    (:`Is Valid`
      (if _returnvalue_2
        ;[1 1 1] Check if connected to a persistable Object
        (`/Engine/EditorBlueprintResources/StandardMacros.IsValid` _returnvalue_3
          (:`Is Valid`
            (return (make `/XR_Toolkit/XR_Toolkit/Core/Scene/Persistence/FXRCore_ConnectionData` true (`self.GetUUID` _returnvalue_3) (`XRConnectorSocket.GetSocketID` _outconnectedsocket))))
          (:`Is Not Valid`
            _))))
    (:`Is Not Valid`
      _))
  (return (make `/XR_Toolkit/XR_Toolkit/Core/Scene/Persistence/FXRCore_ConnectionData` false)))

(fn `Save Persistent Object`
  (bind _xrcore_persistence_manager (`self.XRCore Persistence Manager`)
    (:`then`
      (`/XR_Toolkit/XR_Toolkit/Core/Scene/Persistence/BP_XRCore_PersistenceManager.SavePersistentObject` _xrcore_persistence_manager (`self.Construct XRPersistent Object Data`)))
    (:`else`)))
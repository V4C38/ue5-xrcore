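; XR game mode that gives each player a pawn on login, based on whether a head-mounted display is enabled.
; With a headset, it spawns and possesses the MR or VR pawn class according to PassthrpoughMode, then destroys any previously controlled pawn.
; Without one, it possesses a third-person debug pawn instead.
; Spawn transforms come from randomly picked BP_XR_PlayerSpawnPoint actors in the level.
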(event `self.K2_PostLogin`
  (params (NewPlayer :type "PlayerController Object Reference"))
  (if (`HeadMountedDisplayFunctionLibrary.IsHeadMountedDisplayEnabled`)
    (`self.CreateAndPosess_XRPawn` NewPlayer (`self.Passthrpough Mode`))
    (else
      (`self.CreateAndPosess_Debug3PP Pawn` NewPlayer))))

(fn `CreateAndPosess_Debug3PP Pawn`
  (params (InPlayerController :type "PlayerController Object Reference"))
  (bind (_returnvalue_location _returnvalue_rotation) (`KismetMathLibrary.BreakTransform` (`self.GetTransform` (`self.GetRandomSpawnPoint`))))
  (bind _returnvalue (`|SpawnActorFromClass` "/XR_Toolkit/XR_Toolkit/Core/Base/BP_XRPawn_ThirdPerson.BP_XRPawn_ThirdPerson_C" (`KismetMathLibrary.MakeTransform` _returnvalue_location _returnvalue_rotation) "Undefined" "OverrideRootScale" InPlayerController null))
  (`Controller.Possess` InPlayerController _returnvalue))

(fn `CreateAndPosess_XRPawn`
  (params (InPlayerController :type "PlayerController Object Reference") (bInPassthrpoughMode :type Boolean))
  (locals (Loc_ExistomgControlledPawn :type "Pawn Object Reference"))
  (bind _returnvalue (`Controller.K2_GetPawn` InPlayerController))
  (bind _inplayercontroller (`local.InPlayerController`))
  (bind (_returnvalue_location _returnvalue_rotation) (`KismetMathLibrary.BreakTransform` (`self.GetTransform` (`self.GetRandomSpawnPoint`))))
  (bind _location (.location (`KismetMathLibrary.MakeTransform` _returnvalue_location _returnvalue_rotation)))
  (bind _rotation (.rotation (`KismetMathLibrary.MakeTransform` _returnvalue_location _returnvalue_rotation)))
  (`/Engine/EditorBlueprintResources/StandardMacros.IsValid` _returnvalue
    (:`Is Valid`
      (set `local.Loc_ExistomgControlledPawn` _returnvalue))
    (:`Is Not Valid`
      _))
  (if (`HeadMountedDisplayFunctionLibrary.IsHeadMountedDisplayEnabled`)
    (if (`local.bInPassthrpoughMode`)
      (bind _returnvalue_2 (`|SpawnActorFromClass` (`self.MRPawnClass`) (`KismetMathLibrary.MakeTransform` _location _rotation) "Undefined" "OverrideRootScale" _inplayercontroller null))
      (`Controller.Possess` (`local.InPlayerController`) _returnvalue_2)
      (else
        (bind _returnvalue_3 (`|SpawnActorFromClass` (`self.VRPawnClass`) (`KismetMathLibrary.MakeTransform` _location _rotation) "Undefined" "OverrideRootScale" _inplayercontroller null))
        (`Controller.Possess` (`local.InPlayerController`) _returnvalue_3)))
    (bind _loc_existomgcontrolledpawn (`local.Loc_ExistomgControlledPawn`)
      (:`then`
        (`self.K2_DestroyActor` _loc_existomgcontrolledpawn))
      (:`else`))))

(fn `GetRandomSpawnPoint`
  (returns (Output :type "/XR_Toolkit/XR_Toolkit/Core/Base/BP_XR_PlayerSpawnPoint Object Reference"))
  (bind _outactors (`GameplayStatics.GetAllActorsOfClass` "/XR_Toolkit/XR_Toolkit/Core/Base/BP_XR_PlayerSpawnPoint.BP_XR_PlayerSpawnPoint_C"))
  (return (`|GetArrayItem` _outactors (`KismetMathLibrary.RandomInteger` (`KismetArrayLibrary.Array_Length` _outactors)))))

(fn `UserConstructionScript`)
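; BP_XRHand is a replicated XR hand actor that turns per-hand controller input into interactions and animated hand poses.
; Deadzone-gated primary input starts an XRInteractor interaction or falls back to the laser; secondary input triggers follow-up interactions while primary is held.
; The interactor smoothly follows the thumb-index midpoint, and trigger and grip values drive the hand AnimBP.
; The local owner sends transform and pose to the server each tick; non-local instances interpolate toward that data.
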(event `EnhancedInput|/XR_Toolkit/XR_Toolkit/Core/Input/InputAction_XR_Primary_Touched_L`
  (params (ActionValue :type "Float (double-precision)") (ElapsedSeconds :type "Float (double-precision)") (TriggeredSeconds :type "Float (double-precision)") (InputAction :type "InputAction Object Reference" :default "/XR_Toolkit/XR_Toolkit/Core/Input/InputAction_XR_Primary_Touched_L.InputAction_XR_Primary_Touched_L"))
  ;[0 0 0] Input
  (:`Triggered`
    (`self.IsValidInput` "Left" :!label _label
      (:`true`
        (`self.Input Set Controller Value Trigger Touched` ActionValue))))
  (:`Started`
    (goto _label))
  (:`Canceled`
    (`self.IsValidInput` "Left" :!label _label_2
      (:`true`
        (`self.Input Set Controller Value Trigger Touched` 0.0))))
  (:`Completed`
    (goto _label_2)))

(event `EnhancedInput|/XR_Toolkit/XR_Toolkit/Core/Input/InputAction_XR_Primary_Touched_R`
  (params (ActionValue :type "Float (double-precision)") (ElapsedSeconds :type "Float (double-precision)") (TriggeredSeconds :type "Float (double-precision)") (InputAction :type "InputAction Object Reference" :default "/XR_Toolkit/XR_Toolkit/Core/Input/InputAction_XR_Primary_Touched_R.InputAction_XR_Primary_Touched_R"))
  ;[0 0 0] Input
  (:`Triggered`
    (`self.IsValidInput` "Right" :!label _label_3
      (:`true`
        (`self.Input Set Controller Value Trigger Touched` ActionValue))))
  (:`Started`
    (goto _label_3))
  (:`Canceled`
    (`self.IsValidInput` "Right" :!label _label_4
      (:`true`
        (`self.Input Set Controller Value Trigger Touched` 0.0))))
  (:`Completed`
    (goto _label_4)))

(event `EnhancedInput|/XR_Toolkit/XR_Toolkit/Core/Input/InputAction_XR_Primary_R`
  (params (ActionValue :type "Float (double-precision)") (ElapsedSeconds :type "Float (double-precision)") (TriggeredSeconds :type "Float (double-precision)") (InputAction :type "InputAction Object Reference" :default "/XR_Toolkit/XR_Toolkit/Core/Input/InputAction_XR_Primary_R.InputAction_XR_Primary_R"))
  ;[0 0 0] Input
  (:`Triggered`
    (`self.IsValidInput` "Right"
      (:`true`
        (`self.PrimaryInput_Triggered` ActionValue))))
  (:`Canceled`
    (`self.IsValidInput` "Right" :!label _label_5
      (:`true`
        (`self.PrimaryInput_Triggered` 0.0))))
  (:`Completed`
    (goto _label_5)))

(event `EnhancedInput|/XR_Toolkit/XR_Toolkit/Core/Input/InputAction_XR_Primary_L`
  (params (ActionValue :type "Float (double-precision)") (ElapsedSeconds :type "Float (double-precision)") (TriggeredSeconds :type "Float (double-precision)") (InputAction :type "InputAction Object Reference" :default "/XR_Toolkit/XR_Toolkit/Core/Input/InputAction_XR_Primary_L.InputAction_XR_Primary_L"))
  ;[0 0 0] Input
  (:`Triggered`
    (`self.IsValidInput` "Left"
      (:`true`
        (`self.PrimaryInput_Triggered` ActionValue))))
  (:`Canceled`
    (`self.IsValidInput` "Left" :!label _label_6
      (:`true`
        (`self.PrimaryInput_Triggered` 0.0))))
  (:`Completed`
    (goto _label_6)))

(event `EnhancedInput|/XR_Toolkit/XR_Toolkit/Core/Input/InputAction_XR_Secondary_L`
  (params (ActionValue :type "Float (double-precision)") (ElapsedSeconds :type "Float (double-precision)") (TriggeredSeconds :type "Float (double-precision)") (InputAction :type "InputAction Object Reference" :default "/XR_Toolkit/XR_Toolkit/Core/Input/InputAction_XR_Secondary_L.InputAction_XR_Secondary_L"))
  ;[0 0 0] Input
  (:`Triggered`
    (`self.IsValidInput` "Left"
      (:`true`
        (`self.SecondaryInput_Triggered` ActionValue))))
  (:`Canceled`
    (`self.IsValidInput` "Left" :!label _label_7
      (:`true`
        (`self.SecondaryInput_Triggered` 0.0))))
  (:`Completed`
    (goto _label_7)))

(event `EnhancedInput|/XR_Toolkit/XR_Toolkit/Core/Input/InputAction_XR_Secondary_R`
  (params (ActionValue :type "Float (double-precision)") (ElapsedSeconds :type "Float (double-precision)") (TriggeredSeconds :type "Float (double-precision)") (InputAction :type "InputAction Object Reference" :default "/XR_Toolkit/XR_Toolkit/Core/Input/InputAction_XR_Secondary_R.InputAction_XR_Secondary_R"))
  ;[0 0 0] Input
  (:`Triggered`
    (`self.IsValidInput` "Right"
      (:`true`
        (`self.SecondaryInput_Triggered` ActionValue))))
  (:`Canceled`
    (`self.IsValidInput` "Right" :!label _label_8
      (:`true`
        (`self.SecondaryInput_Triggered` 0.0))))
  (:`Completed`
    (goto _label_8)))

(event `self.ReceiveBeginPlay`
  (bind _bp_handtrackingsystemcomponent (`self.BP_HandTrackingSystemComponent`))
  ;[1 1 1] Init
  (bind _aspawn (cast `Pawn` (`self.GetOwner`)))
  (set `self.OwningPawn` _aspawn)
  (`|ExecutionSequence`
    (:`then_0`
      (set `self.bIsLocallyControlled` (`Pawn.IsLocallyControlled` (`self.OwningPawn`))))
    (:`then_1`
      (`XRInteractorComponent.SetPhysicsConstraint` (`self.XRInteractor`) (`self.XRInteractor_PhysicsConstraint`))
      (`XRInteractorComponent.SetAdditionalColliders` (`self.XRInteractor`) (`|MakeArray` (`self.Sphere_Center`) (`self.Sphere_Thumb`) :!type "PrimitiveComponent Object Reference")))
    (:`then_2`
      (set `/XR_Toolkit/XR_Toolkit/Core/Laser/BP_XRLaserComponent.XRController Hand` (`self.ControllerHand`) (`self.BP_XRLaserComponent`)))
    (:`then_3`
      (bind _asabp_xrcore_hand (cast `/XR_Toolkit/XR_Toolkit/Assets/Meshes/HandModel/ABP_XRCoreHand` (`SkeletalMeshComponent.GetAnimInstance` (`self.SK_Hand`))))
      (set `self.ABP XRCore Hand` _asabp_xrcore_hand))
    (:`then_4`
      (`/XR_Toolkit/XR_Toolkit/Core/Hands/HandTracking/BP_HandTrackingSystemComponent.SetControllerHand` _bp_handtrackingsystemcomponent (`self.ControllerHand`))
      (`/XR_Toolkit/XR_Toolkit/Core/Hands/HandTracking/BP_HandTrackingSystemComponent.AssignAnimBP` _bp_handtrackingsystemcomponent (`self.ABP XRCore Hand`)))))

(event `self.ReceiveTick`
  (params (DeltaSeconds :type "Float (single-precision)"))
  (bind _returnvalue (`GameplayStatics.GetWorldDeltaSeconds`))
  (bind (_returnvalue_location _returnvalue_rotation) (`KismetMathLibrary.BreakTransform` (`self.GetTransform`)))
  (bind _replicationsmoothingspeed (`self.ReplicationSmoothingSpeed`))
  (bind _modifiedroot (`self.ModifiedRoot`))
  (bind (_latestreplicationdata_location_worldspace _latestreplicationdata_rotation_worldspace) (break `/XR_Toolkit/XR_Toolkit/Core/Hands/F_XRHand_ReplicationData` (`self.LatestReplicationData`)))
  (`|ExecutionSequence`
    (:`then_0`
      (`self.UpdateInteractionRoot`))
    (:`then_1`
      (`self.InterpolateXRInteractorTransform`))
    (:`then_2`
      (if (`self.bIsLocallyControlled`)
        ;[1 1 1] Sending Client
        (set `self.ElapsedTimeSinceReplication` DeltaSeconds)
        (bind _motioncontrollerdata (`HeadMountedDisplayFunctionLibrary.GetMotionControllerData` self (`self.ControllerHand`)))
        (if (`.bValid` (break `XRMotionControllerData` _motioncontrollerdata))
          (`self.Server_SetReplicationData` (make `/XR_Toolkit/XR_Toolkit/Core/Hands/F_XRHand_ReplicationData` (`SceneComponent.K2_GetComponentLocation` _modifiedroot) (`SceneComponent.K2_GetComponentRotation` _modifiedroot) (make `/XR_Toolkit/XR_Toolkit/Core/Hands/F_XRHand_HandPoseReplicationData` (`self.Local_TriggerAxis`) (`self.Local_TriggerTouch`) (`self.Local_GripAxis`)))))
        (else
          ;[1 1 1] Receivers
          (`|ExecutionSequence`
            (:`then_0`
              (`SceneComponent.K2_SetWorldLocationAndRotation` (`self.ModifiedRoot`) (`KismetMathLibrary.VInterpTo` _returnvalue_location _latestreplicationdata_location_worldspace _returnvalue _replicationsmoothingspeed) (`KismetMathLibrary.RInterpTo` _returnvalue_rotation _latestreplicationdata_rotation_worldspace _returnvalue _replicationsmoothingspeed) false false))
            (:`then_1`
              (`self.Update Hand Pose`))))))))

(event `Server_SetReplicationData`
  (params (InReplicationData :type "/XR_Toolkit/XR_Toolkit/Core/Hands/F_XRHand_ReplicationData Structure"))
  ;[0 0 0] RPC
  (set `self.LatestReplicationData` InReplicationData))

(fn `GetControllerHand`
  (returns (OutControllerHand :type "EControllerHand Enum"))
  (return (`self.ControllerHand`)))

(fn `Input Set Controller Value Grip`
  (params (InAxisValue :type "Float (double-precision)"))
  (set `self.Local_GripAxis` InAxisValue)
  (bind _abp_xrcore_hand (`self.ABP XRCore Hand`)
    (:`then`
      (`/XR_Toolkit/XR_Toolkit/Assets/Meshes/HandModel/ABP_XRCoreHand.Set ControllerValue_Grip` _abp_xrcore_hand InAxisValue))
    (:`else`)))

(fn `Input Set Controller Value Trigger`
  (params (InAxisValue :type "Float (double-precision)"))
  (set `self.Local_TriggerAxis` InAxisValue)
  (bind _abp_xrcore_hand (`self.ABP XRCore Hand`)
    (:`then`
      (`/XR_Toolkit/XR_Toolkit/Assets/Meshes/HandModel/ABP_XRCoreHand.Set ControllerValue_Trigger` _abp_xrcore_hand InAxisValue))
    (:`else`)))

(fn `Input Set Controller Value Trigger Touched`
  (params (Local_TriggerTouch :type "Float (double-precision)"))
  (bind _abp_xrcore_hand (`self.ABP XRCore Hand`)
    (:`then`
      (set `/XR_Toolkit/XR_Toolkit/Assets/Meshes/HandModel/ABP_XRCoreHand.Input_Trigger_Touch` Local_TriggerTouch _abp_xrcore_hand))
    (:`else`)))

(fn `InterpolateXRInteractorTransform`
  (bind _returnvalue (`GameplayStatics.GetWorldDeltaSeconds`))
  (bind _xrinteractor (`self.XRInteractor`))
  (bind _xrinteractorroot (`self.XRInteractorRoot`))
  (`SceneComponent.K2_SetWorldLocationAndRotation` (`self.XRInteractor`) (`KismetMathLibrary.VInterpTo` (`SceneComponent.K2_GetComponentLocation` _xrinteractor) (`SceneComponent.K2_GetComponentLocation` _xrinteractorroot) _returnvalue 30.0) (`KismetMathLibrary.RInterpTo` (`SceneComponent.K2_GetComponentRotation` _xrinteractor) (`SceneComponent.K2_GetComponentRotation` _xrinteractorroot) _returnvalue 7.0) false false))

(fn `PrimaryInput_End`
  (`|ExecutionSequence`
    (:`then_0`
      (set `self.bCurrentPrimaryInput` false))
    (:`then_1`
      ;[1 1 1] Handle Interactions
      (if (`/XR_Toolkit/XR_Toolkit/Core/Laser/BP_XRLaserComponent.IsLaserActive` (`self.BP_XRLaserComponent`))
        (`/XR_Toolkit/XR_Toolkit/Core/Laser/BP_XRLaserComponent.Server_DisableLaser` (`self.BP_XRLaserComponent`))
        (else
          (`XRInteractorComponent.StopAllXRInteractions` (`self.XRInteractor`)))))
    (:`then_2`
      ;[1 1 1] HandPose
      (set `self.Local_TriggerAxis` 0.0)
      (bind _abp_xrcore_hand (`self.ABP XRCore Hand`)
        (:`then`
          (`/XR_Toolkit/XR_Toolkit/Assets/Meshes/HandModel/ABP_XRCoreHand.Set ControllerValue_Trigger` _abp_xrcore_hand 0.0))
        (:`else`)))))

(fn `PrimaryInput_Triggered`
  (params (InAxisValue :type "Float (double-precision)"))
  (bind _inaxisvalue (`local.InAxisValue`))
  (bind _xrinteractor (`self.XRInteractor`))
  (`|ExecutionSequence`
    (:`then_0`
      (`self.UpdateInteractionRoot`))
    (:`then_1`
      ;[1 1 1] AxisValue Deadzone gate
      (if (`self.bCurrentPrimaryInput`)
        (if (not (> (`local.InAxisValue`) (- (`self.InputAxisDeadzone`) 0.1)))
          (set `self.bCurrentPrimaryInput` false)
          ;[1 1 1] End Interactions
          (if (`/XR_Toolkit/XR_Toolkit/Core/Laser/BP_XRLaserComponent.IsLaserActive` (`self.BP_XRLaserComponent`))
            (`/XR_Toolkit/XR_Toolkit/Core/Laser/BP_XRLaserComponent.Server_DisableLaser` (`self.BP_XRLaserComponent`))
            (else
              (`XRInteractorComponent.StopAllXRInteractions` (`self.XRInteractor`)))))
        (elif (> (`local.InAxisValue`) (`self.InputAxisDeadzone`))
          (set `self.bCurrentPrimaryInput` true)
          ;[1 1 1] Start Interactions
          ; Laser or Interact
          (if (`/XR_Toolkit/XR_Toolkit/Core/Laser/BP_XRLaserComponent.IsLaserActive` (`self.BP_XRLaserComponent`))
            (`XRInteractorComponent.StartXRInteractionByPriority` (`self.XRInteractor`) 1 "LowerEqual" :!label _label)
            (elif (or (`.ReturnValue` (`XRInteractorComponent.CanInteract` _xrinteractor null 0 "LowerEqual")) (`XRInteractorComponent.IsInteracting` _xrinteractor))
              (goto _label)
              (else
                (`/XR_Toolkit/XR_Toolkit/Core/Laser/BP_XRLaserComponent.Server_EnableLaser` (`self.BP_XRLaserComponent`))))))))
    (:`then_2`
      ;[1 1 1] HandPose
      (set `self.Local_TriggerAxis` _inaxisvalue)
      (bind _abp_xrcore_hand (`self.ABP XRCore Hand`)
        (:`then`
          (`/XR_Toolkit/XR_Toolkit/Assets/Meshes/HandModel/ABP_XRCoreHand.Set ControllerValue_Trigger` _abp_xrcore_hand _inaxisvalue))
        (:`else`)))))

(fn `SecondaryInput_End`
  (bind _xrinteractor (`/XR_Toolkit/XR_Toolkit/Core/Laser/BP_XRLaserComponent.GetXRInteractor` (`self.BP_XRLaserComponent`)))
  (`|ExecutionSequence`
    (:`then_0`
      (set `self.bCurrentSecondaryInput` false))
    (:`then_1`
      ;[1 1 1] Handle Interactions
      (if (`/XR_Toolkit/XR_Toolkit/Core/Laser/BP_XRLaserComponent.IsLaserActive` (`self.BP_XRLaserComponent`))
        (`/Engine/EditorBlueprintResources/StandardMacros.IsValid` _xrinteractor
          (:`Is Valid`
            (`XRInteractorComponent.StopAllXRInteractions` _xrinteractor)))
        (else
          (`XRInteractorComponent.StopXRInteractionByPriority` (`self.XRInteractor`) 2 "Equal"))))
    (:`then_2`
      ;[1 1 1] HandPose
      (set `self.Local_GripAxis` 0.0)
      (bind _abp_xrcore_hand (`self.ABP XRCore Hand`)
        (:`then`
          (`/XR_Toolkit/XR_Toolkit/Assets/Meshes/HandModel/ABP_XRCoreHand.Set ControllerValue_Grip` _abp_xrcore_hand 0.0))
        (:`else`)))))

(fn `SecondaryInput_Triggered`
  (params (InAxisValue :type "Float (double-precision)"))
  (bind _inaxisvalue (`local.InAxisValue`))
  (bind _xrinteractor (`/XR_Toolkit/XR_Toolkit/Core/Laser/BP_XRLaserComponent.GetXRInteractor` (`self.BP_XRLaserComponent`)))
  (bind _xrinteractor_2 (`/XR_Toolkit/XR_Toolkit/Core/Laser/BP_XRLaserComponent.GetXRInteractor` (`self.BP_XRLaserComponent`)))
  (bind _returnvalue (> (`local.InAxisValue`) (/ (`self.InputAxisDeadzone`) 2.0)))
  (`|ExecutionSequence`
    (:`then_0`
      ;[1 1 1] AxisValue Deadzone gate
      (if (`self.bCurrentSecondaryInput`)
        (if (not _returnvalue)
          (set `self.bCurrentSecondaryInput` false)
          ;[1 1 1] Stop Interactions
          (if (`/XR_Toolkit/XR_Toolkit/Core/Laser/BP_XRLaserComponent.IsLaserActive` (`self.BP_XRLaserComponent`))
            (`/Engine/EditorBlueprintResources/StandardMacros.IsValid` _xrinteractor_2
              (:`Is Valid`
                (`XRInteractorComponent.StopAllXRInteractions` _xrinteractor_2)))
            (else
              (`XRInteractorComponent.StopXRInteractionByPriority` (`self.XRInteractor`) 2 "LowerEqual"))))
        (elif _returnvalue
          (set `self.bCurrentSecondaryInput` true)
          ;[1 1 1] Interactions
          ; Start Next Interaction
          (if (`self.bCurrentPrimaryInput`)
            (if (`/XR_Toolkit/XR_Toolkit/Core/Laser/BP_XRLaserComponent.IsLaserActive` (`self.BP_XRLaserComponent`))
              (`/Engine/EditorBlueprintResources/StandardMacros.IsValid` _xrinteractor
                (:`Is Valid`
                  (`XRInteractorComponent.StartXRInteractionByPriority` _xrinteractor 1 "LowerEqual")))
              (else
                (`XRInteractorComponent.StartXRInteractionByPriority` (`self.XRInteractor`) 2 "LowerEqual")))))))
    (:`then_1`
      ;[1 1 1] HandPose
      (set `self.Local_GripAxis` _inaxisvalue)
      (bind _abp_xrcore_hand (`self.ABP XRCore Hand`)
        (:`then`
          (`/XR_Toolkit/XR_Toolkit/Assets/Meshes/HandModel/ABP_XRCoreHand.Set ControllerValue_Grip` _abp_xrcore_hand _inaxisvalue))
        (:`else`)))))

(fn `SetControllerHand`
  (params (ControllerHand :type "EControllerHand Enum" :default "Left"))
  (set `self.ControllerHand` ControllerHand))

(fn `ShouldReplicate`
  (params (InDeltaTime :type "Float (double-precision)"))
  (returns (OutShouldReplicate :type Boolean)))

(fn `Update Hand Pose`
  (bind _returnvalue (`GameplayStatics.GetWorldDeltaSeconds`))
  (bind (_triggeraxis _triggertouched _gripaxis) (break `/XR_Toolkit/XR_Toolkit/Core/Hands/F_XRHand_HandPoseReplicationData` (`.HandPoseAxis_11_0280A96848F6A398B1E653B05B765F49` (break `/XR_Toolkit/XR_Toolkit/Core/Hands/F_XRHand_ReplicationData` (`self.LatestReplicationData`)))))
  (`|ExecutionSequence`
    (:`then_0`
      (`self.Input Set Controller Value Trigger` (`KismetMathLibrary.FInterpTo` (`self.Local_TriggerAxis`) _triggeraxis _returnvalue 1.0)))
    (:`then_1`
      (`self.Input Set Controller Value Grip` (`KismetMathLibrary.FInterpTo` (`self.Local_GripAxis`) _gripaxis _returnvalue 1.0)))
    (:`then_2`
      (`/XR_Toolkit/XR_Toolkit/Assets/Meshes/HandModel/ABP_XRCoreHand.Set ControllerValue_Trigger_Touched` (`self.ABP XRCore Hand`) (`KismetMathLibrary.FInterpTo` (`self.Local_TriggerTouch`) _triggertouched _returnvalue 1.0)))))

(fn `UpdateInteractionRoot`
  (bind _sk_hand (`self.SK_Hand`))
  (`|ExecutionSequence`
    (:`then_0`
      (`SceneComponent.K2_SetWorldLocation` (`self.XRInteractorRoot`) (/ (+ (`SceneComponent.GetSocketLocation` _sk_hand "b_l_thumb_nullSocket") (`SceneComponent.GetSocketLocation` _sk_hand "b_l_index_nullSocket")) 2.0) false false))
    (:`then_1`
      (`SceneComponent.SetVisibility` (`self.RootSphere`) (`self.bCurrentPrimaryInput`) false))))

(fn `UserConstructionScript`
  (`|ExecutionSequence`
    (:`then_0`
      (`SceneComponent.SetHiddenInGame` (`self.Arrow1`) (not (`self.bDebugMode`)) false)
      (`SceneComponent.SetHiddenInGame` (`self.Arrow`) (not (`self.bDebugMode`)) false)
      (`SceneComponent.SetHiddenInGame` (`self.XRInteractor`) (not (`self.bDebugMode`)) false))
    (:`then_1`
      (`SceneComponent.K2_SetRelativeTransform` (`self.ModifiedRoot`) (select `EXRStandard` (`XRToolsUtilityFunctions.GetXRStandard`) :`OpenXR` (`KismetMathLibrary.MakeTransform` (0.0 0.0 0.0)) :`MetaXR` (`KismetMathLibrary.MakeTransform` (-3.0 0.0 -5.0) (struct :`Pitch` 75.0))) false false))
    (:`then_2`
      (`SceneComponent.SetWorldScale3D` (`self.ModifiedRoot`) (`KismetMathLibrary.MakeVector` 1.0 (select `byte` (`/XR_Toolkit/XR_Toolkit/Core/Utilities/FL_XRUtilityFunctions.ReduceControllerHandEnum` (`self.ControllerHand`)) :`0` 1.0 :`1` -1.0 :`2` 0.0) 1.0)))))
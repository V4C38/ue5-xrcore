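; Hand gesture classifier component for XR hand tracking, meant to recognize fist, pinch, pinch-fist and flat open poses.
; Its detection logic compares fingertip and bone distances to thresholds, plus hand orientation for the flat pose, and announces pose changes.
; That logic is disconnected: Tick does nothing, the pose check returns a default, and initialization clears the Oculus hand reference.
; Only tick toggling and the current pose getter remain live.
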(event `self.ReceiveTick`
  (params (DeltaSeconds :type "Float (single-precision)")))

(fn `CheckBoneDistance`
  (params (Bone1 :type Byte :default 0) (Bone2 :type Byte :default 0) (DistanceTreshold :type "Float (double-precision)"))
  (returns (TreshholdReached :type Boolean)))

(fn `CheckForValidHandPose`
  (returns (Result_HandPose :type Byte))
  (locals (Local_HandPose_Current :type Byte :default 0))
  (return 0))

(fn `GetCurrentHandPose`
  (returns (CurrentHandPose :type Byte))
  (return (`self.CurrentHandPose`)))

(fn `InitializeComponent`
  (params (OculusHand_Component :type "Object Object Reference") (bEnabled :type Boolean))
  (set `self.OculusHand_Component` null)
  (`self.SetComponentEnabled` bEnabled))

(fn `SetComponentEnabled`
  (params (bEnabled :type Boolean))
  (`self.SetComponentTickEnabled` bEnabled))
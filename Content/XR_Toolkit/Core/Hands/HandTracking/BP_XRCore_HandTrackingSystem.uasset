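; Hand tracking component for BP_XRHand that turns finger pinches into simulated controller input.
; Each tick it caches hand keypoints when tracking data exists, then fires the hand's primary and secondary inputs from two thumb-to-index distance thresholds.
; It derives an interaction root at the thumb-index tip midpoint, aimed from the index root.
; In debug mode, an attached billboard shows thumb-to-index and thumb-to-middle distances.
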(event `self.ReceiveBeginPlay`
  (`|ExecutionSequence`
    (:`then_0`
      (bind _asbp_xrhand (cast `/XR_Toolkit/XR_Toolkit/Core/Hands/BP_XRHand` (`self.GetOwner`)))
      (set `self.OwningXRHand` _asbp_xrhand))
    (:`then_1`
      (`self.SetupDebugMode`))))

(event `self.ReceiveTick`
  (params (DeltaSeconds :type "Float (single-precision)"))
  (bind _owningxrhand (`self.OwningXRHand`)
    (:`then`
      (bind _motioncontrollerdata (`HeadMountedDisplayFunctionLibrary.GetMotionControllerData` _owningxrhand (`/XR_Toolkit/XR_Toolkit/Core/Hands/BP_XRHand.GetControllerHand` _owningxrhand)))
      (bind _output_get (set `self.bIsHandTracking` (> (`KismetArrayLibrary.Array_Length` (`.HandKeyPositions` (break `XRMotionControllerData` _motioncontrollerdata))) 0)))
      (if _output_get
        (set `self.Location_ThumbTip` (`|GetArrayItem` (`.HandKeyPositions` (break `XRMotionControllerData` _motioncontrollerdata)) 5))
        (set `self.Location_IndexRoot` (`|GetArrayItem` (`.HandKeyPositions` (break `XRMotionControllerData` _motioncontrollerdata)) 6))
        (set `self.Location_IndexTip` (`|GetArrayItem` (`.HandKeyPositions` (break `XRMotionControllerData` _motioncontrollerdata)) 10))
        (set `self.Location_MiddleTip` (`|GetArrayItem` (`.HandKeyPositions` (break `XRMotionControllerData` _motioncontrollerdata)) 15))
        (set `self.Rotation_Wrist` (`KismetMathLibrary.Quat_Rotator` (`|GetArrayItem` (`.HandKeyRotations` (break `XRMotionControllerData` _motioncontrollerdata)) 1)))
        (`|ExecutionSequence`
          (:`then_0`
            (`self.ResolveInput`))
          (:`then_1`
            (`self.UpdateDebug`)))))
    (:`else`)))

(fn `AssignAnimBP`
  (params (`InABP XRCore Hand` :type "/XR_Toolkit/XR_Toolkit/Assets/Meshes/HandModel/ABP_XRCoreHand Object Reference"))
  (set `self.Assigned ABP XRCore Hand` `InABP XRCore Hand`))

(fn `GetInteractionRootLocation`
  (returns (OutLocation :type "Vector Structure"))
  (return (* (+ (`self.Location_ThumbTip`) (`self.Location_IndexTip`)) 0.5)))

(fn `GetInteractionRootRotation`
  (returns (OutRotation :type "Rotator Structure"))
  (return (`KismetMathLibrary.FindLookAtRotation` (`self.Location_IndexRoot`) (`self.GetInteractionRootLocation`))))

(fn `ResolveInput`
  (bind _distance_thumbindex (`self.Distance_ThumbIndex`))
  (bind _owningxrhand (`self.OwningXRHand`))
  (bind _owningxrhand_2 (`self.OwningXRHand`))
  (set `self.Distance_ThumbIndex` (`KismetMathLibrary.Vector_Distance` (`self.Location_IndexTip`) (`self.Location_ThumbTip`)))
  (set `self.Distance_ThumbMiddle` (`KismetMathLibrary.Vector_Distance` (`self.Location_MiddleTip`) (`self.Location_ThumbTip`)))
  ;[1 1 1] Simulate Input
  (if (< _distance_thumbindex 5.0)
    (`/XR_Toolkit/XR_Toolkit/Core/Hands/BP_XRHand.PrimaryInput_Triggered` _owningxrhand_2 1.0)
    (else
      (`/XR_Toolkit/XR_Toolkit/Core/Hands/BP_XRHand.PrimaryInput_Triggered` _owningxrhand_2 0.0)))
  (if (< _distance_thumbindex 2.0)
    (`/XR_Toolkit/XR_Toolkit/Core/Hands/BP_XRHand.SecondaryInput_Triggered` _owningxrhand 1.0)
    (else
      (`/XR_Toolkit/XR_Toolkit/Core/Hands/BP_XRHand.SecondaryInput_Triggered` _owningxrhand 0.0))))

(fn `SetControllerHand`
  (params (InControllerHand :type "EControllerHand Enum" :default "Left"))
  (`|ExecutionSequence`
    (:`then_0`
      (set `self.ControllerHand` InControllerHand))
    (:`then_1`
      (`self.SetComponentTickEnabled` true))
    (:`then_2`
      (switch `EControllerHand` InControllerHand
        (:`Right`
          (bind _bp_debughelper (`self.BP_DebugHelper`)
            (:`then`
              (`Actor.SetActorScale3D` _bp_debughelper (-1.0 1.0 1.0))
              (`SceneComponent.K2_SetRelativeLocation` (`/XR_Toolkit/XR_Toolkit/Core/Hands/HandTracking/BP_DEBUG_StringBillboard.TextRoot` _bp_debughelper) (-1.5 0.0 0.0) false false))
            (:`else`)))))))

(fn `SetupDebugMode`
  (bind _owningxrhand (`self.OwningXRHand`)
    (:`then`
      (if (`/XR_Toolkit/XR_Toolkit/Core/Hands/BP_XRHand.bDebugMode` _owningxrhand)
        (bind _returnvalue (`|SpawnActorFromClass` "/XR_Toolkit/XR_Toolkit/Core/Hands/HandTracking/BP_DEBUG_StringBillboard.BP_DEBUG_StringBillboard_C" (`KismetMathLibrary.MakeTransform` (0.0 0.0 0.0)) "Undefined" "MultiplyWithRoot" (`self.GetOwner`) null))
        (bind _output_get (set `self.BP_DebugHelper` _returnvalue))
        (`Actor.K2_AttachToComponent` _output_get (`/XR_Toolkit/XR_Toolkit/Core/Hands/BP_XRHand.XRInteractorRoot` (`self.OwningXRHand`)) "None" "SnapToTarget" "SnapToTarget" "KeepWorld" true)))
    (:`else`)))

(fn `UpdateDebug`
  ;[1 1 1] DEBUG
  (bind _bp_debughelper (`self.BP_DebugHelper`)
    (:`then`
      (`/XR_Toolkit/XR_Toolkit/Core/Hands/HandTracking/BP_DEBUG_StringBillboard.UpdateText` _bp_debughelper (`KismetStringLibrary.Concat_StrStr` "Distance Index" " " (`KismetStringLibrary.Conv_DoubleToString` (`self.Distance_ThumbIndex`))) (`KismetStringLibrary.Concat_StrStr` "Distance Middle" " " (`KismetStringLibrary.Conv_DoubleToString` (`self.Distance_ThumbMiddle`))) ""))
    (:`else`)))
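; World-space annotation actor for the XR Toolkit that displays a title and subtitle beside an owning component, facing the player camera.
; Title, background and subtitle widgets receive the text and show/hide messages, with text applied on BeginPlay.
; Show snaps the actor to the component plus an offset and enables tick; Hide disables tick.
; When dynamic, Tick follows and re-faces the camera, interpolated by FollowSpeed or snapping if zero.
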(event `self.ReceiveBeginPlay`
  (`self.CacheAndConfigureWidget`)
  (if (not (`self.bInitiallyVisible`))
    (`/XR_Toolkit/XR_Toolkit/Core/Utilities/XRAnnotation/BPI_XRCoreUI.Hide`)))

(event `/XR_Toolkit/XR_Toolkit/Core/Utilities/XRAnnotation/BPI_XRCoreUI.Show`
  ;[0 0 0] Show
  (`self.K2_SetActorLocationAndRotation` (+ (`SceneComponent.K2_GetComponentLocation` (`self.OwningComponent`)) (`self.Offset`)) (`KismetMathLibrary.FindLookAtRotation` (`self.K2_GetActorLocation`) (`PlayerCameraManager.GetCameraLocation` (`GameplayStatics.GetPlayerCameraManager` 0))))
  (`|ExecutionSequence`
    (:`then_0`
      (`self.SetActorTickEnabled` true))
    (:`then_1`
      (message `/XR_Toolkit/XR_Toolkit/Core/Utilities/XRAnnotation/BPI_XRCoreUI.Show` (`WidgetComponent.GetUserWidgetObject` (`self.Widget_Title`)))
      (message `/XR_Toolkit/XR_Toolkit/Core/Utilities/XRAnnotation/BPI_XRCoreUI.Show` (`WidgetComponent.GetUserWidgetObject` (`self.Widget_Background`)))
      (message `/XR_Toolkit/XR_Toolkit/Core/Utilities/XRAnnotation/BPI_XRCoreUI.Show` (`WidgetComponent.GetUserWidgetObject` (`self.Widget_Subtitle`))))))

(event `/XR_Toolkit/XR_Toolkit/Core/Utilities/XRAnnotation/BPI_XRCoreUI.SetTitle`
  (params (InTitle :type Text))
  (message `/XR_Toolkit/XR_Toolkit/Core/Utilities/XRAnnotation/BPI_XRCoreUI.SetTitle` (`WidgetComponent.GetUserWidgetObject` (`self.Widget_Title`)) InTitle)
  (message `/XR_Toolkit/XR_Toolkit/Core/Utilities/XRAnnotation/BPI_XRCoreUI.SetTitle` (`WidgetComponent.GetUserWidgetObject` (`self.Widget_Background`)) InTitle))

(event `/XR_Toolkit/XR_Toolkit/Core/Utilities/XRAnnotation/BPI_XRCoreUI.Hide`
  ;[0 0 0] Hide
  (message `/XR_Toolkit/XR_Toolkit/Core/Utilities/XRAnnotation/BPI_XRCoreUI.Hide` (`WidgetComponent.GetUserWidgetObject` (`self.Widget_Title`)))
  (message `/XR_Toolkit/XR_Toolkit/Core/Utilities/XRAnnotation/BPI_XRCoreUI.Hide` (`WidgetComponent.GetUserWidgetObject` (`self.Widget_Background`)))
  (message `/XR_Toolkit/XR_Toolkit/Core/Utilities/XRAnnotation/BPI_XRCoreUI.Hide` (`WidgetComponent.GetUserWidgetObject` (`self.Widget_Subtitle`)))
  (`self.SetActorTickEnabled` false))

(event `/XR_Toolkit/XR_Toolkit/Core/Utilities/XRAnnotation/BPI_XRCoreUI.SetSubtitle`
  (params (InSubtitle :type Text))
  (message `/XR_Toolkit/XR_Toolkit/Core/Utilities/XRAnnotation/BPI_XRCoreUI.SetSubtitle` (`WidgetComponent.GetUserWidgetObject` (`self.Widget_Title`)) InSubtitle)
  (message `/XR_Toolkit/XR_Toolkit/Core/Utilities/XRAnnotation/BPI_XRCoreUI.SetSubtitle` (`WidgetComponent.GetUserWidgetObject` (`self.Widget_Subtitle`)) InSubtitle))

(event `self.ReceiveTick`
  (params (DeltaSeconds :type "Float (single-precision)"))
  (bind _returnvalue (> (`self.FollowSpeed`) 0.0))
  (bind _returnvalue_2 (`KismetMathLibrary.FindLookAtRotation` (`self.K2_GetActorLocation`) (`PlayerCameraManager.GetCameraLocation` (`GameplayStatics.GetPlayerCameraManager` 0))))
  (bind _returnvalue_3 (+ (`SceneComponent.K2_GetComponentLocation` (`self.OwningComponent`)) (`self.Offset`)))
  ;[1 1 1] Move to Target Loc
  (if (`self.bIsDynamic`)
    (`self.K2_SetActorLocationAndRotation` (select `bool` _returnvalue :`false` _returnvalue_3 :`true` (`KismetMathLibrary.VInterpTo` (`self.K2_GetActorLocation`) _returnvalue_3 DeltaSeconds (* (`self.FollowSpeed`) 10.0))) (select `bool` _returnvalue :`false` _returnvalue_2 :`true` (`KismetMathLibrary.RInterpTo` (`self.K2_GetActorRotation`) _returnvalue_2 DeltaSeconds (* (`self.FollowSpeed`) 6.0))))))

(fn `CacheAndConfigureWidget`
  (`/XR_Toolkit/XR_Toolkit/Core/Utilities/XRAnnotation/BPI_XRCoreUI.SetTitle` (`self.Title`))
  (`/XR_Toolkit/XR_Toolkit/Core/Utilities/XRAnnotation/BPI_XRCoreUI.SetSubtitle` (`self.Subtitle`)))

(fn `UserConstructionScript`)
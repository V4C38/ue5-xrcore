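; A reusable 3D XR button with separate title and background widget components, offering highlight, selected, active and show/hide states.
; Presses come from the background widget's button or the XR interaction trigger, then play an animation and fire the OnXRButtonPressed dispatcher.
; Timelines and helper functions offset both widgets for press and hover feedback.
; State changes reach the widgets through messages, and selection suppresses highlight updates.
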(event `self.ReceiveBeginPlay`
  (`|ExecutionSequence`
    (:`then_0`
      (`self.SetTitle` (`self.Title`))
      (message `/XR_Toolkit/XR_Toolkit/Core/Utilities/XRAnnotation/BPI_XRCoreUI.SetActiveState` (`WidgetComponent.GetUserWidgetObject` (`self.Widget_Title`)) (`self.bIsActivated`)))
    (:`then_1`
      (bind _aswbp_xrbutton_background (cast `/XR_Toolkit/XR_Toolkit/Core/Utilities/XRButton/WBP_XRButton_Background` (`WidgetComponent.GetUserWidgetObject` (`self.Widget_Background`))))
      (bind _button (`/XR_Toolkit/XR_Toolkit/Core/Utilities/XRButton/WBP_XRButton_Background.Button` _aswbp_xrbutton_background))
      (add `Button.OnPressed` _button (delegate `OnPressed_Event`))
      (add `Button.OnHovered` _button (`|CreateDelegate` :!event `UpdateHighlightState`))
      (add `Button.OnUnhovered` _button (`|CreateDelegate` :!event `UpdateHighlightState`)))))

(event `OnPressed_Event`
  (`self.XRButtonPressed` null))

(event `self.XRInteractionTrigger.OnInteractionStarted`
  (params (Sender :type "XRInteractionComponent Object Reference") (XRInteractorComponent :type "XRInteractorComponent Object Reference"))
  ;[1 1 1] XRInteraction
  (`self.XRButtonPressed` XRInteractorComponent))

(event `self.XRInteractionTrigger.OnInteractionEnded`
  (params (Sender :type "XRInteractionComponent Object Reference") (XRInteractorComponent :type "XRInteractorComponent Object Reference"))
  ;[1 1 1] XRInteraction
)

(event `self.XRInteractionTrigger.OnInteractionHovered`
  (params (Sender :type "XRInteractionComponent Object Reference") (HoveringXRInteractor :type "XRInteractorComponent Object Reference") (bHovered :type Boolean))
  ;[1 1 1] XRInteraction
  (`/XR_Toolkit/XR_Toolkit/Core/Utilities/XRAnnotation/BPI_XRCoreUI.SetHighlighted` bHovered HoveringXRInteractor))

(event `/XR_Toolkit/XR_Toolkit/Core/Utilities/XRAnnotation/BPI_XRCoreUI.SetTitle`
  (params (InTitle :type Text))
  (message `/XR_Toolkit/XR_Toolkit/Core/Utilities/XRAnnotation/BPI_XRCoreUI.SetTitle` (`WidgetComponent.GetUserWidgetObject` (`self.Widget_Title`)) InTitle)
  (message `/XR_Toolkit/XR_Toolkit/Core/Utilities/XRAnnotation/BPI_XRCoreUI.SetTitle` (`WidgetComponent.GetUserWidgetObject` (`self.Widget_Background`)) InTitle))

(event `XRButtonPressed`
  (params (XRInteractor :type "XRInteractorComponent Object Reference"))
  (`self.AnimatePressEvent`)
  (`self.OnXRButtonPressed` self XRInteractor))

(event `/XR_Toolkit/XR_Toolkit/Core/Utilities/XRAnnotation/BPI_XRCoreUI.SetHighlighted`
  (params (bInHighlightState :type Boolean) (InXRInteractor :type "XRInteractorComponent Object Reference"))
  ;[1 1 1] Highlighting
  (set `self.bHighlightState` bInHighlightState)
  (if (not (`self.bIsSelected`))
    (message `/XR_Toolkit/XR_Toolkit/Core/Utilities/XRAnnotation/BPI_XRCoreUI.SetHighlighted` (`WidgetComponent.GetUserWidgetObject` (`self.Widget_Background`)) bInHighlightState InXRInteractor)
    (`self.Set Cosmetic Button State` bInHighlightState)
    (`self.OnXRButtonHighlighted` self InXRInteractor bInHighlightState)))

(event `/XR_Toolkit/XR_Toolkit/Core/Utilities/XRAnnotation/BPI_XRCoreUI.SetSelected`
  (params (InSelected :type Boolean) (InXRInteractor :type "XRInteractorComponent Object Reference"))
  ;[1 1 1] Highlighting
  (bind _output_get (set `self.bIsSelected` InSelected))
  (message `/XR_Toolkit/XR_Toolkit/Core/Utilities/XRAnnotation/BPI_XRCoreUI.SetSelected` (`WidgetComponent.GetUserWidgetObject` (`self.Widget_Background`)) _output_get InXRInteractor)
  (if _output_get
    (`self.Set Cosmetic Button State` true)
    (else
      (`/XR_Toolkit/XR_Toolkit/Core/Utilities/XRAnnotation/BPI_XRCoreUI.SetHighlighted` (`self.bHighlightState`) InXRInteractor))))

(event `/XR_Toolkit/XR_Toolkit/Core/Utilities/XRAnnotation/BPI_XRCoreUI.SetActiveState`
  (params (bInActive :type Boolean))
  (message `/XR_Toolkit/XR_Toolkit/Core/Utilities/XRAnnotation/BPI_XRCoreUI.SetActiveState` (`WidgetComponent.GetUserWidgetObject` (`self.Widget_Title`)) bInActive))

(event `/XR_Toolkit/XR_Toolkit/Core/Utilities/XRAnnotation/BPI_XRCoreUI.Show`
  (if (not (`self.bIsVisible`))
    (set `self.bIsVisible` true)
    (message `/XR_Toolkit/XR_Toolkit/Core/Utilities/XRAnnotation/BPI_XRCoreUI.Show` (`WidgetComponent.GetUserWidgetObject` (`self.Widget_Title`)))
    (message `/XR_Toolkit/XR_Toolkit/Core/Utilities/XRAnnotation/BPI_XRCoreUI.Show` (`WidgetComponent.GetUserWidgetObject` (`self.Widget_Background`)))))

(event `/XR_Toolkit/XR_Toolkit/Core/Utilities/XRAnnotation/BPI_XRCoreUI.Hide`
  (if (`self.bIsVisible`)
    (set `self.bIsVisible` false)
    (message `/XR_Toolkit/XR_Toolkit/Core/Utilities/XRAnnotation/BPI_XRCoreUI.Hide` (`WidgetComponent.GetUserWidgetObject` (`self.Widget_Title`)))
    (message `/XR_Toolkit/XR_Toolkit/Core/Utilities/XRAnnotation/BPI_XRCoreUI.Hide` (`WidgetComponent.GetUserWidgetObject` (`self.Widget_Background`)))))

(event `AnimatePressEvent`
  ;[1 1 1] Animation
  (`TimelineComponent.SetPlayRate` (`self.Timeline_Pressed`) 5.0)
  (bind (_direction _titleposition) (`Timeline|Timeline_Pressed` :!via `PlayFromStart`)
    (:`Update`
      (`SceneComponent.K2_SetRelativeLocation` (`self.Widget_Title`) (`KismetMathLibrary.VLerp` (`self.GetDesiredTitleLocation` (`self.IsHovered`)) (0.5 -1.0 2.0) _titleposition) false false)
      (`SceneComponent.K2_SetRelativeLocation` (`self.Widget_Background`) (`KismetMathLibrary.VLerp` (`self.GetDesiredBackgroundLocation` (`self.IsHovered`)) (0.25 0.0 1.75) _titleposition) false false))
    (:`Finished`
      (`self.UpdateHighlightState`))))

(event `UpdateHighlightState`
  ;[1 1 1] Animation
  (`TimelineComponent.SetPlayRate` (`self.Timeline_Highlighted`) 8.0)
  (bind (_direction _location_alpha) (`Timeline|Timeline_Highlighted` :!via `PlayFromStart`)
    (:`Update`
      (if (not (`TimelineComponent.IsPlaying` (`self.Timeline_Pressed`)))
        (`SceneComponent.K2_SetRelativeLocation` (`self.Widget_Title`) (`KismetMathLibrary.VLerp` (`SceneComponent.RelativeLocation` (`self.Widget_Title`)) (`self.GetDesiredTitleLocation` (`self.IsHovered`)) _location_alpha) false false)
        (`SceneComponent.K2_SetRelativeLocation` (`self.Widget_Background`) (`KismetMathLibrary.VLerp` (`SceneComponent.RelativeLocation` (`self.Widget_Background`)) (`self.GetDesiredBackgroundLocation` (`self.IsHovered`)) _location_alpha) false false)))))

(fn `GetDesiredBackgroundLocation`
  (params (bInState :type Boolean))
  (returns (OutRelativeLocation :type "Vector Structure"))
  (return (select `bool` bInState :`false` (0.0 0.0 1.75) :`true` (0.5 0.0 1.75) :!type "Vector Structure")))

(fn `GetDesiredTitleLocation`
  (params (bInState :type Boolean))
  (returns (OutRelativeLocation :type "Vector Structure"))
  (return (select `bool` bInState :`false` (1.0 -1.0 2.0) :`true` (2.0 -1.0 2.0) :!type "Vector Structure")))

(fn `IsHovered`
  (returns (bOutIsHovered :type Boolean))
  (return (or (`Widget.IsHovered` (`WidgetComponent.GetUserWidgetObject` (`self.Widget_Background`))) (`.ReturnValue` (`XRInteractionComponent.IsHovered` (`self.XRInteractionTrigger`))))))

(fn `IsVisible`
  (returns (bOutIsVisible :type Boolean))
  (return (`self.bIsVisible`)))

(fn `Set Cosmetic Button State`
  (params (bInState :type Boolean))
  (if (not (`TimelineComponent.IsPlaying` (`self.Timeline_Pressed`)))
    (`SceneComponent.K2_SetRelativeLocation` (`self.Widget_Title`) (`self.GetDesiredTitleLocation` (`local.bInState`)) false false)))

(fn `UserConstructionScript`
  (bind _title (`self.Title`))
  (message `/XR_Toolkit/XR_Toolkit/Core/Utilities/XRAnnotation/BPI_XRCoreUI.SetTitle` (`WidgetComponent.GetWidget` (`self.Widget_Title`)) _title)
  (message `/XR_Toolkit/XR_Toolkit/Core/Utilities/XRAnnotation/BPI_XRCoreUI.SetTitle` (`WidgetComponent.GetWidget` (`self.Widget_Background`)) _title))
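; Actor component in the XR Toolkit that holds whether hand tracking is active and replicates mode changes.
; A server event stores the flag and multicasts it, firing the OnHandTrackingModeChanged dispatcher; a getter exposes the state.
; BeginPlay sets the tick interval from UpdateFrequency, but the experimental automatic switch is disconnected, so Tick does nothing and nothing here triggers the server event.
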(event `self.ReceiveBeginPlay`
  (`self.SetComponentTickInterval` (`self.UpdateFrequency`)))

(event `self.ReceiveTick`
  (params (DeltaSeconds :type "Float (single-precision)"))
  ;[0.3281 0.3281 0.3281] - Experimental -
  ; HandTracking Switch
)

(event `Server_SetIsUsingHandtracking`
  (params (bIsUsingHandTracking :type Boolean))
  ;[0.3281 0.3281 0.3281] - Experimental -
  ; HandTracking Switch
  (set `self.bIsHandTrackingActive` bIsUsingHandTracking)
  (`self.Multicast_SetIsUsingHandtracking` bIsUsingHandTracking))

(event `Multicast_SetIsUsingHandtracking`
  (params (bIsUsingHandTracking :type Boolean))
  ;[0.3281 0.3281 0.3281] - Experimental -
  ; HandTracking Switch
  (`self.OnHandTrackingModeChanged` bIsUsingHandTracking))

(fn `IsHandTrackingActive`
  (returns (bIsHandTrackingActive :type Boolean))
  (return (`self.bIsHandTrackingActive`)))
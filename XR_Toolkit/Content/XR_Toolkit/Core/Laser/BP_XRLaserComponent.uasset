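; XR laser component that gives its owner a networked laser with an XR interactor, tied to a controller hand.
; On BeginPlay the server spawns a replicated BP_XRLaser, starting disabled, and OnRep_XRLaser attaches it to the component, copies config and sets the interactor's owning pawn.
; Server events toggle LaserActive and multicast the change, showing the laser only for the local pawn unless ReplicateLaser is set.
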(event `self.ReceiveBeginPlay`
  ;[0 0 0] Init
  (`|ExecutionSequence`
    (:`then_0`
      (bind _aspawn (cast `Pawn` (`self.GetOwner`)))
      (set `self.bIsLocalLaserComponent` (`Pawn.IsLocallyControlled` _aspawn)))
    (:`then_1`
      (if (`KismetSystemLibrary.IsServer`)
        (`self.Server_SpawnXRLaser`)))))

(event `Server_EnableLaser`
  ;[1 1 1] API
  (set `self.bLaserActive` true)
  (`self.Multicast_EnableLaser`))

(event `Multicast_EnableLaser`
  ;[1 1 1] API
  (if (and (`self.IsActive`) (`self.IsLaserVisibleOnThisClient`))
    (bind _xrlaser (`self.XRLaser`)
      (:`then`
        (`/XR_Toolkit/XR_Toolkit/Core/Laser/BP_XRLaser.OnLaserEnabled` _xrlaser))
      (:`else`))))

(event `Server_DisableLaser`
  ;[1 1 1] API
  (set `self.bLaserActive` false)
  (`self.Multicast_DisableLaser`))

(event `Multicast_DisableLaser`
  ;[1 1 1] API
  (bind _xrlaser (`self.XRLaser`)
    (:`then`
      (`/XR_Toolkit/XR_Toolkit/Core/Laser/BP_XRLaser.OnLaserDisabled` _xrlaser))
    (:`else`)))

(event `Server_SpawnXRLaser`
  ;[0 0 0] Spawn XRLaser Actor
  (`self.XRLaser`
    (:`then`)
    (:`else`
      (bind _returnvalue (`|SpawnActorFromClass` "/XR_Toolkit/XR_Toolkit/Core/Laser/BP_XRLaser.BP_XRLaser_C" (`KismetMathLibrary.MakeTransform` (0.0 0.0 0.0)) "Undefined" "MultiplyWithRoot" (`self.GetOwner`) (`self.MaxLength`) self null))
      (`Actor.SetReplicates` _returnvalue true)
      (bind _output_get (set `self.XRLaser` _returnvalue))
      (`self.Server_DisableLaser`)
      (`/XR_Toolkit/XR_Toolkit/Core/Laser/BP_XRLaser.Server_SetControllerHand` _output_get (`self.Get Controller Hand`)))))

(fn `Get Controller Hand`
  (returns (`XRController Hand` :type "EControllerHand Enum"))
  (return (`self.XRController Hand`)))

(fn `GetXRInteractor`
  (returns (XRInteractor :type "XRInteractorComponent Object Reference"))
  (bind _xrlaser (`self.XRLaser`)
    (:`then`
      (return (`/XR_Toolkit/XR_Toolkit/Core/Laser/BP_XRLaser.XRInteractor` _xrlaser)))
    (:`else`)))

(fn `GetXRLaser`
  (returns (OutXRLaser :type "/XR_Toolkit/XR_Toolkit/Core/Laser/BP_XRLaser Object Reference"))
  (return (`self.XRLaser`)))

(fn `IsLaserActive`
  (returns (bLaserActive :type Boolean))
  (return (`self.bLaserActive`)))

(fn `IsLaserVisibleOnThisClient`
  (returns (ReturnValue :type Boolean))
  (return (or (`self.bReplicateLaser`) (`self.bIsLocalLaserComponent`))))

(fn `OnRep_XRLaser`
  (bind _xrlaser (`self.XRLaser`))
  (`self.XRLaser`
    (:`then`
      (`|ExecutionSequence`
        (:`then_0`
          (`self.K2_AttachToComponent` (`/XR_Toolkit/XR_Toolkit/Core/Laser/BP_XRLaser.LaserRoot` (`self.XRLaser`)) self "None" "SnapToTarget" "SnapToTarget" "KeepRelative" true))
        (:`then_1`
          ;[1 1 1] Set Config Variables on XRLaser
          (set `/XR_Toolkit/XR_Toolkit/Core/Laser/BP_XRLaser.SmoothingFactor` (`self.SmoothingFactor`) _xrlaser)
          (set `/XR_Toolkit/XR_Toolkit/Core/Laser/BP_XRLaser.bInstantlyShowLaser` (not (`self.bAnimateLaserBuildup`)) _xrlaser)
          (set `/XR_Toolkit/XR_Toolkit/Core/Laser/BP_XRLaser.DynamicLengthGrab_Speed` (`self.Dynamic Length Grab Speed`) _xrlaser)
          (set `/XR_Toolkit/XR_Toolkit/Core/Laser/BP_XRLaser.Thickness_Max` (`self.Thickness Max`) _xrlaser)
          (set `/XR_Toolkit/XR_Toolkit/Core/Laser/BP_XRLaser.Thickness_Min` (`self.Thickness Min`) _xrlaser))
        (:`then_2`
          (bind _aspawn (cast `Pawn` (`self.GetOwner`)))
          (`XRInteractorComponent.SetOwningPawn` (`/XR_Toolkit/XR_Toolkit/Core/Laser/BP_XRLaser.XRInteractor` (`self.XRLaser`)) _aspawn))))
    (:`else`)))
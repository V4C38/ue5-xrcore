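; BP_XRLaser is a runtime-spawned XR laser pointer that lets a hand's XRInteractor interact with objects at range.
; A line trace sets length and validity; the interpolated tip drives a rebuilt spline-mesh beam, target sphere and timeline buildup.
; During interactions, the component's laser behavior disables the laser, allows GoGo-style length changes from hand movement, or snaps the tip to it.
; Snapped interactions fade with aim deviation and are terminated by the server beyond a threshold.
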(event `self.ReceiveBeginPlay`
  ;[1 1 1] Init
  ; - Actor is spawned at runtime (Config vars exposed on spawn)
  (`|ExecutionSequence`
    (:`then_0`
      (if (`KismetSystemLibrary.IsServer`)
        (`XRInteractorComponent.Server_SetXRControllerHand` (`self.XRInteractor`) (`self.In XRController Hand`))))
    (:`then_1`
      (`SceneComponent.K2_SetRelativeLocation` (`self.Direction`) (`KismetMathLibrary.MakeVector` (`self.MaxLenght`)) false false)
      (`self.ConfigureLaserMaterial`))
    (:`then_2`
      (set `self.SmoothingStartDistance` (* (`self.MaxLenght`) 0.2)))
    (:`then_3`
      (`self.SetActorHiddenInGame` true))))

(event `self.ReceiveTick`
  (params (DeltaSeconds :type "Float (single-precision)"))
  (bind _bshowlaserasvalid (`self.bShowLaserAsValid`))
  ;[1 1 1] Tick
  (`|ExecutionSequence`
    (:`then_0`
      (if (`self.bLineTracing`)
        (bind _outfoundvalidhit (`self.UpdateLaserLengthFromLineTrace`))
        (set `self.bShowLaserAsValid` _outfoundvalidhit)
        (else
          (switch `EXRLaserBehavior` (`self.InteractionLaserSettings`)
            (:`Enabled`
              (`self.UpdateDynamicLengthModifier`)
              (set `self.bShowLaserAsValid` true))
            (:`Snap`
              (bind _outinteractionvalid (`self.ShouldInteractionGetCancelled` :!label _label))
              (set `self.bShowLaserAsValid` _outinteractionvalid))
            (:`SnapMove`
              (goto _label)))))
      (`self.Interpolate Tip Position` DeltaSeconds)
      (`self.UpdateTargetSphereState` _bshowlaserasvalid)
      (`self.UpdateBeam` _bshowlaserasvalid))
    (:`then_1`
      (`self.HandleXRInteractorRotation` DeltaSeconds))))

(event `OnLaserEnabled`
  ;[1 1 1] Set State
  (if (not (`self.bIsActive`))
    (set `self.bIsActive` true)
    (`self.UpdateLaserLengthFromLineTrace`)
    (if (`self.bInstantlyShowLaser`) :!label _label_2
      (`self.Set Active State` (`self.bIsActive`) :!label _label_3)
      (elif (and (< (`self.Length_Base`) (`self.SmoothingStartDistance`)) (`self.bIsActive`))
        (goto _label_3)
        (else
          (`self.AnimateLaserBuildup`))))))

(event `OnLaserDisabled`
  ;[1 1 1] Set State
  (if (`self.bIsActive`)
    (set `self.bIsActive` false)
    (`XRInteractorComponent.StopAllXRInteractions` (`self.XRInteractor`))
    (goto _label_2)))

(event `AnimateLaserBuildup`
  ;[0 0 0] Buildup
  (`TimelineComponent.SetPlayRate` (`self.Timeline_LaserBuildup`) (`self.GetBuildupSpeed`))
  (`self.Set Buildup State`)
  (if (`self.bIsActive`)
    (bind (_direction _buildupalpha) (`Timeline|Timeline_LaserBuildup` :!label _label_4)
      (:`Update`
        (`self.UpdateDynaMat` _buildupalpha true)
        (`SceneComponent.SetRelativeScale3D` (`self.LaserRoot`) (`KismetMathLibrary.Conv_DoubleToVector` _buildupalpha))
        (`SceneComponent.SetRelativeScale3D` (`self.TargetSphere`) (`KismetMathLibrary.Conv_DoubleToVector` (* (`self.GetTargetSpehreScale`) _buildupalpha))))
      (:`Finished`
        (`self.Set Active State` (`self.bIsActive`))))
    (else
      (goto _label_4 :!via `Reverse`))))

(event `self.XRInteractor.OnStartedInteracting`
  (params (Sender :type "XRInteractorComponent Object Reference") (XRInteractionComponent :type "XRInteractionComponent Object Reference"))
  ;[0 0 0] XRInteraction - Dynamic Length Grab
  (if (`KismetSystemLibrary.IsServer`)
    (set `self.Length_Modifier` 0.0)
    (switch `EXRLaserBehavior` (`XRInteractionComponent.GetLaserBehavior` XRInteractionComponent)
      (:`Disabled`
        (`/XR_Toolkit/XR_Toolkit/Core/Laser/BP_XRLaserComponent.Server_DisableLaser` (`self.OwningXRLaserComponent`) :!label _label_5))
      (:`Supress`
        (goto _label_5))
      (:`Enabled`
        (`self.OnXRInteractionStarted` XRInteractionComponent :!label _label_6))
      (:`Snap`
        (goto _label_6))
      (:`SnapMove`
        (goto _label_6)))))

(event `self.XRInteractor.OnStoppedInteracting`
  (params (Sender :type "XRInteractorComponent Object Reference") (XRInteractionComponent :type "XRInteractionComponent Object Reference"))
  ;[0 0 0] XRInteraction - Dynamic Length Grab
  (`self.OnEndXRInteraction`))

(event `Server_SetLengthModifier`
  (params (Length_Modifier :type "Float (double-precision)"))
  (set `self.Length_Modifier` Length_Modifier))

(event `Server_SetControllerHand`
  (params (`In XRController Hand` :type "EControllerHand Enum" :default "Left"))
  (bind _output_get (set `self.In XRController Hand` `In XRController Hand`))
  (`XRInteractorComponent.Server_SetXRControllerHand` (`self.XRInteractor`) _output_get))

(fn `ClearSplineMesh`
  (bind _splinemeshes (`self.SplineMeshes`))
  (for _array_element _splinemeshes
    (`ActorComponent.K2_DestroyComponent` _array_element))
  (`KismetArrayLibrary.Array_Clear` _splinemeshes)
  (return))

(fn `ConfigureLaserMaterial`
  (bind _returnvalue (`KismetMaterialLibrary.CreateDynamicMaterialInstance` "/XR_Toolkit/XR_Toolkit/Assets/MaterialLibrary/Interaction/MI_XRLaserBeam.MI_XRLaserBeam"))
  (bind _output_get (set `self.DynaMat_SplineMesh` _returnvalue))
  (`MaterialInstanceDynamic.SetScalarParameterValue` _output_get "LaserLength_Max" (`self.MaxLenght`)) ; Used to determine Laser Thickness in the Shader
  (`MaterialInstanceDynamic.SetScalarParameterValue` _output_get "Thickness" (`self.Thickness`)) ; Used to determine Laser Thickness in the Shader
)

(fn `Get Controller Hand`
  (returns (`XRController Hand` :type "EControllerHand Enum"))
  (return (`self.In XRController Hand`)))

(fn `GetBuildupSpeed`
  (returns (ReturnValue :type "Float (single-precision)"))
  (return (* (`KismetMathLibrary.MapRangeClamped` (`self.Length_Base`) (`self.SmoothingStartDistance`) (`self.MaxLenght`) 12.0 3.0) (`self.BuildupSpeed`))))

(fn `GetDesiredTipLocation`
  (params (InModifiedLaserLength :type "Float (double-precision)"))
  (returns (OutDesiredTipLocation :type "Vector Structure"))
  (return (+ (`SceneComponent.K2_GetComponentLocation` (`self.LaserRoot`)) (* (`KismetMathLibrary.GetDirectionUnitVector` (`SceneComponent.K2_GetComponentLocation` (`self.LaserRoot`)) (`SceneComponent.K2_GetComponentLocation` (`self.Direction`))) (`local.InModifiedLaserLength`)))))

(fn `GetInterpolationSpeedByDistance`
  (returns (OutInterpolationSpeed :type "Float (double-precision)"))
  (bind _maxlenght (`self.MaxLenght`))
  (return (* (`KismetMathLibrary.MapRangeClamped` (`self.GetModifiedXRLaserLenght`) (* _maxlenght 0.25) (* _maxlenght 0.8) 25.0 12.0) (* (`self.SmoothingFactor`) (`self.SmoothingFactorModifier`)))))

(fn `GetLengthModifier`
  (returns (OutLength_Modifier :type "Float (double-precision)"))
  (return (`self.Length_Modifier`)))

(fn `GetModifiedXRLaserLenght`
  (returns (OutModifiedLaserLength :type "Float (double-precision)"))
  (return (`KismetMathLibrary.FClamp` (+ (`self.Length_Base`) (`self.Length_Modifier`)) 0.0 (`self.MaxLenght`))))

(fn `GetTargetSpehreScale`
  (returns (OutScale :type "Float (double-precision)"))
  (return (`KismetMathLibrary.MapRangeClamped` (`self.GetModifiedXRLaserLenght`) 100.0 (`self.MaxLenght`) 0.005 (`KismetMathLibrary.MapRangeClamped` (`self.MaxLenght`) 500.0 2500.0 0.01 0.04))))

(fn `HandleXRInteractorRotation`
  (params (InDeltaTime :type "Float (single-precision)"))
  (if (`XRInteractorComponent.IsInteracting` (`self.XRInteractor`))
    _))

(fn `Interpolate Tip Position`
  (params (InDeltaTime :type "Float (single-precision)"))
  (locals (Loc_DesiredTipLocation :type "Vector Structure" :default (0.0 0.0 0.0)) (Loc_ModifiedLength :type "Float (double-precision)" :default 0.0))
  (bind _tip (`self.Tip`))
  (bind _returnvalue (`KismetMathLibrary.VInterpTo` (`SceneComponent.K2_GetComponentLocation` (`self.Tip`)) (`self.GetDesiredTipLocation` (`self.GetModifiedXRLaserLenght`)) (`local.InDeltaTime`) (`self.GetInterpolationSpeedByDistance`)))
  (`|ExecutionSequence`
    (:`then_0`
      ;[1 1 1] Location
      (if (`self.bLineTracing`)
        (bind _output_get (set `self.CurrentTipLocation` _returnvalue))
        (`SceneComponent.K2_SetWorldLocation` _tip _output_get false false)
        (else
          (switch `EXRLaserBehavior` (`self.InteractionLaserSettings`)
            (:`Enabled`
              (bind _output_get_2 (set `self.CurrentTipLocation` _returnvalue))
              (`SceneComponent.K2_SetWorldLocation` _tip _output_get_2 false false))))))
    (:`then_1`
      ;[1 1 1] Rotation
      (`SceneComponent.K2_SetWorldRotation` (`self.Tip`) (`KismetMathLibrary.RInterpTo` (`SceneComponent.K2_GetComponentRotation` (`self.Tip`)) (`SceneComponent.K2_GetComponentRotation` (`self.LaserRoot`)) (`local.InDeltaTime`) 4.5) false false))))

(fn `OnEndXRInteraction`
  (if (`KismetSystemLibrary.IsServer`)
    (set `self.Length_Modifier` 0.0)
    (set `self.bLineTracing` true)
    (set `self.SmoothingFactorModifier` 1.0)
    (`SceneComponent.K2_DetachFromComponent` (`self.Tip`) "KeepWorld" "KeepWorld" "KeepWorld" true)))

(fn `OnXRInteractionStarted`
  (params (InXRInteraction :type "XRInteractionComponent Object Reference"))
  (if (`KismetSystemLibrary.IsServer`)
    (set `self.bLineTracing` false)
    (set `self.SmoothingFactorModifier` 0.5)
    (set `self.InteractionLaserSettings` (`XRInteractionComponent.GetLaserBehavior` (`local.InXRInteraction`))))
  (if (select `EXRLaserBehavior` (`self.InteractionLaserSettings`) :`Snap` true :`SnapMove` true)
    (`SceneComponent.K2_AttachToComponent` (`self.Tip`) (`local.InXRInteraction`) "None" "SnapToTarget" "SnapToTarget" "KeepWorld" true)))

(fn `Set Active State`
  (params (bCurrentlyActive :type Boolean))
  (`|ExecutionSequence`
    (:`then_0`
      (if (`local.bCurrentlyActive`)
        (`self.SetActorHiddenInGame` false)
        (`self.SetActorTickEnabled` true)
        (`self.SetActorEnableCollision` true)
        (`self.UpdateDynaMat` 1.0 true)
        (else
          (`self.SetActorHiddenInGame` true)
          (`self.SetActorTickEnabled` false)
          (`self.SetActorEnableCollision` false)
          (`self.UpdateDynaMat` 0.0 true))))
    (:`then_1`
      (set `self.bCompletedBuildup` true))))

(fn `Set Buildup State`
  (`self.SetActorHiddenInGame` false)
  (`self.SetActorTickEnabled` true)
  (`self.UpdateDynaMat` 0.0)
  (set `self.bCompletedBuildup` false))

(fn `ShouldInteractionGetCancelled`
  (returns (OutInteractionValid :type Boolean))
  (locals (Loc_CurrentDirectionDelta :type "Float (double-precision)"))
  (bind _loc_currentdirectiondelta (`local.Loc_CurrentDirectionDelta`))
  ;[0 0 0] Cache Direction Data
  (set `local.Loc_CurrentDirectionDelta` (`KismetMathLibrary.Dot_VectorVector` (`KismetMathLibrary.GetDirectionUnitVector` (`SceneComponent.K2_GetComponentLocation` (`self.LaserRoot`)) (`SceneComponent.K2_GetComponentLocation` (`self.Direction`))) (`KismetMathLibrary.GetDirectionUnitVector` (`SceneComponent.K2_GetComponentLocation` (`self.LaserRoot`)) (`SceneComponent.K2_GetComponentLocation` (`self.Tip`)))))
  ;[1 1 1] Set Beam Color based on Direction
  (`MaterialInstanceDynamic.SetScalarParameterValue` (`self.DynaMat_SplineMesh`) "Opacity" (select `bool` (> 0.995 (`local.Loc_CurrentDirectionDelta`)) :`false` (`KismetMathLibrary.MapRangeClamped` _loc_currentdirectiondelta 1.0 0.995 1.0 0.35) :`true` (`KismetMathLibrary.MapRangeClamped` _loc_currentdirectiondelta 0.995 0.96 0.35 0.1) :!type "Float (single-precision)"))
  ;[1 1 1] Check if Interaction Direction is within Termination Treshold
  (if (< (`local.Loc_CurrentDirectionDelta`) 0.96)
    (if (`KismetSystemLibrary.IsServer`)
      (`self.Terminate Active Interaction`)
      (return false)
      (else
        (return false)))
    (else
      (return true))))

(fn `Terminate Active Interaction`
  (`|ExecutionSequence`
    (:`then_0`
      (bind _owningxrlasercomponent (`self.OwningXRLaserComponent`)
        (:`then`
          (`/XR_Toolkit/XR_Toolkit/Core/Laser/BP_XRLaserComponent.Server_DisableLaser` _owningxrlasercomponent))
        (:`else`)))
    (:`then_1`
      (`XRInteractorComponent.StopAllXRInteractions` (`self.XRInteractor`)))))

(fn `UpdateBeam`
  (params (bSetAsValid :type Boolean))
  (`self.ClearSplineMesh`)
  (`self.UpdateSpline`)
  (`self.UpdateSplineMesh`)
  (if (`self.bCompletedBuildup`)
    (`self.UpdateDynaMat` 1.0 (select `EXRLaserBehavior` (`self.InteractionLaserSettings`) :`Enabled` true))))

(fn `UpdateDynaMat`
  (params (InLocationAlpha :type "Float (single-precision)") (SetOpacity :type Boolean))
  (bind _dynamat_splinemesh (`self.DynaMat_SplineMesh`))
  (bind (_returnvalue_x _returnvalue_y _returnvalue_z) (`KismetMathLibrary.BreakVector` (`SceneComponent.K2_GetComponentLocation` (`self.LaserRoot`))))
  (`|ExecutionSequence`
    (:`then_0`
      (`MaterialInstanceDynamic.SetVectorParameterValue` _dynamat_splinemesh "AWP_Root" (make `LinearColor` _returnvalue_x _returnvalue_y _returnvalue_z 1.0)))
    (:`then_1`
      (`MaterialInstanceDynamic.SetScalarParameterValue` _dynamat_splinemesh "VisibilityDistance" (`KismetMathLibrary.MapRangeClamped` (`local.InLocationAlpha`) 0.0 1.0 0.0 (`self.MaxLenght`))))
    (:`then_2`
      (if (`local.SetOpacity`)
        (`MaterialInstanceDynamic.SetScalarParameterValue` (`self.DynaMat_SplineMesh`) "Opacity" (select `bool` (`self.bShowLaserAsValid`) :`false` 0.15 :`true` 0.5))))))

(fn `UpdateDynamicLengthModifier`
  (locals (Loc_CurrentLaserLocation :type "Vector Structure" :default (0.0 0.0 0.0)) (Loc_DirectionDOT :type "Float (double-precision)" :default 0.0) (Loc_MovementVelocity :type "Float (double-precision)" :default 0.0))
  (bind _outmodifiedlaserlength (`self.GetModifiedXRLaserLenght`))
  (bind _loc_directiondot (`local.Loc_DirectionDOT`))
  (bind _returnvalue (+ (`self.Length_Modifier`) (* (* _outmodifiedlaserlength (`KismetMathLibrary.MapRangeClamped` _outmodifiedlaserlength 150.0 (* (`self.Length_Base`) 1.5) 0.01 0.03) (`KismetMathLibrary.MapRangeClamped` (`local.Loc_MovementVelocity`) 0.05 1.0 0.1 1.0) (select `bool` (> (`local.Loc_DirectionDOT`) 0.0) :`false` 1 :`true` -1)) (`self.DynamicLengthGrab_Speed`))))
  (if (`KismetSystemLibrary.IsServer`)
    (set `local.Loc_CurrentLaserLocation` (`SceneComponent.K2_GetComponentLocation` (`self.LaserRoot`)))
    ;[0 0 0] Cache Movement Data
    (set `local.Loc_DirectionDOT` (`KismetMathLibrary.Dot_VectorVector` (`KismetMathLibrary.GetDirectionUnitVector` (`local.Loc_CurrentLaserLocation`) (`self.LastLaserLocation`)) (`KismetMathLibrary.GetDirectionUnitVector` (`SceneComponent.K2_GetComponentLocation` (`self.LaserRoot`)) (`SceneComponent.K2_GetComponentLocation` (`self.Tip`)))))
    (set `local.Loc_MovementVelocity` (`KismetMathLibrary.VSize` (- (`local.Loc_CurrentLaserLocation`) (`self.LastLaserLocation`))))
    (`|ExecutionSequence`
      (:`then_0`
        (set `self.LastLaserLocation` (`SceneComponent.K2_GetComponentLocation` (`self.LaserRoot`))))
      (:`then_1`
        ;[1 1 1] Only apply GoGo when moving in Object Direction
        ; - more leeway when moving towards
        (if (or (> _loc_directiondot 0.45) (< _loc_directiondot -0.35))
          ;[0 0 0] Apply if in Valid Range
          (if (`KismetMathLibrary.InRange_FloatFloat` (+ _returnvalue (`self.Length_Base`)) 15.0 (`self.MaxLenght`))
            (set `self.Length_Modifier` _returnvalue)))))
    (else
      (return))))

(fn `UpdateLaserLengthFromLineTrace`
  (returns (OutFoundValidHit :type Boolean))
  (locals (Loc_TraceHit :type "HitResult Structure") (Loc_FoundValidHit :type Boolean :default false))
  (bind (_bblockinghit _binitialoverlap _time _distance _location _impactpoint _normal _impactnormal _physmat _hitactor) (`GameplayStatics.BreakHitResult` (`local.Loc_TraceHit`)))
  ;[1 1 1] Trace Locally for Actors
  (bind (_outhit _returnvalue) (`KismetSystemLibrary.LineTraceSingle` (`SceneComponent.K2_GetComponentLocation` (`self.LaserRoot`)) (`SceneComponent.K2_GetComponentLocation` (`self.Direction`)) "TraceTypeQuery1" true (`|MakeArray` (`self.GetOwner`)) "None" false))
  (set `local.Loc_TraceHit` _outhit)
  (if _returnvalue
    (set `self.Last_TraceImpactPoint` _impactpoint)
    (set `self.Length_Base` _distance)
    (set `local.Loc_FoundValidHit` (`.ReturnValue` (`XRToolsUtilityFunctions.IsActorInteractive` _hitactor)))
    (else
      (set `self.Length_Base` (`self.MaxLenght`))))
  (set `self.Length_Modifier` 0.0) ; Ignore Lenght Modifier when Line Tracing
  (return (`local.Loc_FoundValidHit`)))

(fn `UpdateSpline`
  (bind _spline (`self.Spline`))
  (bind _returnvalue (* (`KismetMathLibrary.GetDirectionUnitVector` (`SceneComponent.K2_GetComponentLocation` (`self.LaserRoot`)) (`SceneComponent.K2_GetComponentLocation` (`self.Direction`))) (* (`self.GetModifiedXRLaserLenght`) 0.2)))
  (`SplineComponent.ClearSplinePoints` (`self.Spline`) true)
  (`|ExecutionSequence`
    (:`then_0`
      (`SplineComponent.AddSplinePoint` (`self.Spline`) (`SceneComponent.K2_GetComponentLocation` (`self.LaserRoot`)) "World" false))
    (:`then_1`
      ;[1 1 1] Midpoint based on distance to the Target
      (`SplineComponent.AddSplinePoint` _spline (+ _returnvalue (`SceneComponent.K2_GetComponentLocation` (`self.LaserRoot`))) "World" false)
      ;;[0 0 0] Smooth Tangent
      (`SplineComponent.SetTangentAtSplinePoint` _spline 1 (* _returnvalue 4.0) "World" false))
    (:`then_2`
      (`SplineComponent.AddSplinePoint` (`self.Spline`) (`SceneComponent.K2_GetComponentLocation` (`self.Tip`)) "World" true))
    (:`then_3`
      (return))))

(fn `UpdateSplineMesh`
  (bind _spline (`self.Spline`))
  ;[1 1 1] Set Spline MeshComponents
  (for _index (range (+ (- (`SplineComponent.GetNumberOfSplinePoints` (`self.Spline`)) 2) 1))
    (bind _returnvalue (`AddComponent|NODE_AddSplineMeshComponent-0` :`bManualAttachment` true :`RelativeTransform` (`KismetMathLibrary.MakeTransform` (0.0 0.0 0.0)))) ; Add new cylinder mesh
    (`PrimitiveComponent.SetMaterial` _returnvalue 0 (`self.DynaMat_SplineMesh`))
    (`KismetArrayLibrary.Array_Add` (`self.SplineMeshes`) _returnvalue)
    (bind _returnvalue_2 (+ _index 1))
    (`SplineMeshComponent.SetStartAndEnd` _returnvalue (`SplineComponent.GetLocationAtSplinePoint` (`self.Spline`) _index "Local") (`SplineComponent.GetTangentAtSplinePoint` _spline _index "Local") (`SplineComponent.GetLocationAtSplinePoint` (`self.Spline`) _returnvalue_2 "Local") (`SplineComponent.GetTangentAtSplinePoint` _spline _returnvalue_2 "Local") true) ; Set the tangents and position to build slightly bend the cylinder. All cylinders combined create a smooth arc.
  )
  (return))

(fn `UpdateTargetSphereState`
  (params (bSetAsValid :type Boolean))
  (`|ExecutionSequence`
    (:`then_0`
      ;[0 0 0] Target Sphere Appearance
      (`MeshComponent.SetScalarParameterValueOnMaterials` (`self.TargetSphere`) "Opacity" (select `bool` (`local.bSetAsValid`) :`false` 0.15 :`true` 1.0 :!type "Float (single-precision)"))
      (if (`self.bCompletedBuildup`)
        (`SceneComponent.SetWorldScale3D` (`self.TargetSphere`) (`KismetMathLibrary.Conv_DoubleToVector` (`self.GetTargetSpehreScale`)))))
    (:`then_1`
      (`PrimitiveComponent.SetCollisionEnabled` (`self.XRInteractor`) (select `bool` (`local.bSetAsValid`) :`false` "NoCollision" :`true` "QueryOnly" :!type "ECollisionEnabled Enum")))))

(fn `UserConstructionScript`
  (`XRInteractorComponent.SetAssignedPhysicsConstraint` (`self.XRInteractor`) (`self.XRInteractor_PhysicsConstraint_Laser`)))
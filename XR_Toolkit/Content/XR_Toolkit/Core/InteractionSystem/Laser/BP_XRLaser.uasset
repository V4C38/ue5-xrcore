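; BP_XRLaser is an XR laser pointer for interacting with actors whose XRInteractionComponent allows laser interaction.
; Each tick a line trace sets beam length and validity, which drives beam opacity, target sphere look and XRInteractor collision.
; The tip interpolates at a distance-based speed, bending a spline beam rebuilt every frame from spline meshes.
; A timeline animates enabling and disabling, while tracing can be suppressed, optionally snapping to the last impact.
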(event `self.ReceiveBeginPlay`
  (`|ExecutionSequence`
    (:`then_0`
      (if (`KismetSystemLibrary.IsServer`)
        (`XRInteractorComponent.Server_SetHandType` (`self.XRInteractor`) (`self.HandType`))))
    (:`then_1`
      (`SceneComponent.K2_SetRelativeLocation` (`self.Direction`) (`KismetMathLibrary.MakeVector` (`self.LaserMaxRange`)) false false)
      (bind _returnvalue (`KismetMaterialLibrary.CreateDynamicMaterialInstance` "/XR_Toolkit/XR_Toolkit/Assets/MaterialLibrary/InteractionDefaults/LaserInteraction/MI_LaserBeam.MI_LaserBeam"))
      (set `self.DynaMat_SplineMesh` _returnvalue))))

(event `self.ReceiveTick`
  (params (DeltaSeconds :type "Float (single-precision)"))
  (bind _bshowlaserasvalid (`self.bShowLaserAsValid`))
  (if (`self.bSupressLineTrace`)
    (set `self.bShowLaserAsValid` true)
    (else
      (bind _outfoundvalidhit (`self.UpdateLaserLengthFromLineTrace`))
      (set `self.bShowLaserAsValid` _outfoundvalidhit)))
  (`self.Interpolate Tip Position` DeltaSeconds)
  (`self.UpdateTargetSphere` _bshowlaserasvalid)
  (`self.UpdateBeam` _bshowlaserasvalid))

(event `Server_SetLengthModifier`
  (params (InLengthModifier :type "Float (double-precision)"))
  ;[1 1 1] Config Setters
  (set `self.Length_Modifier` InLengthModifier))

(event `SetSmoothingActive`
  (params (bInSmoothingActive :type Boolean))
  ;[1 1 1] Config Setters
  (set `self.bSmoothingActive` bInSmoothingActive))

(event `Server_SupressLineTrace`
  (params (bSupress :type Boolean) (bSnapToLastImpact :type Boolean))
  ;[1 1 1] Config Setters
  (set `self.bSupressLineTrace` bSupress)
  (set `self.Snap to Last Impact` bSnapToLastImpact))

(event `OnLaserEnabled`
  ;[1 1 1] Buildup
  (set `self.bBuildUp` true)
  (`self.PRIVATE_AnimateLaserBuildup` :!label _label)
  (`SceneComponent.K2_SetWorldLocation` (`self.Tip`) (`self.GetDesiredTipLocation`) false false))

(event `OnLaserDisabled`
  ;[1 1 1] Buildup
  (set `self.bBuildUp` false)
  (goto _label))

(event `PRIVATE_AnimateLaserBuildup`
  ;[1 1 1] Buildup
  (set `self.bIsActivated` false)
  (`SceneComponent.SetVisibility` (`self.TargetSphere`) false false)
  (`TimelineComponent.SetPlayRate` (`self.Timeline_LaserBuildup`) (`self.GetBuildupSpeed`))
  (if (`self.bBuildUp`)
    (`self.SetActorHiddenInGame` false)
    (`self.SetActorTickEnabled` true)
    (`self.SetActorEnableCollision` true)
    (bind (_direction _buildupalpha) (`Timeline|Timeline_LaserBuildup` :!label _label_2)
      (:`Update`
        (`MaterialInstanceDynamic.SetScalarParameterValue` (`self.DynaMat_SplineMesh`) "DistanceDivider" (* _buildupalpha (`self.GetModifiedXRLaserLenght`)))
        (`SceneComponent.K2_SetWorldLocation` (`self.XRInteractor`) (`self.GetDesiredTipLocation`) false false))
      (:`Finished`
        (if (`self.bBuildUp`)
          (`self.SetActorEnableCollision` true)
          (`SceneComponent.SetVisibility` (`self.TargetSphere`) true false)
          (set `self.bIsActivated` true)
          (else
            (`self.SetActorHiddenInGame` true)
            (`self.SetActorTickEnabled` false)
            (`self.SetActorEnableCollision` false)))
        (`SceneComponent.K2_SetRelativeLocation` (`self.XRInteractor`) (0.0 0.0 0.0) false false)))
    (else
      (goto _label_2 :!via `Reverse`))))

(fn `ClearSplineMesh`
  (bind _splinemeshes (`self.SplineMeshes`))
  (for _array_element _splinemeshes
    (`ActorComponent.K2_DestroyComponent` _array_element))
  (`KismetArrayLibrary.Array_Clear` _splinemeshes)
  (return))

(fn `GetBuildupSpeed`
  (returns (ReturnValue :type "Float (single-precision)"))
  (bind _buildupspeed (`self.BuildUpSpeed`))
  (return (select `bool` (>= (`self.Length_Base`) 100.0) :`false` (* (`self.BuildUpSpeed`) 5.0) :`true` (`KismetMathLibrary.MapRangeClamped` (`self.Length_Base`) 100.0 (`self.LaserMaxRange`) (* _buildupspeed 2.0) (* _buildupspeed 0.5)))))

(fn `GetDesiredTipLocation`
  (returns (OutDesiredTipLocation :type "Vector Structure"))
  (return (+ (`SceneComponent.K2_GetComponentLocation` (`self.LaserRoot`)) (* (`KismetMathLibrary.GetDirectionUnitVector` (`SceneComponent.K2_GetComponentLocation` (`self.LaserRoot`)) (`SceneComponent.K2_GetComponentLocation` (`self.Direction`))) (`self.GetModifiedXRLaserLenght`)))))

(fn `GetHandType`
  (returns (HandType :type "EXRHandType Enum"))
  (return (`self.HandType`)))

(fn `GetInterpolationSpeedByDistance`
  (returns (OutInterpolationSpeed :type "Float (double-precision)"))
  (bind _lasermaxrange (`self.LaserMaxRange`))
  (return (* (`KismetMathLibrary.MapRangeClamped` (`self.GetModifiedXRLaserLenght`) (* _lasermaxrange 0.25) (* _lasermaxrange 0.8) 8.0 3.0) (`self.SmoothingAmount`))))

(fn `GetModifiedXRLaserLenght`
  (returns (OutModifiedLaserLength :type "Float (double-precision)"))
  (return (`KismetMathLibrary.FClamp` (+ (`self.Length_Base`) (`self.Length_Modifier`)) 0.0 (`self.LaserMaxRange`))))

(fn `GetOverlappingInteractionComponents`
  (returns (FoundXRInteractionComps :type "Array of XRInteractionComponent Object Reference"))
  (return))

(fn `HasActorXRInteractionComponent`
  (params (InActor :type "Actor Object Reference"))
  (returns (bFoundXRInteractionComp :type Boolean))
  (bind _returnvalue (`self.GetComponentByClass` InActor "/Script/XR_Toolkit.XRInteractionComponent"))
  (`/Engine/EditorBlueprintResources/StandardMacros.IsValid` _returnvalue
    (:`Is Valid`
      (return (`XRInteractionComponent.IsLaserInteractionEnabled` _returnvalue)))
    (:`Is Not Valid`
      (return false))))

(fn `Interpolate Tip Position`
  (params (InDeltaTime :type "Float (single-precision)"))
  (locals (Loc_DesiredTipLocation :type "Vector Structure" :default (0.0 0.0 0.0)))
  (bind _tip (`self.Tip`))
  (bind _returnvalue (`KismetMathLibrary.VInterpTo` (`SceneComponent.K2_GetComponentLocation` (`self.Tip`)) (`self.GetDesiredTipLocation`) (`local.InDeltaTime`) (`self.GetInterpolationSpeedByDistance`)))
  (if (`self.bSupressLineTrace`)
    (bind _output_get (set `self.CurrentTipLocation` (select `bool` (`self.Snap to Last Impact`) :`false` _returnvalue :`true` (`self.Last_TraceImpactPoint`))))
    (`SceneComponent.K2_SetWorldLocation` _tip _output_get false false)
    (else
      (bind _output_get_2 (set `self.CurrentTipLocation` _returnvalue))
      (`SceneComponent.K2_SetWorldLocation` _tip _output_get_2 false false))))

(fn `UpdateBeam`
  (params (bSetAsValid :type Boolean))
  (`self.ClearSplineMesh`)
  (`self.UpdateSpline`)
  (`self.UpdateSplineMesh` bSetAsValid))

(fn `UpdateLaserLengthFromLineTrace`
  (returns (OutFoundValidHit :type Boolean))
  (locals (Loc_TraceHit :type "HitResult Structure") (Loc_FoundValidHit :type Boolean :default false))
  (bind (_bblockinghit _binitialoverlap _time _distance _location _impactpoint _normal _impactnormal _physmat _hitactor) (`GameplayStatics.BreakHitResult` (`local.Loc_TraceHit`)))
  ;[1 1 1] Trace Locally for Actors
  (bind (_outhit _returnvalue) (`KismetSystemLibrary.LineTraceSingle` (`SceneComponent.K2_GetComponentLocation` (`self.LaserRoot`)) (`SceneComponent.K2_GetComponentLocation` (`self.Direction`)) "TraceTypeQuery1" true (`|MakeArray` (`self.GetOwner`)) "None" false))
  (set `local.Loc_TraceHit` _outhit)
  (if _returnvalue
    (set `self.Last_TraceImpactPoint` _impactpoint)
    (set `self.Length_Base` _distance)
    (set `local.Loc_FoundValidHit` (`self.HasActorXRInteractionComponent` _hitactor))
    (else
      (set `self.Length_Base` (`self.LaserMaxRange`))))
  (set `self.Length_Modifier` 0.0) ; Ignore Lenght Modifier when Line Tracing
  (return (`local.Loc_FoundValidHit`)))

(fn `UpdateSpline`
  (bind _spline (`self.Spline`))
  (bind _returnvalue (* (`KismetMathLibrary.GetDirectionUnitVector` (`SceneComponent.K2_GetComponentLocation` (`self.LaserRoot`)) (`SceneComponent.K2_GetComponentLocation` (`self.Direction`))) (* (`self.GetModifiedXRLaserLenght`) 0.2)))
  (`SplineComponent.ClearSplinePoints` (`self.Spline`) true)
  (`|ExecutionSequence`
    (:`then_0`
      (`SplineComponent.AddSplinePoint` (`self.Spline`) (`SceneComponent.K2_GetComponentLocation` (`self.LaserRoot`)) "World" false))
    (:`then_1`
      ;[1 1 1] Midpoint based on distance to the Target
      (`SplineComponent.AddSplinePoint` _spline (+ _returnvalue (`SceneComponent.K2_GetComponentLocation` (`self.LaserRoot`))) "World" false)
      ;;[0 0 0] Smooth Tangent
      (`SplineComponent.SetTangentAtSplinePoint` _spline 1 (* _returnvalue 4.0) "World" false))
    (:`then_2`
      (`SplineComponent.AddSplinePoint` (`self.Spline`) (`self.CurrentTipLocation`) "World" true))
    (:`then_3`
      (return))))

(fn `UpdateSplineMesh`
  (params (InSetIsValid :type Boolean))
  (bind _spline (`self.Spline`))
  (`MaterialInstanceDynamic.SetScalarParameterValue` (`self.DynaMat_SplineMesh`) "Opacity" (select `bool` InSetIsValid :`false` 0.15 :`true` 0.5))
  ;[1 1 1] Set Spline MeshComponents
  (for _index (range (+ (- (`SplineComponent.GetNumberOfSplinePoints` (`self.Spline`)) 2) 1))
    (bind _returnvalue (`AddComponent|NODE_AddSplineMeshComponent-0` :`bManualAttachment` true :`RelativeTransform` (`KismetMathLibrary.MakeTransform` (0.0 0.0 0.0)))) ; Add new cylinder mesh
    (`PrimitiveComponent.SetMaterial` _returnvalue 0 (`self.DynaMat_SplineMesh`))
    (`KismetArrayLibrary.Array_Add` (`self.SplineMeshes`) _returnvalue)
    (bind _returnvalue_2 (+ _index 1))
    (`SplineMeshComponent.SetStartAndEnd` _returnvalue (`SplineComponent.GetLocationAtSplinePoint` (`self.Spline`) _index "Local") (`SplineComponent.GetTangentAtSplinePoint` _spline _index "Local") (`SplineComponent.GetLocationAtSplinePoint` (`self.Spline`) _returnvalue_2 "Local") (`SplineComponent.GetTangentAtSplinePoint` _spline _returnvalue_2 "Local") true) ; Set the tangents and position to build slightly bend the cylinder. All cylinders combined create a smooth arc.
  )
  (return))

(fn `UpdateTargetSphere`
  (params (bSetAsValid :type Boolean))
  (`|ExecutionSequence`
    (:`then_0`
      ;[0 0 0] Target Sphere Appearance
      (`MeshComponent.SetScalarParameterValueOnMaterials` (`self.TargetSphere`) "Opacity" (select `bool` (`local.bSetAsValid`) :`false` 0.15 :`true` 1.0 :!type "Float (single-precision)"))
      (`SceneComponent.SetWorldScale3D` (`self.TargetSphere`) (`KismetMathLibrary.Conv_DoubleToVector` (`KismetMathLibrary.MapRangeClamped` (`self.GetModifiedXRLaserLenght`) 100.0 (`self.LaserMaxRange`) 0.01 0.1))))
    (:`then_1`
      (`PrimitiveComponent.SetCollisionEnabled` (`self.XRInteractor`) (select `bool` (`local.bSetAsValid`) :`false` "NoCollision" :`true` "QueryOnly" :!type "ECollisionEnabled Enum")))))

(fn `UserConstructionScript`
  (`XRInteractorComponent.SetAssignedPhysicsConstraint` (`self.XRInteractor`) (`self.XRInteractor_PhysicsConstraint_Laser`)))
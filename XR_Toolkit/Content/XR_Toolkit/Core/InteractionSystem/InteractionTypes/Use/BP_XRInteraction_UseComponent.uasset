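; XR interaction component that gives an actor a replicated boolean use state, driven by interacting or hovering.
; Interaction start toggles the state, optionally reverting on end, while UseOnHover mode sets it from hover and disables laser snapping.
; Only the server writes the state, and its OnRep broadcasts OnUseStateChanged.
; An optional cooldown timer temporarily deactivates the component after interaction, and hovering can blend in a hand pose.
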(event `self.ReceiveBeginPlay`
  (if (`KismetSystemLibrary.IsServer`)
    (if (`self.bUseOnHover`)
      (`self.SetSnapXRLaserToActor` false))))

(event `self.OnLocalInteractionStart`
  (params (InInteractor :type "XRInteractorComponent Object Reference"))
  (if (not (`self.bUseOnHover`))
    (`self.SetUseState` (not (`self.UseState`)))
    (if (not (`self.GetIsContinuousInteraction`))
      (`self.ApplyCoolDown`))))

(event `self.OnLocalInteractionEnd`
  (params (InInteractor :type "XRInteractorComponent Object Reference"))
  (if (not (`self.bUseOnHover`))
    (`self.ApplyCoolDown`)
    (if (`self.bResetAfterInteractionEnd`)
      (`self.SetUseState` (not (`self.UseState`))))))

(event `ApplyCoolDown`
  (if (`self.HasCooldown`)
    (`self.SetActive` false)
    (bind _returnvalue (`KismetSystemLibrary.K2_SetTimerDelegate` (delegate `EndCooldown`) (`self.CooldownDuration`)))
    (set `self.CooldownTimer` _returnvalue)))

(event `EndCooldown`
  (`self.SetActive` true))

(event `self.OnLocalInteractionHovered`
  (params (bHovering :type Boolean) (HoveringXRInteractor :type "XRInteractorComponent Object Reference"))
  (`/Engine/EditorBlueprintResources/StandardMacros.DoOnce` false :!label _label
    (:`Completed`
      (`|ExecutionSequence`
        (:`then_0`
          (if (`self.bHasHoverHandPose`)
            (`/XR_Toolkit/XR_Toolkit/Core/FL/ML_XRToolkit_ComponentUtilities.XRInteraction_HoverHandPose` bHovering HoveringXRInteractor (`self.Hand Pose Hover`) (`self.Blend Start Range`) (`self.Fully Blended Range`) (`self.Max Hand Pose Blend Amount`))))
        (:`then_1`
          (if (`self.bUseOnHover`)
            (if bHovering
              (`self.SetUseState` true)
              (elif (`self.bResetAfterInteractionEnd`)
                (`self.SetUseState` false)))))
        (:`then_2`
          (goto _label :!via `Reset`))))))

(fn `GetUseState`
  (returns (UseState :type Boolean))
  (return (`self.UseState`)))

(fn `HasCooldown`
  (returns (ReturnValue :type Boolean))
  (return (> (`self.CooldownDuration`) 0.0)))

(fn `OnRep_State`
  (`self.OnUseStateChanged` (`self.UseState`)))

(fn `SetUseState`
  (params (State :type Boolean))
  (if (`KismetSystemLibrary.IsServer`)
    (if (!= (`local.State`) (`self.GetUseState`))
      (set `self.UseState` State))))
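; XR climbing component that lets the owning pawn pull itself around by a climb interactor.
; While climbing, Tick offsets the pawn by the dampened gap between the grab pivot and interactor, streaming its location through the pawn replication component when networked.
; Overlapping a tagged blocker actor pushes the pawn away and up, then ends the climb.
; Client start/end events toggle Tick and report climb state to the server, which multicasts it.
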(event `self.ReceiveBeginPlay`
  (`self.CacheRequiredVars`))

(event `self.ReceiveTick`
  (params (DeltaSeconds :type "Float (single-precision)"))
  (bind (_returnvalue _blockingactor) (`self.IsOverlappingClimbingBlocker`))
  (bind _owningpawn (`self.OwningPawn`))
  (bind _returnvalue_2 (`Actor.K2_GetActorLocation` (`self.OwningPawn`)))
  (bind (_returnvalue_x _returnvalue_y _returnvalue_z) (`KismetMathLibrary.BreakVector` (+ _returnvalue_2 (* (`KismetMathLibrary.GetDirectionUnitVector` (`Actor.K2_GetActorLocation` _blockingactor) _returnvalue_2) (`self.ClimbingBlockPushbackAmount`)))))
  ;[0 0 0] TICK
  (`self.ClimbInteractor`
    (:`then`
      (if _returnvalue
        ;[1 1 1] Push back and end climb grip
        (`/Engine/EditorBlueprintResources/StandardMacros.IsValid` _blockingactor
          (:`Is Valid`
            (`self.SetComponentTickEnabled` false)
            (`Actor.K2_SetActorLocation` (`self.OwningPawn`) (`KismetMathLibrary.MakeVector` _returnvalue_x _returnvalue_y (+ _returnvalue_z (`self.ClimbingBlockPushbackAmount`))) false false)
            (`self.Client_EndClimbing` (`self.ClimbInteractor`))))
        (else
          (`Actor.K2_AddActorWorldOffset` (`self.OwningPawn`) (* (- (`self.Pivot`) (`SceneComponent.K2_GetComponentLocation` (`self.ClimbInteractor`))) (`self.GetVelocityDampeningFactor`)) false false)
          (if (not (`KismetSystemLibrary.IsStandalone`))
            (`/XR_Toolkit/XR_Toolkit/Core/ReplicationSystem/BP_PawnReplicationSystem.Server_Continuous_SetPawnLocation` (`self.PawnReplicationComponent`) (`Actor.K2_GetActorLocation` _owningpawn) _owningpawn)))))
    (:`else`)))

(event `Client_StartClimbing`
  (params (RequestingClimbInteractor :type "XRInteractorComponent Object Reference") (ClimbedActor :type "Actor Object Reference"))
  ;[1 1 1] Climbing Events
  (if (`self.CanStartClimbing` RequestingClimbInteractor ClimbedActor)
    (`|ExecutionSequence`
      (:`then_0`
        (bind _output_get (set `self.ClimbInteractor` RequestingClimbInteractor))
        (set `self.Pivot` (`SceneComponent.K2_GetComponentLocation` _output_get))
        (`self.SetComponentTickEnabled` true))
      (:`then_1`
        (bind _output_get_2 (set `self.Climbed Actor` ClimbedActor))
        (`self.RequestClimbAudio` _output_get_2))
      (:`then_2`
        (`self.Server_SetClimbState` true)))))

(event `Client_EndClimbing`
  (params (RequestingClimbInteractor :type "XRInteractorComponent Object Reference"))
  ;[1 1 1] Climbing Events
  (if (== RequestingClimbInteractor (`self.ClimbInteractor`))
    (`|ExecutionSequence`
      (:`then_0`
        (`self.SetComponentTickEnabled` false)
        (set `self.ClimbInteractor` null))
      (:`then_1`
        (`self.RequestClimbAudio` (`self.Climbed Actor`) 1)
        (set `self.Climbed Actor` null))
      (:`then_2`
        (`self.Server_SetClimbState` true)))))

(event `Server_SetClimbState`
  (params (bIsClimbing :type Boolean))
  ;[1 1 1] Notifies
  (bind _output_get (set `self.bIsClimbing` bIsClimbing))
  (`self.Multicast_SetClimbState` _output_get))

(event `Multicast_SetClimbState`
  (params (bIsClimbing :type Boolean))
  ;[1 1 1] Notifies
  (if bIsClimbing
    (`self.OnClimbStarted`)
    (else
      (`self.OnClimbEnded`))))

(fn `CacheRequiredVars`
  (bind _returnvalue (`Actor.GetComponentByClass` (`self.GetOwner`) "/XR_Toolkit/XR_Toolkit/Core/ReplicationSystem/BP_PawnReplicationSystem.BP_PawnReplicationSystem_C"))
  (`|ExecutionSequence`
    (:`then_0`
      (bind _aspawn (cast `Pawn` (`self.GetOwner`))
        (:`then`
          (set `self.OwningPawn` _aspawn))
        (:`CastFailed`
          (`/XR_Toolkit/XR_Toolkit/Core/FL/FL_XRUtilityFunctions.CustomDebugWarning` "NewEnumerator0" self (`KismetSystemLibrary.GetDisplayName` self) " must be owned by a pawn."))))
    (:`then_1`
      (`/Engine/EditorBlueprintResources/StandardMacros.IsValid` _returnvalue
        (:`Is Valid`
          (set `self.PawnReplicationComponent` _returnvalue))
        (:`Is Not Valid`
          (`/XR_Toolkit/XR_Toolkit/Core/FL/FL_XRUtilityFunctions.CustomDebugWarning` "NewEnumerator0" self (`KismetSystemLibrary.GetDisplayName` self) "Requires a PawnReplicationComponent to work - add one to the owning pawn."))))))

(fn `CanStartClimbing`
  (params (RequestingClimbInteractor :type "Object Object Reference") (ClimbedActor :type "Object Object Reference"))
  (returns (ReturnValue :type Boolean))
  (return (and (`self.IsActive`) (`KismetSystemLibrary.IsValid` RequestingClimbInteractor) (`KismetSystemLibrary.IsValid` ClimbedActor))))

(fn `GetCurrentClimbInteractor`
  (returns (ClimbXRInteractor :type "XRInteractorComponent Object Reference"))
  (return (`self.ClimbInteractor`)))

(fn `GetVelocityDampeningFactor`
  (returns (VelocityDampeningFactor :type "Float (double-precision)"))
  (return (`self.VelocityDampeningFactor`)))

(fn `IsClimbActive`
  (returns (bIsClimbing :type Boolean))
  (return (`self.bIsClimbing`)))

(fn `IsOverlappingClimbableSurface`
  (params (Collision :type "PrimitiveComponent Object Reference"))
  (returns (bDoesOverlap :type Boolean) (OutActor :type "Actor Object Reference"))
  (for _array_element (`PrimitiveComponent.GetOverlappingActors` Collision null)
    (`/Engine/EditorBlueprintResources/StandardMacros.IsValid` (`Actor.GetComponentByClass` _array_element null)
      (:`Is Valid`
        (return true _array_element))))
  (return false null))

(fn `IsOverlappingClimbingBlocker`
  (returns (ReturnValue :type Boolean) (BlockingActor :type "Actor Object Reference"))
  (bind _returnvalue (`Actor.GetComponentByClass` (`self.OwningPawn`) "/Script/Engine.CapsuleComponent"))
  ;[1 1 1] Echtwelt Specific
  (`/Engine/EditorBlueprintResources/StandardMacros.IsValid` _returnvalue
    (:`Is Valid`
      (for _array_element (`PrimitiveComponent.GetOverlappingActors` _returnvalue null)
        (`/Engine/EditorBlueprintResources/StandardMacros.IsValid` _array_element
          (:`Is Valid`
            (for _array_element_2 (`self.ClimbingBlockTags`)
              (if (`KismetArrayLibrary.Array_Contains` (`Actor.Tags` _array_element) _array_element_2)
                (return true _array_element)
                (else
                  (return true null)))))
          (:`Is Not Valid`
            _))
        (return true null))
      (return false null))
    (:`Is Not Valid`
      (return true null))))

(fn `RequestClimbAudio`
  (params (`Climbed Actor` :type "Actor Object Reference") (XRAudioIndex :type Integer)))

(fn `SetVelocityDampeningFactor`
  (params (InVelocityDampeningFactor :type "Float (double-precision)"))
  (set `self.VelocityDampeningFactor` InVelocityDampeningFactor))
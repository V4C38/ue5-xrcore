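; BP_XRLocomotionSystemComponent is a locomotion component in the XR Toolkit that handles discrete rotation requests for its owning actor.
; RequestRotate uses the sign of the input axis to add or subtract a fixed RotationAngle from the owner's current yaw.
; It passes the target yaw through an OnExecuteRotate dispatcher rather than rotating the actor itself, and prints a warning when the component is inactive.
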(event `self.ReceiveBeginPlay`)

(fn `RequestRotate`
  (params (InputAxis_Value :type "Float (double-precision)"))
  (bind _rotationangle (`self.RotationAngle`))
  (bind (_returnvalue_roll _returnvalue_pitch _returnvalue_yaw) (`KismetMathLibrary.BreakRotator` (`Actor.K2_GetActorRotation` (`self.GetOwner`))))
  (if (`self.IsActive`)
    (if (> InputAxis_Value 0.0)
      (`self.OnExecuteRotate` (+ _returnvalue_yaw _rotationangle))
      (else
        (`self.OnExecuteRotate` (- _returnvalue_yaw _rotationangle))))
    (else
      (`KismetSystemLibrary.PrintString` "Warning: Rotate requested but Component is disabled." true true (struct :`R` 1.0 :`G` 0.90008 :`A` 1.0) 1.0))))
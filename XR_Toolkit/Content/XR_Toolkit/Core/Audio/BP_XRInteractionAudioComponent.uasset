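; Audio component that plays sounds when its assigned XR interaction starts, ends or is hovered.
; It binds the interaction's events on BeginPlay and plays enabled sound waves from its interaction sound data with attenuation settings.
; Playback is limited to the locally controlled interactor unless audio replication is set.
; A short timer suppresses hover sounds after start or end, and hover audio can be restricted to laser interactors.
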(event `AssignXRInteraction`
  (params (AssignedXRInteraction :type "XRInteractionComponent Object Reference"))
  (`self.AssignedXRInteraction`
    (:`then`)
    (:`else`
      (set `self.AssignedXRInteraction` AssignedXRInteraction))))

(event `self.ReceiveBeginPlay`
  (bind _assignedxrinteraction (`self.AssignedXRInteraction`)
    (:`then`
      (add `XRInteractionComponent.OnInteractionStarted` _assignedxrinteraction (delegate `OnInteractionStarted`))
      (add `XRInteractionComponent.OnInteractionEnded` _assignedxrinteraction (delegate `OnInteractionEnded`))
      (add `XRInteractionComponent.OnInteractionHovered` _assignedxrinteraction (delegate `OnInteractionHovered_Event_0`)))
    (:`else`)))

(event `OnInteractionEnded`
  (params (Sender :type "XRInteractionComponent Object Reference") (XRInteractorComponent :type "XRInteractorComponent Object Reference"))
  (bind (_breplicatexrinteractionaudio _interactionstart _interactionend) (break `/XR_Toolkit/XR_Toolkit/Core/Audio/FXRInteractionAudioData` (`self.InteractionSoundData`)))
  (`self.Client_PlayAudio` XRInteractorComponent _interactionend _breplicatexrinteractionaudio)
  (`self.DelayHoverStart`))

(event `OnInteractionStarted`
  (params (Sender :type "XRInteractionComponent Object Reference") (XRInteractorComponent :type "XRInteractorComponent Object Reference"))
  (bind (_breplicatexrinteractionaudio _interactionstart) (break `/XR_Toolkit/XR_Toolkit/Core/Audio/FXRInteractionAudioData` (`self.InteractionSoundData`)))
  (`self.Client_PlayAudio` XRInteractorComponent _interactionstart _breplicatexrinteractionaudio)
  (`self.DelayHoverStart`))

(event `OnInteractionHovered_Event_0`
  (params (Sender :type "XRInteractionComponent Object Reference") (HoveringXRInteractor :type "XRInteractorComponent Object Reference") (bHovered :type Boolean))
  (bind (_breplicatexrinteractionaudio _interactionstart _interactionend _interactionhovered) (break `/XR_Toolkit/XR_Toolkit/Core/Audio/FXRInteractionAudioData` (`self.InteractionSoundData`)))
  (if (`self.CanPlayHoverSound` HoveringXRInteractor)
    (`self.Client_PlayAudio` HoveringXRInteractor _interactionhovered _breplicatexrinteractionaudio)))

(event `DelayHoverStart`
  ;[1 1 1] Prevent HoverSound from occuring directly after InteractionEnd
  (`KismetSystemLibrary.K2_ClearAndInvalidateTimerHandle` (`self.HoverTimer`))
  (set `self.bHoverCooldown` true)
  (bind _returnvalue (`KismetSystemLibrary.K2_SetTimerDelegate` (delegate `ReEnableHover`) 0.25))
  (set `self.HoverTimer` _returnvalue))

(event `ReEnableHover`
  ;[1 1 1] Prevent HoverSound from occuring directly after InteractionEnd
  (set `self.bHoverCooldown` false))

(fn `CanPlayHoverSound`
  (params (HoveringXRInteractor :type "XRInteractorComponent Object Reference"))
  (returns (bAllowed :type Boolean))
  (if (`self.bHoverCooldown`)
    (return false)
    (elif (`XRInteractorComponent.IsLaserInteractor` (`local.HoveringXRInteractor`))
      (return true)
      (elif (`self.bAllowHoverSoundOnlyForLaser`)
        (return false)
        (else
          (return true))))))

(fn `Client_PlayAudio`
  (params (InXRInteractor :type "XRInteractorComponent Object Reference") (InFXRAudioData :type "/XR_Toolkit/XR_Toolkit/Core/Audio/FXRAudioData Structure (by ref)") (InReplicateAudio :type Boolean))
  (bind (_infxraudiodata_enabled _infxraudiodata_sound _infxraudiodata_attenuationsettings) (break `/XR_Toolkit/XR_Toolkit/Core/Audio/FXRAudioData` (`local.InFXRAudioData`)))
  (if InReplicateAudio
    (if _infxraudiodata_enabled :!label _label
      (`self.PlaySingleSoundWave` _infxraudiodata_sound _infxraudiodata_attenuationsettings))
    (elif (`XRInteractorComponent.IsLocallyControlled` (`local.InXRInteractor`))
      (goto _label))))
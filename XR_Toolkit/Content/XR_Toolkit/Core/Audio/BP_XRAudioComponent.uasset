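; XR Toolkit audio component that plays one-shot sounds at its owning actor's location.
; Sounds are played directly or by index from AudioData, which skips invalid or disabled entries and supplies the sound and attenuation.
; Playback is gated by a Cooldown flag and starts a CooldownDuration timer, with ResetCooldown clearing the flag.
; None of the graphs shown sets Cooldown to true.
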(fn `PlaySingleSoundWave`
  (params (Sound :type "SoundBase Object Reference") (AttenuationSettings :type "SoundAttenuation Object Reference"))
  (if (not (`self.Cooldown`))
    (`self.StartCooldown`)
    (`GameplayStatics.PlaySoundAtLocation` Sound (`Actor.K2_GetActorLocation` (`self.GetOwner`)) (struct) 1.0 1.0 0.0 AttenuationSettings null null null)))

(fn `PlaySoundByAudioDataIndex`
  (params (InIndex :type Integer))
  (bind _audiodata (`self.AudioData`))
  (bind (_enabled _sound _attenuationsettings) (break `/XR_Toolkit/XR_Toolkit/Core/Audio/FXRAudioData` (`|GetArrayItem` _audiodata InIndex)))
  (if (and (`KismetArrayLibrary.Array_IsValidIndex` _audiodata InIndex) _enabled)
    (`self.PlaySingleSoundWave` _sound _attenuationsettings)))

(fn `ResetCooldown`
  (set `self.Cooldown` false))

(fn `StartCooldown`
  (bind _returnvalue (`KismetSystemLibrary.K2_SetTimerDelegate` (`|CreateDelegate` :!event `ResetCooldown`) (`self.CooldownDuration`)))
  (set `self.Timer_SingleSoundCooldown` _returnvalue))
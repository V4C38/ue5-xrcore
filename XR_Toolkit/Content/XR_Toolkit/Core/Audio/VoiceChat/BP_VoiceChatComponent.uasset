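; BP_VoiceChatComponent is an unfinished voice chat component for the XR pawn, with empty BeginPlay and Server_SendAudioData events.
; StopRecording saves submix output to a SoundWave and prints its name.
; Disconnected setup logic would add a server-side AudioCaptureComponent at the pawn's HeadContainer transform, send it to a voice chat submix, start recording and loop StopRecording on a timer.
; GetPawn caches the owning BP_XR_Pawn, warning if the cast fails.
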(event `self.ReceiveBeginPlay`)

(event `Stop Recording`
  (bind _returnvalue (`AudioMixerBlueprintLibrary.StopRecordingOutput` "SoundWave" "SoundWave" "/Game/_Cleanup/SoundRecordings" (`self.SubMix`) (`self.RecordedSound`)))
  (bind _output_get (set `self.RecordedSound` _returnvalue))
  (`KismetSystemLibrary.PrintString` (`KismetSystemLibrary.GetDisplayName` _output_get)))

(event `Server_SendAudioData`)
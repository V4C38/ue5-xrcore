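; XR Toolkit game mode that spawns and possesses a pawn for each player on login.
; Players using an HMD get the MR or VR pawn class based on the passthrough mode flag; others get a third-person debug pawn.
; Spawn transforms come from randomly chosen BP_XR_PlayerSpawnPoint actors.
; The optional existing-pawn replacement input on the XR spawn function is not wired into spawning.
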(event `self.K2_PostLogin`
  (params (NewPlayer :type "PlayerController Object Reference"))
  (bind _asbp_xr_player_controller (cast `/XR_Toolkit/XR_Toolkit/Core/Base/BP_XR_PlayerController` NewPlayer))
  (if (`/XR_Toolkit/XR_Toolkit/Core/Base/BP_XR_PlayerController.GetIsUsingHMD` _asbp_xr_player_controller)
    (`self.CreateAndPosess_XRPawn` NewPlayer (`self.Passthrpough Mode`))
    (else
      (`self.CreateAndPosess_Debug3PP Pawn` NewPlayer))))

(fn `CreateAndPosess_Debug3PP Pawn`
  (params (InPlayerController :type "PlayerController Object Reference"))
  (bind (_returnvalue_location _returnvalue_rotation) (`KismetMathLibrary.BreakTransform` (`self.GetTransform` (`self.GetRandomSpawnPoint`))))
  (bind _returnvalue (`|SpawnActorFromClass` "/XR_Toolkit/XR_Toolkit/Core/Base/BP_XRPawn_ThirdPerson.BP_XRPawn_ThirdPerson_C" (`KismetMathLibrary.MakeTransform` _returnvalue_location _returnvalue_rotation) "Undefined" "OverrideRootScale" InPlayerController null))
  (`Controller.Possess` InPlayerController _returnvalue))

(fn `CreateAndPosess_XRPawn`
  (params (InPlayerController :type "PlayerController Object Reference") (bInPassthrpoughMode :type Boolean) (Opt_ExistingPawnToReplace :type "Pawn Object Reference"))
  (bind _inplayercontroller (`local.InPlayerController`))
  (bind (_returnvalue_location _returnvalue_rotation) (`KismetMathLibrary.BreakTransform` (`self.GetTransform` (`self.GetRandomSpawnPoint`))))
  (bind _location (.location (`KismetMathLibrary.MakeTransform` _returnvalue_location _returnvalue_rotation)))
  (bind _rotation (.rotation (`KismetMathLibrary.MakeTransform` _returnvalue_location _returnvalue_rotation)))
  (bind _asbp_xr_player_controller (cast `/XR_Toolkit/XR_Toolkit/Core/Base/BP_XR_PlayerController` InPlayerController))
  (if (`/XR_Toolkit/XR_Toolkit/Core/Base/BP_XR_PlayerController.GetIsUsingHMD` _asbp_xr_player_controller)
    (if (`local.bInPassthrpoughMode`)
      (`|SpawnActorFromClass` (`self.MRPawnClass`) (`KismetMathLibrary.MakeTransform` _location _rotation) "Undefined" "OverrideRootScale" _inplayercontroller null)
      (`Controller.Possess` (`local.InPlayerController`) null)
      (else
        (`|SpawnActorFromClass` (`self.VRPawnClass`) (`KismetMathLibrary.MakeTransform` _location _rotation) "Undefined" "OverrideRootScale" _inplayercontroller null)
        (`Controller.Possess` (`local.InPlayerController`) null)))))

(fn `GetRandomSpawnPoint`
  (returns (Output :type "/XR_Toolkit/XR_Toolkit/Core/Base/Spawning/BP_XR_PlayerSpawnPoint Object Reference"))
  (bind _outactors (`GameplayStatics.GetAllActorsOfClass` "/XR_Toolkit/XR_Toolkit/Core/Base/Spawning/BP_XR_PlayerSpawnPoint.BP_XR_PlayerSpawnPoint_C"))
  (return (`|GetArrayItem` _outactors (`KismetMathLibrary.RandomInteger` (`KismetArrayLibrary.Array_Length` _outactors)))))

(fn `UserConstructionScript`)
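; Non-VR debug pawn for the XR Toolkit that stands in mouse input for XR controls.
; Mouse movement turns actor and camera, replicating through the pawn replication system and a server-to-multicast camera event.
; Left button drives laser, widget presses and interaction, or aborts teleport; right button teleports, or runs another interaction priority while lasing, with the wheel rotating the target.
; Interactions can suppress the laser, and UI input toggles the wrist menu.
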(event `self.ReceiveBeginPlay`
  (`/XR_Toolkit/XR_Toolkit/Core/FL/FL_XRUtilityFunctions.CustomDebugWarning` "NewEnumerator1" (`GameplayStatics.GetPlayerController` 0) "Non-VR Mode: Using " (`KismetSystemLibrary.GetDisplayName` self)))

(event `InputAxis|Mouse_X`
  (params (AxisValue :type "Float (single-precision)"))
  (bind (_returnvalue_roll _returnvalue_pitch _returnvalue_yaw) (`KismetMathLibrary.BreakRotator` (`self.K2_GetActorRotation`)))
  (bind _returnvalue (+ AxisValue _returnvalue_yaw))
  ;[1 1 1] Mouse Look & Rotate
  (`self.K2_SetActorRotation` self (`KismetMathLibrary.MakeRotator` 0.0 0.0 _returnvalue) false)
  (`/XR_Toolkit/XR_Toolkit/Core/ReplicationSystem/BP_PawnReplicationSystem.Server_ExecuteRotate` (`self.BP_PawnReplicationSystem`) (`KismetMathLibrary.MakeRotator` 0.0 0.0 _returnvalue) self))

(event `InputAxis|Mouse_Y`
  (params (AxisValue :type "Float (single-precision)"))
  (bind (_returnvalue_roll _returnvalue_pitch _returnvalue_yaw) (`KismetMathLibrary.BreakRotator` (`SceneComponent.K2_GetComponentRotation` (`self.Camera`))))
  (bind _returnvalue (`KismetMathLibrary.MakeRotator` _returnvalue_roll (+ AxisValue _returnvalue_pitch) _returnvalue_yaw))
  ;[1 1 1] Mouse Look & Rotate
  (`SceneComponent.K2_SetWorldRotation` (`self.Camera`) _returnvalue false false)
  (`self.Server_SetCameraRotation` _returnvalue self))

(event `InputAction|PrimaryInput_Right`
  (params (Key :type "Key Structure"))
  (bind _bp_xrlasercomponent (`self.BP_XRLaserComponent`))
  (bind _xrinteractor (`/XR_Toolkit/XR_Toolkit/Core/InteractionSystem/Laser/BP_XRLaserComponent.GetXRInteractor` (`self.BP_XRLaserComponent`)))
  (bind _xrinteractor_2 (`/XR_Toolkit/XR_Toolkit/Core/InteractionSystem/Laser/BP_XRLaserComponent.GetXRInteractor` (`self.BP_XRLaserComponent`)))
  (bind _output (`|GetArrayItem` (`XRInteractorComponent.GetGetClosestXRInteractions` _xrinteractor_2 1)))
  ;[1 1 1] LMB
  (:`Pressed`
    (set `self.bIsMLMBDown` true)
    (if (`/XR_Toolkit/XR_Toolkit/Core/LocomotionSystem/Teleportation/BP_XRTeleportSystemComponent.GetIsTeleportActive` (`self.BP_XRTeleportSystemComponent`))
      (`/XR_Toolkit/XR_Toolkit/Core/LocomotionSystem/Teleportation/BP_XRTeleportSystemComponent.Server_RequestTeleport_Abort` (`self.BP_XRTeleportSystemComponent`))
      (else
        (`/XR_Toolkit/XR_Toolkit/Core/InteractionSystem/Laser/BP_XRLaserComponent.Server_EnableLaser` (`self.BP_XRLaserComponent`))
        (`/XR_Toolkit/XR_Toolkit/Core/UI/BP_XRWidgetInteractionComponent.XRUI Input Press Pointer Key` (`self.BP_XRWidgetInteractionComponent`) _bp_xrlasercomponent _bp_xrlasercomponent)
        (if (`XRInteractorComponent.IsInteractionActive` _xrinteractor_2)
          ;[1 0 0] TEMP Workaround until XRLaser GoGo work has been done
          (`/Engine/EditorBlueprintResources/StandardMacros.IsValid` _xrinteractor_2
            (:`Is Valid`
              (`/Engine/EditorBlueprintResources/StandardMacros.IsValid` _output
                (:`Is Valid`
                  (`XRInteractionSystemComponent.Server_StartInteraction` (`self.XRInteractionSystem`) _output _xrinteractor_2)))))))))
  (:`Released`
    (set `self.bIsMLMBDown` false)
    (`/XR_Toolkit/XR_Toolkit/Core/InteractionSystem/Laser/BP_XRLaserComponent.Server_DisableLaser` (`self.BP_XRLaserComponent`))
    (`/XR_Toolkit/XR_Toolkit/Core/UI/BP_XRWidgetInteractionComponent.Input_ReleasePointerKey` (`self.BP_XRWidgetInteractionComponent`))
    (if (`XRInteractorComponent.IsInteractionActive` _xrinteractor)
      (`XRInteractionSystemComponent.Server_StopInteracting` (`self.XRInteractionSystem`) _xrinteractor 1))))

(event `Server_SetCameraRotation`
  (params (NewRotation :type "Rotator Structure") (Pawn :type "Pawn Object Reference"))
  ;[1 1 1] Mouse Look & Rotate
  ;;[0 0 0] Mouse Movement / Rotation
  (`self.Multicast_SetCameraRotation` NewRotation Pawn))

(event `InputAction|SecondaryInput_Right`
  (params (Key :type "Key Structure"))
  ;[1 1 1] RMB
  (:`Pressed`
    (if (`/XR_Toolkit/XR_Toolkit/Core/InteractionSystem/Laser/BP_XRLaserComponent.IsLaserActive` (`self.BP_XRLaserComponent`))
      (`XRInteractionSystemComponent.Server_StartInteracting` (`self.XRInteractionSystem`) (`/XR_Toolkit/XR_Toolkit/Core/InteractionSystem/Laser/BP_XRLaserComponent.GetXRInteractor` (`self.BP_XRLaserComponent`)) 0)
      (else
        (`/XR_Toolkit/XR_Toolkit/Core/LocomotionSystem/Teleportation/BP_XRTeleportSystemComponent.Server_RequestTeleport_Start` (`self.BP_XRTeleportSystemComponent`) "None" (`self.BP_XRLaserComponent`) (`self.Camera`)))))
  (:`Released`
    (if (`/XR_Toolkit/XR_Toolkit/Core/LocomotionSystem/Teleportation/BP_XRTeleportSystemComponent.GetIsTeleportActive` (`self.BP_XRTeleportSystemComponent`))
      (`/XR_Toolkit/XR_Toolkit/Core/LocomotionSystem/Teleportation/BP_XRTeleportSystemComponent.Server_RequestTeleport_Execute` (`self.BP_XRTeleportSystemComponent`)))
    (`XRInteractionSystemComponent.Server_StopInteracting` (`self.XRInteractionSystem`) (`/XR_Toolkit/XR_Toolkit/Core/InteractionSystem/Laser/BP_XRLaserComponent.GetXRInteractor` (`self.BP_XRLaserComponent`)) 0)))

(event `Multicast_SetCameraRotation`
  (params (NewRotation :type "Rotator Structure") (Pawn :type "Pawn Object Reference"))
  ;[1 1 1] Mouse Look & Rotate
  ;;[0 0 0] Mouse Movement / Rotation
  (if (not (`self.IsLocallyControlled` Pawn))
    (`SceneComponent.K2_SetWorldRotation` (`self.InteractionRoot`) NewRotation false false)))

(event `Key|MouseScrollUp`
  (params (Key :type "Key Structure"))
  (bind _bp_xrteleportsystemcomponent (`self.BP_XRTeleportSystemComponent`))
  (bind (_teleport_rotation_roll _teleport_rotation_pitch _teleport_rotation_yaw) (`KismetMathLibrary.BreakRotator` (`/XR_Toolkit/XR_Toolkit/Core/LocomotionSystem/Teleportation/BP_XRTeleportSystemComponent.GetTeleportRotation` _bp_xrteleportsystemcomponent)))
  ;[1 1 1] MouseWheel
  (:`Pressed`
    (if (`/XR_Toolkit/XR_Toolkit/Core/LocomotionSystem/Teleportation/BP_XRTeleportSystemComponent.GetIsTeleportActive` _bp_xrteleportsystemcomponent)
      (`/XR_Toolkit/XR_Toolkit/Core/LocomotionSystem/Teleportation/BP_XRTeleportSystemComponent.Server_RequestTeleport_SetRotation` _bp_xrteleportsystemcomponent (`KismetMathLibrary.MakeRotator` 0.0 0.0 (+ (`self.TeleportRotationIncrements`) _teleport_rotation_yaw))))))

(event `self.BP_XRTeleportSystemComponent.OnExecuteTeleport`
  (params (TeleportLocation :type "Vector Structure") (TeleportRotation :type "Rotator Structure"))
  ;[0 0 0] BPC PawnReplicationComponent
  (`/XR_Toolkit/XR_Toolkit/Core/ReplicationSystem/BP_PawnReplicationSystem.Server_ExecuteTeleport` (`self.BP_PawnReplicationSystem`) TeleportLocation TeleportRotation self))

(event `Key|MouseScrollDown`
  (params (Key :type "Key Structure"))
  (bind _bp_xrteleportsystemcomponent (`self.BP_XRTeleportSystemComponent`))
  (bind (_teleport_rotation_roll _teleport_rotation_pitch _teleport_rotation_yaw) (`KismetMathLibrary.BreakRotator` (`/XR_Toolkit/XR_Toolkit/Core/LocomotionSystem/Teleportation/BP_XRTeleportSystemComponent.GetTeleportRotation` _bp_xrteleportsystemcomponent)))
  ;[1 1 1] MouseWheel
  (:`Pressed`
    (if (`/XR_Toolkit/XR_Toolkit/Core/LocomotionSystem/Teleportation/BP_XRTeleportSystemComponent.GetIsTeleportActive` _bp_xrteleportsystemcomponent)
      (`/XR_Toolkit/XR_Toolkit/Core/LocomotionSystem/Teleportation/BP_XRTeleportSystemComponent.Server_RequestTeleport_SetRotation` _bp_xrteleportsystemcomponent (`KismetMathLibrary.MakeRotator` 0.0 0.0 (- _teleport_rotation_yaw (`self.TeleportRotationIncrements`)))))))

(event `InputAction|UI_Right`
  (params (Key :type "Key Structure"))
  (bind _bp_xrwristmenucomponent (`self.BP_XRWristMenuComponent`))
  ;[1 1 1] Player UI
  (:`Pressed`
    (`/XR_Toolkit/XR_Toolkit/Core/UI/XR_WristMenu/BP_XRWristMenuComponent.SetMenuActive` _bp_xrwristmenucomponent (not (`/XR_Toolkit/XR_Toolkit/Core/UI/XR_WristMenu/BP_XRWristMenuComponent.GetIsMenuActive` _bp_xrwristmenucomponent)))))

(event `self.BP_XRWristMenuComponent.OnXRWristMenuCommand`
  (params (Sender :type "/XR_Toolkit/XR_Toolkit/Core/UI/XR_WristMenu/BP_XRWristMenuComponent Object Reference") (CommandIdentifier :type String) (AdditionalData :type String))
  ;[1 1 1] Player UI
  (switch `string` CommandIdentifier
    (:`Close`
      (`/XR_Toolkit/XR_Toolkit/Core/UI/XR_WristMenu/BP_XRWristMenuComponent.SetMenuActive` (`self.BP_XRWristMenuComponent`) false))))

(event `self.XRInteractionSystem.OnInteractionStart`
  (params (Sender :type "XRInteractionSystemComponent Object Reference") (XRInteractionComponent :type "XRInteractionComponent Object Reference") (XRInteractorComponent :type "XRInteractorComponent Object Reference"))
  ;[1 1 1] Disable XRLaser when Interaction rrequests it
  (if (`XRInteractionComponent.GetSupressLaserWhenInteracting` XRInteractionComponent)
    (`/XR_Toolkit/XR_Toolkit/Core/InteractionSystem/Laser/BP_XRLaserComponent.Server_DisableLaser` (`self.BP_XRLaserComponent`))))

(event `self.XRInteractionSystem.OnInteractionEnd`
  (params (Sender :type "XRInteractionSystemComponent Object Reference") (XRInteractionComponent :type "XRInteractionComponent Object Reference") (XRInteractorComponent :type "XRInteractorComponent Object Reference"))
  ;[1 1 1] Disable XRLaser when Interaction rrequests it
  (if (`XRInteractionComponent.GetSupressLaserWhenInteracting` XRInteractionComponent)
    (if (`self.bIsMLMBDown`)
      (`/XR_Toolkit/XR_Toolkit/Core/InteractionSystem/Laser/BP_XRLaserComponent.Server_EnableLaser` (`self.BP_XRLaserComponent`)))))

(fn `UserConstructionScript`
  (`XRInteractorComponent.SetAssignedPhysicsConstraint` (`self.XRInteractor`) (`self.XRInteractor_PhysicsConstraint_NonVR`)))
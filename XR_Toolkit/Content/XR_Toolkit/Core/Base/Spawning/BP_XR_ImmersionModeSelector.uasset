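; Interactable selector that switches a player between VR and MR (passthrough) immersion in the XR toolkit.
; On interaction start, the server resolves the player controller from the interactor's owning pawn and has BP_XRGameMode replace that pawn using the trigger state as passthrough mode.
; A text label follows trigger state changes, initialized from the game mode's passthrough setting at BeginPlay, which warns if that game mode is absent.
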(event `self.ReceiveBeginPlay`
  (`parent.ReceiveBeginPlay`)
  (bind _asbp_xrgame_mode (cast `/XR_Toolkit/XR_Toolkit/Core/Base/BP_XRGameMode` (`GameplayStatics.GetGameMode`))
    (:`then`
      (bind _output_get (set `self.As BP XRGame Mode` _asbp_xrgame_mode))
      (`self.UpdateStateText` (`/XR_Toolkit/XR_Toolkit/Core/Base/BP_XRGameMode.Passthrpough Mode` _output_get)))
    (:`CastFailed`
      (`/XR_Toolkit/XR_Toolkit/Core/FL/FL_XRUtilityFunctions.CustomDebugWarning` "NewEnumerator1" self "XRGameMode not used: " "Cannot change immersion mode between VR and MR"))))

(event `self.XRInteractionTrigger.OnInteractionStarted`
  (params (Sender :type "XRInteractionComponent Object Reference") (XRInteractorComponent :type "XRInteractorComponent Object Reference"))
  (if (`KismetSystemLibrary.IsServer`)
    (bind (_asplayer_controller _aspawn) (`self.GetPlayerControllerFromXRInteractor` XRInteractorComponent))
    (`/Engine/EditorBlueprintResources/StandardMacros.IsValid` _asplayer_controller
      (:`Is Valid`
        (bind _as_bp_xrgame_mode (`self.As BP XRGame Mode`)
          (:`then`
            (`/XR_Toolkit/XR_Toolkit/Core/Base/BP_XRGameMode.CreateAndPosess_XRPawn` _as_bp_xrgame_mode _asplayer_controller (`XRInteractionTrigger.GetTriggerState` (`self.XRInteractionTrigger`)) _aspawn))
          (:`else`))))))

(event `self.XRInteractionTrigger.OnTriggerStateChanged`
  (params (Sender :type "XRInteractionTrigger Object Reference") (State :type Boolean))
  (`self.UpdateStateText` State))

(fn `GetPlayerControllerFromXRInteractor`
  (params (`XRInteractor Component` :type "XRInteractorComponent Object Reference"))
  (returns (`AsPlayer Controller` :type "PlayerController Object Reference") (AsPawn :type "Pawn Object Reference"))
  (bind _aspawn (cast `Pawn` (`KismetMathLibrary.SelectObject` (`ActorComponent.GetOwner` `XRInteractor Component`) (`ActorComponent.GetOwner` `XRInteractor Component`) (`XRInteractorComponent.IsLaserInteractor` `XRInteractor Component`))))
  (bind _asplayer_controller (cast `PlayerController` (`Pawn.GetController` _aspawn)))
  (return _asplayer_controller _aspawn))

(fn `UpdateStateText`
  (params (bState :type Boolean))
  (`TextRenderComponent.K2_SetText` (`self.Text_State`) (select `bool` bState :`false` "Off - VR" :`true` "On - MR")))

(fn `UserConstructionScript`)
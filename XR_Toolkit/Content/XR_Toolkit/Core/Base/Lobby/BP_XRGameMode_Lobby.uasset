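; BP_XRGameMode_Lobby is the lobby game mode of the XR Toolkit, providing the pawns that players control in the lobby.
; One function spawns the XR lobby pawn and another spawns a non-VR lobby pawn for third-person debugging.
; Each places its pawn at a random spawn point, sets the player controller as owner and possesses it.
; The event graph holds only disabled placeholder events.
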(fn `CreateAndPosess_Debug3PP Pawn`
  (params (InPlayerController :type "PlayerController Object Reference"))
  (bind (_returnvalue_location _returnvalue_rotation) (`KismetMathLibrary.BreakTransform` (`self.GetTransform` (`self.GetRandomSpawnPoint`))))
  (bind _returnvalue (`|SpawnActorFromClass` "/XR_Toolkit/XR_Toolkit/Core/Base/Lobby/BP_XR_NonVR_Pawn_Lobby.BP_XR_NonVR_Pawn_Lobby_C" (`KismetMathLibrary.MakeTransform` _returnvalue_location _returnvalue_rotation) "Undefined" "OverrideRootScale" InPlayerController null))
  (`Controller.Possess` InPlayerController _returnvalue))

(fn `CreateAndPosess_XRPawn`
  (params (InPlayerController :type "PlayerController Object Reference"))
  (bind (_returnvalue_location _returnvalue_rotation) (`KismetMathLibrary.BreakTransform` (`self.GetTransform` (`self.GetRandomSpawnPoint`))))
  (bind _returnvalue (`|SpawnActorFromClass` "/XR_Toolkit/XR_Toolkit/Core/Base/Lobby/BP_XR_Pawn_Lobby.BP_XR_Pawn_Lobby_C" (`KismetMathLibrary.MakeTransform` _returnvalue_location _returnvalue_rotation) "Undefined" "OverrideRootScale" InPlayerController null))
  (`Controller.Possess` InPlayerController _returnvalue))

(fn `UserConstructionScript`
  (`parent.UserConstructionScript`))
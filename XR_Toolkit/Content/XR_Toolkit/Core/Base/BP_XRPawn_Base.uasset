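; Base VR pawn for the XR Toolkit that sets up input, hands and head replication for a player.
; BeginPlay adds the XR input mapping context, has the server spawn replicated left and right BP_XRHand actors, and links the camera to the head replicator.
; RepNotifies on the hand references set each hand's side and attach it to its motion controller for the local player.
; Helper functions look up hands, lasers and interactors by side.
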(event `self.ReceiveBeginPlay`
  ;[0 0 0] Initial Setup
  (`|ExecutionSequence`
    (:`then_0`
      ;;[1 1 1] Setup Input
      (bind _asplayer_controller (cast `PlayerController` (`self.GetController`)))
      (bind _returnvalue (pcsubsystem `EnhancedInputLocalPlayerSubsystem` _asplayer_controller))
      (`/Engine/EditorBlueprintResources/StandardMacros.IsValid` _returnvalue
        (:`Is Valid`
          (`EnhancedInputSubsystemInterface.AddMappingContext` _returnvalue "/XR_Toolkit/XR_Toolkit/Core/InputActions/InputMappingContext_XRTools.InputMappingContext_XRTools" 0 (struct)))))
    (:`then_1`
      (if (`KismetSystemLibrary.IsServer`)
        (`self.Server_SpawnXRHands`)))
    (:`then_2`
      ;;[1 1 1] Setup Head Replication
      (`/XR_Toolkit/XR_Toolkit/Core/ReplicationSystem/BP_ProxyComponentReplicator.Init Components` (`self.BP_ProxyComponentReplicator_Head`) self (`self.Camera`) (`self.Head_Container`)))
    (:`then_3`
      (`/XR_Toolkit/XR_Toolkit/Core/Utilities/FL_XRUtilityFunctions.CustomDebugWarning` "NewEnumerator3" (`GameplayStatics.GetPlayerController` 0) "VR Mode: Using " (`KismetSystemLibrary.GetDisplayName` self)))))

(event `Server_SpawnXRHands`
  ;[1 1 1] Spawn XRHands
  (`|ExecutionSequence`
    (:`then_0`
      (bind _returnvalue (`|SpawnActorFromClass` "/XR_Toolkit/XR_Toolkit/Core/Hands/BP_XRHand.BP_XRHand_C" (`KismetMathLibrary.MakeTransform` (0.0 0.0 0.0)) "Undefined" "MultiplyWithRoot" self null))
      (bind _output_get (set `self.XRHand_Right` _returnvalue))
      (`self.SetReplicates` _output_get true)
      (set `/XR_Toolkit/XR_Toolkit/Core/Hands/BP_XRHand.ControllerHand` "Right" _returnvalue))
    (:`then_1`
      (bind _returnvalue_2 (`|SpawnActorFromClass` "/XR_Toolkit/XR_Toolkit/Core/Hands/BP_XRHand.BP_XRHand_C" (`KismetMathLibrary.MakeTransform` (0.0 0.0 0.0)) "Undefined" "MultiplyWithRoot" self null))
      (bind _output_get_2 (set `self.XRHand_Left` _returnvalue_2))
      (`self.SetReplicates` _output_get_2 true)
      (set `/XR_Toolkit/XR_Toolkit/Core/Hands/BP_XRHand.ControllerHand` "Left" _returnvalue_2))))

(fn `Get XRInteractor By Hand`
  (params (InControllerHand :type "EControllerHand Enum" :default "Left"))
  (returns (OutXRInteractor :type "XRInteractorComponent Object Reference"))
  (bind _xrhand_right (`self.XRHand_Right`))
  (bind _xrhand_left (`self.XRHand_Left`))
  (switch `/XR_Toolkit/XR_Toolkit/Core/Utilities/EN_SimplifiedControllerHand` (`/XR_Toolkit/XR_Toolkit/Core/Utilities/FL_XRUtilityFunctions.SimplifyControllerHand` InControllerHand)
    (:`NewEnumerator0`
      (`/Engine/EditorBlueprintResources/StandardMacros.IsValid` _xrhand_left
        (:`Is Valid`
          (return (`/XR_Toolkit/XR_Toolkit/Core/Hands/BP_XRHand.XRInteractor` _xrhand_left)))))
    (:`NewEnumerator1`
      (`/Engine/EditorBlueprintResources/StandardMacros.IsValid` _xrhand_right
        (:`Is Valid`
          (return (`/XR_Toolkit/XR_Toolkit/Core/Hands/BP_XRHand.XRInteractor` _xrhand_right)))))))

(fn `Get XRLaser By Hand`
  (params (InControllerHand :type "EControllerHand Enum" :default "Left"))
  (returns (OutXRLaserComponent :type "/XR_Toolkit/XR_Toolkit/Core/Laser/BP_XRLaserComponent Object Reference"))
  (bind _returnvalue (`self.GetXRHand` InControllerHand))
  (bind _bp_xrlasercomponent (`/XR_Toolkit/XR_Toolkit/Core/Hands/BP_XRHand.BP_XRLaserComponent` _returnvalue))
  (`/Engine/EditorBlueprintResources/StandardMacros.IsValid` _returnvalue
    (:`Is Valid`
      (`/Engine/EditorBlueprintResources/StandardMacros.IsValid` _bp_xrlasercomponent
        (:`Is Valid`
          (return _bp_xrlasercomponent))
        (:`Is Not Valid`
          _)))
    (:`Is Not Valid`
      _))
  (`/XR_Toolkit/XR_Toolkit/Core/Utilities/FL_XRUtilityFunctions.CustomDebugWarning` "NewEnumerator0" self "Failed to return valid XRLaser for XRHand: ")
  (return null))

(fn `GetXRHand`
  (params (InControllerHand :type "EControllerHand Enum" :default "Left"))
  (returns (ReturnValue :type "/XR_Toolkit/XR_Toolkit/Core/Hands/BP_XRHand Object Reference"))
  (return (select `/XR_Toolkit/XR_Toolkit/Core/Utilities/EN_SimplifiedControllerHand` (`/XR_Toolkit/XR_Toolkit/Core/Utilities/FL_XRUtilityFunctions.SimplifyControllerHand` InControllerHand) :`NewEnumerator0` (`self.XRHand_Left`) :`NewEnumerator1` (`self.XRHand_Right`))))

(fn `OnRep_XRHand_Left`
  (`|ExecutionSequence`
    (:`then_0`
      (`/XR_Toolkit/XR_Toolkit/Core/Hands/BP_XRHand.Server_SetControllerHand` (`self.XRHand_Left`) "Left"))
    (:`then_1`
      (if (`self.IsLocallyControlled`)
        (`self.K2_AttachToComponent` (`self.XRHand_Left`) (`self.MotionController_L`) "None" "SnapToTarget" "SnapToTarget" "KeepWorld" true)))))

(fn `OnRep_XRHand_Right`
  (`|ExecutionSequence`
    (:`then_0`
      (if (`KismetSystemLibrary.IsServer`)
        (`/XR_Toolkit/XR_Toolkit/Core/Hands/BP_XRHand.Server_SetControllerHand` (`self.XRHand_Right`) "Right")))
    (:`then_1`
      (if (`self.IsLocallyControlled`)
        (`self.K2_AttachToComponent` (`self.XRHand_Right`) (`self.MotionController_R`) "None" "SnapToTarget" "SnapToTarget" "KeepWorld" true)))))

(fn `UserConstructionScript`)
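; Network component in the XR Toolkit replication system that assigns ownership of its actor to a player controller.
; On BeginPlay, a server-only helper polls for player controller index 0, retrying after a short delay until it is valid.
; It then sets that controller as the actor's owner and fires the authority-received dispatcher through a notify event, passing itself.
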(event `self.ReceiveBeginPlay`
  (bind _validplayercontroller (`self.Server_GetPlayerController`)
    (:`Out_Exec`
      (`Actor.SetOwner` (`self.GetOwner`) _validplayercontroller)
      (`self.PRIVATE_Server_NotifyClients`))))

(event `PRIVATE_Server_NotifyClients`
  (`self.Server_OnAuthorityReceived` self))
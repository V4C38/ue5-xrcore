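; Actor component that replicates an XR pawn's head, hands, controller hand animation and movement in multiplayer.
; Once a locally controlled pawn registers, Tick sends camera, controller and input data through Server-to-Multicast RPCs onto pawn containers and hand AnimBPs.
; Teleport, rotation and continuous movement share that relay; continuous movement moves the local pawn only when client-server mismatch exceeds a threshold.
; Hand-tracking gesture replication is an unimplemented stub.
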(event `self.ReceiveTick`
  (params (DeltaSeconds :type "Float (single-precision)"))
  (`|ExecutionSequence`
    (:`then_0`
      ;[1 1 1] Update Pawn Transform
      (`self.Server_UpdatePawnTransformData` (`self.GetLocalPawnTransformData`)))
    (:`then_1`
      ;[1 1 1] Update Pawn Hands
      (`self.Server_UpdateControllerHandPoses` (`self.GetLocalControllerHandData`)))))

(event `Server_ExecuteTeleport`
  (params (NewLocation :type "Vector Structure") (NewRotation :type "Rotator Structure") (Pawn :type "Pawn Object Reference"))
  ;[1 1 1] Teleportation (Called by TeleportComponent or manually)
  (`self.Multicast_ExecuteTeleport` NewLocation NewRotation Pawn))

(event `Server_UpdateControllerHandPoses`
  (params (ControllerHandData :type "/XR_Toolkit/XR_Toolkit/Core/ReplicationSystem/FControllerHandData_BP Structure"))
  ;[1 1 1] Network_UpdateHandAnimation
  (`self.Multicast_UpdateControllerHandPoses` ControllerHandData))

(event `Multicast_UpdateControllerHandPoses`
  (params (ControllerHandData :type "/XR_Toolkit/XR_Toolkit/Core/ReplicationSystem/FControllerHandData_BP Structure"))
  ;[1 1 1] Network_UpdateHandAnimation
  (`self.ApplyControllerHandPoses` ControllerHandData))

(event `Server_UpdatePawnTransformData`
  (params (PawnTransformData :type "/XR_Toolkit/XR_Toolkit/Core/ReplicationSystem/FPawnTransformData_BP Structure"))
  ;[1 1 1] ApplyPawnComponentsTransformData
  ; - Head
  ; - Hands
  (`self.Multicast_UpdatePawnTransformData` PawnTransformData))

(event `Multicast_ExecuteTeleport`
  (params (NewLocation :type "Vector Structure") (NewRotation :type "Rotator Structure") (Pawn :type "Pawn Object Reference"))
  ;[1 1 1] Teleportation (Called by TeleportComponent or manually)
  (`Actor.K2_SetActorLocationAndRotation` Pawn NewLocation NewRotation false false)
  (if (`Pawn.IsLocallyControlled` Pawn)
    (`HeadMountedDisplayFunctionLibrary.ResetOrientationAndPosition` 0.0)))

(event `Multicast_UpdatePawnTransformData`
  (params (PawnTransformData :type "/XR_Toolkit/XR_Toolkit/Core/ReplicationSystem/FPawnTransformData_BP Structure"))
  ;[1 1 1] ApplyPawnComponentsTransformData
  ; - Head
  ; - Hands
  (`self.ApplyPawnTransformData` PawnTransformData))

(event `Server_UpdateHandTrackingGesture`
  (params (HandSide :type Byte :default 0) (NewHandGesture :type "EXRHandTrackingGesture Enum" :default "None"))
  ;[1 1 1] Network_UpdateHandAnimation
)

(event `Multicast_UpdateHandTrackingGesture`
  (params (HandSide :type Byte :default 0) (NewHandGesture :type "EXRHandTrackingGesture Enum" :default "None"))
  ;[1 1 1] Network_UpdateHandAnimation
)

(event `Server_ExecuteRotate`
  (params (NewRotation :type "Rotator Structure") (Pawn :type "Pawn Object Reference"))
  ;[1 1 1] Rotation (Called by TeleportComponent or manually)
  (`self.Multicast_ExecuteRotate` NewRotation Pawn))

(event `Server_Continuous_SetPawnLocation`
  (params (NewLocation :type "Vector Structure") (Pawn :type "Pawn Object Reference"))
  ;[1 1 1] Continuous Movement
  ; Will not update the Locally Controlled pawn unless the discrepancy between Server and the Local Client exceeds the treshold (MaxLocationServerClientMismatch)
  (`self.Multicast_Continuous_SetPawnLocation` NewLocation Pawn (`Actor.K2_GetActorLocation` Pawn)))

(event `Multicast_Continuous_SetPawnLocation`
  (params (NewLocation :type "Vector Structure") (Pawn :type "Pawn Object Reference") (ServerLocation :type "Vector Structure"))
  ;[1 1 1] Continuous Movement
  ; Will not update the Locally Controlled pawn unless the discrepancy between Server and the Local Client exceeds the treshold (MaxLocationServerClientMismatch)
  (if (`Pawn.IsLocallyControlled` Pawn)
    (if (not (`self.DoesClientMatchServerLocation` NewLocation ServerLocation))
      (`Actor.K2_SetActorLocation` Pawn NewLocation false false))
    (else
      (`Actor.K2_SetActorLocation` Pawn NewLocation false false))))

(event `Multicast_ExecuteRotate`
  (params (NewRotation :type "Rotator Structure") (Pawn :type "Pawn Object Reference"))
  ;[1 1 1] Rotation (Called by TeleportComponent or manually)
  (if (not (`Pawn.IsLocallyControlled` Pawn))
    (if (!= NewRotation (`Actor.K2_GetActorRotation` Pawn) :`ErrorTolerance` 0.1)
      (`Actor.K2_SetActorRotation` Pawn NewRotation false))
    (if (`Pawn.IsLocallyControlled` Pawn)
      (`HeadMountedDisplayFunctionLibrary.ResetOrientationAndPosition` 0.0 "Position"))))

(fn `ApplyControllerHandPoses`
  (params (ControllerHandData :type "/XR_Toolkit/XR_Toolkit/Core/ReplicationSystem/FControllerHandData_BP Structure"))
  (bind _xrpawn (`self.XRPawn`))
  (bind (_controllerhanddata_input_grip_r _controllerhanddata_input_grip_l _controllerhanddata_input_trigger_r _controllerhanddata_input_trigger_l _controllerhanddata_input_trigger_r_touch _controllerhanddata_input_trigger_l_touch) (break `/XR_Toolkit/XR_Toolkit/Core/ReplicationSystem/FControllerHandData_BP` (`local.ControllerHandData`)))
  (bind _animbp_hand_r (`/XR_Toolkit/XR_Toolkit/Core/Base/BP_XRPawn_Base.AnimBP_Hand_R` _xrpawn))
  (bind _animbp_hand_l (`/XR_Toolkit/XR_Toolkit/Core/Base/BP_XRPawn_Base.AnimBP_Hand_L` _xrpawn))
  (bind _xrpawn_2 (`self.XRPawn`)
    (:`then`
      (if (and (`KismetSystemLibrary.IsValid` (`/XR_Toolkit/XR_Toolkit/Core/Base/BP_XRPawn_Base.AnimBP_Hand_L` _xrpawn_2)) (`KismetSystemLibrary.IsValid` (`/XR_Toolkit/XR_Toolkit/Core/Base/BP_XRPawn_Base.AnimBP_Hand_R` _xrpawn_2)))
        (set `/XR_Toolkit/XR_Toolkit/Assets/Meshes/HandModel/ABP_XROculusHand.Input_Grip` _controllerhanddata_input_grip_r _animbp_hand_r)
        (set `/XR_Toolkit/XR_Toolkit/Assets/Meshes/HandModel/ABP_XROculusHand.Input_Grip` _controllerhanddata_input_grip_l _animbp_hand_l)
        (set `/XR_Toolkit/XR_Toolkit/Assets/Meshes/HandModel/ABP_XROculusHand.Input_Trigger` _controllerhanddata_input_trigger_r _animbp_hand_r)
        (set `/XR_Toolkit/XR_Toolkit/Assets/Meshes/HandModel/ABP_XROculusHand.Input_Trigger` _controllerhanddata_input_trigger_l _animbp_hand_l)
        (set `/XR_Toolkit/XR_Toolkit/Assets/Meshes/HandModel/ABP_XROculusHand.Input_Trigger_Touch` _controllerhanddata_input_trigger_r_touch _animbp_hand_r)
        (set `/XR_Toolkit/XR_Toolkit/Assets/Meshes/HandModel/ABP_XROculusHand.Input_Trigger_Touch` _controllerhanddata_input_trigger_l_touch _animbp_hand_l)))
    (:`else`)))

(fn `ApplyPawnTransformData`
  (params (PawnTransformData :type "/XR_Toolkit/XR_Toolkit/Core/ReplicationSystem/FPawnTransformData_BP Structure"))
  (bind (_pawntransformdata_head_location _pawntransformdata_head_rotation _pawntransformdata_rhand_location _pawntransformdata_rhand_rotation _pawntransformdata_lhand_location _pawntransformdata_lhand_rotation) (break `/XR_Toolkit/XR_Toolkit/Core/ReplicationSystem/FPawnTransformData_BP` (`local.PawnTransformData`)))
  (bind (_pawntransformdata_head_location_2 _pawntransformdata_head_rotation_2) (break `/XR_Toolkit/XR_Toolkit/Core/ReplicationSystem/FPawnTransformData_BP` (`local.PawnTransformData`)))
  (bind (_pawntransformdata_head_location_3 _pawntransformdata_head_rotation_3 _pawntransformdata_rhand_location_2 _pawntransformdata_rhand_rotation_2) (break `/XR_Toolkit/XR_Toolkit/Core/ReplicationSystem/FPawnTransformData_BP` (`local.PawnTransformData`)))
  (`self.XRPawn`
    (:`then`
      (`|ExecutionSequence`
        (:`then_0`
          (`SceneComponent.K2_SetWorldTransform` (`/XR_Toolkit/XR_Toolkit/Core/Base/BP_XRPawn_Base.Head_Container` (`self.XRPawn`)) (`KismetMathLibrary.MakeTransform` _pawntransformdata_head_location_2 _pawntransformdata_head_rotation_2) false false))
        (:`then_1`
          (`SceneComponent.K2_SetWorldTransform` (`/XR_Toolkit/XR_Toolkit/Core/Base/BP_XRPawn_Base.MotionController_Container_R` (`self.XRPawn`)) (`KismetMathLibrary.MakeTransform` _pawntransformdata_rhand_location_2 _pawntransformdata_rhand_rotation_2) false false))
        (:`then_2`
          (`SceneComponent.K2_SetWorldTransform` (`/XR_Toolkit/XR_Toolkit/Core/Base/BP_XRPawn_Base.MotionController_Container_L` (`self.XRPawn`)) (`KismetMathLibrary.MakeTransform` _pawntransformdata_lhand_location _pawntransformdata_lhand_rotation) false false))))
    (:`else`)))

(fn `DeRegisterXRPawn`
  (set `self.XRPawn` null)
  (`self.SetComponentTickEnabled` false))

(fn `DoesClientMatchServerLocation`
  (params (ClientLocation :type "Vector Structure") (ServerLocation :type "Vector Structure"))
  (returns (ReturnValue :type Boolean))
  (return (== ClientLocation ServerLocation :`ErrorTolerance` (`self.MaxLocationServerClientMismatch`))))

(fn `GetLocalControllerHandData`
  (returns (OutControllerHandData :type "/XR_Toolkit/XR_Toolkit/Core/ReplicationSystem/FControllerHandData_BP Structure"))
  (bind _xrpawn (`self.XRPawn`)
    (:`then`
      (return (make `/XR_Toolkit/XR_Toolkit/Core/ReplicationSystem/FControllerHandData_BP` (`/XR_Toolkit/XR_Toolkit/Core/Base/BP_XRPawn_Base.Input_Get_R_Grip` _xrpawn) (`/XR_Toolkit/XR_Toolkit/Core/Base/BP_XRPawn_Base.Input_Get_L_Grip` _xrpawn) (`/XR_Toolkit/XR_Toolkit/Core/Base/BP_XRPawn_Base.Input_Get_R_Trigger` _xrpawn) (`/XR_Toolkit/XR_Toolkit/Core/Base/BP_XRPawn_Base.Input_Get_L_Trigger` _xrpawn) (`/XR_Toolkit/XR_Toolkit/Core/Base/BP_XRPawn_Base.Input_Get_R_TriggerTouch` _xrpawn) (`/XR_Toolkit/XR_Toolkit/Core/Base/BP_XRPawn_Base.Input_Get_L_TriggerTouch` _xrpawn))))
    (:`else`)))

(fn `GetLocalHandTrackingData`)

(fn `GetLocalPawnTransformData`
  (returns (OutPawnTransformData :type "/XR_Toolkit/XR_Toolkit/Core/ReplicationSystem/FPawnTransformData_BP Structure"))
  (bind _xrpawn (`self.XRPawn`))
  (bind _motioncontroller_l (`/XR_Toolkit/XR_Toolkit/Core/Base/BP_XRPawn_Base.MotionController_L` _xrpawn))
  (bind _motioncontroller_r (`/XR_Toolkit/XR_Toolkit/Core/Base/BP_XRPawn_Base.MotionController_R` _xrpawn))
  (bind _camera (`/XR_Toolkit/XR_Toolkit/Core/Base/BP_XRPawn_Base.Camera` _xrpawn))
  (return (make `/XR_Toolkit/XR_Toolkit/Core/ReplicationSystem/FPawnTransformData_BP` (`SceneComponent.K2_GetComponentLocation` _camera) (`SceneComponent.K2_GetComponentRotation` _camera) (`SceneComponent.K2_GetComponentLocation` _motioncontroller_r) (`SceneComponent.K2_GetComponentRotation` _motioncontroller_r) (`SceneComponent.K2_GetComponentLocation` _motioncontroller_l) (`SceneComponent.K2_GetComponentRotation` _motioncontroller_l))))

(fn `Register XRPawn`
  (params (XRPawn :type "/XR_Toolkit/XR_Toolkit/Core/Base/BP_XRPawn_Base Object Reference"))
  (bind _output_get (set `self.XRPawn` XRPawn))
  (`/Engine/EditorBlueprintResources/StandardMacros.IsValid` _output_get
    (:`Is Valid`
      (if (`Pawn.IsLocallyControlled` _output_get)
        (`self.SetComponentTickEnabled` true)))
    (:`Is Not Valid`
      (`/XR_Toolkit/XR_Toolkit/Core/FL/FL_XRUtilityFunctions.CustomDebugWarning` "NewEnumerator1" self "Registered Pawn is not valid. Replication can not be initialized."))))
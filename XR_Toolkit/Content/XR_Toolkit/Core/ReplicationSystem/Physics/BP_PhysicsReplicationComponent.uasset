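; Component that smooths manually replicated physics actor transforms on clients in the XR Toolkit.
; Received transforms become a target that Tick interpolates the owner toward with teleporting moves, using the config's ReplicationInterval as speed, until replication ends.
; Client and server events toggle physics simulation on the stored static meshes.
; Registration with the manual replication system and the body of InitializePhysicsOnOwner are disconnected, so neither runs.
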(event `self.ReceiveBeginPlay`
  (if (not (`KismetSystemLibrary.IsServer`))
    (set `self.OwningPlayer` (`GameplayStatics.GetPlayerController` 0))))

(event `OnReplicatePhysicsActor`
  (params (NewTransform :type "Transform Structure (by ref)"))
  (set `self.ServerTargetTransform` NewTransform)
  (if (not (`self.IsComponentTickEnabled`))
    (`self.SetComponentTickEnabled` true))
  (`/XR_Toolkit/XR_Toolkit/Core/FL/FL_XRUtilityFunctions.CustomDebugWarning` "NewEnumerator3" (`self.GetOwner` self) " transform was replicated (Pysics)"))

(event `Client_SetReplicatePhysics`
  (params (bReplicatePhysics :type Boolean) (bClientSimulatePhysics :type Boolean))
  (`/Engine/EditorBlueprintResources/StandardMacros.IsValid` (`self.OwningPlayer`)
    (:`Is Valid`
      (`|ExecutionSequence`
        (:`then_0`
          (`self.SetOwnerSimulatePhysics` bClientSimulatePhysics))))))

(event `OnEndReplication`
  (`self.SetComponentTickEnabled` false)
  (`/XR_Toolkit/XR_Toolkit/Core/FL/FL_XRUtilityFunctions.CustomDebugWarning` "NewEnumerator3" (`self.GetOwner` self) "was removed from replication on client: " (`KismetSystemLibrary.GetDisplayName` (`self.OwningPlayer`))))

(event `SetOwnerSimulatePhysics`
  (params (Simulate :type Boolean))
  (for _array_element (`self.PhysicsStaticMeshes`)
    (`PrimitiveComponent.SetSimulatePhysics` _array_element Simulate)))

(event `self.ReceiveTick`
  (params (DeltaSeconds :type "Float (single-precision)"))
  (`Actor.K2_SetActorTransform` (`self.GetOwner`) (`KismetMathLibrary.TInterpTo` (`Actor.GetTransform` (`self.GetOwner`)) (`self.ServerTargetTransform`) DeltaSeconds (`.ReplicationInterval` (`/XR_Toolkit/XR_Toolkit/Core/FL/FL_XRUtilityFunctions.GetPhysicsConfig`))) false true))

(event `OnServer_SetOwnerSimulatePhysics`
  (params (InputPin :type Boolean))
  (if (`KismetSystemLibrary.IsServer`)
    (for _array_element (`self.PhysicsStaticMeshes`)
      (`PrimitiveComponent.SetSimulatePhysics` _array_element InputPin))))

(fn `Initialize Physics on Owner`
  (params (PhysicsStaticMeshes :type "Array of StaticMeshComponent Object Reference") (UseDefaultSettings :type Boolean)))
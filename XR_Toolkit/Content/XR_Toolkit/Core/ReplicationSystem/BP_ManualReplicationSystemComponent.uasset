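; XR Toolkit component that manually replicates actor transforms from the server, covering registered physics actors and on-request syncs for non-physics actors, such as on late join.
; The server ticks at a configured interval, snapshots each registered component's owner transform and multicasts the list.
; Receivers pass the server transform to the physics replication component only where its owning client is locally controlled and drift exceeds configured tolerances.
; On-request syncs multicast a teleport to the server transform.
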(event `self.ReceiveBeginPlay`
  ;[0.3646 0.3646 0.3646] Init
  ; Only Tick on Server
  (if (`KismetSystemLibrary.IsServer`)
    (`self.SetComponentTickEnabled` true)
    (`self.SetComponentTickInterval` (`.ReplicationInterval` (`/XR_Toolkit/XR_Toolkit/Core/FL/FL_XRUtilityFunctions.GetPhysicsConfig`)))))

(event `Server_AuthorizeActorRPCs`
  (params (Actor :type "Actor Object Reference"))
  (`Actor.SetOwner` Actor (`GameplayStatics.GetPlayerController` 0)))

(event `self.ReceiveTick`
  (params (DeltaSeconds :type "Float (single-precision)"))
  (`self.ReplicatePhysicsActors`))

(event `Client_RequestActorTransformReplication`
  (params (ActorToReplicate :type "Actor Object Reference"))
  (`self.Server_RequestActorTransformReplication` ActorToReplicate))

(event `Server_RequestActorTransformReplication`
  (params (ActorToReplicate :type "Actor Object Reference"))
  ;[1 1 1] Manual Replicate (non Physics - LateJoin)
  (`self.Multicast_ManualActorReplication` ActorToReplicate (`Actor.GetTransform` ActorToReplicate)))

(event `Multicast_ReplicatePhysicsTransforms`
  (params (RegisteredPhysicsReplicationComponents :type "Array of /XR_Toolkit/XR_Toolkit/Core/ReplicationSystem/Physics/FPhysicsReplicationData Structure (by ref)"))
  ;[1 1 1] Physics Actors
  (for _array_element RegisteredPhysicsReplicationComponents
    (`self.Validated Replicate` _array_element)))

(event `Multicast_ManualActorReplication`
  (params (ActorToReplicate :type "Actor Object Reference") (ServerTransform :type "Transform Structure"))
  ;[1 1 1] Manual Replicate (non Physics - LateJoin)
  (`Actor.K2_SetActorTransform` ActorToReplicate ServerTransform false true))

(event `Server_RegisterForPhysicsReplication`
  (params (PhysicsReplicationComponent :type "/XR_Toolkit/XR_Toolkit/Core/ReplicationSystem/Physics/FPhysicsReplicationData Structure (by ref)"))
  (bind (_physicsreplicationcomponent _owningclient) (break `/XR_Toolkit/XR_Toolkit/Core/ReplicationSystem/Physics/FPhysicsReplicationData` PhysicsReplicationComponent))
  ;[1 1 1] Physics Actors
  (`KismetArrayLibrary.Array_AddUnique` (`self.RegisteredPhysicsReplicationComponents`) PhysicsReplicationComponent)
  (`self.Validated Replicate` PhysicsReplicationComponent)
  (`/XR_Toolkit/XR_Toolkit/Core/FL/FL_XRUtilityFunctions.CustomDebugWarning` "NewEnumerator3" (`self.GetOwner` _physicsreplicationcomponent) "Replicating Physics" (`KismetSystemLibrary.GetDisplayName` _owningclient)))

(event `Server_DeregisterFromPhysicsReplication`
  (params (PhysicsReplicationComponent :type "/XR_Toolkit/XR_Toolkit/Core/ReplicationSystem/Physics/FPhysicsReplicationData Structure (by ref)"))
  (bind (_physicsreplicationcomponent _owningclient) (break `/XR_Toolkit/XR_Toolkit/Core/ReplicationSystem/Physics/FPhysicsReplicationData` PhysicsReplicationComponent))
  ;[1 1 1] Physics Actors
  (`KismetArrayLibrary.Array_RemoveItem` (`self.RegisteredPhysicsReplicationComponents`) PhysicsReplicationComponent)
  (`/XR_Toolkit/XR_Toolkit/Core/FL/FL_XRUtilityFunctions.CustomDebugWarning` "NewEnumerator3" (`self.GetOwner` _physicsreplicationcomponent) "Stop Replicating Physics" (`KismetSystemLibrary.GetDisplayName` _owningclient)))

(fn `ReplicatePhysicsActors`
  (for (_array_element _array_index) (`self.RegisteredPhysicsReplicationComponents`)
    (bind (_physicsreplicationcomponent _owningclient) (break `/XR_Toolkit/XR_Toolkit/Core/ReplicationSystem/Physics/FPhysicsReplicationData` _array_element))
    (`KismetArrayLibrary.Array_Set` (`self.RegisteredPhysicsReplicationComponents`) _array_index (make `/XR_Toolkit/XR_Toolkit/Core/ReplicationSystem/Physics/FPhysicsReplicationData` _physicsreplicationcomponent _owningclient (`Actor.GetTransform` (`self.GetOwner` _physicsreplicationcomponent)))))
  (`self.Multicast_ReplicatePhysicsTransforms` (`self.RegisteredPhysicsReplicationComponents`)))

(fn `RequestActorTransformReplication`
  (params (ActorToReplicate :type "Actor Object Reference"))
  (`self.Client_RequestActorTransformReplication` ActorToReplicate))

(fn `Validated Replicate`
  (params (PhysicsReplicationData :type "/XR_Toolkit/XR_Toolkit/Core/ReplicationSystem/Physics/FPhysicsReplicationData Structure (by ref)"))
  (bind (_defaultlineardamping _defaultangulardamping _replicationinterval _replication_locationtolerance _replication_rotationtolerance) (`/XR_Toolkit/XR_Toolkit/Core/FL/FL_XRUtilityFunctions.GetPhysicsConfig`))
  (bind (_physicsreplicationdata_physicsreplicationcomponent _physicsreplicationdata_owningclient _physicsreplicationdata_currentservertransform) (break `/XR_Toolkit/XR_Toolkit/Core/ReplicationSystem/Physics/FPhysicsReplicationData` (`local.PhysicsReplicationData`)))
  (bind (_physicsreplicationdata_physicsreplicationcomponent_2 _physicsreplicationdata_owningclient_2 _physicsreplicationdata_currentservertransform_2) (break `/XR_Toolkit/XR_Toolkit/Core/ReplicationSystem/Physics/FPhysicsReplicationData` (`local.PhysicsReplicationData`)))
  (`/Engine/EditorBlueprintResources/StandardMacros.IsValid` _physicsreplicationdata_owningclient_2
    (:`Is Valid`
      (if (`Controller.IsLocalController` _physicsreplicationdata_owningclient_2)
        (if (not (`KismetMathLibrary.NearlyEqual_TransformTransform` (`Actor.GetTransform` (`self.GetOwner` _physicsreplicationdata_physicsreplicationcomponent_2)) _physicsreplicationdata_currentservertransform_2 _replication_locationtolerance _replication_rotationtolerance))
          (`/XR_Toolkit/XR_Toolkit/Core/ReplicationSystem/Physics/BP_PhysicsReplicationComponent.OnReplicatePhysicsActor` _physicsreplicationdata_physicsreplicationcomponent _physicsreplicationdata_currentservertransform))))))
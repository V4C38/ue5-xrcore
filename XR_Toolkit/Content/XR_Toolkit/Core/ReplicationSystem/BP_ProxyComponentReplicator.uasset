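; BP_ProxyComponentReplicator mirrors a locally controlled pawn's source component transform onto a proxy target component for remote clients.
; InitComponents hides the target as configured, attaches it to the source locally and registers it with the server.
; OnRep_TargetComponent enables ticking, throttled to the replication interval on the sender.
; The sender's tick sends world location and rotation to the server, while receivers interpolate the target toward that data.
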(event `Server_SetTargetComponent`
  (params (TargetComponent :type "SceneComponent Object Reference"))
  (set `self.TargetComponent` TargetComponent))

(event `Server_ReplicateLocalToRemote`
  (params (InTargetData :type "/XR_Toolkit/XR_Toolkit/Core/ReplicationSystem/FLocationAndRotation Structure"))
  (set `self.TargetData` InTargetData))

(event `self.ReceiveTick`
  (params (DeltaSeconds :type "Float (single-precision)"))
  (bind _sourcecomponent (`self.SourceComponent`))
  (bind (_targetdata_location _targetdata_rotation) (break `/XR_Toolkit/XR_Toolkit/Core/ReplicationSystem/FLocationAndRotation` (`self.TargetData`)))
  (bind _targetcomponent (`self.TargetComponent`))
  (if (`self.bIsLocalComponent`)
    ;[1 1 1] Set Component Location directly on Sending Client
    (`self.Server_ReplicateLocalToRemote` (make `/XR_Toolkit/XR_Toolkit/Core/ReplicationSystem/FLocationAndRotation` (`SceneComponent.K2_GetComponentLocation` _sourcecomponent) (`SceneComponent.K2_GetComponentRotation` _sourcecomponent)))
    (else
      ;[1 1 1] Interpolate to Target on Receiving Client
      (`SceneComponent.K2_SetWorldLocationAndRotation` (`self.TargetComponent`) (`KismetMathLibrary.VInterpTo` (`SceneComponent.K2_GetComponentLocation` _targetcomponent) _targetdata_location DeltaSeconds 5.0) (`KismetMathLibrary.RInterpTo` (`SceneComponent.K2_GetComponentRotation` _targetcomponent) _targetdata_rotation DeltaSeconds 5.0) false false))))

(fn `Init Components`
  (params (RequestingPawn :type "Pawn Object Reference") (InLocalSource :type "SceneComponent Object Reference") (InRemoteTarget :type "SceneComponent Object Reference"))
  (if (and (`KismetSystemLibrary.IsValid` RequestingPawn) (`KismetSystemLibrary.IsValid` InLocalSource) (`KismetSystemLibrary.IsValid` InRemoteTarget))
    (bind _output_get (set `self.bIsLocalComponent` (`Pawn.IsLocallyControlled` (`local.RequestingPawn`))))
    (if _output_get
      ;[1 1 1] Initialize Replication on the Sending Client
      (`|ExecutionSequence`
        (:`then_0`
          (`SceneComponent.SetHiddenInGame` (`local.InRemoteTarget`) (`self.bTargetHiddenOnLocal`) false)
          (`SceneComponent.K2_AttachToComponent` (`local.InRemoteTarget`) (`self.SourceComponent`) "None" "SnapToTarget" "SnapToTarget" "KeepWorld" true))
        (:`then_1`
          (set `self.SourceComponent` (`local.InLocalSource`)))
        (:`then_2`
          (`self.Server_SetTargetComponent` (`local.InRemoteTarget`)))))))

(fn `OnRep_TargetComponent`
  (`|ExecutionSequence`
    (:`then_0`
      (if (`self.bIsLocalComponent`)
        (`self.SetComponentTickInterval` (`self.ReplicationInterval`))
        (else
          (`self.SetComponentTickInterval` 0.0))))
    (:`then_1`
      (`self.SetComponentTickEnabled` (`KismetSystemLibrary.IsValid` (`self.TargetComponent`))))))
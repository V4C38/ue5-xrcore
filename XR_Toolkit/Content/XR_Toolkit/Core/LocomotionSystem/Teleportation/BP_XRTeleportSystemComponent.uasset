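; Pawn component that coordinates networked XR teleportation, from aiming through execute or abort.
; The locally controlled pawn has the server spawn a replicated BP_XRTeleportOrigin, which traces for valid locations while the component ticks during aiming.
; Start, rotate, execute and abort requests run as server-to-multicast RPCs, with aiming shown remotely only if indicator replication is enabled.
; Dispatchers report active state, hand and valid destination, leaving the actual move to listeners.
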(event `self.ReceiveBeginPlay`
  (bind _aspawn (cast `Pawn` (`self.GetOwner`)))
  (bind _output_get (set `self.bIsLocalTeleporter` (`Pawn.IsLocallyControlled` _aspawn)))
  (if _output_get
    (`self.Server_SpawnXRTeleportOrigin`)))

(event `self.ReceiveTick`
  (params (DeltaSeconds :type "Float (single-precision)"))
  (`self.BP_XRTeleportOrigin`
    (:`then`
      (`/XR_Toolkit/XR_Toolkit/Core/LocomotionSystem/Teleportation/BP_XRTeleportOrigin.TraceTeleportLocation` (`self.BP_XRTeleportOrigin`)))
    (:`else`)))

(event `Server_SpawnXRTeleportOrigin`
  ;[1 1 1] Spawn TeleportOrigin
  (`self.BP_XRTeleportOrigin`
    (:`then`)
    (:`else`
      (bind _returnvalue (`|SpawnActorFromClass` "/XR_Toolkit/XR_Toolkit/Core/LocomotionSystem/Teleportation/BP_XRTeleportOrigin.BP_XRTeleportOrigin_C" (`KismetMathLibrary.MakeTransform` (0.0 0.0 0.0)) "Undefined" "OverrideRootScale" (`self.GetOwner`) (`self.TeleportReadySpeed`) (`self.TeleportRotation`) (`self.AllowTeleportOnActorsWithTags`) null))
      (`Actor.SetReplicates` _returnvalue true)
      (set `self.BP_XRTeleportOrigin` _returnvalue))))

(event `Server_RequestTeleport_Start`
  (params (InRequestingHand :type "EXRHandType Enum" :default "None") (RootComponent :type "SceneComponent Object Reference") (PlayerCamera :type "SceneComponent Object Reference"))
  ;[1 1 1] Request Start
  (set `self.TeleportHand` InRequestingHand)
  (`self.Multicast_RequestTeleport_Start` RootComponent PlayerCamera))

(event `Multicast_RequestTeleport_Start`
  (params (RootComponent :type "SceneComponent Object Reference") (PlayerCamera :type "SceneComponent Object Reference"))
  (bind (_returnvalue_roll _returnvalue_pitch _returnvalue_yaw) (`KismetMathLibrary.BreakRotator` (`SceneComponent.K2_GetComponentRotation` PlayerCamera)))
  ;[1 1 1] Request Start
  (if (`self.IsActive`)
    (if (`self.IsTeleporterVisibleOnThisClient`)
      (`self.SetComponentTickEnabled` true)
      (`|ExecutionSequence`
        (:`then_0`
          (bind _bp_xrteleportorigin (`self.BP_XRTeleportOrigin`)
            (:`then`
              (`Actor.K2_AttachToComponent` _bp_xrteleportorigin RootComponent "None" "SnapToTarget" "SnapToTarget" "KeepRelative" false))
            (:`else`)))
        (:`then_1`
          (bind _bp_xrteleportorigin_2 (`self.BP_XRTeleportOrigin`)
            (:`then`
              (`/XR_Toolkit/XR_Toolkit/Core/LocomotionSystem/Teleportation/BP_XRTeleportOrigin.InitializeTeleport` _bp_xrteleportorigin_2)
              (`self.Server_RequestTeleport_SetRotation` (`KismetMathLibrary.MakeRotator` 0.0 0.0 _returnvalue_yaw)))
            (:`else`)))
        (:`then_2`
          (bind _output_get (set `self.bIsTeleportActive` true))
          (`self.OnTeleportActive` _output_get (`self.TeleportHand`)))))
    (else
      (`self.Server_RequestTeleport_Abort`))))

(event `Server_RequestTeleport_Execute`
  ;[1 1 1] Execute Teleport
  (`self.Multicast_RequestTeleport_Execute`))

(event `Multicast_RequestTeleport_Execute`
  (bind (_trace_result_is_valid_location _teleportlocation _teleportrotation) (`/XR_Toolkit/XR_Toolkit/Core/LocomotionSystem/Teleportation/BP_XRTeleportOrigin.GetTeleportData` (`self.BP_XRTeleportOrigin`)))
  ;[1 1 1] Execute Teleport
  (if (`self.bIsTeleportActive`)
    (`self.SetComponentTickEnabled` false)
    (if (`/XR_Toolkit/XR_Toolkit/Core/LocomotionSystem/Teleportation/BP_XRTeleportOrigin.IsTeleportAllowed` (`self.BP_XRTeleportOrigin`))
      (`|ExecutionSequence`
        (:`then_0`
          (`/XR_Toolkit/XR_Toolkit/Core/LocomotionSystem/Teleportation/BP_XRTeleportOrigin.StopXRTeleportOrigin` (`self.BP_XRTeleportOrigin`) :!label _label))
        (:`then_1`
          (if _trace_result_is_valid_location
            (`self.OnExecuteTeleport` _teleportlocation _teleportrotation))
          (bind _output_get (set `self.bIsTeleportActive` false :!label _label_2))
          (`self.OnTeleportActive` _output_get (`self.TeleportHand`))))
      (else
        (`|ExecutionSequence`
          (:`then_0`
            (goto _label))
          (:`then_1`
            (goto _label_2)))))))

(event `Server_RequestTeleport_SetRotation`
  (params (TeleportRotation :type "Rotator Structure"))
  ;[1 1 1] Rotation
  (bind _output_get (set `self.TeleportRotation` TeleportRotation))
  (`self.Multicast_RequestTeleport_SetRotation` _output_get))

(event `Multicast_RequestTeleport_SetRotation`
  (params (TeleportRotation :type "Rotator Structure"))
  ;[1 1 1] Rotation
  (bind _bp_xrteleportorigin (`self.BP_XRTeleportOrigin`)
    (:`then`
      (`/XR_Toolkit/XR_Toolkit/Core/LocomotionSystem/Teleportation/BP_XRTeleportOrigin.SetTeleportRotation` _bp_xrteleportorigin TeleportRotation))
    (:`else`)))

(event `Server_RequestTeleport_Abort`
  ;[1 1 1] Abort
  (`self.Multicast_RequestTeleport_Abort`))

(event `Multicast_RequestTeleport_Abort`
  ;[1 1 1] Abort
  (bind _bp_xrteleportorigin (`self.BP_XRTeleportOrigin`)
    (:`then`
      (`/XR_Toolkit/XR_Toolkit/Core/LocomotionSystem/Teleportation/BP_XRTeleportOrigin.StopXRTeleportOrigin` _bp_xrteleportorigin)
      (`self.SetComponentTickEnabled` false)
      (bind _output_get (set `self.bIsTeleportActive` false))
      (`self.OnTeleportActive` _output_get (`self.TeleportHand`)))
    (:`else`)))

(fn `CanTeleport`
  (returns (Allowed :type Boolean))
  (return (not (`self.bIsTeleportActive`))))

(fn `GetIsTeleportActive`
  (returns (bTeleportActive :type Boolean))
  (return (`self.bIsTeleportActive`)))

(fn `GetTeleportHand`
  (returns (OutTeleportingHand :type "EXRHandType Enum"))
  (return (`self.TeleportHand`)))

(fn `GetTeleportRotation`
  (returns (`Teleport Rotation` :type "Rotator Structure"))
  (return (`self.TeleportRotation`)))

(fn `IsTeleporterVisibleOnThisClient`
  (returns (bIsVisibleOnClient :type Boolean))
  (return (or (`self.bReplicateTeleportationIndicator`) (`self.bIsLocalTeleporter`))))
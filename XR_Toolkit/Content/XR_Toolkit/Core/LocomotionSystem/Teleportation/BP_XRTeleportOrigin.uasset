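; XR teleport origin actor that traces and draws the teleport arc and landing indicator, and supplies destination, rotation and validity.
; A predicted projectile path feeds a spline, rebuilt as spline meshes on each trace; hit actors need a valid tag.
; On initialization, timelines animate the arc material, then scale up the landing cylinder before allowing teleport.
; Build-up speed varies with target distance, playing faster for nearby targets.
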(event `self.ReceiveBeginPlay`
  (`self.GetDynaMat`))

(event `self.ReceiveTick`
  (params (DeltaSeconds :type "Float (single-precision)"))
  (bind (_traceresult_pathpoints _traceresult_lasttracedestination _traceresult_bisvalidlocation) (break `/XR_Toolkit/XR_Toolkit/Core/LocomotionSystem/Teleportation/FTeleportTraceResult_BP` (`self.TraceResult`)))
  (`self.SetVisualIndicatorMaterials` _traceresult_bisvalidlocation))

(event `InitializeTeleport`
  ;[1 1 1] Teleport Arc and Location PopUp
  (`|ExecutionSequence`
    (:`then_0`
      (set `self.bAllowTeleport` false)
      (set `self.Timer_InitializeTeleport` (struct))
      (`self.SetActorHiddenInGame` false)
      (`self.SetActorTickEnabled` false)
      (`self.SetVisualIndicatorMaterials` false)
      (`SceneComponent.SetRelativeScale3D` (`self.TeleportCylinder`) (0.0 0.0 0.0)))
    (:`then_1`
      (`TimelineComponent.SetPlayRate` (`self.Timeline_BuildUp`) (* (`self.InitializePlayRate`) (`self.Get Distance Based Buildup Factor`)))
      (bind (_direction _curve_range _beamopacity) (`Timeline|Timeline_BuildUp` :!via `PlayFromStart`)
        (:`Update`
          (bind _output_get (`self.GetDynaMat`))
          (`MaterialInstanceDynamic.SetScalarParameterValue` _output_get "DistanceDivider" (* _curve_range (`self.VisibilityRange`)))
          (`MaterialInstanceDynamic.SetScalarParameterValue` _output_get "Emissive" _beamopacity))
        (:`Finished`
          (`TimelineComponent.SetPlayRate` (`self.Timeline_ScaleUp`) 7.0)
          (bind (_direction_2 _teleportcircle_scale) (`Timeline|Timeline_ScaleUp` :!via `PlayFromStart`)
            (:`Update`
              (`SceneComponent.SetRelativeScale3D` (`self.TeleportCylinder`) (`KismetMathLibrary.Conv_DoubleToVector` _teleportcircle_scale)))
            (:`Finished`
              (`self.SetActorTickEnabled` true)
              (set `self.bAllowTeleport` true))))))))

(fn `CheckActorForValidTags`
  (params (InActorToCheck :type "Actor Object Reference"))
  (returns (bHasValidTag :type Boolean))
  (locals (bLocal_FoundTag :type Boolean :default false))
  (`/Engine/EditorBlueprintResources/StandardMacros.IsValid` InActorToCheck
    (:`Is Valid`
      (for _array_element (`Actor.Tags` InActorToCheck)
        (if (`KismetArrayLibrary.Array_Contains` (`self.ValidTraceTags`) _array_element)
          (set `local.bLocal_FoundTag` true)))
      (return (`local.bLocal_FoundTag`)))))

(fn `ClearArc`
  (bind _splinemeshes (`self.SplineMeshes`))
  (`ActorComponent.K2_DestroyComponent` _splinemeshes)
  (`KismetArrayLibrary.Array_Clear` _splinemeshes)
  (`SplineComponent.ClearSplinePoints` (`self.ArcSpline`) true))

(fn `Get Distance Based Buildup Factor`
  (returns (OutPlayRate :type "Float (double-precision)"))
  (bind _quickteleportdistancetreshold (`self.QuickTeleportDistanceTreshold`))
  (bind _arcdirection (`self.ArcDirection`))
  (bind _quickteleportdistancetreshold_2 (`self.QuickTeleportDistanceTreshold`))
  (bind _outhit (`GameplayStatics.Blueprint_PredictProjectilePath_ByObjectType` :`StartPos` (`SceneComponent.K2_GetComponentLocation` _arcdirection) :`LaunchVelocity` (* (`SceneComponent.GetForwardVector` _arcdirection) (`self.TeleportLaunchVelocity`)) :`ObjectTypes` (`|MakeArray` "ObjectTypeQuery1" "ObjectTypeQuery2" "ObjectTypeQuery4" :!type "EObjectTypeQuery Enum") :`SimFrequency` 30.0)) ; Simulate throwing a projectile (including gravity) to find a teleport location.
  (bind _returnvalue (`KismetMathLibrary.Vector_Distance` (`.ImpactPoint` (`GameplayStatics.BreakHitResult` _outhit)) (`SceneComponent.K2_GetComponentLocation` (`self.ArcDirection`))))
  (return (`KismetMathLibrary.MapRangeClamped` _returnvalue _quickteleportdistancetreshold_2 (* _quickteleportdistancetreshold_2 5.0) (select `bool` (< _returnvalue _quickteleportdistancetreshold) :`false` 1.0 :`true` (`KismetMathLibrary.MapRangeClamped` _returnvalue 0.0 _quickteleportdistancetreshold 5.0 1.0)) 0.75)))

(fn `GetDynaMat`
  (returns (Output_Get :type "MaterialInstanceDynamic Object Reference"))
  (bind _dynamat_arc (`self.DynaMat_Arc`)
    (:`then`
      (return _dynamat_arc))
    (:`else`
      (bind _returnvalue (`KismetMaterialLibrary.CreateDynamicMaterialInstance` "/XR_Toolkit/XR_Toolkit/Assets/MaterialLibrary/InteractionDefaults/Teleportation/MI_TeleportSpline.MI_TeleportSpline"))
      (bind _output_get (set `self.DynaMat_Arc` _returnvalue))
      (return _output_get))))

(fn `GetTeleportData`
  (returns (`Trace Result Is Valid Location` :type Boolean) (TeleportLocation :type "Vector Structure") (TeleportRotation :type "Rotator Structure"))
  (bind (_traceresult_pathpoints _traceresult_lasttracedestination _traceresult_bisvalidlocation) (break `/XR_Toolkit/XR_Toolkit/Core/LocomotionSystem/Teleportation/FTeleportTraceResult_BP` (`self.TraceResult`)))
  (return _traceresult_bisvalidlocation _traceresult_lasttracedestination (`self.TeleportRotation`)))

(fn `IsTeleportAllowed`
  (returns (bAllowTeleport :type Boolean))
  (return (`self.bAllowTeleport`)))

(fn `SetTeleportRotation`
  (params (TeleportRotation :type "Rotator Structure"))
  (set `self.TeleportRotation` TeleportRotation))

(fn `Setup Visual Teleport Indicators`
  (bind _teleportcylinder (`self.TeleportCylinder`))
  (bind (_traceresult_pathpoints _traceresult_lasttracedestination _traceresult_bisvalidlocation) (break `/XR_Toolkit/XR_Toolkit/Core/LocomotionSystem/Teleportation/FTeleportTraceResult_BP` (`self.TraceResult`)))
  (`|ExecutionSequence`
    (:`then_0`
      ;[0 0 0] Setup Arc
      (`self.ClearArc`)
      (`self.UpdateArc`))
    (:`then_1`
      ;[0 0 0] Only Set Circle visible when location is valid
      (`SceneComponent.SetVisibility` _teleportcylinder _traceresult_bisvalidlocation false)
      (`SceneComponent.SetVisibility` (`self.RotationIndicator`) _traceresult_bisvalidlocation false)
      (`SceneComponent.SetVisibility` (`self.Sphere_Tip`) _traceresult_bisvalidlocation false)
      (bind _output_get (set `self.LastValidLocation` _traceresult_lasttracedestination))
      (`SceneComponent.K2_SetWorldLocation` _teleportcylinder _output_get false false)
      (`SceneComponent.K2_SetWorldRotation` _teleportcylinder (`self.TeleportRotation`) false false))))

(fn `SetVisualIndicatorMaterials`
  (params (bCanTeleport :type Boolean))
  (bind _returnvalue (select `bool` bCanTeleport :`false` 0.1 :`true` 1.0))
  (`MeshComponent.SetScalarParameterValueOnMaterials` (`self.TeleportCylinder`) "Emissive" _returnvalue)
  (bind _output_get (`self.GetDynaMat`))
  (`MaterialInstanceDynamic.SetScalarParameterValue` _output_get "Emissive" _returnvalue))

(fn `StopXRTeleportOrigin`
  (`self.SetActorHiddenInGame` true)
  (`self.SetActorTickEnabled` false)
  (`self.ClearArc`)
  (`KismetSystemLibrary.K2_ClearAndInvalidateTimerHandle` (`self.Timer_InitializeTeleport`)))

(fn `TraceTeleportLocation`
  (bind _arcdirection (`self.ArcDirection`))
  (bind (_traceresult_pathpoints _traceresult_lasttracedestination) (break `/XR_Toolkit/XR_Toolkit/Core/LocomotionSystem/Teleportation/FTeleportTraceResult_BP` (`self.TraceResult`)))
  (bind (_outhit _outpathpositions _outlasttracedestination _returnvalue) (`GameplayStatics.Blueprint_PredictProjectilePath_ByObjectType` (`SceneComponent.K2_GetComponentLocation` _arcdirection) (* (`SceneComponent.GetForwardVector` _arcdirection) (`self.TeleportLaunchVelocity`)) true 0.0 (`|MakeArray` "ObjectTypeQuery1" "ObjectTypeQuery2" "ObjectTypeQuery4" :!type "EObjectTypeQuery Enum") false (`|MakeArray` (`self.GetOwner`)) "None" 0.0 30.0)) ; Simulate throwing a projectile (including gravity) to find a teleport location.
  (if _returnvalue
    (bind (_bblockinghit _binitialoverlap _time _distance _location _impactpoint _normal _impactnormal _physmat _hitactor) (`GameplayStatics.BreakHitResult` _outhit))
    (set `self.TraceResult` (make `/XR_Toolkit/XR_Toolkit/Core/LocomotionSystem/Teleportation/FTeleportTraceResult_BP` _outpathpositions _impactpoint (`self.CheckActorForValidTags` _hitactor)))
    (else
      (set `self.TraceResult` (make `/XR_Toolkit/XR_Toolkit/Core/LocomotionSystem/Teleportation/FTeleportTraceResult_BP` _traceresult_pathpoints _traceresult_lasttracedestination))))
  (`self.Setup Visual Teleport Indicators`))

(fn `UpdateArc`
  (bind _traceresult_pathpoints (break `/XR_Toolkit/XR_Toolkit/Core/LocomotionSystem/Teleportation/FTeleportTraceResult_BP` (`self.TraceResult`)))
  (bind _arcspline (`self.ArcSpline`))
  (bind (_traceresult_pathpoints_2 _traceresult_lasttracedestination _traceresult_bisvalidlocation) (break `/XR_Toolkit/XR_Toolkit/Core/LocomotionSystem/Teleportation/FTeleportTraceResult_BP` (`self.TraceResult`)))
  (bind _arcendpoint (`self.ArcEndPoint`))
  (bind _arcspline_2 (`self.ArcSpline`))
  (bind _traceresult_pathpoints_3 (break `/XR_Toolkit/XR_Toolkit/Core/LocomotionSystem/Teleportation/FTeleportTraceResult_BP` (`self.TraceResult`)))
  ;[1 1 1] Add Spline points
  ; (+ configure last point)
  (for _array_element _traceresult_pathpoints_3
    (`SplineComponent.AddSplinePoint` _arcspline_2 _array_element "Local" false) ; Build a spline from all trace points. This generates tangets we can use to build a smoothly curved spline mesh
  )
  (`SplineComponent.SetSplinePointType` _arcspline_2 (`KismetArrayLibrary.Array_LastIndex` _traceresult_pathpoints_3) "CurveClamped" true) ; Update the point type to create the curve
  ;[1 1 1] Set Spline MeshComponents
  (for _index (range (+ (- (`SplineComponent.GetNumberOfSplinePoints` (`self.ArcSpline`)) 2) 1))
    (bind _returnvalue (`AddComponent|NODE_AddSplineMeshComponent-0` :`bManualAttachment` true :`RelativeTransform` (`KismetMathLibrary.MakeTransform` (0.0 0.0 0.0)))) ; Add new cylinder mesh
    (`PrimitiveComponent.SetMaterial` _returnvalue 0 (`self.DynaMat_Arc`))
    (`KismetArrayLibrary.Array_Add` (`self.SplineMeshes`) _returnvalue)
    (bind _returnvalue_2 (+ _index 1))
    (`SplineMeshComponent.SetStartAndEnd` _returnvalue (`|GetArrayItem` _traceresult_pathpoints _index) (`SplineComponent.GetTangentAtSplinePoint` _arcspline _index "Local") (`|GetArrayItem` _traceresult_pathpoints _returnvalue_2) (`SplineComponent.GetTangentAtSplinePoint` _arcspline _returnvalue_2 "Local") true) ; Set the tangents and position to build slightly bend the cylinder. All cylinders combined create a smooth arc.
    ;[1 1 1] Set EndPoint to Teleport Location
    (`SceneComponent.SetVisibility` _arcendpoint (xor _traceresult_bisvalidlocation (not (`self.bAllowTeleport`))) false)
    (`SceneComponent.K2_SetWorldLocation` _arcendpoint _traceresult_lasttracedestination false true)))

(fn `UserConstructionScript`)
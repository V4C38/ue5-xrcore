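; Actor component that feeds XR hand-tracking data into an assigned XR core hand Anim Blueprint, apparently still a debug-stage prototype.
; Each tick it copies hand key position 10 from motion controller data into the AnimBP's index-tip control transform, with no rotation.
; It always reads the right hand, ignoring the settable ControllerHand, and prints the position and key count on screen.
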(event `self.ReceiveBeginPlay`)

(event `self.ReceiveTick`
  (params (DeltaSeconds :type "Float (single-precision)"))
  (`self.Assigned ABP XRCore Hand`
    (:`then`
      (bind _motioncontrollerdata (`HeadMountedDisplayFunctionLibrary.GetMotionControllerData` self "Right"))
      (bind (_bvalid _devicename _applicationinstanceid _devicevisualtype _handindex _trackingstatus _gripposition _griprotation _aimposition _aimrotation _palmposition _palmrotation _handkeypositions) (break `XRMotionControllerData` _motioncontrollerdata))
      (bind _output (`|GetArrayItem` _handkeypositions 10))
      (set `/XR_Toolkit/XR_Toolkit/Assets/Meshes/HandModel/ABP_XRCoreHand.Control Index Tip` (`KismetMathLibrary.MakeTransform` _output) (`self.Assigned ABP XRCore Hand`))
      (`KismetSystemLibrary.PrintString` (`KismetStringLibrary.Conv_VectorToString` _output) true true (struct :`G` 0.66 :`B` 1.0 :`A` 1.0) 2.0 "1")
      (`KismetSystemLibrary.PrintString` (`KismetStringLibrary.Conv_IntToString` (`KismetArrayLibrary.Array_Length` _handkeypositions)) true true (struct :`R` 1.0 :`G` 0.014541 :`A` 1.0) 2.0 "2"))
    (:`else`)))

(fn `AssignAnimBP`
  (params (`InABP XRCore Hand` :type "/XR_Toolkit/XR_Toolkit/Assets/Meshes/HandModel/ABP_XRCoreHand Object Reference"))
  (set `self.Assigned ABP XRCore Hand` `InABP XRCore Hand`))

(fn `SetControllerHand`
  (params (InControllerHand :type "EControllerHand Enum" :default "Left"))
  (set `self.ControllerHand` InControllerHand))
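; Pawn component that holds and replicates an XR user's data, including a username persisted in a local file.
; On BeginPlay, the locally controlled pawn waits briefly, loads the saved name from the project content directory and sends it via server RPC.
; The RepNotify on the user data writes the name back to that file for the local user and calls the update dispatcher for listeners.
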(event `self.ReceiveBeginPlay`
  (bind _aspawn (cast `Pawn` (`self.GetOwner`)))
  (bind _output_get (set `self.bIsLocalUser` (`Pawn.IsLocallyControlled` _aspawn)))
  (if _output_get
    (`KismetSystemLibrary.Delay` 1.0)
    (`self.SetUsername` (`self.GetLocalXRUserName`))))

(event `Server_SetXRUserData`
  (params (`XRUser Data` :type "/XR_Toolkit/XR_Toolkit/_Cleanup/Data/FXRConfig Structure"))
  ;[0 0 0] RPC Username | LocalFile
  (set `self.XRUser Data` `XRUser Data`))

(fn `GetLocalXRUserName`
  (returns (ReturnValue :type String))
  (if (`self.bIsLocalUser`)
    (return (`XRLocalFileHandler.LoadFromLocalFile` (`KismetStringLibrary.Concat_StrStr` (`KismetSystemLibrary.GetProjectContentDirectory`) (`self.LocalUserNameFileName`))))))

(fn `GetXRUserData`
  (returns (`XRUser Data` :type "/XR_Toolkit/XR_Toolkit/_Cleanup/Data/FXRConfig Structure"))
  (return (`self.XRUser Data`)))

(fn `OnRep_XRUser Data`
  (`|ExecutionSequence`
    (:`then_0`
      (if (`self.bIsLocalUser`)
        (`self.UpdateLocalUsernameFile` (`.Username_8_C8CC84EC4491675B2FEC54AFE39496CE` (break `/XR_Toolkit/XR_Toolkit/_Cleanup/Data/FXRConfig` (`self.XRUser Data`))))))
    (:`then_1`
      (`self.OnUpdatedUserData` (`self.XRUser Data`)))))

(fn `SetUsername`
  (params (Username :type String))
  (bind _structout (setmembers `/XR_Toolkit/XR_Toolkit/_Cleanup/Data/FXRConfig` :`StructRef` (`self.XRUser Data`) :`Username` Username))
  (`self.Server_SetXRUserData` _structout))

(fn `UpdateLocalUsernameFile`
  (params (Username :type String))
  (if (`self.bIsLocalUser`)
    (`XRLocalFileHandler.SaveToLocalFile` Username (`KismetStringLibrary.Concat_StrStr` (`KismetSystemLibrary.GetProjectContentDirectory`) (`self.LocalUserNameFileName`)))))